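; Captain Jack's dialogue component, scripting a story conversation in which he tells Peter to stay in the dormitory while he heads to the lower deck.
; The Dialogue override calls its parent, then chains AddDialogue nodes linearly, each with speaker, line, single option and animation.
; The last line closes the conversation, opens the next map and restores game-only input.
; Disconnected leftovers include tree-index branching, alternate lines and progress-reset calls that never run.
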(fn `AC_Dialogue_CaptainJack_AutoGenFunc`)

(fn `Dialogue`
  (locals (RefCaptainJack :type "/Game/ChildrenOfAndromeda/Dialogue/NPC_CaptainJack Object Reference") (`ref Black screen` :type "/Game/Afonso/CutScenes/BP_BlackScreen Object Reference"))
  (bind _returnvalue (`GameplayStatics.GetPlayerController` 0))
  (`parent.Dialogue`)
  (bind _state (`self.AddDialogue` "Captain Jack" "Footsteps. You walk like you're about to argue with someone. Relax, kid. Come look at this." (`|MakeArray` "Next" :!type "Text") null "/Game/ChildrenOfAndromeda/Dialogue/Anims/Anim_Conversation.Anim_Conversation"))
  (switch `/Game/ChildrenOfAndromeda/Dialogue/Enum_DialogueState` _state
    (:`NewEnumerator0`
      (bind _state_2 (`self.AddDialogue` "Captain Jack" "People back on Earth still think \"space\" means a dark empty nothing. But look at that. That's not nothing. That's everything they never got to see." (`|MakeArray` "You sound like Professor Solari  \nwhen she talks about the plant research." :!type "Text") null "/Game/ChildrenOfAndromeda/Dialogue/Anims/NewAnimation_Montage.NewAnimation_Montage"))
      (switch `/Game/ChildrenOfAndromeda/Dialogue/Enum_DialogueState` _state_2
        (:`NewEnumerator0`
          (bind _state_3 (`self.AddDialogue` "Peter" "Captain, what’s going on? What was that thing?" (`|MakeArray` "Next" :!type "Text") null "/Game/ChildrenOfAndromeda/Dialogue/Anims/NewAnimation_Montage.NewAnimation_Montage"))
          (switch `/Game/ChildrenOfAndromeda/Dialogue/Enum_DialogueState` _state_3
            (:`NewEnumerator0`
              (bind _state_4 (`self.AddDialogue` "Captain Jack" "I don’t know, Peter. Those creatures got onto the ship without me noticing." (`|MakeArray` "We have to go back. We left the teacher alone. She might still" :!type "Text") null "/Game/ChildrenOfAndromeda/Dialogue/Anims/Anim_Conversation.Anim_Conversation"))
              (switch `/Game/ChildrenOfAndromeda/Dialogue/Enum_DialogueState` _state_4
                (:`NewEnumerator0`
                  (bind _state_5 (`self.AddDialogue` "Captain Jack" "Peter, it’s too dangerous. There was nothing else we could have done." (`|MakeArray` "Next" :!type "Text") null "/Game/ChildrenOfAndromeda/Dialogue/Anims/Anim_Conversation.Anim_Conversation"))
                  (switch `/Game/ChildrenOfAndromeda/Dialogue/Enum_DialogueState` _state_5
                    (:`NewEnumerator0`
                      (bind _state_6 (`self.AddDialogue` "Captain Jack" "Stay in the dormitory. I’m going to try to get to the lower deck of the ship and take this ship to a safe place where they can rescue us." (`|MakeArray` "Next" :!type "Text") null "/Game/ChildrenOfAndromeda/Dialogue/Anims/Anim_Conversation.Anim_Conversation"))
                      (switch `/Game/ChildrenOfAndromeda/Dialogue/Enum_DialogueState` _state_6
                        (:`NewEnumerator0`
                          (bind _state_7 (`self.AddDialogue` "Captain Jack" "As long as you’re here, you’re safe; out there, you’re not." (`|MakeArray` "Next" :!type "Text") null "/Game/ChildrenOfAndromeda/Dialogue/Anims/Anim_Conversation.Anim_Conversation"))
                          (switch `/Game/ChildrenOfAndromeda/Dialogue/Enum_DialogueState` _state_7
                            (:`NewEnumerator0`
                              (bind _state_8 (`self.AddDialogue` "Captain Jack" "I’m leaving. Please don’t do anything stupid while I’m gone. \n" (`|MakeArray` "End conversation" :!type "Text") null "/Game/ChildrenOfAndromeda/Dialogue/Anims/Anim_Conversation.Anim_Conversation"))
                              (switch `/Game/ChildrenOfAndromeda/Dialogue/Enum_DialogueState` _state_8
                                (:`NewEnumerator0`
                                  (`self.CloseConversation`)
                                  (`GameplayStatics.OpenLevelBySoftObjectPtr` "/Game/MAPAFINAL/Map_After_.Map_After_")
                                  (set `PlayerController.bShowMouseCursor` false _returnvalue)
                                  (`WidgetBlueprintLibrary.SetInputMode_GameOnly` _returnvalue))))))))))))))))))