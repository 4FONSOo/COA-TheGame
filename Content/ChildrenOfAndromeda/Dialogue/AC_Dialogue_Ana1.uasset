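; Dialogue component for NPC_Ana1 that plays the scene where Peter persuades a worried Ana to let him investigate the Professor's fate.
; Overrides Dialogue with a linear chain of single-option AddDialogue steps, each playing an animation.
; The last step closes the conversation, hides the cursor, reveals the security room key card and hides Ana, using class lookups.
; Captain Jack lines and tree-index branching remain as unconnected nodes.
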(fn `Dialogue`
  (locals (RefPlayer :type "/Game/ChildrenOfAndromeda/Character/BP_Character/BP_Resident_HorrorV1 Object Reference") (`1CardRef` :type "/Game/sistemas/InteractableSystem/InitialKeyBP Object Reference") (RefAna :type "/Game/ChildrenOfAndromeda/Dialogue/NPC_Ana Object Reference"))
  (`parent.Dialogue`)
  (bind _state (`self.AddDialogue` "Ana" "Footsteps. You walk like you're about to argue with someone. Relax, kid. Come look at this." (`|MakeArray` "Next" :!type "Text") null "/Game/ChildrenOfAndromeda/Dialogue/Anims/Anim_Conversation.Anim_Conversation"))
  (switch `/Game/ChildrenOfAndromeda/Dialogue/Enum_DialogueState` _state
    (:`NewEnumerator0`
      (bind _state_2 (`self.AddDialogue` "Ana" "If we hadn't taken so many detours, we could already be home." (`|MakeArray` "Is everything okay? You seem upset about something." :!type "Text") null "/Game/ChildrenOfAndromeda/Dialogue/Anims/NewAnimation_Montage.NewAnimation_Montage"))
      (switch `/Game/ChildrenOfAndromeda/Dialogue/Enum_DialogueState` _state_2
        (:`NewEnumerator0`
          (bind _state_3 (`self.AddDialogue` "Peter" "The captain must be joking. I can’t just stand here." (`|MakeArray` "Next" :!type "Text") null "/Game/ChildrenOfAndromeda/Dialogue/Anims/NewAnimation_Montage.NewAnimation_Montage"))
          (switch `/Game/ChildrenOfAndromeda/Dialogue/Enum_DialogueState` _state_3
            (:`NewEnumerator0`
              (bind _state_4 (`self.AddDialogue` "Ana" "Peter, the ship’s been invaded—it’s not safe. What do you want to do?" (`|MakeArray` "I need to go back to the corridor  \nto find out what really happened to the Professor." :!type "Text") null "/Game/ChildrenOfAndromeda/Dialogue/Anims/Anim_Conversation.Anim_Conversation"))
              (switch `/Game/ChildrenOfAndromeda/Dialogue/Enum_DialogueState` _state_4
                (:`NewEnumerator0`
                  (bind _state_5 (`self.AddDialogue` "Ana" "That’s way too dangerous." (`|MakeArray` "Here, this is a communicator. We can stay in constant contact.  \nAt the first sign of danger, I’ll come right back here. \nI promise." :!type "Text") null "/Game/ChildrenOfAndromeda/Dialogue/Anims/Anim_Conversation.Anim_Conversation"))
                  (switch `/Game/ChildrenOfAndromeda/Dialogue/Enum_DialogueState` _state_5
                    (:`NewEnumerator0`
                      (bind _state_6 (`self.AddDialogue` "Ana" "This isn’t going to end well. We don’t know what that thing was, or if there are more like it." (`|MakeArray` "Yeah, I know, but I have to investigate." :!type "Text") null "/Game/ChildrenOfAndromeda/Dialogue/Anims/Anim_Conversation.Anim_Conversation"))
                      (switch `/Game/ChildrenOfAndromeda/Dialogue/Enum_DialogueState` _state_6
                        (:`NewEnumerator0`
                          (`self.CloseConversation`)
                          (set `PlayerController.bShowMouseCursor` false (`GameplayStatics.GetPlayerController` 0))
                          (cast `/Game/ChildrenOfAndromeda/Dialogue/NPC_Ana1` (`self.GetOwner`))
                          (bind _outactors (`GameplayStatics.GetAllActorsOfClass` "/Game/sistemas/InteractableSystem/SecurityRoomKeyBP1.SecurityRoomKeyBP1_C"))
                          (`/Game/sistemas/InteractableSystem/BaseInteractable_BP.ShowCard` (`|GetArrayItem` _outactors))
                          (bind _outactors_2 (`GameplayStatics.GetAllActorsOfClass` "/Game/ChildrenOfAndromeda/Dialogue/NPC_Ana1.NPC_Ana1_C"))
                          (`Actor.SetActorHiddenInGame` (`|GetArrayItem` _outactors_2) true))))))))))))))