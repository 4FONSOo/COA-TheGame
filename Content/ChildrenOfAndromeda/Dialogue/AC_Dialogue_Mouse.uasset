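; Dialogue component that scripts Captain Jack's shipboard conversation with the player, a biology student, on the way to Saturnio.
; Its Dialogue function calls the parent, then runs a linear chain of AddDialogue steps, each with one response and an animation, before closing the conversation.
; The opening two lines appear twice in the chain.
; Unconnected nodes hold an unused tree-index switch, randomized repeat-click lines, a quit prompt and progress-reset logic.
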(fn `Dialogue`
  (`parent.Dialogue`)
  (bind _state (`self.AddDialogue` "Captain Jack" "Footsteps. You walk like you're about to argue with someone. Relax, kid. Come look at this." (`|MakeArray` "Next" :!type "Text") null "/Game/ChildrenOfAndromeda/Dialogue/Anims/Anim_Conversation.Anim_Conversation"))
  (switch `/Game/ChildrenOfAndromeda/Dialogue/Enum_DialogueState` _state
    (:`NewEnumerator0`
      (bind _state_2 (`self.AddDialogue` "Captain Jack" "People back on Earth still think \"space\" means a dark empty nothing. But look at that. That's not nothing. That's everything they never got to see." (`|MakeArray` "You sound like Professor Solari  \nwhen she talks about the plant research." :!type "Text") null "/Game/ChildrenOfAndromeda/Dialogue/Anims/NewAnimation_Montage.NewAnimation_Montage"))
      (switch `/Game/ChildrenOfAndromeda/Dialogue/Enum_DialogueState` _state_2
        (:`NewEnumerator0`
          (bind _state_3 (`self.AddDialogue` "Captain Jack" "You know, the first I flew past Saturn's rings - the old one, back in the Solar system - I cried. Don't tell anyone." (`|MakeArray` "...I won't. How'd you even know I was here?" :!type "Text") null "/Game/ChildrenOfAndromeda/Dialogue/Anims/NewAnimation_Montage.NewAnimation_Montage"))
          (switch `/Game/ChildrenOfAndromeda/Dialogue/Enum_DialogueState` _state_3
            (:`NewEnumerator0`
              (bind _state_4 (`self.AddDialogue` "Captain Jack" "Footsteps. You walk like you're about to argue with someone. Relax, kid. Come look at this." (`|MakeArray` "Next" :!type "Text") null "/Game/ChildrenOfAndromeda/Dialogue/Anims/Anim_Conversation.Anim_Conversation"))
              (switch `/Game/ChildrenOfAndromeda/Dialogue/Enum_DialogueState` _state_4
                (:`NewEnumerator0`
                  (bind _state_5 (`self.AddDialogue` "Captain Jack" "People back on Earth still think \"space\" means a dark empty nothing. But look at that. That's not nothing. That's everything they never got to see." (`|MakeArray` "You sound like Professor Solari  \nwhen she talks about the plant research" :!type "Text") null "/Game/ChildrenOfAndromeda/Dialogue/Anims/Anim_Conversation.Anim_Conversation"))
                  (switch `/Game/ChildrenOfAndromeda/Dialogue/Enum_DialogueState` _state_5
                    (:`NewEnumerator0`
                      (bind _state_6 (`self.AddDialogue` "Captain Jack" "Ha. Maybe. She's a good woman, your professor. Knows what she's looking for. That's rarer than you'd think out here — most people just drift." (`|MakeArray` "What about you? What are you looking for?" :!type "Text") null "/Game/ChildrenOfAndromeda/Dialogue/Anims/Anim_Conversation.Anim_Conversation"))
                      (switch `/Game/ChildrenOfAndromeda/Dialogue/Enum_DialogueState` _state_6
                        (:`NewEnumerator0`
                          (bind _state_7 (`self.AddDialogue` "Captain Jack" "Right now? Saturnio. Same as you. After that... we'll see." (`|MakeArray` "Next" :!type "Text") null "/Game/ChildrenOfAndromeda/Dialogue/Anims/Anim_Conversation.Anim_Conversation"))
                          (switch `/Game/ChildrenOfAndromeda/Dialogue/Enum_DialogueState` _state_7
                            (:`NewEnumerator0`
                              (bind _state_8 (`self.AddDialogue` "Captain Jack" "You nervous about landing on a planet outside the solar system for the first time?" (`|MakeArray` "A little. Ana's more nervous than me, I think. \nShe almost didn't come." :!type "Text") null "/Game/ChildrenOfAndromeda/Dialogue/Anims/Anim_Conversation.Anim_Conversation"))
                              (switch `/Game/ChildrenOfAndromeda/Dialogue/Enum_DialogueState` _state_8
                                (:`NewEnumerator0`
                                  (bind _state_9 (`self.AddDialogue` "Captain Jack" "But she did. That's what matters. Fear's fine. Fear means you understand what's at stake." (`|MakeArray` "Next" :!type "Text") null "/Game/ChildrenOfAndromeda/Dialogue/Anims/Anim_Conversation.Anim_Conversation"))
                                  (switch `/Game/ChildrenOfAndromeda/Dialogue/Enum_DialogueState` _state_9
                                    (:`NewEnumerator0`
                                      (bind _state_10 (`self.AddDialogue` "Captain Jack" "What about you what's your stake in all this? You're a biology student. Why does a biology student care this much about a plant on the other side of the galaxy?" (`|MakeArray` "Someone I care about needs what that plant  \ncan do. That's it. That's the whole reason." :!type "Text") null "/Game/ChildrenOfAndromeda/Dialogue/Anims/Anim_Conversation.Anim_Conversation"))
                                      (switch `/Game/ChildrenOfAndromeda/Dialogue/Enum_DialogueState` _state_10
                                        (:`NewEnumerator0`
                                          (bind _state_11 (`self.AddDialogue` "Captain Jack" "Yeah. Then you'd better make sure nothing goes wrong on my ship. I run a clean operation." (`|MakeArray` "...Is that supposed to be reassuring?" :!type "Text") null "/Game/ChildrenOfAndromeda/Dialogue/Anims/Anim_Conversation.Anim_Conversation"))
                                          (switch `/Game/ChildrenOfAndromeda/Dialogue/Enum_DialogueState` _state_11
                                            (:`NewEnumerator0`
                                              (bind _state_12 (`self.AddDialogue` "Captain Jack" "Get some sleep, kid. We arrive at Saturnio in thirty-six hours. Trust me — you'll want to be rested." (`|MakeArray` "End conversation" :!type "Text") null "/Game/ChildrenOfAndromeda/Dialogue/Anims/Anim_Conversation.Anim_Conversation"))
                                              (switch `/Game/ChildrenOfAndromeda/Dialogue/Enum_DialogueState` _state_12
                                                (:`NewEnumerator0`
                                                  (`self.CloseConversation`))))))))))))))))))))))))))