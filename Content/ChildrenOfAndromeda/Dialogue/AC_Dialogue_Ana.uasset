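; Dialogue component for the NPC Ana that plays her linear conversation with the player about detours, the broken shower and class grades.
; Dialogue overrides the parent and chains AddDialogue calls, each with one reply and usually a conversation animation, advancing on Pass Trough.
; The end closes the conversation and, if the owner is NPC_Ana, calls ShowCard on the first InitialKeyBP found.
; Captain Jack lines and tree-index logic remain as unconnected nodes.
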(fn `Dialogue`
  (locals (RefPlayer :type "/Game/ChildrenOfAndromeda/Character/BP_Character/BP_Resident_HorrorV1 Object Reference") (`1CardRef` :type "/Game/sistemas/InteractableSystem/InitialKeyBP Object Reference") (RefAna :type "/Game/ChildrenOfAndromeda/Dialogue/NPC_Ana Object Reference"))
  (`parent.Dialogue`)
  (bind _state (`self.AddDialogue` "Ana" "Footsteps. You walk like you're about to argue with someone. Relax, kid. Come look at this." (`|MakeArray` "Next" :!type "Text") null "/Game/ChildrenOfAndromeda/Dialogue/Anims/Anim_Conversation.Anim_Conversation"))
  (switch `/Game/ChildrenOfAndromeda/Dialogue/Enum_DialogueState` _state
    (:`NewEnumerator0`
      (bind _state_2 (`self.AddDialogue` "Ana" "If we hadn't taken so many detours, we could already be home." (`|MakeArray` "Is everything okay? You seem upset about something." :!type "Text") null "/Game/ChildrenOfAndromeda/Dialogue/Anims/NewAnimation_Montage.NewAnimation_Montage"))
      (switch `/Game/ChildrenOfAndromeda/Dialogue/Enum_DialogueState` _state_2
        (:`NewEnumerator0`
          (bind _state_3 (`self.AddDialogue` "Peter" "Are you worried about the detour?" (`|MakeArray` "Next" :!type "Text") null "/Game/ChildrenOfAndromeda/Dialogue/Anims/NewAnimation_Montage.NewAnimation_Montage"))
          (switch `/Game/ChildrenOfAndromeda/Dialogue/Enum_DialogueState` _state_3
            (:`NewEnumerator0`
              (bind _state_4 (`self.AddDialogue` "Ana" "No, we've had several along the way. We rarely stick to our original route." (`|MakeArray` "Next" :!type "Text") null "/Game/ChildrenOfAndromeda/Dialogue/Anims/Anim_Conversation.Anim_Conversation"))
              (switch `/Game/ChildrenOfAndromeda/Dialogue/Enum_DialogueState` _state_4
                (:`NewEnumerator0`
                  (bind _state_5 (`self.AddDialogue` "Ana" "If we hadn’t taken so many detours, we could already be home." (`|MakeArray` "Is everything okay? You seem upset about something." :!type "Text") null "/Game/ChildrenOfAndromeda/Dialogue/Anims/Anim_Conversation.Anim_Conversation"))
                  (switch `/Game/ChildrenOfAndromeda/Dialogue/Enum_DialogueState` _state_5
                    (:`NewEnumerator0`
                      (bind _state_6 (`self.AddDialogue` "Ana" "They still haven’t fixed the shower problem, when are we going to be able to take a shower?" (`|MakeArray` "Yeah… they should have fixed it by now." :!type "Text") null "/Game/ChildrenOfAndromeda/Dialogue/Anims/Anim_Conversation.Anim_Conversation"))
                      (switch `/Game/ChildrenOfAndromeda/Dialogue/Enum_DialogueState` _state_6
                        (:`NewEnumerator0`
                          (bind _state_7 (`self.AddDialogue` "Ana" "On top of that, Professor Birra’s grades are out. Can you believe he gave me a 19.9 on my paper?" (`|MakeArray` "He didn’t round it up?" :!type "Text") null "/Game/ChildrenOfAndromeda/Dialogue/Anims/Anim_Conversation.Anim_Conversation"))
                          (switch `/Game/ChildrenOfAndromeda/Dialogue/Enum_DialogueState` _state_7
                            (:`NewEnumerator0`
                              (bind _state_8 (`self.AddDialogue` "Ana" "NO! Seriously! I hate him." (`|MakeArray` "Next" :!type "Text") null "/Game/ChildrenOfAndromeda/Dialogue/Anims/Anim_Conversation.Anim_Conversation"))
                              (switch `/Game/ChildrenOfAndromeda/Dialogue/Enum_DialogueState` _state_8
                                (:`NewEnumerator0`
                                  (`self.AddDialogue` "Ana" "You got a 10.4. What happened?" (`|MakeArray` "I’ve been really focused on Professor Solaris’s research project. So focused that I haven’t had time for anything else." :!type "Text") null "/Game/ChildrenOfAndromeda/Dialogue/Anims/Anim_Conversation.Anim_Conversation")
                                  (switch `/Game/ChildrenOfAndromeda/Dialogue/Enum_DialogueState` "NewEnumerator0"
                                    (:`NewEnumerator0`
                                      (bind _state_9 (`self.AddDialogue` "Ana" "I understand, but you shouldn’t let your other classes suffer." (`|MakeArray` "Yeah, I know." :!type "Text") null "/Game/ChildrenOfAndromeda/Dialogue/Anims/Anim_Conversation.Anim_Conversation"))
                                      (switch `/Game/ChildrenOfAndromeda/Dialogue/Enum_DialogueState` _state_9
                                        (:`NewEnumerator0`
                                          (`self.CloseConversation`)
                                          (cast `/Game/ChildrenOfAndromeda/Dialogue/NPC_Ana` (`self.GetOwner`))
                                          (bind _outactors (`GameplayStatics.GetAllActorsOfClass` "/Game/sistemas/InteractableSystem/InitialKeyBP.InitialKeyBP_C"))
                                          (`/Game/sistemas/InteractableSystem/BaseInteractable_BP.ShowCard` (`|GetArrayItem` _outactors)))))))))))))))))))))))