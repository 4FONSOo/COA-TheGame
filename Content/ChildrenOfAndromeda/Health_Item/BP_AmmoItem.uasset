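; Ammo pickup that resupplies the player's current weapon on contact.
; When its Trigger is overlapped by an actor tagged Player, it casts to BP_Resident_HorrorV1 and checks for a valid CurrentWeapon.
; If reserve ammo is below maximum, it calls the weapon's AmmoPickupo and destroys itself; at maximum it stays in place.
; Portuguese debug prints trace most branches.
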(event `self.Trigger.OnComponentBeginOverlap`
  (params (OverlappedComponent :type "PrimitiveComponent Object Reference") (OtherActor :type "Actor Object Reference") (OtherComp :type "PrimitiveComponent Object Reference") (OtherBodyIndex :type Integer) (bFromSweep :type Boolean) (SweepResult :type "HitResult Structure (by ref)"))
  (`KismetSystemLibrary.PrintString` "entrou trigger")
  (if (`self.ActorHasTag` OtherActor "Player")
    (`KismetSystemLibrary.PrintString` "entrou branch hastag")
    (bind _asbp_resident_horror_v1 (cast `/Game/ChildrenOfAndromeda/Character/BP_Character/BP_Resident_HorrorV1` OtherActor)
      (:`then`
        (bind _currentweapon (`/Game/ChildrenOfAndromeda/Character/BP_Character/BP_Resident_HorrorV1.CurrentWeapon` _asbp_resident_horror_v1)
          (:`then`
            (if (< (`/Game/ChildrenOfAndromeda/Weapons/BP_baseWeapon.CurrentReserveAmmo` _currentweapon) (`/Game/ChildrenOfAndromeda/Weapons/BP_baseWeapon.MaxReserveAmmo` _currentweapon))
              (`KismetSystemLibrary.PrintString` "castou")
              (`/Game/ChildrenOfAndromeda/Weapons/BP_baseWeapon.AmmoPickupo` _currentweapon)
              (`self.K2_DestroyActor`)
              (`KismetSystemLibrary.PrintString` "destruiu")
              (else
                (`KismetSystemLibrary.PrintString` "municao maxima"))))
          (:`else`)))
      (:`CastFailed`
        (`KismetSystemLibrary.PrintString` "castou fail")))))

(fn `UserConstructionScript`)