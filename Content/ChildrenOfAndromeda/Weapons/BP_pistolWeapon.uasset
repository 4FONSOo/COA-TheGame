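; BP_pistolWeapon is a child weapon Blueprint for a pistol that fires trace-based shots with a limited fire rate.
; Shoot calls the parent implementation, then, if CanShoot is set, clears that flag and calls CreateShotTrace with the weapon's Range.
; A timer lasting FireRate then triggers ResetShot, which re-enables shooting.
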(event `self.Shoot`
  (`parent.Shoot`)
  (if (`self.CanShoot?`)
    (set `self.CanShoot?` false)
    (`self.CreateShotTrace` (`self.Range`))
    (`KismetSystemLibrary.K2_SetTimerDelegate` (delegate `ResetShot`) (`self.FireRate`))))

(event `ResetShot`
  (set `self.CanShoot?` true))

(fn `UserConstructionScript`
  (`parent.UserConstructionScript`))