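; Base weapon Blueprint that handles hitscan shooting, ammo and reloading for the BP_Resident_HorrorV1 player, with Shoot and EndShoot left empty.
; CreateShotTrace decrements the magazine, then either reloads at zero or line-traces for Pawns, spawning Niagara impacts and applying damage to every hit.
; An optional TRON beam fires through a BP_TRON_BeamSpawner found in the level; a call without a cached spawner only looks it up.
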(event `self.ReceiveBeginPlay`
  (bind _asbp_resident_horror_v1 (cast `/Game/ChildrenOfAndromeda/Character/BP_Character/BP_Resident_HorrorV1` (`GameplayStatics.GetPlayerCharacter` 0)))
  (set `self.PlayerCharacter` _asbp_resident_horror_v1))

(event `Shoot`)

(event `CreateShotTrace`
  (params (range :type "Float (double-precision)"))
  (bind _shootarrow (`self.ShootArrow`))
  (bind _returnvalue (`SceneComponent.K2_GetComponentLocation` _shootarrow))
  (bind _output_get (set `self.CurrentMagAmmo` (`KismetMathLibrary.Clamp` (- (`self.CurrentMagAmmo`) 1) 0 (`self.MaxMagAmmo`))))
  (`/Game/ChildrenOfAndromeda/Character/BP_Character/BP_Resident_HorrorV1.UpdateAmmo` (`self.PlayerCharacter`) _output_get (`self.CurrentReserveAmmo`))
  (if (<= _output_get 0)
    (`self.ReloadWeapon`)
    (else
      ;[1 0.1167 0] Acrescenta Isto
      (`self.FireTRONBeam_FromWeapon`)
      (bind (_outhits _returnvalue_2) (`KismetSystemLibrary.LineTraceMultiForObjects` :`Start` _returnvalue :`End` (+ _returnvalue (* (`KismetMathLibrary.GetForwardVector` (`SceneComponent.K2_GetComponentRotation` _shootarrow)) range)) :`ObjectTypes` (`|MakeArray` "ObjectTypeQuery3" :!type "EObjectTypeQuery Enum") :`DrawDebugType` "ForDuration"))
      (if _returnvalue_2
        (for _array_element _outhits
          (bind (_bblockinghit _binitialoverlap _time _distance _location _impactpoint _normal _impactnormal _physmat _hitactor) (`GameplayStatics.BreakHitResult` _array_element))
          (`NiagaraFunctionLibrary.SpawnSystemAtLocation` "/Game/Birra_New/07_TRON/Niagara/NS_TronImpact.NS_TronImpact" _location)
          (`GameplayStatics.ApplyDamage` _hitactor (`self.Base Damage`)))))))

(event `EndShoot`)

(event `ReloadWeapon`
  (if (== (`self.CurrentMagAmmo`) (`self.MaxMagAmmo`))
    _
    (elif (not (<= (`self.CurrentReserveAmmo`) 0))
      (`self.EndShoot`)
      (bind _output_get (set `self.NeededAmmo` (- (`self.MaxMagAmmo`) (`self.CurrentMagAmmo`))))
      (if (>= (`self.CurrentReserveAmmo`) _output_get)
        (set `self.CurrentMagAmmo` (+ (`self.NeededAmmo`) (`self.CurrentMagAmmo`)))
        (set `self.CurrentReserveAmmo` (- (`self.CurrentReserveAmmo`) (`self.NeededAmmo`)))
        (`/Game/ChildrenOfAndromeda/Character/BP_Character/BP_Resident_HorrorV1.Reload` (`self.PlayerCharacter`))
        (else
          (set `self.CurrentMagAmmo` (+ (`self.CurrentReserveAmmo`) (`self.CurrentMagAmmo`)))
          (set `self.CurrentReserveAmmo` 0)
          (`/Game/ChildrenOfAndromeda/Character/BP_Character/BP_Resident_HorrorV1.Reload` (`self.PlayerCharacter`)))))))

(fn `FindTRONBeamSpawner`
  (`/Engine/EditorBlueprintResources/StandardMacros.IsValid` (`self.TRONBeamSpawnerRef`)
    (:`Is Not Valid`
      (bind _outactors (`GameplayStatics.GetAllActorsOfClass` "/Game/Birra_New/07_TRON/BP/BP_TRON_BeamSpawner.BP_TRON_BeamSpawner_C"))
      (set `self.TRONBeamSpawnerRef` (`|GetArrayItem` _outactors))
      (return))))

(fn `FireTRONBeam_FromWeapon`
  (locals (StartRaw :type "Vector Structure" :default (0.0 0.0 0.0)) (FireDirection :type "Vector Structure") (StartLocaiton :type "Vector Structure"))
  (bind _tronbeamspawnerref (`self.TRONBeamSpawnerRef`))
  (bind _shootarrow (`self.ShootArrow`))
  (if (`self.bUseTRONBeam`)
    (`/Engine/EditorBlueprintResources/StandardMacros.IsValid` _tronbeamspawnerref
      (:`Is Valid`
        (if (`KismetSystemLibrary.IsValid` _tronbeamspawnerref)
          (bind _output_get (set `local.StartRaw` (`SceneComponent.K2_GetComponentLocation` _shootarrow)))
          (bind _output_get_2 (set `local.FireDirection` (`SceneComponent.GetForwardVector` _shootarrow)))
          (bind _output_get_3 (set `local.StartLocaiton` (+ _output_get (* _output_get_2 (`self.TRONStartForwardOffset`)))))
          (`/Game/Birra_New/07_TRON/BP/BP_TRON_BeamSpawner.FireTRONFromResident_WithTrace` (`self.TRONBeamSpawnerRef`) (`self.PlayerCharacter`) _output_get_3 _output_get_2 (`self.bTRONForceImpactMode`))
          (else
            (return))))
      (:`Is Not Valid`
        (`self.FindTRONBeamSpawner`)))
    (else
      (return))))

(fn `UserConstructionScript`)