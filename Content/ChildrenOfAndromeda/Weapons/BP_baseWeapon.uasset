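; Base weapon Blueprint for the Resident_Horror player character, handling magazine and reserve ammo, hitscan damage, reloads and ammo pickups, with empty Shoot and EndShoot events.
; CreateShotTrace spends a round, then either auto-reloads on empty or fires a TRON beam through the level's first beam spawner and multi-traces pawns for impact effects and damage.
; Reloads and capped pickups adjust reserves and notify the player character.
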(event `AmmoPickupo`
  (`KismetSystemLibrary.PrintString` "entrou ammo pickup")
  (if (<= (+ (`self.CurrentReserveAmmo`) (`self.ammopickup`)) (`self.MaxReserveAmmo`))
    (bind _output_get (set `self.CurrentReserveAmmo` (+ (`self.ammopickup`) (`self.CurrentReserveAmmo`))))
    (`KismetSystemLibrary.PrintString` (`KismetStringLibrary.Conv_IntToString` _output_get))
    (`/Game/ChildrenOfAndromeda/Character/BP_Character/BP_Resident_HorrorV1.AtualizarAmmo` (`self.PlayerCharacter`))
    (else
      (bind _output_get_2 (set `self.CurrentReserveAmmo` (`self.MaxReserveAmmo`)))
      (`KismetSystemLibrary.PrintString` (`KismetStringLibrary.Conv_IntToString` _output_get_2))
      (`/Game/ChildrenOfAndromeda/Character/BP_Character/BP_Resident_HorrorV1.AtualizarAmmo` (`self.PlayerCharacter`)))))

(event `self.ReceiveBeginPlay`
  (bind _asbp_resident_horror_v1 (cast `/Game/ChildrenOfAndromeda/Character/BP_Character/BP_Resident_HorrorV1` (`GameplayStatics.GetPlayerCharacter` 0)))
  (set `self.PlayerCharacter` _asbp_resident_horror_v1))

(event `Shoot`)

(event `CreateShotTrace`
  (params (range :type "Float (double-precision)"))
  (bind _shootarrow (`self.ShootArrow`))
  (bind _returnvalue (`SceneComponent.K2_GetComponentLocation` _shootarrow))
  (bind _output_get (set `self.CurrentMagAmmo` (`KismetMathLibrary.Clamp` (- (`self.CurrentMagAmmo`) 1) 0 (`self.MaxMagAmmo`))))
  (`/Game/ChildrenOfAndromeda/Character/BP_Character/BP_Resident_HorrorV1.UpdateAmmo` (`self.PlayerCharacter`) _output_get (`self.CurrentReserveAmmo`))
  (if (<= _output_get 0)
    (`self.ReloadWeapon`)
    (else
      (`self.FireTRON_FromWeapon`)
      (bind (_outhits _returnvalue_2) (`KismetSystemLibrary.LineTraceMultiForObjects` _returnvalue (+ _returnvalue (* (`KismetMathLibrary.GetForwardVector` (`SceneComponent.K2_GetComponentRotation` _shootarrow)) range)) (`|MakeArray` "ObjectTypeQuery3" :!type "EObjectTypeQuery Enum")))
      (if _returnvalue_2
        (for _array_element _outhits
          (bind (_bblockinghit _binitialoverlap _time _distance _location _impactpoint _normal _impactnormal _physmat _hitactor) (`GameplayStatics.BreakHitResult` _array_element))
          (`NiagaraFunctionLibrary.SpawnSystemAtLocation` "/Game/Birra_New/07_TRON/Niagara/NS_TronImpact.NS_TronImpact" _location)
          (`GameplayStatics.ApplyDamage` _hitactor (`self.Base Damage`)))))))

(event `EndShoot`)

(event `ReloadWeapon`
  (if (== (`self.CurrentMagAmmo`) (`self.MaxMagAmmo`))
    _
    (elif (not (<= (`self.CurrentReserveAmmo`) 0))
      (`self.EndShoot`)
      (bind _output_get (set `self.NeededAmmo` (- (`self.MaxMagAmmo`) (`self.CurrentMagAmmo`))))
      (if (>= (`self.CurrentReserveAmmo`) _output_get)
        (set `self.CurrentMagAmmo` (+ (`self.NeededAmmo`) (`self.CurrentMagAmmo`)))
        (set `self.CurrentReserveAmmo` (- (`self.CurrentReserveAmmo`) (`self.NeededAmmo`)))
        (`/Game/ChildrenOfAndromeda/Character/BP_Character/BP_Resident_HorrorV1.Reload` (`self.PlayerCharacter`))
        (else
          (set `self.CurrentMagAmmo` (+ (`self.CurrentReserveAmmo`) (`self.CurrentMagAmmo`)))
          (set `self.CurrentReserveAmmo` 0)
          (`/Game/ChildrenOfAndromeda/Character/BP_Character/BP_Resident_HorrorV1.Reload` (`self.PlayerCharacter`)))))))

(fn `FireTRON_FromWeapon`
  (bind _shootarrow (`self.ShootArrow`))
  (bind _returnvalue (`SceneComponent.GetForwardVector` _shootarrow))
  (bind _outactors (`GameplayStatics.GetAllActorsOfClass` "/Game/Birra_New/07_TRON/BP/BP_TRON_BeamSpawner.BP_TRON_BeamSpawner_C"))
  (`KismetSystemLibrary.PrintString` "entrou tron")
  (bind _output (`|GetArrayItem` _outactors))
  (`/Engine/EditorBlueprintResources/StandardMacros.IsValid` _output
    (:`Is Valid`
      (bind _output_get (set `self.TRONBeamSpawnerRef` _output))
      (`/Game/Birra_New/07_TRON/BP/BP_TRON_BeamSpawner.FireTRONFromResident_WithTrace` _output (`self.PlayerCharacter`) (+ (`SceneComponent.K2_GetComponentLocation` _shootarrow) (* _returnvalue (`self.TRONStartForwardOffset`))) _returnvalue false)
      (`/Game/Birra_New/07_TRON/BP/BP_TRON_BeamSpawner.FireTRONFromResident_WithTrace` _output_get (`self.PlayerCharacter`) (+ (`SceneComponent.K2_GetComponentLocation` _shootarrow) (* _returnvalue (`self.TRONStartForwardOffset`))) _returnvalue false))))

(fn `UserConstructionScript`)