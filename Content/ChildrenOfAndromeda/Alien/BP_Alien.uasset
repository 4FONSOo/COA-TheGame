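; BP_Alien is an alien actor with health and a floating health bar widget.
; Overlap of its Sphere with BP_Resident_HorrorV1 subtracts health and updates W_AlienHP, then destroys the actor if IsDead.
; Tick refreshes the bar's percent and turns it toward the player camera.
; AnyDamage leaves Health unchanged, and the zero-health check that sets IsDead is unconnected, so nothing here triggers death.
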(event `self.ReceiveTick`
  (params (DeltaSeconds :type "Float (single-precision)"))
  (bind _healthbarwidget (`self.HealthBarWidget`))
  (bind _asw_alien_hp (cast `/Game/ChildrenOfAndromeda/Alien/W_AlienHP` (`WidgetComponent.GetWidget` (`self.HealthBarWidget`))))
  (`ProgressBar.SetPercent` (`/Game/ChildrenOfAndromeda/Alien/W_AlienHP.AlienHB` _asw_alien_hp) (/ (`self.health`) 30.0))
  (`SceneComponent.K2_SetWorldRotation` _healthbarwidget (`KismetMathLibrary.FindLookAtRotation` (`SceneComponent.K2_GetComponentLocation` _healthbarwidget) (`SceneComponent.K2_GetComponentLocation` (`PlayerCameraManager.TransformComponent` (`GameplayStatics.GetPlayerCameraManager` 0)))) false false))

(event `self.ReceiveAnyDamage`
  (params (Damage :type "Float (single-precision)") (DamageType :type "DamageType Object Reference") (InstigatedBy :type "Controller Object Reference") (DamageCauser :type "Actor Object Reference"))
  (if (not (`self.isDead?`))
    (bind _output_get (set `self.health` (`self.health`)))
    (`self.UpdateHealthAlien`)))

(event `self.ReceiveBeginPlay`
  (`self.UpdateHealthAlien`))

(event `self.Sphere.OnComponentBeginOverlap`
  (params (OverlappedComponent :type "PrimitiveComponent Object Reference") (OtherActor :type "Actor Object Reference") (OtherComp :type "PrimitiveComponent Object Reference") (OtherBodyIndex :type Integer) (bFromSweep :type Boolean) (SweepResult :type "HitResult Structure (by ref)"))
  (bind _asbp_resident_horror_v1 (cast `/Game/ChildrenOfAndromeda/Character/BP_Character/BP_Resident_HorrorV1` OtherActor))
  (`/Engine/EditorBlueprintResources/StandardMacros.IsValid` _asbp_resident_horror_v1
    (:`Is Valid`
      (set `self.health` (- (`self.health`) 15.0))
      (`self.UpdateHealthAlien`)
      (if (`self.isDead?`)
        (`self.K2_DestroyActor`)))))

(fn `UpdateHealthAlien`
  (bind _asw_alien_hp (cast `/Game/ChildrenOfAndromeda/Alien/W_AlienHP` (`WidgetComponent.GetUserWidgetObject` (`self.HealthBarWidget`))))
  (`/Engine/EditorBlueprintResources/StandardMacros.IsValid` _asw_alien_hp
    (:`Is Valid`
      (set `/Game/ChildrenOfAndromeda/Alien/W_AlienHP.alienHealth` (`self.health`) _asw_alien_hp)
      (return))))

(fn `UserConstructionScript`
  (`parent.UserConstructionScript`))