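; BP_porta is an automatic four-panel door that opens when a BP_Resident_HorrorV1 enters its trigger box and closes when that actor leaves.
; Box overlap events cast to that class, then play or reverse two timelines together.
; The Door timeline slides one pair of cube meshes along local X, while the second timeline slides the other pair along Z.
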(event `self.ReceiveBeginPlay`)

(event `OpenDoor`
  (bind (_direction _door_1 _door_2) (`Timeline|Door` :!label _label)
    (:`Update`
      (`SceneComponent.K2_SetRelativeLocation` (`self.Cube_111`) (`KismetMathLibrary.MakeVector` _door_1) false false)
      (`SceneComponent.K2_SetRelativeLocation` (`self.Cube_110`) (`KismetMathLibrary.MakeVector` _door_2) false false))))

(event `CloseDoor1`
  (goto _label :!via `Reverse`))

(event `OpenDoor2`
  (bind (_direction _door_1 _door_2) (`Timeline|Timeline` :!label _label_2)
    (:`Update`
      (`SceneComponent.K2_SetRelativeLocation` (`self.Cube_109`) (`KismetMathLibrary.MakeVector` 0.0 0.0 _door_1) false false)
      (`SceneComponent.K2_SetRelativeLocation` (`self.Cube_112`) (`KismetMathLibrary.MakeVector` 0.0 0.0 _door_2) false false))))

(event `CloseDoor2`
  (goto _label_2 :!via `Reverse`))

(event `self.Box.OnComponentBeginOverlap`
  (params (OverlappedComponent :type "PrimitiveComponent Object Reference") (OtherActor :type "Actor Object Reference") (OtherComp :type "PrimitiveComponent Object Reference") (OtherBodyIndex :type Integer) (bFromSweep :type Boolean) (SweepResult :type "HitResult Structure (by ref)"))
  (cast `/Game/ChildrenOfAndromeda/Character/BP_Character/BP_Resident_HorrorV1` OtherActor)
  (`self.OpenDoor`)
  (`self.OpenDoor2`))

(event `self.Box.OnComponentEndOverlap`
  (params (OverlappedComponent :type "PrimitiveComponent Object Reference") (OtherActor :type "Actor Object Reference") (OtherComp :type "PrimitiveComponent Object Reference") (OtherBodyIndex :type Integer))
  (cast `/Game/ChildrenOfAndromeda/Character/BP_Character/BP_Resident_HorrorV1` OtherActor)
  (`self.CloseDoor1`)
  (`self.CloseDoor2`))

(fn `UserConstructionScript`)