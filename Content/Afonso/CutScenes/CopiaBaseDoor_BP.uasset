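; Interactable door Blueprint in the CutScenes folder, apparently a copy of a base door, that can be locked by a named key.
; On Interact, an unlocked door fires both open events, while a locked one passes its DoorName to the Character's UseKeyMessage and unlocks and opens on success.
; Each open event plays its own timeline, though no timeline outputs drive movement in this graph.
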(event `OpenDoor`
  (`Timeline|Linha do tempo`))

(event `OpenDoor2`
  (`Timeline|Linha do tempo_0`))

(event `self.Interact`
  (params (Character :type "Actor Object Reference"))
  (`KismetSystemLibrary.PrintString` "porta")
  (if (`self.Unlocked`)
    (`self.OpenDoor`)
    (`self.OpenDoor2`)
    (else
      (bind _door_unlocked (message `/Game/sistemas/InteractableSystem/Interface/CharacterBPInterface.UseKey` Character (`self.DoorName`)))
      (if _door_unlocked
        (set `self.Unlocked` true)
        (`self.OpenDoor`)
        (`self.OpenDoor2`)
        (`KismetSystemLibrary.PrintString` "DoorUnlocked")))))

(fn `UserConstructionScript`
  (`parent.UserConstructionScript`))