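; Trigger actor that runs the Peter and teacher death cutscene when BP_Resident_HorrorV1 overlaps its box.
; It plays the teacher's death and a level sequence, disabling player input while a timed Peter monologue widget shows.
; It then destroys itself and the blocker, teleports the player and restores input.
; Finally it spawns NPC_Ana2, removes Ana's first dialogue actor, moves BP_Ana and reveals the lab key card, all at hard-coded locations.
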(event `self.Box.OnComponentBeginOverlap`
  (params (OverlappedComponent :type "PrimitiveComponent Object Reference") (OtherActor :type "Actor Object Reference") (OtherComp :type "PrimitiveComponent Object Reference") (OtherBodyIndex :type Integer) (bFromSweep :type Boolean) (SweepResult :type "HitResult Structure (by ref)"))
  (cast `/Game/ChildrenOfAndromeda/Character/BP_Character/BP_Resident_HorrorV1` OtherActor)
  (`/Game/Afonso/professora/Professora.PlayTeacherDeath` (`self.TeacherRef`))
  (bind (_outactor _returnvalue) (`LevelSequencePlayer.CreateLevelSequencePlayer` (`self.CutScene`)))
  (`MovieSceneSequencePlayer.Play` _returnvalue)
  (`self.DisableInput` (`GameplayStatics.GetPlayerCharacter` 0) (`GameplayStatics.GetPlayerController` 0))
  (bind _returnvalue_2 (`|CreateWidget` "/Game/ChildrenOfAndromeda/Dialogue/PeterMonologo.PeterMonologo_C"))
  (bind _output_get (set `self.Ref Peter Dialogue` _returnvalue_2))
  (`KismetSystemLibrary.Delay` 0.5)
  (`/Game/ChildrenOfAndromeda/Dialogue/PeterMonologo.SetText3` _returnvalue_2)
  (`UserWidget.AddToViewport` _output_get 0)
  (`KismetSystemLibrary.Delay` 3.0)
  (`Widget.RemoveFromParent` (`self.Ref Peter Dialogue`))
  (`self.K2_DestroyActor`)
  (`self.K2_DestroyActor` (`self.RefBloqueio`))
  (`self.K2_TeleportTo` (`GameplayStatics.GetPlayerCharacter` 0) (98.234165 -2416.832278 1687.0) (struct))
  (`self.EnableInput` (`GameplayStatics.GetPlayerCharacter` 0) (`GameplayStatics.GetPlayerController` 0))
  (`|SpawnActorFromClass` "/Game/ChildrenOfAndromeda/Dialogue/NPC_Ana2.NPC_Ana2_C" (`KismetMathLibrary.MakeTransform` (2.0 -2726.0 1649.0) (struct :`Yaw` 90.0)) "AlwaysSpawn" "MultiplyWithRoot" null null)
  (`self.K2_DestroyActor` (`self.RefDialogoAna1`))
  (bind _outactors (`GameplayStatics.GetAllActorsOfClass` "/Game/Afonso/ana/BP_Ana.BP_Ana_C"))
  (`self.K2_TeleportTo` (`|GetArrayItem` _outactors) (2.0 -2726.0 1590.0) (struct))
  (bind _outactors_2 (`GameplayStatics.GetAllActorsOfClass` "/Game/sistemas/InteractableSystem/LaboratorioKey.LaboratorioKey_C"))
  (`/Game/sistemas/InteractableSystem/BaseInteractable_BP.ShowCard` (`|GetArrayItem` _outactors_2)))

(fn `UserConstructionScript`)