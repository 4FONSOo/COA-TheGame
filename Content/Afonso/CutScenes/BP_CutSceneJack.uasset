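; BP_CutSceneJack is a box trigger that starts the Captain Jack cutscene when BP_Resident_HorrorV1 overlaps it.
; The overlap plays the level sequence, disables input, swaps Ana's mesh for her seated version and spawns NPC_CaptainJack.
; A short timer is meant to teleport the player and captain references to fixed locations.
; The trigger destroys itself before setting that timer, so the teleport likely never fires.
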(event `self.Box.OnComponentBeginOverlap`
  (params (OverlappedComponent :type "PrimitiveComponent Object Reference") (OtherActor :type "Actor Object Reference") (OtherComp :type "PrimitiveComponent Object Reference") (OtherBodyIndex :type Integer) (bFromSweep :type Boolean) (SweepResult :type "HitResult Structure (by ref)"))
  (cast `/Game/ChildrenOfAndromeda/Character/BP_Character/BP_Resident_HorrorV1` OtherActor)
  (bind (_outactor _returnvalue) (`LevelSequencePlayer.CreateLevelSequencePlayer` (`self.CutScene`)))
  (`MovieSceneSequencePlayer.Play` _returnvalue)
  (`self.DisableInput` (`GameplayStatics.GetPlayerController` 0) null)
  (`self.K2_DestroyActor`)
  (`KismetSystemLibrary.K2_SetTimerDelegate` (delegate `TimerTeleport`) 0.3)
  (`self.K2_DestroyActor` (`self.RefAnaMesh`))
  (`/Game/Afonso/ana/BP_AnaSentada.ShowAnaSentada` (`self.RefAnaMeshSentada`))
  (`|SpawnActorFromClass` "/Game/ChildrenOfAndromeda/Dialogue/NPC_CaptainJack.NPC_CaptainJack_C" (`KismetMathLibrary.MakeTransform` (237.0 -2463.0 1662.0) (struct :`Yaw` 180.0)) "AlwaysSpawn" "MultiplyWithRoot" null null))

(event `TimerTeleport`
  (`self.K2_SetActorLocation` (`self.RefPlayer`) (8246.0 -1790.0 8848.0) false true)
  (`self.K2_SetActorLocation` (`self.RefCapitao`) (8246.0 -1792.0 8848.0) false true))

(fn `UserConstructionScript`)