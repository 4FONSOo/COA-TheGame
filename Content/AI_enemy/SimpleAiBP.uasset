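; Simple enemy AI pawn that wanders at random, chases pawns it sees and plays a mutant jump attack on reaching them.
; From BeginPlay, Patrol loops AIMoveTo calls to random reachable points around its current location.
; PawnSensing sightings start ChaseTarget, which falls back to Patrol only if the move fails.
; A CanAttack flag blocks repeat attacks until the montage completes or is interrupted.
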(event `self.ReceiveBeginPlay`
  (`self.Patrol`))

(event `Patrol`
  (`|AIMoveTo` self (`NavigationSystemV1.K2_GetRandomReachablePointInRadius` (`self.K2_GetActorLocation`) 500.0 null null) null
    (:`OnSuccess`
      (`KismetSystemLibrary.Delay` 0.2))
    (:`OnFail`
      _))
  (`self.Patrol`))

(event `self.PawnSensing.OnSeePawn`
  (params (Pawn :type "Pawn Object Reference"))
  (`self.ChaseTarget` Pawn))

(event `ChaseTarget`
  (params (TargetActor :type "Actor Object Reference"))
  (`|AIMoveTo` self (0.0 0.0 0.0) TargetActor
    (:`OnSuccess`
      (if (`self.CanAttack`)
        (`|PlayMontage` (`self.Mesh`) "/Game/Mutant/Demo/Mutant_Jump_Animation_Montage.Mutant_Jump_Animation_Montage"
          (:`then`
            (set `self.CanAttack` false))
          (:`OnCompleted`
            (set `self.CanAttack` true :!label _label))
          (:`OnInterrupted`
            (goto _label)))))
    (:`OnFail`
      (`self.Patrol`))))

(fn `UserConstructionScript`)