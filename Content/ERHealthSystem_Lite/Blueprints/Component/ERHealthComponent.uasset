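; Replicated health component that handles damage, healing, death and regeneration for its owning actor.
; On authority it binds to the owner's OnTakeAnyDamage, treating positive damage as harm and other values as healing, then updates clamped health and state flags.
; A looping timer drives regeneration, delayed after damage.
; OnRep_Health broadcasts health, death, damage, heal and full-health dispatchers, while public events control invincibility, healing pause, health and regeneration settings.
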(event `self.ReceiveBeginPlay`
  ;[0.02353 0.149 0.04444 0.25 24] Begin Play / Healing Events (Update Health - Damage Functions / Healing Functions)
  ;;[0.01 0.01 0.01] Switch Authority And Update Health Variable By Binding To (On Take Any Damage Event) If Server
  (`/Engine/EditorBlueprintResources/ActorComponentMacros.Switch Has Authority`
    (:`Authority`
      (add `Actor.OnTakeAnyDamage` (`self.GetOwner`) (delegate `Event On Take AnyDamage`))
      (`self.Regenerate Health?`) ; Check If Health Regen Is Needed On Begin Play
    )))

(event `ROS_Update Health`
  (params (`CallEventDispatchers?` :type Boolean) (Health :type "Float (double-precision)") (`Max Health` :type "Float (double-precision)"))
  ;[0.02353 0.149 0.04444 0.25 24] Begin Play / Healing Events (Update Health - Damage Functions / Healing Functions)
  ;;[0.01 0.01 0.01] Server Update Health Function (Private)
  (set `self.CallEventDispatchers?` `CallEventDispatchers?`)
  (`self.Update Health Function` Health `Max Health`))

(event `Event On Take AnyDamage`
  (params (DamagedActor :type "Actor Object Reference") (Damage :type "Float (single-precision)") (DamageType :type "DamageType Object Reference") (InstigatedBy :type "Controller Object Reference") (DamageCauser :type "Actor Object Reference"))
  ;[0.02353 0.149 0.04444 0.25 24] Begin Play / Healing Events (Update Health - Damage Functions / Healing Functions)
  ;;[0.01 0.01 0.01] Switch Authority And Update Health Variable By Binding To (On Take Any Damage Event) If Server
  (`self.On Take Any Damage` DamagedActor Damage DamageType InstigatedBy DamageCauser) ; Damage And Healing Functions
)

(event `Health Regeneration`
  ;[0.02353 0.149 0.04444 0.25 24] Begin Play / Healing Events (Update Health - Damage Functions / Healing Functions)
  ;;[0.01 0.01 0.01] Regenerate Health If (CanRegenerateHealth) Is True
  (if (`self.CanHeal?`)
    (`self.Heal Function` (`self.RegenerationAmount`))
    (elif (`KismetSystemLibrary.K2_IsValidTimerHandle` (`self.RegenerateHealthTimer`))
      (`KismetSystemLibrary.K2_ClearAndInvalidateTimerHandle` (`self.RegenerateHealthTimer`)))))

(event `PauseHealing`
  (params (`PauseHealing?` :type Boolean))
  ;[0.02353 0.149 0.04444 0.25 24] Begin Play / Healing Events (Update Health - Damage Functions / Healing Functions)
  ;;[0.01 0.01 0.01] Pause Healing By Setting (CanHeal?) To False And Heal Over Time When Pause Healing Is False (Public)
  (set `self.CanHeal?` (not `PauseHealing?`))
  (`self.Regenerate Health?`))

(event `Update Health`
  (params (Health :type "Float (double-precision)") (`Max Health` :type "Float (double-precision)"))
  ;[0.02353 0.149 0.04444 0.25 24] Begin Play / Healing Events (Update Health - Damage Functions / Healing Functions)
  ;;[0.01 0.01 0.01] Update Health Variable (Public)
  (`self.ROS_Update Health` false Health `Max Health`))

(event `Update Health Regeneration`
  (params (`CanRegenerateHealth?` :type Boolean) (RegenerationAmount :type "Float (double-precision)") (RegenerationRate :type "Float (single-precision)") (RegenerationDelay :type "Float (double-precision)"))
  ;[0.02353 0.149 0.04444 0.25 24] Begin Play / Healing Events (Update Health - Damage Functions / Healing Functions)
  ;;[0.01 0.01 0.01] Update Health Regeneration (Public)
  (`self.On Health Regeneration Updated` `CanRegenerateHealth?` RegenerationAmount RegenerationRate RegenerationDelay))

(event `Invincibility`
  (params (`Invincible?` :type Boolean))
  ;[0.02353 0.149 0.04444 0.25 24] Begin Play / Healing Events (Update Health - Damage Functions / Healing Functions)
  ;;[0.01 0.01 0.01] Give The Actor Calling This Event Invincibility By Setting (Can be Damaged?) To False (Public)
  (set `self.CanBeDamaged?` (not `Invincible?`)))

(fn `Call On Any Damaged`
  (`self.On Any Damage` (`self.Damaged Actor`) (`self.DamageAmount`) (`self.Health`) (`self.MaxHealth`) (`self.LastUpdatedHealth`) (`self.Damage Type`) (`self.Instigated By`) (`self.Damage Causer`)))

(fn `Call On Any Heal`
  (`self.On Any Heal` (`self.Damaged Actor`) (`self.HealAmount`) (`self.Health`) (`self.MaxHealth`) (`self.LastUpdatedHealth`) (`self.Damage Type`) (`self.Instigated By`) (`self.Damage Causer`)))

(fn `Call On Death`
  ;[0.01 0.01 0.01] Call On Death Event Dispacher
  (`self.On Death` (`self.Damaged Actor`) (`self.DamageAmount`) (`self.MaxHealth`) (`self.LastUpdatedHealth`) (`self.Damage Type`) (`self.Instigated By`) (`self.Damage Causer`)))

(fn `Call On Full Health`
  (`self.On Full Health` (`self.Damaged Actor`) (`self.HealAmount`) (`self.MaxHealth`) (`self.LastUpdatedHealth`) (`self.Damage Type`) (`self.Instigated By`) (`self.Damage Causer`)))

(fn `Call On Health Updated`
  (`self.On Health Updated` (`self.Health`) (`self.MaxHealth`) (`self.LastUpdatedHealth`)))

(fn `Damage Function`
  (params (`Damage Amount` :type "Float (double-precision)"))
  (locals (`Health (Local)` :type "Float (double-precision)" :default 0.0))
  ;[0.01 0.01 0.01] If The Actor Can Be Damged Subtract The Damage Amoung Form Health Then Set The New Health Value and New Health State
  (if (`self.CanBeDamaged?`)
    (set `self.LastUpdatedHealth` (`self.Health`))
    (bind _output_get (set `local.Health (Local)` (`KismetMathLibrary.FClamp` (- (`self.Health`) (`local.Damage Amount`)) 0.0 (`self.MaxHealth`))))
    (if (<= _output_get 0.0)
      (`self.Dead Function`)
      (else
        (`self.On Damaged Function`)))
    (`self.ROS_Update Health` true (`local.Health (Local)`) (`self.MaxHealth`))))

(fn `Dead Function`
  ;[0.01 0.01 0.01] Set Death Variables
  (set `self.IsDead?` true)
  (set `self.CanHeal?` false)
  (set `self.CanBeDamaged?` false)
  (if (`KismetSystemLibrary.K2_IsValidTimerHandle` (`self.RegenerateHealthTimer`))
    (`KismetSystemLibrary.K2_ClearAndInvalidateTimerHandle` (`self.RegenerateHealthTimer`))))

(fn `Heal Function`
  (params (HealAmount :type "Float (double-precision)"))
  (locals (`Health (Local)` :type "Float (double-precision)" :default 0.0))
  ;[0.01 0.01 0.01] If The Actor Can Heal Add The Healing Amount To Health Then Set The New Health Value and New Health State
  (if (and (`self.CanHeal?`) (!= (`self.Health`) (`self.MaxHealth`)))
    (set `self.LastUpdatedHealth` (`self.Health`))
    (set `local.Health (Local)` (`KismetMathLibrary.FClamp` (+ (`self.Health`) (`local.HealAmount`)) 0.0 (`self.MaxHealth`)))
    (`self.On Healed Function`)
    (if (>= (`local.Health (Local)`) (`self.MaxHealth`))
      (`self.On Full Health Function`)
      (`self.ROS_Update Health` true (`local.Health (Local)`) (`self.MaxHealth`))
      (set `self.IsHealing?` false)
      (else
        (`self.ROS_Update Health` true (`local.Health (Local)`) (`self.MaxHealth`))))
    (elif (`KismetSystemLibrary.K2_IsValidTimerHandle` (`self.RegenerateHealthTimer`))
      (`KismetSystemLibrary.K2_ClearAndInvalidateTimerHandle` (`self.RegenerateHealthTimer`)))))

(fn `On Damaged Function`
  ;[0.01 0.01 0.01] Set Variables, Regenerate Health
  (set `self.IsFullHealth?` false)
  (set `self.IsDamaged?` true)
  (set `self.IsHealing?` false)
  (`self.Regenerate Health?`))

(fn `On Full Health Function`
  ;[0.01 0.01 0.01] Set Full Health Variables And Clear Regen Timer If Valid
  (set `self.IsFullHealth?` true)
  (set `self.IsDamaged?` false)
  (if (`KismetSystemLibrary.K2_IsValidTimerHandle` (`self.RegenerateHealthTimer`))
    (`KismetSystemLibrary.K2_ClearTimer` null "HealthRegen")))

(fn `On Healed Function`
  ;[0.01 0.01 0.01] Set Healing Variables
  (set `self.IsHealing?` true)
  (set `self.IsDamaged?` false))

(fn `On Health Regeneration Updated`
  (params (`CanRegenerateHealth?` :type Boolean) (RegenerationAmount :type "Float (double-precision)") (RegenerationRate :type "Float (single-precision)") (RegenerationDelay :type "Float (double-precision)"))
  (set `self.CanRegenerateHealth?` `CanRegenerateHealth?`)
  (set `self.RegenerationAmount` (`local.RegenerationAmount`))
  (set `self.RegenerationRate` (`local.RegenerationRate`))
  (set `self.RegenerationDelay` (`local.RegenerationDelay`))
  (`self.Regenerate Health?`))

(fn `On Take Any Damage`
  (params (`Damaged Actor` :type "Actor Object Reference") (Damage :type "Float (single-precision)") (`Damage Type` :type "DamageType Object Reference") (`Instigated By` :type "Controller Object Reference") (`Damage Causer` :type "Actor Object Reference"))
  ;[0.01 0.01 0.01] Set Damage Variables And Check If Damage Is Greater Than Zero Then Do Damage, If Not Then Heal
  (set `self.Damaged Actor` `Damaged Actor`)
  (set `self.Damage Type` (`local.Damage Type`))
  (set `self.Instigated By` (`local.Instigated By`))
  (set `self.Damage Causer` (`local.Damage Causer`))
  (if (> (`local.Damage`) 0.0)
    (bind _output_get (set `self.DamageAmount` (`local.Damage`)))
    (`self.Damage Function` _output_get)
    (else
      (bind _output_get_2 (set `self.HealAmount` (* (`local.Damage`) -1.0)))
      (`self.Heal Function` _output_get_2))))

(fn `OnRep_Health`
  ;[0.01 0.01 0.01] Update Health And Check Health State Then Call The Related Event Dispatchers
  (`self.Call On Health Updated`)
  (if (`self.CallEventDispatchers?`)
    (`|ExecutionSequence`
      (:`then_0`
        (if (`self.IsDead?`)
          (`self.Call On Death`)))
      (:`then_1`
        (if (`self.IsHealing?`)
          (`self.Call On Any Heal`)))
      (:`then_2`
        (if (`self.IsFullHealth?`)
          (`self.Call On Full Health`)))
      (:`then_3`
        (if (`self.IsDamaged?`)
          (`self.Call On Any Damaged`))))))

(fn `Update Health Function`
  (params (Health :type "Float (double-precision)") (`Max Health` :type "Float (double-precision)"))
  ;[0.01 0.01 0.01] Set Max Health Only If It Changed And Set Health Then Check If Health Regeneration Is Needed
  (if (!= `Max Health` (`self.MaxHealth`))
    (set `self.MaxHealth` (`local.Max Health`)))
  (bind _output_get (set `self.Health` (`local.Health`)))
  (if (and (< _output_get (`self.MaxHealth`)) (not (`KismetSystemLibrary.K2_IsValidTimerHandle` (`self.RegenerateHealthTimer`))))
    (`self.Regenerate Health?`)))