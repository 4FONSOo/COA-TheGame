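; Game mode for the ERHealthSystem Lite demonstration that spawns or respawns players at random Player Start actors.
; SpawnPlayer destroys the controller's existing pawn, spawns a BP_ERHealthCharacter at a random start and possesses it.
; It then calls RestartPlayerAtTransform with a separately rolled random start, which may differ from the spawn location.
; Nothing in this Blueprint calls SpawnPlayer itself.
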(fn `Get Random Player Start`
  (returns (`Player Start Transform` :type "Transform Structure (by ref)"))
  (bind _outactors (`GameplayStatics.GetAllActorsOfClass` "/Script/Engine.PlayerStart"))
  (return (`self.GetTransform` (`|GetArrayItem` _outactors (`KismetMathLibrary.RandomIntegerInRange` 0 (- (`KismetArrayLibrary.Array_Length` _outactors) 1))))))

(fn `Spawn Player`
  (params (`Player Controller` :type "PlayerController Object Reference"))
  (bind _returnvalue (`Controller.K2_GetPawn` `Player Controller`))
  (`/Engine/EditorBlueprintResources/StandardMacros.IsValid` _returnvalue
    (:`Is Valid`
      (`self.K2_DestroyActor` _returnvalue))
    (:`Is Not Valid`
      _))
  (bind _returnvalue_2 (`|SpawnActorFromClass` "/Game/ERHealthSystem_Lite/Demonstration/Blueprints/BP_ERHealthCharacter.BP_ERHealthCharacter_C" (`self.Get Random Player Start`) "Undefined" "MultiplyWithRoot" null null))
  (`Controller.Possess` (`local.Player Controller`) _returnvalue_2)
  (`self.RestartPlayerAtTransform` (`local.Player Controller`) (`self.Get Random Player Start`)))

(fn `UserConstructionScript`)