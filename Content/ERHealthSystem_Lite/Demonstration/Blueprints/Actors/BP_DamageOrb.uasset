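; BP_DamageOrb is an ERHealthSystem demo pickup: a red glowing orb that applies damage to overlapping actors with an ERHealth component.
; On the server, overlap checks CanBeDamaged, applies BaseDamage and hides the orb, with a DoOnce gate preventing repeat hits.
; The HideInGame RepNotify toggles sphere visibility, starts the respawn timer and resets the gate on show.
; Construction sets the dynamic material and server-side InterpToMovement path.
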(event `self.SphereCollision.OnComponentBeginOverlap`
  (params (OverlappedComponent :type "PrimitiveComponent Object Reference") (OtherActor :type "Actor Object Reference") (OtherComp :type "PrimitiveComponent Object Reference") (OtherBodyIndex :type Integer) (bFromSweep :type Boolean) (SweepResult :type "HitResult Structure (by ref)"))
  ;[0.01 0.01 0.01] (Health Pickup Example) On Component Begin Overlap Check If The Actor Has ERHealth Component And Heal Using(ApplyDamage) Then Hide (Sphere) And Show After A Delay
  (`/Engine/EditorBlueprintResources/ActorMacros.Switch Has Authority`
    (:`Authority`
      (bind _output_get (set `self.ERHealthComponent` (`self.GetComponentByClass` OtherActor "/Game/ERHealthSystem_Lite/Blueprints/Component/ERHealthComponent.ERHealthComponent_C")))
      (`/Engine/EditorBlueprintResources/StandardMacros.IsValid` _output_get
        (:`Is Valid`
          (`/Engine/EditorBlueprintResources/StandardMacros.DoOnce` false :!label _label
            (:`Completed`
              (if (`/Game/ERHealthSystem_Lite/Blueprints/Component/ERHealthComponent.CanBeDamaged?` (`self.ERHealthComponent`))
                (`GameplayStatics.ApplyDamage` OtherActor (`self.BaseDamage`) null self)
                (`self.Hide`)
                (else
                  (goto _label :!via `Reset`))))))))))

(event `Reset`
  ;[0.01 0.01 0.01] (Health Pickup Example) On Component Begin Overlap Check If The Actor Has ERHealth Component And Heal Using(ApplyDamage) Then Hide (Sphere) And Show After A Delay
  (goto _label :!via `Reset`))

(event `Hide`
  ;[0.01 0.01 0.01] (Health Pickup Example) On Component Begin Overlap Check If The Actor Has ERHealth Component And Heal Using(ApplyDamage) Then Hide (Sphere) And Show After A Delay
  (set `self.HideInGame?` true))

(event `Show`
  ;[0.01 0.01 0.01] (Health Pickup Example) On Component Begin Overlap Check If The Actor Has ERHealth Component And Heal Using(ApplyDamage) Then Hide (Sphere) And Show After A Delay
  (set `self.HideInGame?` false))

(fn `OnRep_HideInGame?`
  (if (`self.HideInGame?`)
    (`SceneComponent.SetHiddenInGame` (`self.Sphere`) true false)
    (`KismetSystemLibrary.K2_SetTimer` null "Show" (`self.RespawnDelay`))
    (else
      (`SceneComponent.SetHiddenInGame` (`self.Sphere`) false false)
      (`self.Reset`))))

(fn `UserConstructionScript`
  (bind _returnvalue (`PrimitiveComponent.CreateDynamicMaterialInstance` (`self.Sphere`) 0 "/Engine/VREditor/UI/FrameMaterial.FrameMaterial" "None"))
  (`MaterialInstanceDynamic.SetVectorParameterValue` _returnvalue "BaseColor" (struct :`R` 0.301961 :`A` 1.0))
  (`MaterialInstanceDynamic.SetScalarParameterValue` _returnvalue "GlowAmount" 1.0)
  (`/Engine/EditorBlueprintResources/ActorMacros.Switch Has Authority`
    (:`Authority`
      (`InterpToMovementComponent.AddControlPointPosition` (`self.InterpToMovement`) (0.0 0.0 0.0) true)
      (`InterpToMovementComponent.AddControlPointPosition` (`self.InterpToMovement`) (`self.TargetPosition`) true)
      (set `InterpToMovementComponent.Duration` (`self.Duration`) (`self.InterpToMovement`)))))