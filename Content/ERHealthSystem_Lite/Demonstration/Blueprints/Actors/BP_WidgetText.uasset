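; Demonstration actor in ERHealthSystem_Lite that shows a text label in the world when the player is near.
; On BeginPlay it creates a W_Text widget, assigns it to its Widget component and fills it with the Text variable.
; Every Tick it hides or shows the whole actor by checking whether the first player pawn is within WidgetDistance.
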(event `self.ReceiveBeginPlay`
  (bind _returnvalue (`|CreateWidget` "/Game/ERHealthSystem_Lite/Demonstration/Blueprints/Widgets/W_Text.W_Text_C"))
  (`/Engine/EditorBlueprintResources/StandardMacros.IsValid` _returnvalue
    (:`Is Valid`
      (`WidgetComponent.SetWidget` (`self.Widget`) _returnvalue)
      (set `MultiLineEditableTextBox.Text` (`self.Text`) (`/Game/ERHealthSystem_Lite/Demonstration/Blueprints/Widgets/W_Text.Text` _returnvalue)))))

(event `self.ReceiveTick`
  (params (DeltaSeconds :type "Float (single-precision)"))
  (if (`self.Is Player In Range?`)
    (`self.SetActorHiddenInGame` false)
    (else
      (`self.SetActorHiddenInGame` true))))

(fn `Is Player In Range?`
  (returns (PlayerInRange :type Boolean))
  (if (`KismetSystemLibrary.IsValid` (`GameplayStatics.GetPlayerPawn` 0))
    (return (< (`KismetMathLibrary.Vector_Distance` (`self.K2_GetActorLocation`) (`self.K2_GetActorLocation` (`GameplayStatics.GetPlayerPawn` 0))) (`self.WidgetDistance`)))))

(fn `UserConstructionScript`)