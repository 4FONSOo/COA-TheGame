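; BP_Sphere is a demo actor for the ERHealthSystem, an orange sphere with a health component and a health value widget.
; Damage, heal and Tick events push health to the widget, which shows only while the sphere lives and player 0 is within WidgetDistance.
; On death, the authority pops the sphere upward with physics, hides it, then spawns a replacement at its original transform and destroys itself.
; A RepNotify activates its InterpToMovement component.
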(event `self.ReceiveBeginPlay`
  (set `self.Spawn Transform` (`self.GetTransform`))
  (bind _asw_health_value (cast `/Game/ERHealthSystem_Lite/Demonstration/Blueprints/Widgets/W_HealthValue` (`WidgetComponent.GetWidget` (`self.HealthWidget`))))
  (bind _output_get (set `self.As W Health Value` _asw_health_value))
  (`/Game/ERHealthSystem_Lite/Demonstration/Blueprints/Widgets/W_HealthValue.Health Updated_Event` _output_get (`/Game/ERHealthSystem_Lite/Blueprints/Component/ERHealthComponent.Health` (`self.ERHealthComponent`)) (`/Game/ERHealthSystem_Lite/Blueprints/Component/ERHealthComponent.MaxHealth` (`self.ERHealthComponent`))))

(event `self.ReceiveTick`
  (params (DeltaSeconds :type "Float (single-precision)"))
  (if (not (`self.IsDead?`))
    (if (`self.Is Player In Range?`)
      (bind _as_w_health_value (`self.As W Health Value`)
        (:`then`
          (`Widget.SetVisibility` _as_w_health_value "HitTestInvisible")
          (`/Game/ERHealthSystem_Lite/Demonstration/Blueprints/Widgets/W_HealthValue.Health Updated_Event` (`self.As W Health Value`) (`/Game/ERHealthSystem_Lite/Blueprints/Component/ERHealthComponent.Health` (`self.ERHealthComponent`)) (`/Game/ERHealthSystem_Lite/Blueprints/Component/ERHealthComponent.MaxHealth` (`self.ERHealthComponent`))))
        (:`else`))
      (else
        (bind _as_w_health_value_2 (`self.As W Health Value` :!label _label)
          (:`then`
            (`Widget.SetVisibility` _as_w_health_value_2 "Collapsed")
            (`/Game/ERHealthSystem_Lite/Demonstration/Blueprints/Widgets/W_HealthValue.Health Updated_Event` (`self.As W Health Value`) (`/Game/ERHealthSystem_Lite/Blueprints/Component/ERHealthComponent.Health` (`self.ERHealthComponent`)) (`/Game/ERHealthSystem_Lite/Blueprints/Component/ERHealthComponent.MaxHealth` (`self.ERHealthComponent`))))
          (:`else`))))
    (else
      (goto _label))))

(event `self.ERHealthComponent.On Any Damage`
  (params (DamagedActor :type "Actor Object Reference") (DamageAmount :type "Float (double-precision)") (Health :type "Float (double-precision)") (MaxHealth :type "Float (double-precision)") (LastUpdatedHealth :type "Float (double-precision)") (DamageType :type "DamageType Object Reference") (InstigatedBy :type "Controller Object Reference") (DamageCauser :type "Actor Object Reference"))
  (`/Game/ERHealthSystem_Lite/Demonstration/Blueprints/Widgets/W_HealthValue.Health Updated_Event` (`self.As W Health Value`) Health MaxHealth))

(event `self.ERHealthComponent.On Any Heal`
  (params (HealedActor :type "Actor Object Reference") (HealAmount :type "Float (double-precision)") (Health :type "Float (double-precision)") (MaxHealth :type "Float (double-precision)") (LastUpdatedHealth :type "Float (double-precision)") (HealType :type "DamageType Object Reference") (InstigatedBy :type "Controller Object Reference") (HealCauser :type "Actor Object Reference"))
  (`/Game/ERHealthSystem_Lite/Demonstration/Blueprints/Widgets/W_HealthValue.Health Updated_Event` (`self.As W Health Value`) Health MaxHealth))

(event `self.ERHealthComponent.On Death`
  (params (DamagedActor :type "Actor Object Reference") (DamageAmount :type "Float (single-precision)") (MaxHealth :type "Float (double-precision)") (LastUpdatedHealth :type "Float (double-precision)") (DamageType :type "DamageType Object Reference") (InstigatedBy :type "Controller Object Reference") (DamageCauser :type "Actor Object Reference"))
  (`/Engine/EditorBlueprintResources/ActorMacros.Switch Has Authority`
    (:`Authority`
      (set `self.IsDead?` true)
      (`PrimitiveComponent.SetSimulatePhysics` (`self.Sphere`) true)
      (`PrimitiveComponent.AddImpulse` (`self.Sphere`) (0.0 0.0 500.0) "None" true)
      (`KismetSystemLibrary.Delay` 1.0)
      (`SceneComponent.SetVisibility` (`self.Sphere`) false false)
      (`PrimitiveComponent.SetSimulatePhysics` (`self.Sphere`) false)
      (`PrimitiveComponent.SetCollisionEnabled` (`self.Sphere`) "NoCollision")
      (`KismetSystemLibrary.Delay` 1.0)
      (`|SpawnActorFromClass` "BP_Sphere_C" (`self.Spawn Transform`) "AlwaysSpawn" "MultiplyWithRoot" null (`self.WidgetDistance`) null)
      (`self.K2_DestroyActor`))))

(fn `Is Player In Range?`
  (returns (PlayerInRange :type Boolean))
  (if (`KismetSystemLibrary.IsValid` (`GameplayStatics.GetPlayerPawn` 0))
    (return (< (`KismetMathLibrary.Vector_Distance` (`self.K2_GetActorLocation`) (`self.K2_GetActorLocation` (`GameplayStatics.GetPlayerPawn` 0))) (`self.WidgetDistance`)))))

(fn `OnRep_MoveActor?`
  (`ActorComponent.Activate` (`self.InterpToMovement`) false))

(fn `UserConstructionScript`
  (bind _returnvalue (`PrimitiveComponent.CreateDynamicMaterialInstance` (`self.Sphere`) 0 "/Engine/TemplateResources/MI_Template_BaseGray.MI_Template_BaseGray" "None"))
  (bind _output_get (set `self.Material Instance` _returnvalue))
  (`MaterialInstanceDynamic.SetVectorParameterValue` _output_get "DiffuseColor" (struct :`R` 1.0 :`G` 0.5 :`A` 1.0)))