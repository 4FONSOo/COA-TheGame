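; BP_DamageAOE is an ERHealthSystem Lite demo actor that deals damage over time to actors inside its box volume.
; Box overlap events track actors that have an ERHealthComponent in an array, removing them when they leave.
; A looping timer started at BeginPlay applies damage to each tracked actor, only on the authority.
; The construction script gives the cube a dynamic, glowing red material instance.
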(event `self.ReceiveBeginPlay`
  ;[0.01 0.01 0.01] Apply Damage Over Time Example
  (`KismetSystemLibrary.K2_SetTimerDelegate` (delegate `DamageTick`) 0.2 true))

(event `DamageTick`
  ;[0.01 0.01 0.01] Apply Damage Over Time Example
  (for _array_element (`self.OverlappingActors`)
    (`/Engine/EditorBlueprintResources/ActorMacros.Switch Has Authority`
      (:`Authority`
        (`GameplayStatics.ApplyDamage` _array_element (`self.BaseDamage`) null self)))))

(event `self.BoxCollision.OnComponentBeginOverlap`
  (params (OverlappedComponent :type "PrimitiveComponent Object Reference") (OtherActor :type "Actor Object Reference") (OtherComp :type "PrimitiveComponent Object Reference") (OtherBodyIndex :type Integer) (bFromSweep :type Boolean) (SweepResult :type "HitResult Structure (by ref)"))
  ;[0.01 0.01 0.01] On Component Begin Overlap Add Overlapping Actors With ERHealth Component To An Array
  (`/Engine/EditorBlueprintResources/StandardMacros.IsValid` (`self.GetComponentByClass` OtherActor "/Game/ERHealthSystem_Lite/Blueprints/Component/ERHealthComponent.ERHealthComponent_C")
    (:`Is Valid`
      (`KismetArrayLibrary.Array_Add` (`self.OverlappingActors`) OtherActor))))

(event `self.BoxCollision.OnComponentEndOverlap`
  (params (OverlappedComponent :type "PrimitiveComponent Object Reference") (OtherActor :type "Actor Object Reference") (OtherComp :type "PrimitiveComponent Object Reference") (OtherBodyIndex :type Integer))
  (bind _returnvalue (`KismetArrayLibrary.Array_Find` (`self.OverlappingActors`) OtherActor))
  ;[0.01 0.01 0.01] On Component End Overlap Remove Actors From (Overlapping Actors Array)
  (if (>= _returnvalue 0)
    (`KismetArrayLibrary.Array_Remove` (`self.OverlappingActors`) _returnvalue)))

(fn `UserConstructionScript`
  (bind _returnvalue (`PrimitiveComponent.CreateDynamicMaterialInstance` (`self.Cube`) 0 "/Engine/VREditor/UI/FrameMaterial.FrameMaterial" "None"))
  (`MaterialInstanceDynamic.SetVectorParameterValue` _returnvalue "BaseColor" (struct :`R` 0.3 :`A` 1.0))
  (`MaterialInstanceDynamic.SetScalarParameterValue` _returnvalue "GlowAmount" 1.0))