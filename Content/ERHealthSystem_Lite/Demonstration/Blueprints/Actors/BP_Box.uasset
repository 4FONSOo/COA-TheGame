(event `self.ReceiveBeginPlay`
  (bind _as_w_note_text (`self.As W Note Text`))
  (bind _as_w_note_text_2 (`self.As W Note Text`))
  (set `self.Spawn Transform` (`self.GetTransform`))
  (bind _asw_health_value (cast `/Game/ERHealthSystem_Lite/Demonstration/Blueprints/Widgets/W_HealthValue` (`WidgetComponent.GetWidget` (`self.HealthWidget`))))
  (bind _output_get (set `self.As W Health Value` _asw_health_value))
  (`/Game/ERHealthSystem_Lite/Demonstration/Blueprints/Widgets/W_HealthValue.Health Updated_Event` _output_get (`/Game/ERHealthSystem_Lite/Blueprints/Component/ERHealthComponent.Health` (`self.ERHealthComponent`)) (`/Game/ERHealthSystem_Lite/Blueprints/Component/ERHealthComponent.MaxHealth` (`self.ERHealthComponent`)))
  (`Widget.SetVisibility` (`self.As W Health Value`) "Collapsed")
  (if (`self.UseNoteWidget?`)
    (`SceneComponent.SetVisibility` (`self.TextWidget`) true false)
    (bind _asw_note_text (cast `/Game/ERHealthSystem_Lite/Demonstration/Blueprints/Widgets/W_NoteText` (`WidgetComponent.GetWidget` (`self.TextWidget`))))
    (bind _output_get_2 (set `self.As W Note Text` _asw_note_text))
    (`Widget.SetVisibility` _output_get_2 "Collapsed")
    (`/Game/ERHealthSystem_Lite/Blueprints/Component/ERHealthComponent.PauseHealing` (`self.ERHealthComponent`) true)
    (`/Game/ERHealthSystem_Lite/Demonstration/Blueprints/Widgets/W_NoteText.Set Pause Healing` _as_w_note_text "Pause Healing: True")
    (`TextBlock.SetColorAndOpacity` (`/Game/ERHealthSystem_Lite/Demonstration/Blueprints/Widgets/W_NoteText.PauseHealing` _as_w_note_text) (make `SlateColor` (struct :`G` 0.4 :`A` 1.0)))
    (`/Game/ERHealthSystem_Lite/Demonstration/Blueprints/Widgets/W_NoteText.Set Invincible` _as_w_note_text_2 "Invincible: False")
    (`TextBlock.SetColorAndOpacity` (`/Game/ERHealthSystem_Lite/Demonstration/Blueprints/Widgets/W_NoteText.Invincible` _as_w_note_text_2) (make `SlateColor` (struct :`R` 0.4 :`A` 1.0)))
    (bind _returnvalue (`KismetSystemLibrary.K2_SetTimerDelegate` (delegate `Invincible?/PauseHealing?_Event`) 5.0 true))
    (set `self.TimerHandle` _returnvalue)))

(event `self.ReceiveTick`
  (params (DeltaSeconds :type "Float (single-precision)"))
  (if (not (`self.IsDead?`))
    (if (`self.Is Player In Range?`)
      (bind _as_w_health_value (`self.As W Health Value`)
        (:`then`
          (`Widget.SetVisibility` _as_w_health_value "HitTestInvisible")
          (`/Game/ERHealthSystem_Lite/Demonstration/Blueprints/Widgets/W_HealthValue.Health Updated_Event` (`self.As W Health Value`) (`/Game/ERHealthSystem_Lite/Blueprints/Component/ERHealthComponent.Health` (`self.ERHealthComponent`)) (`/Game/ERHealthSystem_Lite/Blueprints/Component/ERHealthComponent.MaxHealth` (`self.ERHealthComponent`))))
        (:`else`
          _))
      (bind _as_w_note_text (`self.As W Note Text`)
        (:`then`
          (`Widget.SetVisibility` _as_w_note_text "HitTestInvisible"))
        (:`else`))
      (else
        (bind _as_w_health_value_2 (`self.As W Health Value` :!label _label)
          (:`then`
            (`Widget.SetVisibility` _as_w_health_value_2 "Collapsed")
            (`/Game/ERHealthSystem_Lite/Demonstration/Blueprints/Widgets/W_HealthValue.Health Updated_Event` (`self.As W Health Value`) (`/Game/ERHealthSystem_Lite/Blueprints/Component/ERHealthComponent.Health` (`self.ERHealthComponent`)) (`/Game/ERHealthSystem_Lite/Blueprints/Component/ERHealthComponent.MaxHealth` (`self.ERHealthComponent`))))
          (:`else`
            _))
        (bind _as_w_note_text_2 (`self.As W Note Text`)
          (:`then`
            (`Widget.SetVisibility` _as_w_note_text_2 "Collapsed"))
          (:`else`))))
    (else
      (goto _label))))

(event `Invincible?/PauseHealing?_Event`
  (bind _as_w_note_text (`self.As W Note Text`))
  (bind _as_w_note_text_2 (`self.As W Note Text`))
  (bind _as_w_note_text_3 (`self.As W Note Text`))
  (bind _as_w_note_text_4 (`self.As W Note Text`))
  (`/Engine/EditorBlueprintResources/StandardMacros.FlipFlop`
    (:`A`
      (`/Game/ERHealthSystem_Lite/Blueprints/Component/ERHealthComponent.Invincibility` (`self.ERHealthComponent`) true)
      (`/Game/ERHealthSystem_Lite/Blueprints/Component/ERHealthComponent.PauseHealing` (`self.ERHealthComponent`) false)
      (`/Game/ERHealthSystem_Lite/Demonstration/Blueprints/Widgets/W_NoteText.Set Pause Healing` _as_w_note_text_2 "Pause Healing: False")
      (`TextBlock.SetColorAndOpacity` (`/Game/ERHealthSystem_Lite/Demonstration/Blueprints/Widgets/W_NoteText.PauseHealing` _as_w_note_text_2) (make `SlateColor` (struct :`R` 0.4 :`A` 1.0)))
      (`/Game/ERHealthSystem_Lite/Demonstration/Blueprints/Widgets/W_NoteText.Set Invincible` _as_w_note_text "Invincible: True")
      (`TextBlock.SetColorAndOpacity` (`/Game/ERHealthSystem_Lite/Demonstration/Blueprints/Widgets/W_NoteText.Invincible` _as_w_note_text) (make `SlateColor` (struct :`G` 0.4 :`A` 1.0))))
    (:`B`
      (`/Game/ERHealthSystem_Lite/Blueprints/Component/ERHealthComponent.Invincibility` (`self.ERHealthComponent`) false)
      (`/Game/ERHealthSystem_Lite/Blueprints/Component/ERHealthComponent.PauseHealing` (`self.ERHealthComponent`) true)
      (`/Game/ERHealthSystem_Lite/Demonstration/Blueprints/Widgets/W_NoteText.Set Pause Healing` _as_w_note_text_3 "Pause Healing: True")
      (`TextBlock.SetColorAndOpacity` (`/Game/ERHealthSystem_Lite/Demonstration/Blueprints/Widgets/W_NoteText.PauseHealing` _as_w_note_text_3) (make `SlateColor` (struct :`G` 0.4 :`A` 1.0)))
      (`/Game/ERHealthSystem_Lite/Demonstration/Blueprints/Widgets/W_NoteText.Set Invincible` _as_w_note_text_4 "Invincible: False")
      (`TextBlock.SetColorAndOpacity` (`/Game/ERHealthSystem_Lite/Demonstration/Blueprints/Widgets/W_NoteText.Invincible` _as_w_note_text_4) (make `SlateColor` (struct :`R` 0.4 :`A` 1.0))))))

(event `self.ERHealthComponent.On Any Damage`
  (params (DamagedActor :type "Actor Object Reference") (DamageAmount :type "Float (double-precision)") (Health :type "Float (double-precision)") (MaxHealth :type "Float (double-precision)") (LastUpdatedHealth :type "Float (double-precision)") (DamageType :type "DamageType Object Reference") (InstigatedBy :type "Controller Object Reference") (DamageCauser :type "Actor Object Reference"))
  (bind _material_instance (`self.Material Instance`))
  (`/Game/ERHealthSystem_Lite/Demonstration/Blueprints/Widgets/W_HealthValue.Health Updated_Event` (`self.As W Health Value`) Health MaxHealth)
  (`|ExecutionSequence`
    (:`then_0`
      (`MaterialInstanceDynamic.SetVectorParameterValue` _material_instance "DiffuseColor" (struct :`R` 0.4 :`A` 1.0)))
    (:`then_1`
      (`KismetSystemLibrary.RetriggerableDelay` 0.05)
      (`MaterialInstanceDynamic.SetVectorParameterValue` _material_instance "DiffuseColor" (struct :`R` 0.003922 :`G` 0.137255 :`B` 0.576471 :`A` 1.0)))))

(event `self.ERHealthComponent.On Death`
  (params (DamagedActor :type "Actor Object Reference") (DamageAmount :type "Float (single-precision)") (MaxHealth :type "Float (double-precision)") (LastUpdatedHealth :type "Float (double-precision)") (DamageType :type "DamageType Object Reference") (InstigatedBy :type "Controller Object Reference") (DamageCauser :type "Actor Object Reference"))
  (`|ExecutionSequence`
    (:`then_0`
      (`/Engine/EditorBlueprintResources/ActorMacros.Switch Has Authority`
        (:`Authority`
          (set `self.IsDead?` true)
          (`PrimitiveComponent.AddImpulse` (`self.Cube`) (0.0 0.0 500.0) "None" true)
          (`KismetSystemLibrary.Delay` 1.0)
          (`SceneComponent.SetVisibility` (`self.Cube`) false false)
          (`PrimitiveComponent.SetSimulatePhysics` (`self.Cube`) false)
          (`PrimitiveComponent.SetCollisionEnabled` (`self.Cube`) "NoCollision")
          (`KismetSystemLibrary.Delay` 1.0)
          (`|SpawnActorFromClass` "BP_Box_C" (`self.Spawn Transform`) "AlwaysSpawn" "MultiplyWithRoot" null (`self.Can RegenerateHealth?`) (`self.UseHealEffect?`) (`self.Health`) (`self.UseNoteWidget?`) (`self.WidgetDistance`) null)
          (`self.K2_DestroyActor`))))
    (:`then_1`
      (bind _as_w_note_text (`self.As W Note Text`)
        (:`then`
          (`Widget.SetVisibility` _as_w_note_text "Collapsed")
          (if (`KismetSystemLibrary.K2_IsValidTimerHandle` (`self.TimerHandle`))
            (`KismetSystemLibrary.K2_ClearAndInvalidateTimerHandle` (`self.TimerHandle`))))
        (:`else`)))))

(event `self.ERHealthComponent.On Any Heal`
  (params (HealedActor :type "Actor Object Reference") (HealAmount :type "Float (double-precision)") (Health :type "Float (double-precision)") (MaxHealth :type "Float (double-precision)") (LastUpdatedHealth :type "Float (double-precision)") (HealType :type "DamageType Object Reference") (InstigatedBy :type "Controller Object Reference") (HealCauser :type "Actor Object Reference"))
  (bind _material_instance (`self.Material Instance`))
  (`/Game/ERHealthSystem_Lite/Demonstration/Blueprints/Widgets/W_HealthValue.Health Updated_Event` (`self.As W Health Value`) Health MaxHealth)
  (if (`self.UseHealEffect?`)
    (`|ExecutionSequence`
      (:`then_0`
        (`MaterialInstanceDynamic.SetVectorParameterValue` _material_instance "DiffuseColor" (struct :`G` 0.301961 :`A` 1.0)))
      (:`then_1`
        (`KismetSystemLibrary.RetriggerableDelay` 0.05)
        (`MaterialInstanceDynamic.SetVectorParameterValue` _material_instance "DiffuseColor" (struct :`R` 0.003922 :`G` 0.137255 :`B` 0.576471 :`A` 1.0))))))

(fn `Is Player In Range?`
  (returns (PlayerInRange :type Boolean))
  (if (`KismetSystemLibrary.IsValid` (`GameplayStatics.GetPlayerPawn` 0))
    (return (< (`KismetMathLibrary.Vector_Distance` (`self.K2_GetActorLocation`) (`self.K2_GetActorLocation` (`GameplayStatics.GetPlayerPawn` 0))) (`self.WidgetDistance`)))))

(fn `UserConstructionScript`
  (bind _returnvalue (`PrimitiveComponent.CreateDynamicMaterialInstance` (`self.Cube`) 0 "/Engine/TemplateResources/MI_Template_BaseGray.MI_Template_BaseGray" "None"))
  (bind _output_get (set `self.Material Instance` _returnvalue))
  (`MaterialInstanceDynamic.SetVectorParameterValue` _output_get "DiffuseColor" (struct :`R` 0.003922 :`G` 0.137255 :`B` 0.576471 :`A` 1.0))
  (set `/Game/ERHealthSystem_Lite/Blueprints/Component/ERHealthComponent.CanRegenerateHealth?` (`self.Can RegenerateHealth?`) (`self.ERHealthComponent`))
  (`/Game/ERHealthSystem_Lite/Blueprints/Component/ERHealthComponent.Update Health` (`self.ERHealthComponent`) (`self.Health`) (`/Game/ERHealthSystem_Lite/Blueprints/Component/ERHealthComponent.MaxHealth` (`self.ERHealthComponent`))))