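; Base interactable door actor that opens on interaction, either when already unlocked or when the character supplies a key for its door name.
; A successful UseKeyMessage call on the character sets Unlocked, so later interactions skip the key check.
; Opening plays two timelines together, sliding one pair of cubes along relative X and the other along relative Z.
; No closing logic exists, and debug strings print on interaction and unlock.
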(event `OpenDoor`
  (bind (_direction _door_1 _door_2) (`Timeline|Linha do tempo`)
    (:`Update`
      (`SceneComponent.K2_SetRelativeLocation` (`self.Cube_104`) (`KismetMathLibrary.MakeVector` _door_1) false false)
      (`SceneComponent.K2_SetRelativeLocation` (`self.Cube_103`) (`KismetMathLibrary.MakeVector` _door_2) false false))))

(event `OpenDoor2`
  (bind (_direction _door_1 _door_2) (`Timeline|Linha do tempo_0`)
    (:`Update`
      (`SceneComponent.K2_SetRelativeLocation` (`self.Cube_102`) (`KismetMathLibrary.MakeVector` 0.0 0.0 _door_1) false false)
      (`SceneComponent.K2_SetRelativeLocation` (`self.Cube_100`) (`KismetMathLibrary.MakeVector` 0.0 0.0 _door_2) false false))))

(event `/Game/sistemas/InteractableSystem/Interface/InteractableInterface.Interact`
  (params (Character :type "Actor Object Reference"))
  (`KismetSystemLibrary.PrintString` "porta")
  (if (`self.Unlocked`)
    (`self.OpenDoor`)
    (`self.OpenDoor2`)
    (else
      (bind _door_unlocked (message `/Game/sistemas/InteractableSystem/Interface/CharacterBPInterface.UseKey` Character (`self.DoorName`)))
      (if _door_unlocked
        (set `self.Unlocked` true)
        (`self.OpenDoor`)
        (`self.OpenDoor2`)
        (`KismetSystemLibrary.PrintString` "DoorUnlocked")))))

(fn `UserConstructionScript`
  (`parent.UserConstructionScript`))