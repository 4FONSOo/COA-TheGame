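; Light-sequence trigger that stages a blackout when the player enters it, then relights the rect lights in red and starts the alarms.
; After a delay, ApagarProximaLuz re-enters a timed loop that turns off one light and hides its paired mesh per step, with sound.
; ReacenderTodas then spawns an effect, hides the sky actor, restores lights and meshes and plays sound cues.
; An old E-key start remains; the red-light flicker is left disconnected.
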(event `self.TriggerInteracao.OnComponentBeginOverlap`
  (params (OverlappedComponent :type "PrimitiveComponent Object Reference") (OtherActor :type "Actor Object Reference") (OtherComp :type "PrimitiveComponent Object Reference") (OtherBodyIndex :type Integer) (bFromSweep :type Boolean) (SweepResult :type "HitResult Structure (by ref)"))
  (bind _indiceactual (`self.IndiceActual`))
  (bind _output (`|GetArrayItem` (`self.Luzes`) (`self.IndiceActual`)))
  (bind _output_2 (`|GetArrayItem` (`self.MeshesParaEsconder`) _indiceactual))
  (`GameplayStatics.SpawnSound2D` null 1.0 1.0 0.0 null)
  (if (== OtherActor (`GameplayStatics.GetPlayerCharacter` 0))
    (set `self.JogadorDentro` true)
    (`self.EnableInput` (`GameplayStatics.GetPlayerController` 0))
    (`KismetSystemLibrary.Delay` 5.0)
    (if (< (`self.IndiceActual`) (`KismetArrayLibrary.Array_Length` (`self.Luzes`))) :!label _label
      (if (`KismetSystemLibrary.IsValid` _output)
        (`GameplayStatics.SpawnSoundAtLocation` null (`self.K2_GetActorLocation` _output) (struct) 1.0 1.0 0.0 null null)
        (`SceneComponent.SetVisibility` (`RectLight.RectLightComponent` _output) false false)
        (if (`KismetSystemLibrary.IsValid` _output_2)
          (`SceneComponent.SetHiddenInGame` (`StaticMeshActor.StaticMeshComponent` _output_2) true false))
        (set `self.IndiceActual` (+ _indiceactual 1))
        (`KismetSystemLibrary.Delay` (`self.TempoEntreLuzes`))
        (`self.ApagarProximaLuz`)
        (`ActorComponent.K2_DestroyComponent` (`self.TriggerInteracao`)))
      (else
        (`KismetSystemLibrary.Delay` (`self.Reacender`))
        (`self.ReacenderTodas`)))))

(event `ApagarProximaLuz`
  (goto _label))

(event `self.TriggerInteracao.OnComponentEndOverlap`
  (params (OverlappedComponent :type "PrimitiveComponent Object Reference") (OtherActor :type "Actor Object Reference") (OtherComp :type "PrimitiveComponent Object Reference") (OtherBodyIndex :type Integer))
  (if (== OtherActor (`GameplayStatics.GetPlayerCharacter` 0))
    (set `self.JogadorDentro` false)
    (`self.DisableInput` (`GameplayStatics.GetPlayerController` 0))))

(event `Key|E`
  (params (Key :type "Key Structure"))
  ; Old Key
  (:`Pressed`
    (`KismetSystemLibrary.Delay` 2.0)
    (if (`self.JogadorDentro`)
      (if (not (`self.SequenciaEmCurso`))
        (set `self.SequenciaEmCurso` true)
        (set `self.IndiceActual` 0)
        (`self.ApagarProximaLuz`)))))

(event `ReacenderTodas`
  (bind _returnvalue (`self.K2_GetActorLocation` (`self.ref_Smoke`)))
  (`GameplayStatics.SpawnSoundAtLocation` null _returnvalue (struct) 1.0 1.0 0.0 null null)
  (`GameplayStatics.SpawnEmitterAtLocation` null _returnvalue)
  (`self.SetActorHiddenInGame` (`self.ref_Sky`) true)
  (`KismetSystemLibrary.Delay` 5.0)
  (for _array_element (`self.Luzes`)
    (if (`KismetSystemLibrary.IsValid` _array_element)
      (bind _rectlightcomponent (`RectLight.RectLightComponent` _array_element))
      (`LightComponent.SetLightColor` _rectlightcomponent (`self.Vermelho`) true)
      (`SceneComponent.SetVisibility` _rectlightcomponent true false)
      (`GameplayStatics.SpawnSound2D` null 1.0 1.0 0.0 null)
      (for _array_element_2 (`self.MeshesParaEsconder`)
        (if (`KismetSystemLibrary.IsValid` _array_element_2)
          (`SceneComponent.SetHiddenInGame` (`StaticMeshActor.StaticMeshComponent` _array_element_2) false false)))
      (set `self.SequenciaEmCurso` false)
      (`GameplayStatics.SpawnSound2D` null 1.0 1.0 0.0 null)
      (for _array_element_3 (`self.Alarmes`)
        (if (`KismetSystemLibrary.IsValid` _array_element_3)
          (`/Game/Birra_New/11_EasterEggs/EasterEgg_3/BP_Alarme.LigarAlarme` _array_element_3)))
      (`KismetSystemLibrary.Delay` 2.5)
      (`GameplayStatics.SpawnSound2D` null 1.0 1.0 0.0 null)
      (`KismetSystemLibrary.Delay` 5.0)
      (`GameplayStatics.SpawnSound2D` null 1.0 1.0 0.0 null)
      (`KismetSystemLibrary.Delay` 4.0)
      (`GameplayStatics.SpawnSound2D` null 1.0 1.0 0.0 null)
      (`KismetSystemLibrary.Delay` 4.0)
      (`GameplayStatics.SpawnSound2D` null 1.0 1.0 0.0 null))))

(event `AtualizarFlickerVermelhas`
  ; Funciona, mas o efeito é, mehhhhhhh
)

(event `IniciarFlicker`
  ; Funciona, mas o efeito é, mehhhhhhh
  (set `self.FlickerAtivo` true)
  (`KismetSystemLibrary.K2_SetTimerDelegate` (delegate `AtualizarFlickerVermelhas`) (`self.IntervaloFlicker`) true))

(fn `UserConstructionScript`)