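; BP_CCTV is a controllable security camera actor with zoom, pan, tilt and an infrared view mode.
; Zoom events step the camera's field of view within min and max limits, starting from a default on BeginPlay.
; Tilt and pan step separate PitchPivot and YawPivot components within clamped angles, keeping each axis independent.
; Infrared toggles by switching the camera's post-process blend weight between off and fully on.
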(event `self.ReceiveBeginPlay`
  (bind _camera (`self.Camera`))
  (bind _output_get (set `self.CurrentFOV` (`self.DefaultFOV`)))
  (`CameraComponent.SetFieldOfView` _camera _output_get)
  (`CameraComponent.SetPostProcessBlendWeight` _camera 0.0))

(event `CamZoomIn`
  (bind _output_get (set `self.CurrentFOV` (`KismetMathLibrary.FClamp` (- (`self.CurrentFOV`) (`self.ZoomStep`)) (`self.MinFov`) (`self.MaxFov`))))
  (`CameraComponent.SetFieldOfView` (`self.Camera`) _output_get))

(event `CamZoomOut`
  (bind _output_get (set `self.CurrentFOV` (`KismetMathLibrary.FClamp` (+ (`self.CurrentFOV`) (`self.ZoomStep`)) (`self.MinFov`) (`self.MaxFov`))))
  (`CameraComponent.SetFieldOfView` (`self.Camera`) _output_get))

(event `CamTiltUp`
  (bind _pitchpivot (`self.PitchPivot`))
  (`SceneComponent.K2_SetRelativeRotation` _pitchpivot (`KismetMathLibrary.MakeRotator` 0.0 (`KismetMathLibrary.FClamp` (+ (.pitch (`SceneComponent.RelativeRotation` _pitchpivot)) (`self.TiltStep`)) (`self.MinPitch`) (`self.MaxPitch`))) false false))

(event `CamTiltDown`
  (bind _pitchpivot (`self.PitchPivot`))
  (`SceneComponent.K2_SetRelativeRotation` _pitchpivot (`KismetMathLibrary.MakeRotator` 0.0 (`KismetMathLibrary.FClamp` (- (.pitch (`SceneComponent.RelativeRotation` _pitchpivot)) (`self.TiltStep`)) (`self.MinPitch`) (`self.MaxPitch`))) false false))

(event `CamPanLeft`
  (bind _yawpivot (`self.YawPivot`))
  (`SceneComponent.K2_SetRelativeRotation` _yawpivot (`KismetMathLibrary.MakeRotator` 0.0 0.0 (`KismetMathLibrary.FClamp` (- (.yaw (`SceneComponent.RelativeRotation` _yawpivot)) (`self.PanStep`)) (`self.MinYaw`) (`self.MaxYaw`))) false false))

(event `CamPanRight`
  (bind _yawpivot (`self.YawPivot`))
  (`SceneComponent.K2_SetRelativeRotation` _yawpivot (`KismetMathLibrary.MakeRotator` 0.0 0.0 (`KismetMathLibrary.FClamp` (+ (.yaw (`SceneComponent.RelativeRotation` _yawpivot)) (`self.PanStep`)) (`self.MinYaw`) (`self.MaxYaw`))) false false))

(event `ToggleInfraRed`
  (bind _camera (`self.Camera`))
  (if (`self.bInfraRedOn`)
    (set `self.bInfraRedOn` false)
    (`CameraComponent.SetPostProcessBlendWeight` _camera 0.0)
    (else
      (set `self.bInfraRedOn` true)
      (`CameraComponent.SetPostProcessBlendWeight` _camera 1.0))))

(fn `UserConstructionScript`)