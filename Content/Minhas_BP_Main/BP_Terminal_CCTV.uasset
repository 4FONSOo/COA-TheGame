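; CCTV terminal actor that lets the first-person player view security cameras by pressing E after entering its collision box.
; Using it locks move and look input and blends the view through the Cameras array, with A/D cycling and wrapping.
; Wheel and arrow keys call zoom, pan and tilt on the whole array, ungated by terminal use.
; E again, or leaving the box while active, restores player view and input.
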(event `self.ReceiveBeginPlay`
  (bind _output_get (set `self.PCRef` (`GameplayStatics.GetPlayerController` 0)))
  (bind _asbp_first_person_character (cast `/Game/FirstPerson/Blueprints/BP_FirstPersonCharacter` (`GameplayStatics.GetPlayerCharacter` 0)))
  (set `self.PlayerRef` _asbp_first_person_character)
  (`self.EnableInput` _output_get))

(event `self.BoxColisao.OnComponentBeginOverlap`
  (params (OverlappedComponent :type "PrimitiveComponent Object Reference") (OtherActor :type "Actor Object Reference") (OtherComp :type "PrimitiveComponent Object Reference") (OtherBodyIndex :type Integer) (bFromSweep :type Boolean) (SweepResult :type "HitResult Structure (by ref)"))
  (if (== OtherActor (`self.PlayerRef`))
    (set `self.bPlayerInside` true)))

(event `self.BoxColisao.OnComponentEndOverlap`
  (params (OverlappedComponent :type "PrimitiveComponent Object Reference") (OtherActor :type "Actor Object Reference") (OtherComp :type "PrimitiveComponent Object Reference") (OtherBodyIndex :type Integer))
  (bind _busingterminal (`self.bUsingTerminal`))
  (if (== OtherActor (`self.PlayerRef`))
    (if _busingterminal
      (set `self.bPlayerInside` _busingterminal)
      (`self.ExitTerminal`))))

(event `EnterTerminal`
  (bind _pcref (`self.PCRef`))
  (if (> (`KismetArrayLibrary.Array_Length` (`self.Cameras`)) 0)
    (set `self.bUsingTerminal` true)
    (set `self.CurrentIndex` 0)
    (`Controller.SetIgnoreLookInput` _pcref true)
    (`Controller.SetIgnoreMoveInput` _pcref true)
    (`PlayerController.SetViewTargetWithBlend` _pcref (`|GetArrayItem` (`self.Cameras`) (`self.CurrentIndex`)) 0.15 "VTBlend_Linear" 0.0 false)))

(event `ExitTerminal`
  (bind _pcref (`self.PCRef`))
  (set `self.bUsingTerminal` false)
  (`Controller.ResetIgnoreMoveInput` _pcref)
  (`Controller.ResetIgnoreLookInput` _pcref)
  (`PlayerController.SetViewTargetWithBlend` _pcref (`self.PlayerRef`) 0.15 "VTBlend_Linear" 0.0 false))

(event `NextCamera`
  (bind _cameras (`self.Cameras`))
  (bind _returnvalue (`KismetArrayLibrary.Array_Length` _cameras))
  (if (`self.bUsingTerminal`)
    (if (> _returnvalue 0)
      (bind _output_get (set `self.CurrentIndex` (mod (+ (`self.CurrentIndex`) 1) _returnvalue)))
      (`PlayerController.SetViewTargetWithBlend` (`self.PCRef`) (`|GetArrayItem` _cameras _output_get) 0.15 "VTBlend_Linear" 0.0 false))))

(event `Key|E`
  (params (Key :type "Key Structure"))
  (:`Pressed`
    (if (`self.bPlayerInside`)
      (if (`self.bUsingTerminal`)
        (`self.ExitTerminal`)
        (else
          (`self.EnterTerminal`))))))

(event `PreviousCamera`
  (bind _cameras (`self.Cameras`))
  (bind _returnvalue (`KismetArrayLibrary.Array_Length` _cameras))
  (if (`self.bUsingTerminal`)
    (if (> _returnvalue 0)
      (bind _output_get (set `self.CurrentIndex` (mod (+ (- (`self.CurrentIndex`) 1) _returnvalue) _returnvalue)))
      (`PlayerController.SetViewTargetWithBlend` (`self.PCRef`) (`|GetArrayItem` _cameras _output_get) 0.15 "VTBlend_Linear" 0.0 false))))

(event `Key|D`
  (params (Key :type "Key Structure"))
  (:`Pressed`
    (`self.NextCamera`)))

(event `Key|A`
  (params (Key :type "Key Structure"))
  (:`Pressed`
    (`self.PreviousCamera`)))

(event `Key|MouseScrollUp`
  (params (Key :type "Key Structure"))
  (:`Pressed`
    (`/Game/Minhas_BP_Main/BP_CCTV.CamZoomIn` (`self.Cameras`))))

(event `Key|Left`
  (params (Key :type "Key Structure"))
  (:`Pressed`
    (`/Game/Minhas_BP_Main/BP_CCTV.CamPanLeft` (`self.Cameras`))))

(event `Key|MouseScrollDown`
  (params (Key :type "Key Structure"))
  (:`Pressed`
    (`/Game/Minhas_BP_Main/BP_CCTV.CamZoomOut` (`self.Cameras`))))

(event `Key|Right`
  (params (Key :type "Key Structure"))
  (:`Pressed`
    (`/Game/Minhas_BP_Main/BP_CCTV.CamPanRight` (`self.Cameras`))))

(event `Key|Down`
  (params (Key :type "Key Structure"))
  (:`Pressed`
    (`/Game/Minhas_BP_Main/BP_CCTV.CamTiltDown` (`self.Cameras`))))

(event `Key|Up`
  (params (Key :type "Key Structure"))
  (:`Pressed`
    (`/Game/Minhas_BP_Main/BP_CCTV.CamTiltUp` (`self.Cameras`))))

(fn `UserConstructionScript`)