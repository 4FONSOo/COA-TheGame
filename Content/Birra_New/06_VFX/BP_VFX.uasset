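; Actor Blueprint that plays a looping spark effect with sound at randomized intervals, optionally starting on BeginPlay.
; Each firing spawns a chosen Niagara system and plays a random sound from an array at the NSEffect component's location and rotation, each toggleable.
; It then schedules a timer with a random delay between configurable minimum and maximum values, storing the handle.
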(event `CE_StartSparkLoop`
  (set `self.bIsStopped` false)
  (`self.CE_FireSparkPair`))

(event `self.ReceiveBeginPlay`
  (if (`self.bAutoStart`)
    (`self.CE_StartSparkLoop`)))

(event `CE_ScheduleNextSpark`
  (bind _returnvalue (`KismetSystemLibrary.K2_SetTimerDelegate` (`|CreateDelegate` :!event `CE_FireSparkPair`) (`KismetMathLibrary.RandomFloatInRange` (`self.MinSparkInterval`) (`self.MaxSparkInterval`))))
  (set `self.SparkTimerHandle` _returnvalue))

(event `CE_FireSparkPair`
  (bind _sons (`self.Sons`))
  (bind _ns_effect (`self.NS_Effect`))
  (bind _niagara_escolher (`self.NIagara_Escolher`))
  (bind _returnvalue (`KismetArrayLibrary.Array_Length` _sons))
  (bind _returnvalue_2 (`SceneComponent.K2_GetComponentLocation` _ns_effect))
  (bind _returnvalue_3 (`SceneComponent.K2_GetComponentRotation` _ns_effect))
  (`|ExecutionSequence`
    (:`then_0`
      (if (`self.bPlayNiagara`)
        (`/Engine/EditorBlueprintResources/StandardMacros.IsValid` _niagara_escolher
          (:`Is Valid`
            (`NiagaraFunctionLibrary.SpawnSystemAtLocation` _niagara_escolher _returnvalue_2 _returnvalue_3)))))
    (:`then_1`
      (if (`self.bPlaySound`)
        (if (> _returnvalue 0)
          (`GameplayStatics.PlaySoundAtLocation` (`|GetArrayItem` _sons (`KismetMathLibrary.RandomIntegerInRange` 0 (- _returnvalue 1))) _returnvalue_2 _returnvalue_3 1.0 1.0 0.0 "/Game/Birra_New/Managers/Audio/3_Attenuation/ATT_CloseObject.ATT_CloseObject" "/Game/Birra_New/Managers/Audio/5_Concurrency/CONC_OneShot_Close.CONC_OneShot_Close" null null))))
    (:`then_2`
      (`self.CE_ScheduleNextSpark`))))

(fn `UserConstructionScript`)