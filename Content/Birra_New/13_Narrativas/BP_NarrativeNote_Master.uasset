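; Master actor for readable narrative notes that the horror resident character can read and, optionally, collect.
; A data table row drives the paper mesh, dynamic material and behavior flags, with glow and pulse following a visual state.
; Box overlap flags the character as able to interact (unregistering is empty) and shows a camera-facing prompt.
; Opening the reader widget marks the note read, which can collect and hide it; story flags and sounds are only printed or logged.
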(event `self.BoxCollision_Interact.OnComponentBeginOverlap`
  (params (OverlappedComponent :type "PrimitiveComponent Object Reference") (OtherActor :type "Actor Object Reference") (OtherComp :type "PrimitiveComponent Object Reference") (OtherBodyIndex :type Integer) (bFromSweep :type Boolean) (SweepResult :type "HitResult Structure (by ref)"))
  (bind _asbp_resident_horror_v1 (cast `/Game/ChildrenOfAndromeda/Character/BP_Character/BP_Resident_HorrorV1` OtherActor))
  (set `self.bPlayerInside` true)
  (set `self.CurrentInteractor` _asbp_resident_horror_v1)
  (`self.RegisterWithCharacter` _asbp_resident_horror_v1)
  (`self.UpdatePromptState`)
  (`self.UpdateNoteVisualState`))

(event `self.BoxCollision_Interact.OnComponentEndOverlap`
  (params (OverlappedComponent :type "PrimitiveComponent Object Reference") (OtherActor :type "Actor Object Reference") (OtherComp :type "PrimitiveComponent Object Reference") (OtherBodyIndex :type Integer))
  (cast `/Game/ChildrenOfAndromeda/Character/BP_Character/BP_Resident_HorrorV1` OtherActor)
  (set `self.bPlayerInside` false)
  (set `self.CurrentInteractor` null)
  (`self.UnregisterFromCharacter` null)
  (`self.UpdatePromptState`)
  (`self.UpdateNoteVisualState`))

(event `self.ReceiveBeginPlay`
  (set `self.bPlayerInside` false)
  (set `self.bWidgetOpen` false)
  (set `self.bWasRead` false)
  (set `self.bCollected` false)
  (`SceneComponent.SetVisibility` (`self.TextRender_Prompt`) false false)
  (`self.LoadNoteData`)
  (`self.ApplyNoteVisuals`)
  (`self.UpdatePromptState`)
  (`self.UpdateNoteVisualState`))

(event `self.ReceiveTick`
  (params (DeltaSeconds :type "Float (single-precision)"))
  (if (and (`self.bUsePromptBillboard`) (`self.bPlayerInside`) (`SceneComponent.IsVisible` (`self.TextRender_Prompt`)))
    (`self.FacePromptToPlayer`)))

(event `CE_OnNoteWidgetClosed`
  (bind (_currentnotedata_notetitle _currentnotedata_notebody _currentnotedata_noteauthor _currentnotedata_notedate _currentnotedata_papertexture _currentnotedata_paperbacktexture _currentnotedata_papermesh _currentnotedata_papertint _currentnotedata_paperscale3d _currentnotedata_paperrotationoffset _currentnotedata_dirtamount _currentnotedata_damageamount _currentnotedata_edgedarkness _currentnotedata_paperwarpamount _currentnotedata_bglowwhenunread _currentnotedata_bglowwheninrangeonly _currentnotedata_idleemissivestrength _currentnotedata_idlepulsespeed _currentnotedata_idlepulseamount _currentnotedata_focusemissivestrength _currentnotedata_focuspulsespeed _currentnotedata_focuspulseamount _currentnotedata_reademissivestrength _currentnotedata_readpulsespeed _currentnotedata_readpulseamount _currentnotedata_emissivecolor _currentnotedata_bshowtitleinwidget _currentnotedata_bcanbecollected _currentnotedata_bdestroyafterread) (break `/Game/Birra_New/13_Narrativas/ST_NarrativeNoteData` (`self.CurrentNoteData`)))
  (set `self.bWidgetOpen` false)
  (set `self.CurrentReaderWidget` null)
  (if (and _currentnotedata_bdestroyafterread (`self.bCollected`))
    (`self.CE_HideNote`)
    (else
      (`self.UpdatePromptState`)
      (`self.UpdateNoteVisualState`))))

(event `CE_HideNote`
  (bind _staticmesh_paper (`self.StaticMesh_Paper`))
  (`SceneComponent.SetVisibility` _staticmesh_paper false false)
  (`PrimitiveComponent.SetCollisionEnabled` _staticmesh_paper "NoCollision")
  (`PrimitiveComponent.SetCollisionEnabled` (`self.BoxCollision_Interact`) "NoCollision")
  (`SceneComponent.SetVisibility` (`self.TextRender_Prompt`) false false)
  (set `self.bCollected` true)
  (set `self.CurrentVisualState` "NewEnumerator3")
  (`self.ApplyGlowState`))

(event `CE_ShowNote`
  (bind _staticmesh_paper (`self.StaticMesh_Paper`))
  (`SceneComponent.SetVisibility` _staticmesh_paper true false)
  (`PrimitiveComponent.SetCollisionEnabled` _staticmesh_paper "NoCollision")
  (`PrimitiveComponent.SetCollisionEnabled` (`self.BoxCollision_Interact`) "QueryOnly")
  (set `self.bCollected` false)
  (`self.UpdatePromptState`)
  (`self.UpdateNoteVisualState`))

(event `CE_ForceCloseNote`)

(fn `ApplyGlowState`
  (bind (_currentnotedata_notetitle _currentnotedata_notebody _currentnotedata_noteauthor _currentnotedata_notedate _currentnotedata_papertexture _currentnotedata_paperbacktexture _currentnotedata_papermesh _currentnotedata_papertint _currentnotedata_paperscale3d _currentnotedata_paperrotationoffset _currentnotedata_dirtamount _currentnotedata_damageamount _currentnotedata_edgedarkness _currentnotedata_paperwarpamount _currentnotedata_bglowwhenunread _currentnotedata_bglowwheninrangeonly _currentnotedata_idleemissivestrength _currentnotedata_idlepulsespeed _currentnotedata_idlepulseamount _currentnotedata_focusemissivestrength _currentnotedata_focuspulsespeed _currentnotedata_focuspulseamount _currentnotedata_reademissivestrength _currentnotedata_readpulsespeed _currentnotedata_readpulseamount) (break `/Game/Birra_New/13_Narrativas/ST_NarrativeNoteData` (`self.CurrentNoteData`)))
  (bind _papermid (`self.PaperMID`))
  (bind _papermid_2 (`self.PaperMID`))
  (`/Engine/EditorBlueprintResources/StandardMacros.IsValid` (`self.PaperMID`)
    (:`Is Valid`
      (switch `/Game/Birra_New/13_Narrativas/E_NarrativeNoteVisualState` (`self.CurrentVisualState`)
        (:`NewEnumerator0`
          (if _currentnotedata_bglowwhenunread
            (`MaterialInstanceDynamic.SetScalarParameterValue` _papermid_2 "EmissiveStrength" 0.0 :!label _label)
            (`MaterialInstanceDynamic.SetScalarParameterValue` _papermid_2 "PulseSpeed" 0.0)
            (`MaterialInstanceDynamic.SetScalarParameterValue` _papermid_2 "PulseAmount" 0.0)
            (return)
            (elif _currentnotedata_bglowwheninrangeonly
              (`MaterialInstanceDynamic.SetScalarParameterValue` _papermid_2 "EmissiveStrength" 0.0)
              (`MaterialInstanceDynamic.SetScalarParameterValue` _papermid_2 "PulseSpeed" 0.0)
              (`MaterialInstanceDynamic.SetScalarParameterValue` _papermid_2 "PulseAmount" 0.0)
              (return)
              (else
                (`MaterialInstanceDynamic.SetScalarParameterValue` _papermid_2 "EmissiveStrength" _currentnotedata_idleemissivestrength)
                (`MaterialInstanceDynamic.SetScalarParameterValue` _papermid_2 "PulseSpeed" _currentnotedata_idlepulsespeed)
                (`MaterialInstanceDynamic.SetScalarParameterValue` _papermid_2 "PulseAmount" _currentnotedata_idlepulseamount)))))
        (:`NewEnumerator1`
          (`MaterialInstanceDynamic.SetScalarParameterValue` _papermid "EmissiveStrength" _currentnotedata_focusemissivestrength)
          (`MaterialInstanceDynamic.SetScalarParameterValue` _papermid "PulseSpeed" _currentnotedata_focuspulsespeed)
          (`MaterialInstanceDynamic.SetScalarParameterValue` _papermid "PulseAmount" _currentnotedata_focuspulseamount))
        (:`NewEnumerator2`
          (`MaterialInstanceDynamic.SetScalarParameterValue` _papermid "EmissiveStrength" _currentnotedata_reademissivestrength)
          (`MaterialInstanceDynamic.SetScalarParameterValue` _papermid "PulseSpeed" _currentnotedata_readpulsespeed)
          (`MaterialInstanceDynamic.SetScalarParameterValue` _papermid "PulseAmount" _currentnotedata_readpulseamount))
        (:`NewEnumerator3`
          (goto _label))))
    (:`Is Not Valid`
      (return))))

(fn `ApplyNoteVisuals`
  (bind (_currentnotedata_notetitle _currentnotedata_notebody _currentnotedata_noteauthor _currentnotedata_notedate _currentnotedata_papertexture _currentnotedata_paperbacktexture _currentnotedata_papermesh _currentnotedata_papertint _currentnotedata_paperscale3d _currentnotedata_paperrotationoffset _currentnotedata_dirtamount _currentnotedata_damageamount _currentnotedata_edgedarkness _currentnotedata_paperwarpamount _currentnotedata_bglowwhenunread _currentnotedata_bglowwheninrangeonly _currentnotedata_idleemissivestrength _currentnotedata_idlepulsespeed _currentnotedata_idlepulseamount _currentnotedata_focusemissivestrength _currentnotedata_focuspulsespeed _currentnotedata_focuspulseamount _currentnotedata_reademissivestrength _currentnotedata_readpulsespeed _currentnotedata_readpulseamount _currentnotedata_emissivecolor) (break `/Game/Birra_New/13_Narrativas/ST_NarrativeNoteData` (`self.CurrentNoteData`)))
  (bind _staticmesh_paper (`self.StaticMesh_Paper`))
  (bind _papermid (`self.PaperMID`))
  (if (`self.bDataLoaded`)
    (`/Engine/EditorBlueprintResources/StandardMacros.IsValid` _currentnotedata_papermesh
      (:`Is Valid`
        (`StaticMeshComponent.SetStaticMesh` _staticmesh_paper _currentnotedata_papermesh))
      (:`Is Not Valid`
        (`StaticMeshComponent.SetStaticMesh` _staticmesh_paper "/Game/LevelPrototyping/Meshes/SM_Cube.SM_Cube")))
    (`SceneComponent.SetRelativeScale3D` _staticmesh_paper _currentnotedata_paperscale3d)
    (`SceneComponent.K2_SetRelativeRotation` _staticmesh_paper _currentnotedata_paperrotationoffset false false)
    (`self.CreatePaperMID`)
    (`/Engine/EditorBlueprintResources/StandardMacros.IsValid` _papermid
      (:`Is Valid`
        (`MaterialInstanceDynamic.SetTextureParameterValue` _papermid "PaperTexture" _currentnotedata_papertexture)
        (`MaterialInstanceDynamic.SetVectorParameterValue` _papermid "PaperTint" _currentnotedata_papertint)
        (`MaterialInstanceDynamic.SetScalarParameterValue` _papermid "DirtAmount" _currentnotedata_dirtamount)
        (`MaterialInstanceDynamic.SetScalarParameterValue` _papermid "DirtAmount" _currentnotedata_damageamount)
        (`MaterialInstanceDynamic.SetScalarParameterValue` _papermid "EdgeDarkness" _currentnotedata_edgedarkness)
        (`MaterialInstanceDynamic.SetScalarParameterValue` _papermid "PaperWarpAmount" _currentnotedata_paperwarpamount)
        (`MaterialInstanceDynamic.SetVectorParameterValue` _papermid "EmissiveColor" _currentnotedata_emissivecolor)
        (`self.UpdateNoteVisualState`)))
    (else
      (return))))

(fn `CanInteract`
  (returns (CanInteract :type Boolean))
  (bind (_currentnotedata_notetitle _currentnotedata_notebody _currentnotedata_noteauthor _currentnotedata_notedate _currentnotedata_papertexture _currentnotedata_paperbacktexture _currentnotedata_papermesh _currentnotedata_papertint _currentnotedata_paperscale3d _currentnotedata_paperrotationoffset _currentnotedata_dirtamount _currentnotedata_damageamount _currentnotedata_edgedarkness _currentnotedata_paperwarpamount _currentnotedata_bglowwhenunread _currentnotedata_bglowwheninrangeonly _currentnotedata_idleemissivestrength _currentnotedata_idlepulsespeed _currentnotedata_idlepulseamount _currentnotedata_focusemissivestrength _currentnotedata_focuspulsespeed _currentnotedata_focuspulseamount _currentnotedata_reademissivestrength _currentnotedata_readpulsespeed _currentnotedata_readpulseamount _currentnotedata_emissivecolor _currentnotedata_bshowtitleinwidget _currentnotedata_bcanbecollected _currentnotedata_bdestroyafterread _currentnotedata_bshowprompt _currentnotedata_bcanbereread) (break `/Game/Birra_New/13_Narrativas/ST_NarrativeNoteData` (`self.CurrentNoteData`)))
  (if (`self.bDataLoaded`)
    (if (`self.bCollected`)
      _
      (elif (`self.bWidgetOpen`)
        _
        (elif (`KismetMathLibrary.BooleanNAND` (`self.bWasRead`) _currentnotedata_bcanbereread)
          _
          (elif (`self.bPlayerInside`)
            (return true)
            (else
              _))))))
  (return false))

(fn `CollectNote`
  (bind (_currentnotedata_notetitle _currentnotedata_notebody _currentnotedata_noteauthor _currentnotedata_notedate _currentnotedata_papertexture _currentnotedata_paperbacktexture _currentnotedata_papermesh _currentnotedata_papertint _currentnotedata_paperscale3d _currentnotedata_paperrotationoffset _currentnotedata_dirtamount _currentnotedata_damageamount _currentnotedata_edgedarkness _currentnotedata_paperwarpamount _currentnotedata_bglowwhenunread _currentnotedata_bglowwheninrangeonly _currentnotedata_idleemissivestrength _currentnotedata_idlepulsespeed _currentnotedata_idlepulseamount _currentnotedata_focusemissivestrength _currentnotedata_focuspulsespeed _currentnotedata_focuspulseamount _currentnotedata_reademissivestrength _currentnotedata_readpulsespeed _currentnotedata_readpulseamount _currentnotedata_emissivecolor _currentnotedata_bshowtitleinwidget _currentnotedata_bcanbecollected _currentnotedata_bdestroyafterread _currentnotedata_bshowprompt _currentnotedata_bcanbereread _currentnotedata_readsoundname _currentnotedata_closesoundname _currentnotedata_pickupsoundname) (break `/Game/Birra_New/13_Narrativas/ST_NarrativeNoteData` (`self.CurrentNoteData`)))
  (set `self.bCollected` true)
  (`KismetSystemLibrary.LogString` _currentnotedata_pickupsoundname)
  (if _currentnotedata_bdestroyafterread
    (`self.CE_HideNote`)
    (else
      (`self.UpdateNoteVisualState`))))

(fn `CreatePaperMID`
  (bind _staticmesh_paper (`self.StaticMesh_Paper`))
  (bind _returnvalue (`PrimitiveComponent.CreateDynamicMaterialInstance` _staticmesh_paper 0 "/Game/Birra_New/13_Narrativas/MI_Narrative_Paper_Default.MI_Narrative_Paper_Default" "None"))
  (bind _output_get (set `self.PaperMID` _returnvalue))
  (`PrimitiveComponent.SetMaterial` _staticmesh_paper 0 _output_get))

(fn `FacePromptToPlayer`
  (bind _textrender_prompt (`self.TextRender_Prompt`))
  (`SceneComponent.K2_SetWorldRotation` _textrender_prompt (`KismetMathLibrary.FindLookAtRotation` (`SceneComponent.K2_GetComponentLocation` _textrender_prompt) (`PlayerCameraManager.GetCameraLocation` (`GameplayStatics.GetPlayerCameraManager` 0))) false false))

(fn `LoadNoteData`
  (bind _notedatatable (`self.NoteDataTable`))
  (`/Engine/EditorBlueprintResources/StandardMacros.IsValid` _notedatatable
    (:`Is Valid`
      (bind _returnvalue (`|GetDataTableRow` _notedatatable "NoteID")
        (:`then`
          (set `self.CurrentNoteData` _returnvalue)
          (set `self.bDataLoaded` true))
        (:`RowNotFound`
          (`KismetSystemLibrary.PrintString` "BP_NarrativeNote_Master: NoteID não encontrado")
          (set `self.bDataLoaded` false))))
    (:`Is Not Valid`
      (`KismetSystemLibrary.PrintString` "BP_NarrativeNote_Master: DataTable inválida")
      (set `self.bDataLoaded` false)
      (return))))

(fn `MarkNoteAsRead`
  (bind (_currentnotedata_notetitle _currentnotedata_notebody _currentnotedata_noteauthor _currentnotedata_notedate _currentnotedata_papertexture _currentnotedata_paperbacktexture _currentnotedata_papermesh _currentnotedata_papertint _currentnotedata_paperscale3d _currentnotedata_paperrotationoffset _currentnotedata_dirtamount _currentnotedata_damageamount _currentnotedata_edgedarkness _currentnotedata_paperwarpamount _currentnotedata_bglowwhenunread _currentnotedata_bglowwheninrangeonly _currentnotedata_idleemissivestrength _currentnotedata_idlepulsespeed _currentnotedata_idlepulseamount _currentnotedata_focusemissivestrength _currentnotedata_focuspulsespeed _currentnotedata_focuspulseamount _currentnotedata_reademissivestrength _currentnotedata_readpulsespeed _currentnotedata_readpulseamount _currentnotedata_emissivecolor _currentnotedata_bshowtitleinwidget _currentnotedata_bcanbecollected _currentnotedata_bdestroyafterread _currentnotedata_bshowprompt _currentnotedata_bcanbereread _currentnotedata_readsoundname _currentnotedata_closesoundname _currentnotedata_pickupsoundname _currentnotedata_unlocksstoryflag) (break `/Game/Birra_New/13_Narrativas/ST_NarrativeNoteData` (`self.CurrentNoteData`)))
  (if (`self.bWasRead`)
    (return)
    (else
      (set `self.bWasRead` true)
      (if (!= _currentnotedata_unlocksstoryflag "None")
        (`KismetSystemLibrary.PrintString` (`KismetStringLibrary.Concat_StrStr` "Story Flag Unlocked: " (`KismetStringLibrary.Conv_NameToString` _currentnotedata_unlocksstoryflag)))
        (elif _currentnotedata_bcanbecollected
          (`self.CollectNote`)
          (else
            (`self.UpdateNoteVisualState`)))))))

(fn `OpenNoteWidget`
  (bind _playercontrollerref (`self.PlayerControllerRef`))
  (bind (_currentnotedata_notetitle _currentnotedata_notebody _currentnotedata_noteauthor _currentnotedata_notedate _currentnotedata_papertexture _currentnotedata_paperbacktexture _currentnotedata_papermesh _currentnotedata_papertint _currentnotedata_paperscale3d _currentnotedata_paperrotationoffset _currentnotedata_dirtamount _currentnotedata_damageamount _currentnotedata_edgedarkness _currentnotedata_paperwarpamount _currentnotedata_bglowwhenunread _currentnotedata_bglowwheninrangeonly _currentnotedata_idleemissivestrength _currentnotedata_idlepulsespeed _currentnotedata_idlepulseamount _currentnotedata_focusemissivestrength _currentnotedata_focuspulsespeed _currentnotedata_focuspulseamount _currentnotedata_reademissivestrength _currentnotedata_readpulsespeed _currentnotedata_readpulseamount _currentnotedata_emissivecolor _currentnotedata_bshowtitleinwidget _currentnotedata_bcanbecollected _currentnotedata_bdestroyafterread _currentnotedata_bshowprompt _currentnotedata_bcanbereread _currentnotedata_readsoundname) (break `/Game/Birra_New/13_Narrativas/ST_NarrativeNoteData` (`self.CurrentNoteData`)))
  (if (`self.bWidgetOpen`)
    (return)
    (else
      (bind _output_get (set `self.PlayerControllerRef` (`GameplayStatics.GetPlayerController` 0)))
      (bind _returnvalue (`|CreateWidget` "/Game/Birra_New/13_Narrativas/WBP_NoteReader_Generic.WBP_NoteReader_Generic_C" _output_get (`self.CurrentNoteData`) self))
      (bind _output_get_2 (set `self.CurrentReaderWidget` _returnvalue))
      (`UserWidget.AddToViewport` _output_get_2 0)
      (set `self.bWidgetOpen` true)
      (`SceneComponent.SetVisibility` (`self.TextRender_Prompt`) false false)
      (`WidgetBlueprintLibrary.SetInputMode_GameAndUIEx` _playercontrollerref (`self.CurrentReaderWidget`))
      (set `PlayerController.bShowMouseCursor` false _playercontrollerref)
      (`KismetSystemLibrary.PrintString` _currentnotedata_readsoundname)
      (`self.MarkNoteAsRead`)
      (`self.UpdatePromptState`)
      (`self.UpdateNoteVisualState`))))

(fn `RegisterWithCharacter`
  (params (InteractorCharacter :type "/Game/ChildrenOfAndromeda/Character/BP_Character/BP_Resident_HorrorV1 Object Reference"))
  (set `/Game/ChildrenOfAndromeda/Character/BP_Character/BP_Resident_HorrorV1.bCanInteract` true InteractorCharacter))

(fn `UnregisterFromCharacter`
  (params (InteractorCharacter :type "/Game/ChildrenOfAndromeda/Character/BP_Character/BP_Resident_HorrorV1 Object Reference")))

(fn `UpdateNoteVisualState`
  (if (`self.bCollected`)
    (set `self.CurrentVisualState` "NewEnumerator3")
    (`self.ApplyGlowState`)
    (else
      (if (`self.bWasRead`)
        (set `self.CurrentVisualState` "NewEnumerator2")
        (elif (`self.bPlayerInside`)
          (set `self.CurrentVisualState` "NewEnumerator1")
          (else
            (set `self.CurrentVisualState` "NewEnumerator2"))))
      (`self.ApplyGlowState`)))
  (return))

(fn `UpdatePromptState`
  (bind (_currentnotedata_notetitle _currentnotedata_notebody _currentnotedata_noteauthor _currentnotedata_notedate _currentnotedata_papertexture _currentnotedata_paperbacktexture _currentnotedata_papermesh _currentnotedata_papertint _currentnotedata_paperscale3d _currentnotedata_paperrotationoffset _currentnotedata_dirtamount _currentnotedata_damageamount _currentnotedata_edgedarkness _currentnotedata_paperwarpamount _currentnotedata_bglowwhenunread _currentnotedata_bglowwheninrangeonly _currentnotedata_idleemissivestrength _currentnotedata_idlepulsespeed _currentnotedata_idlepulseamount _currentnotedata_focusemissivestrength _currentnotedata_focuspulsespeed _currentnotedata_focuspulseamount _currentnotedata_reademissivestrength _currentnotedata_readpulsespeed _currentnotedata_readpulseamount _currentnotedata_emissivecolor _currentnotedata_bshowtitleinwidget _currentnotedata_bcanbecollected _currentnotedata_bdestroyafterread _currentnotedata_bshowprompt _currentnotedata_bcanbereread) (break `/Game/Birra_New/13_Narrativas/ST_NarrativeNoteData` (`self.CurrentNoteData`)))
  (bind _textrender_prompt (`self.TextRender_Prompt`))
  (if _currentnotedata_bshowprompt
    (if (`self.bCollected`)
      (`SceneComponent.SetVisibility` _textrender_prompt false false :!label _label)
      (return)
      (elif (`KismetMathLibrary.BooleanNAND` (`self.bWasRead`) _currentnotedata_bcanbereread)
        (goto _label)
        (elif (`KismetMathLibrary.BooleanNAND` (`self.bPlayerInside`) (`self.bWidgetOpen`))
          (`TextRenderComponent.K2_SetText` _textrender_prompt (`self.PromptText`))
          (`SceneComponent.SetVisibility` _textrender_prompt true false)
          (else
            (goto _label)))))
    (else
      (`SceneComponent.SetVisibility` _textrender_prompt false false)
      (return))))

(fn `UserConstructionScript`
  (`self.LoadNoteData`)
  (`self.ApplyNoteVisuals`)
  (`self.UpdatePromptState`)
  (`self.UpdateNoteVisualState`))