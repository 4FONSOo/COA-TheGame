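; Interactive button that arms, activates and resets a linked gravity tunnel when the player presses E nearby.
; InteractionZone overlaps toggle input and a state-based text prompt for the player character.
; Armed, used and locked flags drive the press sequence, moving the button mesh, playing audio and calling TargetTunnel.
; Activation and reset lock the button until a delay ends; unused backup logic remains in the graph.
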(event `Key|E`
  (params (Key :type "Key Structure"))
  (bind _pressetext (`self.PressEText`))
  (bind _buttonmesh (`self.ButtonMesh`))
  (bind _pressetext_2 (`self.PressEText`))
  (bind _pressetext_3 (`self.PressEText`))
  (bind _buttonstartlocation (`self.ButtonStartLocation`))
  (bind _resetbuttondelay (`self.ResetButtonDelay`))
  (bind _targettunnel (`self.TargetTunnel`))
  (:`Pressed`
    (if (`self.bPlayerInRange`)
      (if (`self.bButtonLocked`)
        _
        (elif (`self.bButtonUsed`)
          (set `self.bButtonArmed` false)
          (set `self.bButtonLocked` true)
          (`AudioComponent.Play` (`self.ButtonPressAudio`) 0.0)
          (`SceneComponent.SetVisibility` _pressetext false false)
          (`SceneComponent.K2_SetRelativeLocation` _buttonmesh _buttonstartlocation false false)
          (`/Engine/EditorBlueprintResources/StandardMacros.IsValid` _targettunnel
            (:`Is Valid`
              (`/Game/Birra_New/00_GravityTunnel/Bp/BP_GravityTunnel.ResetGravityTunnel` _targettunnel)
              (`KismetSystemLibrary.Delay` _resetbuttondelay)
              (set `self.bButtonLocked` false)
              (if (`self.bPlayerInRange`)
                (`TextRenderComponent.K2_SetText` _pressetext_2 (`KismetTextLibrary.Conv_StringToText` "PRESS E TO ARM"))
                (`SceneComponent.SetVisibility` _pressetext_2 true false)
                (set `self.bButtonUsed` false)
                (set `self.bButtonArmed` false)
                (set `self.bButtonLocked` false))))
          (elif (`self.bButtonArmed`)
            (set `self.bButtonUsed` true)
            (set `self.bButtonLocked` true)
            (`AudioComponent.Play` (`self.ButtonPressAudio`) 0.0)
            (`SceneComponent.SetVisibility` _pressetext false false)
            (`SceneComponent.K2_SetRelativeLocation` _buttonmesh (+ _buttonstartlocation (`self.ButtonPressedOffset`)) false false)
            (`/Engine/EditorBlueprintResources/StandardMacros.IsValid` _targettunnel
              (:`Is Valid`
                (`/Game/Birra_New/00_GravityTunnel/Bp/BP_GravityTunnel.ActivateGravityTunnel` _targettunnel)
                (`KismetSystemLibrary.Delay` _resetbuttondelay)
                (set `self.bButtonLocked` false)
                (if (`self.bPlayerInRange`)
                  (`TextRenderComponent.K2_SetText` _pressetext_2 (`KismetTextLibrary.Conv_StringToText` "PRESS E TO RESET"))
                  (`SceneComponent.SetVisibility` _pressetext_2 false false))))
            (else
              (set `self.bButtonArmed` true)
              (`AudioComponent.Play` (`self.ButtonPressAudio`) 0.0)
              (`TextRenderComponent.K2_SetText` _pressetext_3 (`KismetTextLibrary.Conv_StringToText` "PRESS E TO ARM"))
              (`SceneComponent.SetVisibility` _pressetext_3 true false))))))))

(event `self.InteractionZone.OnComponentBeginOverlap`
  (params (OverlappedComponent :type "PrimitiveComponent Object Reference") (OtherActor :type "Actor Object Reference") (OtherComp :type "PrimitiveComponent Object Reference") (OtherBodyIndex :type Integer) (bFromSweep :type Boolean) (SweepResult :type "HitResult Structure (by ref)"))
  (bind _pressetext (`self.PressEText`))
  (if (== OtherActor (`GameplayStatics.GetPlayerCharacter` 0))
    (set `self.bPlayerInRange` true)
    (`self.EnableInput` (`GameplayStatics.GetPlayerController` 0))
    (if (`self.bButtonLocked`)
      (`TextRenderComponent.K2_SetText` _pressetext (`KismetTextLibrary.Conv_StringToText` "RESET"))
      (elif (`self.bButtonUsed`)
        (`TextRenderComponent.K2_SetText` _pressetext (`KismetTextLibrary.Conv_StringToText` "RESET"))
        (`SceneComponent.SetVisibility` _pressetext true false)
        (elif (`self.bButtonArmed`)
          (`TextRenderComponent.K2_SetText` _pressetext (`KismetTextLibrary.Conv_StringToText` "RELEASE"))
          (`SceneComponent.SetVisibility` _pressetext true false)
          (else
            (`TextRenderComponent.K2_SetText` _pressetext (`KismetTextLibrary.Conv_StringToText` "ARM"))
            (`SceneComponent.SetVisibility` _pressetext true false)))))))

(event `self.InteractionZone.OnComponentEndOverlap`
  (params (OverlappedComponent :type "PrimitiveComponent Object Reference") (OtherActor :type "Actor Object Reference") (OtherComp :type "PrimitiveComponent Object Reference") (OtherBodyIndex :type Integer))
  (if (== OtherActor (`GameplayStatics.GetPlayerCharacter` 0))
    (set `self.bPlayerInRange` false)
    (`SceneComponent.SetVisibility` (`self.PressEText`) false false)
    (`self.DisableInput` (`GameplayStatics.GetPlayerController` 0))))

(event `Key|E`
  (params (Key :type "Key Structure"))
  ; Backup
)

(event `self.ReceiveBeginPlay`
  (set `self.ButtonStartLocation` (`SceneComponent.RelativeLocation` (`self.ButtonMesh`)))
  (`SceneComponent.SetVisibility` (`self.PressEText`) false false)
  (set `self.bButtonArmed` false)
  (set `self.bButtonUsed` false))

(event `CustomEvent`
  (params (OverlappedComponent :type "PrimitiveComponent Object Reference") (OtherActor :type "Actor Object Reference") (OtherComp :type "PrimitiveComponent Object Reference") (OtherBodyIndex :type Integer))
  ;[0.15 0.04616 0.01821 0.5] BackUp
  (if (== OtherActor (`GameplayStatics.GetPlayerCharacter` 0))
    (set `self.bPlayerInRange` true)
    (`SceneComponent.SetVisibility` (`self.PressEText`) false false)
    (`self.DisableInput` (`GameplayStatics.GetPlayerController` 0))))

(fn `UserConstructionScript`)