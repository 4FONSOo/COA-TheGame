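; Gravity tunnel actor the player toggles with E near its button, switching suction and a protective force field.
; Activation starts alarms, lights, VFX and audio, then fades out the force field after a delay; stopping refills it.
; While active, Tick pulls overlapping Characters and physics-simulating BP_GravityObjects toward SuctionTarget via launch or velocity overrides.
; Timelines drive the field's dynamic material, and hits spawn arcs, flicker and throttled impact sounds.
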(event `self.ReceiveBeginPlay`
  (set `self.GravityTunnelState` "NewEnumerator0")
  (set `self.bGravityTunnelActive` false)
  (set `self.bSuctionActive` false)
  (set `self.bCanToggle` true)
  (set `self.bPlayerInRange` false)
  (set `self.SuctionRampAlpha` 0.0)
  (set `self.SuctionRampTimer` 0.0)
  (set `self.LastImpactTime` -999.0)
  (set `self.ButtonStartLocation` (`SceneComponent.RelativeLocation` (`self.SM_ButtonPress`)))
  (`SceneComponent.SetVisibility` (`self.TextRender`) false false)
  (`SceneComponent.SetVisibility` (`self.SM_ForceField`) true false)
  (`PrimitiveComponent.SetCollisionEnabled` (`self.ForceFieldCollision`) "QueryAndPhysics")
  (`self.EnsureForceFieldMaterial`)
  (`AudioComponent.Stop` (`self.Audio_AlarmLoop`))
  (`AudioComponent.Stop` (`self.Audio_SuctionLoop`)))

(event `self.InteractionZone.OnComponentBeginOverlap`
  (params (OverlappedComponent :type "PrimitiveComponent Object Reference") (OtherActor :type "Actor Object Reference") (OtherComp :type "PrimitiveComponent Object Reference") (OtherBodyIndex :type Integer) (bFromSweep :type Boolean) (SweepResult :type "HitResult Structure (by ref)"))
  (bind _textrender (`self.TextRender`))
  (if (== OtherActor (`GameplayStatics.GetPlayerCharacter` 0))
    (set `self.bPlayerInRange` true)
    (`self.EnableInput` (`GameplayStatics.GetPlayerController` 0))
    (`SceneComponent.SetVisibility` _textrender true false)
    (`TextRenderComponent.K2_SetText` _textrender (`KismetTextLibrary.Conv_StringToText` "PRESS E"))))

(event `AnimateButtonPress`
  (bind _buttonpressaudio (`self.ButtonPressAudio`))
  (bind _sm_buttonpress (`self.SM_ButtonPress`))
  (bind _buttonstartlocation (`self.ButtonStartLocation`))
  (`/Engine/EditorBlueprintResources/StandardMacros.IsValid` _buttonpressaudio
    (:`Is Valid`
      (`GameplayStatics.PlaySoundAtLocation` _buttonpressaudio (`self.K2_GetActorLocation`) (struct) 1.0 1.0 0.0 null null null null)
      (`SceneComponent.K2_SetRelativeLocation` _sm_buttonpress (+ _buttonstartlocation (`self.ButtonPressedOffset`)) false false)
      (`KismetSystemLibrary.Delay` 0.15)
      (`SceneComponent.K2_SetRelativeLocation` _sm_buttonpress _buttonstartlocation false false))))

(event `self.InteractionZone.OnComponentEndOverlap`
  (params (OverlappedComponent :type "PrimitiveComponent Object Reference") (OtherActor :type "Actor Object Reference") (OtherComp :type "PrimitiveComponent Object Reference") (OtherBodyIndex :type Integer))
  (if (== (`GameplayStatics.GetPlayerCharacter` 0) OtherActor)
    (set `self.bPlayerInRange` false)
    (`SceneComponent.SetVisibility` (`self.TextRender`) false false)))

(event `ToggleGravityTunnel`
  (if (`self.bCanToggle`)
    (set `self.bCanToggle` false)
    (switch `/Game/Birra_New/00_GravityTunnel/Enum/E_GravityTunnelState` (`self.GravityTunnelState`)
      (:`NewEnumerator0`
        (`self.StartGravityTunnel`))
      (:`NewEnumerator1`
        (`self.StopGravityTunnel` :!label _label))
      (:`NewEnumerator2`
        (goto _label)))
    (`KismetSystemLibrary.Delay` (`self.ToggleCooldown`))
    (set `self.bCanToggle` true)))

(event `self.ForceFieldCollision.OnComponentHit`
  (params (HitComponent :type "PrimitiveComponent Object Reference") (OtherActor :type "Actor Object Reference") (OtherComp :type "PrimitiveComponent Object Reference") (NormalImpulse :type "Vector Structure") (Hit :type "HitResult Structure (by ref)"))
  (bind (_bblockinghit _binitialoverlap _time _distance _location _impactpoint _normal) (`GameplayStatics.BreakHitResult` Hit))
  (`NiagaraFunctionLibrary.SpawnSystemAtLocation` (`self.ForceFieldArcVFX`) _location (`KismetMathLibrary.MakeRotFromZ` _normal))
  (`self.PulseForceFieldImpact`)
  (bind _canplay (`self.CanPlayImpactSound` OtherComp))
  (if _canplay
    (`self.PlayImpactSound` _location)))

(event `StartGravityTunnel`
  (set `self.GravityTunnelState` "NewEnumerator2")
  (set `self.bGravityTunnelActive` true)
  (`self.StartSuction`)
  (`self.StartAlarmLights`)
  (`self.StartExternalLights`)
  (`self.StartGravityVFX`)
  (`self.StartExternalVFX`)
  (`self.StartGravityAudio`)
  (`KismetSystemLibrary.Delay` (`self.SuctionStartDelay`))
  (if (`self.bGravityTunnelActive`)
    (`self.StopForceField`)
    (`KismetSystemLibrary.Delay` (`self.ForceFieldFadeOutDuration`))
    (if (`self.bGravityTunnelActive`)
      (`self.StartSuctionVFX`))))

(event `StopGravityTunnel`
  (set `self.GravityTunnelState` "NewEnumerator3")
  (set `self.bGravityTunnelActive` false)
  (`self.StopSuction`)
  (`self.StartForceField`)
  (`self.StopExternalVFX`)
  (`self.StopGravityVFX`)
  (`self.StopGravityAudio`)
  (`self.StopExternalLights`)
  (`self.StopAlarmLights`)
  (set `self.GravityTunnelState` "NewEnumerator4")
  (`KismetSystemLibrary.Delay` 0.4)
  (set `self.GravityTunnelState` "NewEnumerator0"))

(event `StartSuction`
  (set `self.bSuctionActive` true)
  (set `self.SuctionRampAlpha` 0.0)
  (set `self.SuctionRampTimer` 0.0)
  (`self.StartSuctionVFX`)
  (`AudioComponent.FadeIn` (`self.Audio_SuctionLoop`) 0.5 1.0 0.0 "Linear"))

(event `self.ReceiveTick`
  (params (DeltaSeconds :type "Float (single-precision)"))
  (if (`self.bSuctionActive`)
    (`self.UpdateSuctionRamp` DeltaSeconds)
    (`self.ApplySuction`)
    (`self.UpdateSuctionAudioVolume`)))

(event `StopSuction`
  (set `self.bSuctionActive` false)
  (set `self.SuctionRampAlpha` 0.0)
  (set `self.SuctionRampTimer` 0.0)
  (`self.StopSuctionVFX`)
  (`AudioComponent.FadeOut` (`self.Audio_SuctionLoop`) 0.5 0.0 "Linear"))

(event `Key|E`
  (params (Key :type "Key Structure"))
  (:`Pressed`
    (`self.AnimateButtonPress`)
    (`self.ToggleGravityTunnel`)))

(event `StartForceField`
  (`self.BeginForceFieldFill`))

(event `StopForceField`
  (`self.BeginForceFieldFadeOut`))

(event `PulseForceFieldImpact`
  (bind _forcefieldmaterial (`self.ForceFieldMaterial`))
  (`/Engine/EditorBlueprintResources/StandardMacros.IsValid` _forcefieldmaterial
    (:`Is Valid`
      (`MaterialInstanceDynamic.SetScalarParameterValue` _forcefieldmaterial "FlickerAmount" (`self.ForceFieldImpactGlitch`))
      (`KismetSystemLibrary.Delay` (`self.ForceFieldImpactBoostTime`))
      (`MaterialInstanceDynamic.SetScalarParameterValue` _forcefieldmaterial "FlickerAmount" (`self.ForceFieldNormalGlitch`)))))

(event `StartGravityVFX`
  (bind _steamleakpoint (`self.SteamLeakPoint`))
  (bind _activevfxcomponents (`self.ActiveVFXComponents`))
  (bind (_returnvalue_location _returnvalue_rotation) (`KismetMathLibrary.BreakTransform` (`SceneComponent.K2_GetComponentToWorld` (`self.TunnelZone`))))
  (bind (_returnvalue_location_2 _returnvalue_rotation_2) (`KismetMathLibrary.BreakTransform` (`SceneComponent.K2_GetComponentToWorld` _steamleakpoint)))
  (bind _returnvalue (`NiagaraFunctionLibrary.SpawnSystemAtLocation` null _returnvalue_location _returnvalue_rotation))
  (`KismetArrayLibrary.Array_Add` _activevfxcomponents _returnvalue)
  (bind _returnvalue_2 (`NiagaraFunctionLibrary.SpawnSystemAtLocation` (`self.DustAirVFX`) _returnvalue_location _returnvalue_rotation))
  (`KismetArrayLibrary.Array_Add` _activevfxcomponents _returnvalue_2)
  (bind _returnvalue_3 (`NiagaraFunctionLibrary.SpawnSystemAtLocation` (`self.AlarmHazeVFX`) _returnvalue_location _returnvalue_rotation))
  (`KismetArrayLibrary.Array_Add` _activevfxcomponents _returnvalue_3)
  (`/Engine/EditorBlueprintResources/StandardMacros.IsValid` _steamleakpoint
    (:`Is Valid`
      (bind _returnvalue_4 (`NiagaraFunctionLibrary.SpawnSystemAtLocation` (`self.SteamLeakVFX`) _returnvalue_location_2 _returnvalue_rotation_2))
      (`KismetArrayLibrary.Array_Add` _activevfxcomponents _returnvalue_4))))

(event `StopGravityVFX`
  (bind _activevfxcomponents (`self.ActiveVFXComponents`))
  (for _array_element _activevfxcomponents
    (`/Engine/EditorBlueprintResources/StandardMacros.IsValid` _array_element
      (:`Is Valid`
        (`ActorComponent.Deactivate` _array_element))))
  (`KismetArrayLibrary.Array_Clear` _activevfxcomponents))

(event `StartGravityAudio`
  (bind _returnvalue (`self.K2_GetActorLocation`))
  (bind _alarmstartsound (`self.AlarmStartSound`))
  (bind _suctionstartsound (`self.SuctionStartSound`))
  (`/Engine/EditorBlueprintResources/StandardMacros.IsValid` _alarmstartsound
    (:`Is Valid`
      (`GameplayStatics.PlaySoundAtLocation` _alarmstartsound _returnvalue (struct) 1.0 1.0 0.0 null null null null)
      (`AudioComponent.FadeIn` (`self.Audio_AlarmLoop`) 0.5 0.8 0.0 "Linear")
      (`/Engine/EditorBlueprintResources/StandardMacros.IsValid` _suctionstartsound
        (:`Is Valid`
          (`GameplayStatics.PlaySoundAtLocation` _suctionstartsound _returnvalue (struct) 1.0 1.0 0.0 null null null null)
          (`AudioComponent.FadeIn` (`self.Audio_SuctionLoop`) 1.5 0.2 0.0 "Linear"))))))

(event `StopGravityAudio`
  (bind _suctionstopsound (`self.SuctionStopSound`))
  (bind _alarmstopsound (`self.AlarmStopSound`))
  (`AudioComponent.FadeOut` (`self.Audio_SuctionLoop`) 0.8 0.0 "Linear")
  (`AudioComponent.FadeOut` (`self.Audio_AlarmLoop`) 0.5 0.0 "Linear")
  (`/Engine/EditorBlueprintResources/StandardMacros.IsValid` _suctionstopsound
    (:`Is Valid`
      (`GameplayStatics.PlaySoundAtLocation` _suctionstopsound (`self.K2_GetActorLocation`) (struct) 1.0 1.0 0.0 null null null null)
      (`/Engine/EditorBlueprintResources/StandardMacros.IsValid` _alarmstopsound
        (:`Is Valid`
          (`GameplayStatics.PlaySoundAtLocation` _alarmstopsound (0.0 0.0 0.0) (struct) 1.0 1.0 0.0 null null null null))))))

(event `BeginForceFieldFill`
  (bind _sm_forcefield (`self.SM_ForceField`))
  (bind _forcefieldmaterial (`self.ForceFieldMaterial`))
  (`self.EnsureForceFieldMaterial`)
  (`SceneComponent.SetVisibility` _sm_forcefield true false)
  (`PrimitiveComponent.SetCollisionEnabled` (`self.ForceFieldCollision`) "QueryAndPhysics")
  (`PrimitiveComponent.CreateDynamicMaterialInstance` _sm_forcefield 0 _forcefieldmaterial "None")
  (`self.SetForceFieldMaterialNormal`)
  (bind (_direction _fillalpha) (`Timeline|TL_ForceFieldFill` :!via `PlayFromStart`)
    (:`Update`
      (`/Engine/EditorBlueprintResources/StandardMacros.IsValid` (`self.ForceFieldMaterial`)
        (:`Is Valid`
          (set `self.ForceFieldFillAlpha` _fillalpha)
          (`MaterialInstanceDynamic.SetScalarParameterValue` _forcefieldmaterial "Opacity" (`KismetMathLibrary.Lerp` (`self.ForceFieldStartOpacity`) (`self.ForceFieldTargetOpacity`) _fillalpha))
          (`MaterialInstanceDynamic.SetScalarParameterValue` _forcefieldmaterial "EmissiveIntensity" (`KismetMathLibrary.Lerp` (`self.ForceFieldStartEmissive`) (`self.ForceFieldTargetEmissive`) _fillalpha))
          (`MaterialInstanceDynamic.SetScalarParameterValue` _forcefieldmaterial "FlickerAmount" (`KismetMathLibrary.Lerp` (`self.ForceFieldStartGlitch`) (`self.ForceFieldTargetGlitch`) _fillalpha))
          (`MaterialInstanceDynamic.SetVectorParameterValue` _forcefieldmaterial "GlitchColor" (`self.ForceFieldColor`)))))
    (:`Finished`
      (`self.SetForceFieldMaterialNormal`))))

(event `BeginForceFieldFadeOut`
  (bind _forcefieldmaterial (`self.ForceFieldMaterial`))
  (`/Engine/EditorBlueprintResources/StandardMacros.IsValid` _forcefieldmaterial
    (:`Is Valid`
      (`PrimitiveComponent.SetCollisionEnabled` (`self.ForceFieldCollision`) "NoCollision")
      (bind (_direction _fadealpha) (`Timeline|TL_ForceFieldFadeOut` :!via `PlayFromStart`)
        (:`Update`
          (`/Engine/EditorBlueprintResources/StandardMacros.IsValid` (`self.ForceFieldMaterial`)
            (:`Is Valid`
              (`MaterialInstanceDynamic.SetScalarParameterValue` _forcefieldmaterial "Opacity" (`KismetMathLibrary.Lerp` (`self.ForceFieldTargetOpacity`) (`self.ForceFieldHiddenOpacity`) _fadealpha))
              (`MaterialInstanceDynamic.SetScalarParameterValue` _forcefieldmaterial "EmissiveIntensity" (`KismetMathLibrary.Lerp` (`self.ForceFieldTargetEmissive`) 0.0 _fadealpha))
              (`MaterialInstanceDynamic.SetScalarParameterValue` _forcefieldmaterial "FlickerAmount" (`KismetMathLibrary.Lerp` (`self.ForceFieldTargetGlitch`) 0.0 _fadealpha)))))
        (:`Finished`
          (`self.SetForceFieldMaterialHidden`))))))

(event `StartExternalVFX`
  (for _array_element (`self.ForceFieldVFXActors`)
    (`/Engine/EditorBlueprintResources/StandardMacros.IsValid` _array_element
      (:`Is Valid`
        (`self.SetActorHiddenInGame` _array_element false)
        (bind _returnvalue (`self.GetComponentByClass` _array_element "/Script/Niagara.NiagaraComponent"))
        (`/Engine/EditorBlueprintResources/StandardMacros.IsValid` _returnvalue
          (:`Is Valid`
            (`ActorComponent.Activate` _returnvalue false)
            (for _array_element_2 (`self.AmbientVFXActors`)
              (`/Engine/EditorBlueprintResources/StandardMacros.IsValid` _array_element_2
                (:`Is Valid`
                  (`self.SetActorHiddenInGame` _array_element_2 false)
                  (bind _returnvalue_2 (`self.GetComponentByClass` _array_element_2 "/Script/Niagara.NiagaraComponent"))
                  (`/Engine/EditorBlueprintResources/StandardMacros.IsValid` _returnvalue_2
                    (:`Is Valid`
                      (`ActorComponent.Activate` _returnvalue_2 false))))))))))))

(event `StopExternalVFX`
  (for _array_element (`self.SuctionVFXActors`)
    (`/Engine/EditorBlueprintResources/StandardMacros.IsValid` _array_element
      (:`Is Valid`
        (`self.SetActorHiddenInGame` _array_element false)
        (bind _returnvalue (`self.GetComponentByClass` _array_element "/Script/Niagara.NiagaraComponent"))
        (`/Engine/EditorBlueprintResources/StandardMacros.IsValid` _returnvalue
          (:`Is Valid`
            (`ActorComponent.Deactivate` _returnvalue)
            (for _array_element_2 (`self.ForceFieldVFXActors`)
              (`/Engine/EditorBlueprintResources/StandardMacros.IsValid` _array_element_2
                (:`Is Valid`
                  (`self.SetActorHiddenInGame` _array_element_2 false)
                  (bind _returnvalue_2 (`self.GetComponentByClass` _array_element_2 "/Script/Niagara.NiagaraComponent"))
                  (`/Engine/EditorBlueprintResources/StandardMacros.IsValid` _returnvalue_2
                    (:`Is Valid`
                      (`ActorComponent.Deactivate` _returnvalue_2)
                      (for _array_element_3 (`self.AmbientVFXActors`)
                        (`/Engine/EditorBlueprintResources/StandardMacros.IsValid` _array_element_3
                          (:`Is Valid`
                            (`self.SetActorHiddenInGame` _array_element_3 false)
                            (bind _returnvalue_3 (`self.GetComponentByClass` _array_element_3 "/Script/Niagara.NiagaraComponent"))
                            (`/Engine/EditorBlueprintResources/StandardMacros.IsValid` _returnvalue_3
                              (:`Is Valid`
                                (`ActorComponent.Deactivate` _returnvalue_3)))))))))))))))))

(event `StartExternalLights`
  (for _array_element (`self.GravityTunnelLights`)
    (`/Engine/EditorBlueprintResources/StandardMacros.IsValid` _array_element
      (:`Is Valid`
        (for _array_element_2 (`self.K2_GetComponentsByClass` _array_element "/Script/Engine.LightComponent")
          (`SceneComponent.SetVisibility` _array_element_2 true false)
          (`LightComponent.SetIntensity` _array_element_2 5000.0))))))

(event `StopExternalLights`
  (for _array_element (`self.GravityTunnelLights`)
    (`/Engine/EditorBlueprintResources/StandardMacros.IsValid` _array_element
      (:`Is Valid`
        (for _array_element_2 (`self.K2_GetComponentsByClass` _array_element "/Script/Engine.LightComponent")
          (`SceneComponent.SetVisibility` _array_element_2 false false)
          (`LightComponent.SetIntensity` _array_element_2 0.0))))))

(event `StartAlarmLights`
  (for _array_element (`self.AlarmLightActors`)
    (`/Engine/EditorBlueprintResources/StandardMacros.IsValid` _array_element
      (:`Is Valid`
        (`/Game/Birra_New/00_GravityTunnel/Bp/GT_AlarmLight.StartAlarm` _array_element)))))

(event `StopAlarmLights`
  (for _array_element (`self.AlarmLightActors`)
    (`/Engine/EditorBlueprintResources/StandardMacros.IsValid` _array_element
      (:`Is Valid`
        (`/Game/Birra_New/00_GravityTunnel/Bp/GT_AlarmLight.StopAlarm` _array_element)))))

(event `StartSuctionVFX`
  (for _array_element (`self.SuctionVFXActors`)
    (`/Engine/EditorBlueprintResources/StandardMacros.IsValid` _array_element
      (:`Is Valid`
        (`self.SetActorHiddenInGame` _array_element false)
        (for _array_element_2 (`self.K2_GetComponentsByClass` _array_element "/Script/Niagara.NiagaraComponent")
          (`ActorComponent.Activate` _array_element_2 true))))))

(event `StopSuctionVFX`
  (for _array_element (`self.SuctionVFXActors`)
    (`/Engine/EditorBlueprintResources/StandardMacros.IsValid` _array_element
      (:`Is Valid`
        (`self.SetActorHiddenInGame` _array_element true)
        (for _array_element_2 (`self.K2_GetComponentsByClass` _array_element "/Script/Niagara.NiagaraComponent")
          (`ActorComponent.Deactivate` _array_element_2))))))

(fn `ApplyCharacterSuction`
  (params (TargetCharacter :type "Character Object Reference"))
  (`Character.LaunchCharacter` TargetCharacter (* (* (`KismetMathLibrary.Normal` (- (`SceneComponent.K2_GetComponentLocation` (`self.SuctionTarget`)) (`self.K2_GetActorLocation` TargetCharacter))) (`self.PlayerPullVelocity`)) (`self.SuctionRampAlpha`)) true true))

(fn `ApplyPhysicsObjectSuction`
  (params (TargetActor :type "Actor Object Reference") (TargetPrimitive :type "PrimitiveComponent Object Reference"))
  (locals (Const_1 :type "Float (double-precision)" :default 1500.0))
  (`/Engine/EditorBlueprintResources/StandardMacros.IsValid` TargetPrimitive
    (:`Is Valid`
      (`PrimitiveComponent.WakeRigidBody` TargetPrimitive "None")
      (`PrimitiveComponent.SetPhysicsLinearVelocity` TargetPrimitive (+ (* (`KismetMathLibrary.Normal` (- (`SceneComponent.K2_GetComponentLocation` (`self.SuctionTarget`)) (`SceneComponent.K2_GetComponentLocation` TargetPrimitive))) (`self.ObjectSuctionVelocity`)) (`KismetMathLibrary.MakeVector` 0.0 0.0 (`self.ObjectLiftVelocity`))) false "None")
      (`PrimitiveComponent.AddTorqueInRadians` TargetPrimitive (* (* (`KismetMathLibrary.RandomUnitVector`) (`self.ObjectRandomTorqueStrength`)) (`self.SuctionRampAlpha`)) "None" true))))

(fn `ApplySuction`
  (for _array_element (`PrimitiveComponent.GetOverlappingActors` (`self.TunnelZone`) null)
    (`/Engine/EditorBlueprintResources/StandardMacros.IsValid` _array_element
      (:`Is Valid`
        (bind _ascharacter (cast `Character` _array_element)
          (:`then`
            (`self.ApplyCharacterSuction` _ascharacter))
          (:`CastFailed`
            (bind _asbp_gravity_object (cast `/Game/Birra_New/00_GravityTunnel/Bp/BP_GravityObject` _array_element)
              (:`then`
                (bind _mesh (`/Game/Birra_New/00_GravityTunnel/Bp/BP_GravityObject.getObjectMesh` _asbp_gravity_object))
                (if (`SceneComponent.IsSimulatingPhysics` _mesh "None")
                  (`self.ApplyPhysicsObjectSuction` _asbp_gravity_object _mesh)))
              (:`CastFailed`
                (`KismetSystemLibrary.PrintString` "ké esta merda?")))))))))

(fn `CanPlayImpactSound`
  (params (OtherComp :type "PrimitiveComponent Object Reference"))
  (returns (CanPlay :type Boolean))
  (bind _returnvalue (`KismetSystemLibrary.GetGameTimeInSeconds`))
  (`/Engine/EditorBlueprintResources/StandardMacros.IsValid` OtherComp
    (:`Is Valid`
      (bind _returnvalue_2 (`PrimitiveComponent.GetPhysicsLinearVelocity` OtherComp "None"))
      (if (> (`KismetMathLibrary.VSize` _returnvalue_2) (`self.MinImpactVelocity`))
        (if (> (- _returnvalue (`self.LastImpactTime`)) (`self.ImpactCooldown`))
          (set `self.LastImpactTime` _returnvalue)
          (return true)
          (else
            (return false)))
        (else
          (return false))))
    (:`Is Not Valid`
      (return false))))

(fn `EnsureForceFieldMaterial`
  (`/Engine/EditorBlueprintResources/StandardMacros.IsValid` (`self.ForceFieldMaterial`)
    (:`Is Valid`
      (return))
    (:`Is Not Valid`
      (bind _returnvalue (`PrimitiveComponent.CreateDynamicMaterialInstance` (`self.SM_ForceField`) 0 (`self.ForceFieldBaseMaterial`) "None"))
      (set `self.ForceFieldMaterial` _returnvalue))))

(fn `PlayImpactSound`
  (params (HitLocation :type "Vector Structure"))
  (bind _impactsoundarray (`self.ImpactSoundArray`))
  (if (>= (`KismetArrayLibrary.Array_Length` _impactsoundarray) 0)
    (`GameplayStatics.PlaySoundAtLocation` (`KismetArrayLibrary.Array_Random` _impactsoundarray) HitLocation (struct) 1.0 1.0 0.0 null null null null)))

(fn `SetForceFieldMaterialHidden`
  (bind _forcefieldmaterial (`self.ForceFieldMaterial`))
  (`/Engine/EditorBlueprintResources/StandardMacros.IsValid` _forcefieldmaterial
    (:`Is Valid`
      (`MaterialInstanceDynamic.SetScalarParameterValue` _forcefieldmaterial "Opacity" (`self.ForceFieldHiddenOpacity`))
      (`MaterialInstanceDynamic.SetScalarParameterValue` _forcefieldmaterial "FlickerAmount" 0.0))))

(fn `SetForceFieldMaterialNormal`
  (bind _forcefieldmaterial (`self.ForceFieldMaterial`))
  (`/Engine/EditorBlueprintResources/StandardMacros.IsValid` _forcefieldmaterial
    (:`Is Valid`
      (`MaterialInstanceDynamic.SetScalarParameterValue` _forcefieldmaterial "Opacity" (`self.ForceFieldNormalOpacity`))
      (`MaterialInstanceDynamic.SetScalarParameterValue` _forcefieldmaterial "GlitchAmount" (`self.ForceFieldNormalGlitch`))
      (`MaterialInstanceDynamic.SetScalarParameterValue` _forcefieldmaterial "EmissiveIntensity" (`self.ForceFieldEmissive`))
      (`MaterialInstanceDynamic.SetVectorParameterValue` _forcefieldmaterial "GlitchColor" (`self.ForceFieldColor`)))))

(fn `UpdateSuctionAudioVolume`
  (`AudioComponent.SetVolumeMultiplier` (`self.Audio_SuctionLoop`) (`KismetMathLibrary.Lerp` 0.2 1.0 (`self.SuctionRampAlpha`))))

(fn `UpdateSuctionRamp`
  (params (DeltaSeconds :type "Float (double-precision)"))
  (bind (_returnvalue_x _returnvalue_y) (`KismetMathLibrary.BreakVector2D` (`KismetMathLibrary.MakeVector2D` 0.0 1.0)))
  (set `self.SuctionRampAlpha` (`|EaseFunction` "EaseInOut" (`KismetMathLibrary.FClamp` (/ (+ (`self.SuctionRampTimer`) DeltaSeconds) (`self.SuctionRampDuration`))) _returnvalue_x _returnvalue_y)))

(fn `UserConstructionScript`)