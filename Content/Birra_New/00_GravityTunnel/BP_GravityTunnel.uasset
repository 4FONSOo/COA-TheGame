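; Gravity tunnel hazard that stages a one-shot, resettable decompression event, sucking objects and characters in the tunnel.
; Activation closes both doors, starts the alarm and emergency lights, then after delays opens the exterior door and runs timed suction with VFX and audio.
; While suction runs, Tick applies force and random torque to suckable BP_GravityObjects toward SuctionTarget and launches overlapping Characters.
; Reset stops suction, closes all doors and unhides normal lights.
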(event `self.ReceiveBeginPlay`
  (`KismetSystemLibrary.PrintString` "Hello"))

(event `ActivateGravityTunnel`
  (bind _exteriordoor (`self.ExteriorDoor`))
  (bind _door_b (`self.Door_B`))
  (bind _alarm (`self.Alarm`))
  (bind _door_a (`self.Door_A`))
  (if (not (`self.bAlreadyActivated`))
    (set `self.bAlreadyActivated` true)
    (set `self.bTunnelActive` true)
    (`|ExecutionSequence`
      (:`then_0`
        (`/Engine/EditorBlueprintResources/StandardMacros.IsValid` _door_a
          (:`Is Valid`
            (`/Game/Birra/BP_GenericDoor.CloseDoor` _door_a))))
      (:`then_1`
        (`/Engine/EditorBlueprintResources/StandardMacros.IsValid` _door_b
          (:`Is Valid`
            (`/Game/Birra/BP_GenericDoor.CloseDoor` _door_b))))
      (:`then_2`
        (`/Engine/EditorBlueprintResources/StandardMacros.IsValid` _alarm
          (:`Is Valid`
            (`/Game/Birra/BP_GenericAlarm.StartAlarm` _alarm))))
      (:`then_3`
        (`KismetSystemLibrary.Delay` (`self.ExteriorDoorOpenDelay`))
        (`/Engine/EditorBlueprintResources/StandardMacros.IsValid` _exteriordoor
          (:`Is Valid`
            (`/Game/Birra/BP_ExteriorDoor.OpenDoor` _exteriordoor)
            (`AudioComponent.Play` (`self.PreSuctionWarningAudio`) 0.0)
            (`KismetSystemLibrary.Delay` (`self.DramaticPauseDuration`))
            (if (`self.bTunnelActive`)
              (`KismetSystemLibrary.PrintString` "Hello")
              (`self.StartSuction`)))))
      (:`then_4`
        (`self.StartEmergencyLighting`)))))

(event `StartEmergencyLighting`
  (for _array_element (`self.NormalLights`)
    (`/Engine/EditorBlueprintResources/StandardMacros.IsValid` _array_element
      (:`Is Valid`
        (`self.SetActorHiddenInGame` _array_element true))))
  (for _array_element_2 (`self.EmergencyLights`)
    (`/Engine/EditorBlueprintResources/StandardMacros.IsValid` _array_element_2
      (:`Is Valid`
        (`/Game/Birra/BP_EmergencyLight.LigarEmergencyLights` _array_element_2)))))

(event `StartSuction`
  (bind _decompressionaudio_ (`self.DecompressionAudio `))
  (set `self.bSuctionActive` true)
  (`self.StartSuctionVFX`)
  (`AudioComponent.Play` _decompressionaudio_ 0.0)
  (`AudioComponent.FadeIn` _decompressionaudio_ 0.3 1.0 0.0 "Linear")
  (`KismetSystemLibrary.Delay` (`self.SuctionDuration`))
  (`self.StopSuction`))

(event `StopSuction`
  (set `self.bSuctionActive` false)
  (`self.StopSuctionVFX`)
  (`AudioComponent.FadeOut` (`self.DecompressionAudio `) 1.0 0.0 "Linear"))

(event `self.ReceiveTick`
  (params (DeltaSeconds :type "Float (single-precision)"))
  (if (`self.bSuctionActive`)
    (`self.ApplySuction`)))

(event `ApplySuction`
  (for _array_element (`PrimitiveComponent.GetOverlappingActors` (`self.TunnelZone`) "/Script/Engine.Actor")
    (bind _asbp_gravity_object (cast `/Game/Birra_New/00_GravityTunnel/BP_GravityObject` _array_element)
      (:`then`
        (if (`/Game/Birra_New/00_GravityTunnel/BP_GravityObject.CanBeSucked` _asbp_gravity_object)
          (bind _mesh (`/Game/Birra_New/00_GravityTunnel/BP_GravityObject.getObjectMesh` _asbp_gravity_object))
          (bind _returnvalue (`SceneComponent.K2_GetComponentLocation` _mesh))
          (`PrimitiveComponent.AddForce` _mesh (* (`KismetMathLibrary.Normal` (- (`SceneComponent.K2_GetComponentLocation` (`self.SuctionTarget`)) _returnvalue)) (`self.ObjectSuctionForce`)) "None" true)
          (`PrimitiveComponent.AddTorqueInRadians` _mesh (* (`KismetMathLibrary.RandomUnitVector`) (`self.SpinTorqueForce`)) "None" true)))
      (:`CastFailed`
        (bind _ascharacter (cast `Character` _array_element))
        (`Character.LaunchCharacter` _ascharacter (* (`KismetMathLibrary.Normal` (- _returnvalue (`self.K2_GetActorLocation` _ascharacter))) (`self.PlayerPullVelocity`)) true true)))))

(event `self.SuctionEndZone.OnComponentBeginOverlap`
  (params (OverlappedComponent :type "PrimitiveComponent Object Reference") (OtherActor :type "Actor Object Reference") (OtherComp :type "PrimitiveComponent Object Reference") (OtherBodyIndex :type Integer) (bFromSweep :type Boolean) (SweepResult :type "HitResult Structure (by ref)"))
  (if (`self.bSuctionActive`)
    (bind _asbp_gravity_object (cast `/Game/Birra_New/00_GravityTunnel/BP_GravityObject` OtherActor))
    (`GameplayStatics.PlaySoundAtLocation` (`self.ObjectExitSound`) (`self.K2_GetActorLocation` _asbp_gravity_object) (struct) 1.0 1.0 0.0 null null null null)
    (`self.K2_DestroyActor` null)))

(event `StartSuctionVFX`
  (for _array_element (`self.SuctionVFXActors`)
    (`/Engine/EditorBlueprintResources/StandardMacros.IsValid` _array_element
      (:`Is Valid`
        (`/Game/Birra/VFX/BP_SuctionVFX.StartVFX` _array_element (`SceneComponent.K2_GetComponentLocation` (`self.SuctionTarget`)))))))

(event `StopSuctionVFX`
  (for _array_element (`self.SuctionVFXActors`)
    (`/Engine/EditorBlueprintResources/StandardMacros.IsValid` _array_element
      (:`Is Valid`
        (`/Game/Birra/VFX/BP_SuctionVFX.StopVFX` _array_element)))))

(event `StopEmergencyLighting`
  (for _array_element (`self.NormalLights`)
    (`/Engine/EditorBlueprintResources/StandardMacros.IsValid` _array_element
      (:`Is Valid`
        (`self.SetActorHiddenInGame` _array_element false)))))

(event `ResetGravityTunnel`
  (bind _door_a (`self.Door_A`))
  (bind _door_b (`self.Door_B`))
  (bind _exteriordoor (`self.ExteriorDoor`))
  (set `self.bTunnelActive` false)
  (`self.StopSuction`)
  (`|ExecutionSequence`
    (:`then_0`
      (`/Engine/EditorBlueprintResources/StandardMacros.IsValid` _exteriordoor
        (:`Is Valid`
          (`/Game/Birra/BP_ExteriorDoor.CloseDoor` _exteriordoor))))
    (:`then_1`
      (`/Engine/EditorBlueprintResources/StandardMacros.IsValid` _door_a
        (:`Is Valid`
          (`/Game/Birra/BP_GenericDoor.CloseDoor` _door_a))))
    (:`then_2`
      (`/Engine/EditorBlueprintResources/StandardMacros.IsValid` _door_b
        (:`Is Valid`
          (`/Game/Birra/BP_GenericDoor.CloseDoor` _door_b))))
    (:`then_3`
      (`self.StopEmergencyLighting`))
    (:`then_4`
      (set `self.bAlreadyActivated` false))))

(fn `UserConstructionScript`)