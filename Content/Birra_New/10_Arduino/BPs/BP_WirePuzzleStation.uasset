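; Interactable wire puzzle station that mirrors an Arduino-driven puzzle on a world widget and opens a dummy door when solved.
; The trigger box enables input, with E blending the view to the station and D returning it.
; Events from BP_ArduinoWirePuzzleController update three wires on WBP_WirePuzzleVisual.
; Solving runs a timed color blink, restores the player view, fires a completion dispatcher and raises the door, which F also moves for debugging.
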(event `CheckPuzzleSolvedForDoor`
  (bind _arduinopuzzlecontrollerref (`self.ArduinoPuzzleControllerRef`))
  (`/Engine/EditorBlueprintResources/StandardMacros.IsValid` _arduinopuzzlecontrollerref
    (:`Is Valid`
      (if (`/Game/Birra_New/10_Arduino/BPs/BP_ArduinoWirePuzzleController.bPuzzleSolved` _arduinopuzzlecontrollerref)
        (if (not (`self.bDoorAlreadyOpened `))
          (set `self.bDoorAlreadyOpened ` true)
          (`KismetSystemLibrary.PrintString` "Abrir Porta")
          (`self.OpenDummySolvedDoor`))))))

(event `Key|F`
  (params (Key :type "Key Structure"))
  (bind (_dummydoorclosedrelativelocation_x _dummydoorclosedrelativelocation_y _dummydoorclosedrelativelocation_z) (`KismetMathLibrary.BreakVector` (`self.DummyDoorClosedRelativeLocation`)))
  (:`Pressed`
    (`KismetSystemLibrary.PrintString` "DebugPorta")
    (`KismetSystemLibrary.MoveComponentTo` (`self.SM_DummySolvedDoor`) (`KismetMathLibrary.MakeVector` _dummydoorclosedrelativelocation_x _dummydoorclosedrelativelocation_y (+ _dummydoorclosedrelativelocation_z (`self.DummyDoorOpenHeight`))) (struct) true true (`self.DummyDoorOpenTime`) :!label _label)))

(event `OpenDummySolvedDoor`
  (`KismetSystemLibrary.PrintString` "OPEN DUMMY DOOR CALLED")
  (if (`self.bUseDummySolvedDoor`)
    (if (not (`self.bDummyDoorOpened`))
      (set `self.bDummyDoorOpened` true)
      (goto _label))))

(event `Key|D`
  (params (Key :type "Key Structure"))
  (:`Pressed`
    (if (`self.bPuzzleViewActive`)
      (`self.ExitPuzzleView`))))

(event `self.ReceiveBeginPlay`
  (`SceneComponent.SetVisibility` (`self.TextRender_InteractPrompt`) false false)
  (`SceneComponent.SetVisibility` (`self.WidgetComponent_PuzzleVisual`) false false)
  (set `self.bPlayerIsInside` false)
  (set `self.bPuzzleViewActive` false)
  (set `self.bInteractionEnabled` true)
  (`self.FindArduinoPuzzleController`)
  (set `self.DummyDoorClosedRelativeLocation` (`SceneComponent.RelativeLocation` (`self.SM_DummySolvedDoor`))))

(event `self.Box_InteractionTrigger.OnComponentBeginOverlap`
  (params (OverlappedComponent :type "PrimitiveComponent Object Reference") (OtherActor :type "Actor Object Reference") (OtherComp :type "PrimitiveComponent Object Reference") (OtherBodyIndex :type Integer) (bFromSweep :type Boolean) (SweepResult :type "HitResult Structure (by ref)"))
  (bind _ascharacter (cast `Character` OtherActor))
  (set `self.PlayerRef` _ascharacter)
  (bind _output_get (set `self.PlayerControllerRef` (`GameplayStatics.GetPlayerController` 0)))
  (set `self.bPlayerIsInside` true)
  (`SceneComponent.SetVisibility` (`self.TextRender_InteractPrompt`) true false)
  (`self.EnableInput` _output_get)
  (`SceneComponent.SetVisibility` (`self.WidgetComponent_PuzzleVisual`) true false))

(event `self.Box_InteractionTrigger.OnComponentEndOverlap`
  (params (OverlappedComponent :type "PrimitiveComponent Object Reference") (OtherActor :type "Actor Object Reference") (OtherComp :type "PrimitiveComponent Object Reference") (OtherBodyIndex :type Integer))
  (cast `Character` OtherActor)
  (set `self.bPlayerIsInside` false)
  (`SceneComponent.SetVisibility` (`self.TextRender_InteractPrompt`) false false)
  (if (`self.bPuzzleViewActive`)
    (`self.ExitPuzzleView`)
    (else
      (`self.RefreshStationVisualState`)
      (`self.DisableInput` (stale `self.Box_InteractionTrigger.OnComponentBeginOverlap` _output_get)))))

(event `Key|E`
  (params (Key :type "Key Structure"))
  (:`Pressed`
    (if (`self.bPuzzleViewActive`)
      _
      (elif (`self.bPlayerIsInside`)
        (if (`self.bInteractionEnabled`)
          (if (not (`self.bStationCompleted`))
            (`self.EnterPuzzleView`)))))))

(event `OnArduinoWireStateChanged`
  (`KismetSystemLibrary.PrintString` "STATION RECEIVED WIRE CHANGE" true true (struct :`R` 1.0 :`G` 0.803057 :`A` 1.0) 10.0)
  (if (not (`self.bStationCompleted`))
    (`self.UpdateWireVisuals`)))

(event `BlinkPuzzleColors`
  (bind _puzzlewidgetref (`self.PuzzleWidgetRef`))
  (`/Engine/EditorBlueprintResources/StandardMacros.IsValid` _puzzlewidgetref
    (:`Is Valid`
      (`/Game/Birra_New/10_Arduino/UI/WBP_WirePuzzleVisual.RandomBlinkColors_Safe` _puzzlewidgetref))))

(event `OnArduinoPuzzleSolved`
  (`self.StartSolvedBlink`))

(event `OnArduinoPuzzleReset`
  (bind _puzzlewidgetref (`self.PuzzleWidgetRef`))
  (`/Engine/EditorBlueprintResources/StandardMacros.IsValid` _puzzlewidgetref
    (:`Is Valid`
      (`/Game/Birra_New/10_Arduino/UI/WBP_WirePuzzleVisual.HideAllWires` _puzzlewidgetref)
      (`self.UpdateWireVisuals`))))

(event `StartSolvedBlink`
  (if (not (`self.bSolvedSequenceRunning`))
    (set `self.bSolvedSequenceRunning` true)
    (set `self.bInteractionEnabled` false)
    (bind _returnvalue (`KismetSystemLibrary.K2_SetTimer` null "BlinkPuzzleColors" (`self.SolvedBlinkInterval`) true))
    (bind _output_get (set `self.SolvedBlinkTimerHandle` _returnvalue))
    (`KismetSystemLibrary.Delay` (`self.SolvedBlinkDuration`))
    (`KismetSystemLibrary.K2_ClearAndInvalidateTimerHandle` _output_get)
    (`self.EndPuzzleViewSolved`)
    (`self.OpenDummySolvedDoor`)))

(event `OnArduinoPuzzleFailed`)

(event `EndPuzzleViewSolved`
  (bind _playerref (`self.PlayerRef`))
  (bind _puzzlewidgetref (`self.PuzzleWidgetRef`))
  (`KismetSystemLibrary.K2_ClearAndInvalidateTimerHandle` (`self.SolvedBlinkTimerHandle`))
  (`/Engine/EditorBlueprintResources/StandardMacros.IsValid` _puzzlewidgetref
    (:`Is Valid`
      (`/Game/Birra_New/10_Arduino/UI/WBP_WirePuzzleVisual.ApplyWireColors` _puzzlewidgetref)
      (`self.HidePuzzleWidget`)
      (set `self.bStationCompleted` true)
      (set `self.bPuzzleViewActive` false)
      (set `self.bInteractionEnabled` false)
      (set `self.bInteractionEnabled` false)
      (`/Engine/EditorBlueprintResources/StandardMacros.IsValid` _playerref
        (:`Is Valid`
          (`PlayerController.SetViewTargetWithBlend` (`self.PlayerControllerRef`) _playerref (`self.ExitViewBlendTime`) "VTBlend_Linear" 0.0 false)
          (`SceneComponent.SetVisibility` (`self.TextRender_InteractPrompt`) false false)
          (`self.ED_WirePuzzleStationCompleted`)
          (`KismetSystemLibrary.PrintString` "Wire Puzzle Station Completed"))))))

(fn `BindArduinoEvents`
  (bind _arduinopuzzlecontrollerref (`self.ArduinoPuzzleControllerRef`))
  (`KismetSystemLibrary.PrintString` "Binding Arduino EVENTS entrei")
  (if (not (`self.bArduinoEventsBound`))
    (`self.FindArduinoPuzzleController`)
    (`/Engine/EditorBlueprintResources/StandardMacros.IsValid` _arduinopuzzlecontrollerref
      (:`Is Valid`
        (add `/Game/Birra_New/10_Arduino/BPs/BP_ArduinoWirePuzzleController.ED_WirePuzzleChanged` _arduinopuzzlecontrollerref (`|CreateDelegate` :!event `OnArduinoWireStateChanged`))
        (`KismetSystemLibrary.PrintString` "Wire Changed OK")
        (add `/Game/Birra_New/10_Arduino/BPs/BP_ArduinoWirePuzzleController.ED_WirePuzzleSolved` _arduinopuzzlecontrollerref (`|CreateDelegate` :!event `OnArduinoPuzzleSolved`))
        (add `/Game/Birra_New/10_Arduino/BPs/BP_ArduinoWirePuzzleController.ED_WirePuzzleReset` _arduinopuzzlecontrollerref (`|CreateDelegate` :!event `OnArduinoPuzzleReset`))
        (add `/Game/Birra_New/10_Arduino/BPs/BP_ArduinoWirePuzzleController.ED_WirePuzzleFailed` _arduinopuzzlecontrollerref (`|CreateDelegate` :!event `OnArduinoPuzzleFailed`))
        (set `self.bArduinoEventsBound` true))
      (:`Is Not Valid`
        (`KismetSystemLibrary.PrintString` "Falhou Arduino")))))

(fn `EnterPuzzleView`
  (set `self.bPuzzleViewActive` true)
  (set `self.bInteractionEnabled` false)
  (`KismetSystemLibrary.K2_SetTimer` null "CheckPuzzleSolvedForDoor" 0.1)
  (`SceneComponent.SetVisibility` (`self.TextRender_InteractPrompt`) false false)
  (`PlayerController.SetViewTargetWithBlend` (`self.PlayerControllerRef`) self (`self.EnterViewBlendTime`) "VTBlend_Linear" 0.0 false)
  (`self.ShowPuzzleWidget`))

(fn `ExitPuzzleView`
  (bind _playercontrollerref (`self.PlayerControllerRef`))
  (bind _textrender_interactprompt (`self.TextRender_InteractPrompt`))
  (`/Engine/EditorBlueprintResources/StandardMacros.IsValid` _playercontrollerref
    (:`Is Valid`
      (`PlayerController.SetViewTargetWithBlend` _playercontrollerref (`self.PlayerRef`) (`self.ExitViewBlendTime`) "VTBlend_Linear" 0.0 false)
      (set `self.bPuzzleViewActive` false)
      (set `self.bInteractionEnabled` true)
      (`self.HidePuzzleWidget`)
      (if (`self.bPlayerIsInside`)
        (`SceneComponent.SetVisibility` _textrender_interactprompt true false)
        (else
          (`SceneComponent.SetVisibility` _textrender_interactprompt false false)
          (`self.DisableInput` (`self.PlayerControllerRef`))
          (`self.HidePuzzleWidget`)
          (`KismetSystemLibrary.K2_ClearTimer` null))))
    (:`Is Not Valid`
      (return))))

(fn `FindArduinoPuzzleController`
  (`/Engine/EditorBlueprintResources/StandardMacros.IsValid` (`self.ArduinoPuzzleControllerRef`)
    (:`Is Not Valid`
      (bind _returnvalue (`GameplayStatics.GetActorOfClass` "/Game/Birra_New/10_Arduino/BPs/BP_ArduinoWirePuzzleController.BP_ArduinoWirePuzzleController_C"))
      (set `self.ArduinoPuzzleControllerRef` _returnvalue))))

(fn `HidePuzzleWidget`
  (bind _widgetcomponent_puzzlevisual (`self.WidgetComponent_PuzzleVisual`))
  (`/Engine/EditorBlueprintResources/StandardMacros.IsValid` _widgetcomponent_puzzlevisual
    (:`Is Valid`
      (`SceneComponent.SetVisibility` _widgetcomponent_puzzlevisual false false))))

(fn `RefreshStationVisualState`
  (bind _puzzlewidgetref (`self.PuzzleWidgetRef`))
  (`SceneComponent.SetVisibility` (`self.TextRender_InteractPrompt`) false false)
  (`self.HidePuzzleWidget`)
  (`/Engine/EditorBlueprintResources/StandardMacros.IsValid` _puzzlewidgetref
    (:`Is Valid`
      (`/Game/Birra_New/10_Arduino/UI/WBP_WirePuzzleVisual.HideAllWires` _puzzlewidgetref))))

(fn `ShowPuzzleWidget`
  (bind _widgetcomponent_puzzlevisual (`self.WidgetComponent_PuzzleVisual`))
  (`SceneComponent.SetVisibility` _widgetcomponent_puzzlevisual true false)
  (bind _aswbp_wire_puzzle_visual (cast `/Game/Birra_New/10_Arduino/UI/WBP_WirePuzzleVisual` (`WidgetComponent.GetUserWidgetObject` _widgetcomponent_puzzlevisual)))
  (bind _output_get (set `self.PuzzleWidgetRef` _aswbp_wire_puzzle_visual))
  (if (`/Game/Birra_New/10_Arduino/UI/WBP_WirePuzzleVisual.bUseRandomWireColors` _output_get)
    (`/Game/Birra_New/10_Arduino/UI/WBP_WirePuzzleVisual.RandomizeRightSideOnly` _output_get)
    (else
      (`/Game/Birra_New/10_Arduino/UI/WBP_WirePuzzleVisual.ApplyDefaultWireColors` _output_get)))
  (`/Game/Birra_New/10_Arduino/UI/WBP_WirePuzzleVisual.HideAllWires` _output_get)
  (`self.BindArduinoEvents`)
  (`self.UpdateWireVisuals`))

(fn `UpdateWireVisuals`
  (bind _arduinopuzzlecontrollerref (`self.ArduinoPuzzleControllerRef`))
  (bind _puzzlewidgetref (`self.PuzzleWidgetRef`))
  (`KismetSystemLibrary.PrintString` "UPDATE WIRE Visuals")
  (`/Engine/EditorBlueprintResources/StandardMacros.IsValid` _arduinopuzzlecontrollerref
    (:`Is Valid`
      (`/Engine/EditorBlueprintResources/StandardMacros.IsValid` _puzzlewidgetref
        (:`Is Valid`
          (`/Game/Birra_New/10_Arduino/UI/WBP_WirePuzzleVisual.SetWireConnected` _puzzlewidgetref 1 (`/Game/Birra_New/10_Arduino/BPs/BP_ArduinoWirePuzzleController.Wire1Connected` _arduinopuzzlecontrollerref))
          (`/Game/Birra_New/10_Arduino/UI/WBP_WirePuzzleVisual.SetWireConnected` _puzzlewidgetref 2 (`/Game/Birra_New/10_Arduino/BPs/BP_ArduinoWirePuzzleController.Wire2Connected` _arduinopuzzlecontrollerref))
          (`/Game/Birra_New/10_Arduino/UI/WBP_WirePuzzleVisual.SetWireConnected` _puzzlewidgetref 3 (`/Game/Birra_New/10_Arduino/BPs/BP_ArduinoWirePuzzleController.Wire3Connected` _arduinopuzzlecontrollerref)))
        (:`Is Not Valid`
          (return))))
    (:`Is Not Valid`
      (return))))

(fn `UserConstructionScript`)