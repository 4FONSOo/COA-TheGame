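; Three-wire door puzzle that opens a sliding door once all three wires are connected.
; A trigger overlap with the resident horror character enables input, and keys 1-3 toggle wire states.
; Each toggle recolors that wire's indicator mesh, and connecting one beeps and checks for completion.
; Solving starts a looping timer for a brief light show, sets indicators red despite the SetAllGreen name, then a timeline slides the door after a delay.
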(event `CE_OpenDoor`
  (`|ExecutionSequence`
    (:`then_0`
      (`GameplayStatics.PlaySound2D` "/Game/Birra_New/SFX/freesound_community-scifi-door-opening-36171.freesound_community-scifi-door-opening-36171" 1.0 1.0 0.0 null null))
    (:`then_1`
      (bind (_direction _alpha) (`Timeline|TL_OpenDoor` :!via `PlayFromStart`)
        (:`Update`
          (`SceneComponent.K2_SetRelativeLocation` (`self.SM_DOOR`) (`KismetMathLibrary.VLerp` (`self.DoorOpenLocation`) (`self.DoorClosedLocation`) _alpha) false false))))))

(event `Randomize`
  (params (TargetMesh :type "StaticMesh Object Reference") (FinalMaterial :type "MaterialInterface Object Reference"))
  (bind _output (`|GetArrayItem` (`self.RandomPrankMaterials`) (`KismetMathLibrary.RandomIntegerInRange` 0 1)))
  (`PrimitiveComponent.SetMaterial` (`self.SMN_Amarela`) 0 _output)
  (`PrimitiveComponent.SetMaterial` (`self.SMN_Azul`) 0 _output)
  (`PrimitiveComponent.SetMaterial` (`self.SMN_Vermelha`) 0 _output))

(event `CE_SetAllGreen`
  (bind _returnvalue (`KismetSystemLibrary.K2_SetTimerDelegate` (`|CreateDelegate` :!event `ApplyRandomSolvedMaterials`) 0.1 true))
  (bind _output_get (set `self.SolvedRandomTimerHandle` _returnvalue))
  (`KismetSystemLibrary.Delay` 2.5)
  (`KismetSystemLibrary.K2_ClearAndInvalidateTimerHandle` _output_get)
  (`GameplayStatics.PlaySound2D` "/Game/Birra_New/SFX/door_lock_007.door_lock_007" 1.0 1.0 0.0 null null)
  (`PrimitiveComponent.SetMaterial` (`self.SMN_Amarela`) 0 "/Game/Birra_New/10_Arduino/BPs/Ard_Red.Ard_Red")
  (`PrimitiveComponent.SetMaterial` (`self.SMN_Azul`) 0 "/Game/Birra_New/10_Arduino/BPs/Ard_Red.Ard_Red")
  (`PrimitiveComponent.SetMaterial` (`self.SMN_Vermelha`) 0 "/Game/Birra_New/10_Arduino/BPs/Ard_Red.Ard_Red"))

(event `CE_CheckSolved`
  (if (and (and (`self.bWire1Connected`) (`self.bWire2Connected`)) (`self.bWire3Connected`))
    (set `self.bSolved` true)
    (`self.CE_SetAllGreen`)
    (`KismetSystemLibrary.Delay` 5.0)
    (`self.CE_OpenDoor`)))

(event `ApplyRandomSolvedMaterials`
  (bind _randomprankmaterials (`self.RandomPrankMaterials`))
  (bind _output (`|GetArrayItem` _randomprankmaterials (`KismetMathLibrary.RandomIntegerInRange` 0 (- (`KismetArrayLibrary.Array_Length` _randomprankmaterials) 1))))
  (`PrimitiveComponent.SetMaterial` (`self.SMN_Amarela`) 0 _output)
  (`GameplayStatics.PlaySound2D` "/Game/Birra_New/SFX/Bluezone_BC0241_interface_beep_transmission_004.Bluezone_BC0241_interface_beep_transmission_004" 0.5 1.0 0.0 "/Game/Birra_New/Managers/Audio/5_Concurrency/CONC_Machine_OneShot.CONC_Machine_OneShot" null)
  (`PrimitiveComponent.SetMaterial` (`self.SMN_Azul`) 0 _output)
  (`GameplayStatics.PlaySound2D` "/Game/Birra_New/SFX/Bluezone_BC0241_interface_beep_transmission_004.Bluezone_BC0241_interface_beep_transmission_004" 0.5 1.0 0.0 "/Game/Birra_New/Managers/Audio/5_Concurrency/CONC_Machine_OneShot.CONC_Machine_OneShot" null)
  (`PrimitiveComponent.SetMaterial` (`self.SMN_Vermelha`) 0 _output)
  (`GameplayStatics.PlaySound2D` "/Game/Birra_New/SFX/Bluezone_BC0241_interface_beep_transmission_004.Bluezone_BC0241_interface_beep_transmission_004" 0.5 1.0 0.0 "/Game/Birra_New/Managers/Audio/5_Concurrency/CONC_Machine_OneShot.CONC_Machine_OneShot" null))

(event `CE_UpdateWireState`
  (params (WireIndex :type Integer) (bConnected :type Boolean))
  (bind _smn_amarela (`self.SMN_Amarela`))
  (bind _smn_azul (`self.SMN_Azul`))
  (bind _smn_vermelha (`self.SMN_Vermelha`))
  (if (`self.bPuzzleActive`)
    (if (not (`self.bSolved`))
      (switch `int` WireIndex
        (:`0`
          (if (`self.bWire2Connected`) :!label _label
            (`PrimitiveComponent.SetMaterial` _smn_amarela 0 (`self.M_Green`))
            (`GameplayStatics.PlaySound2D` "/Game/Birra_New/SFX/Bluezone_BC0241_interface_beep_transmission_004.Bluezone_BC0241_interface_beep_transmission_004" 0.5 1.0 0.0 "/Game/Birra_New/Managers/Audio/5_Concurrency/CONC_Machine_OneShot.CONC_Machine_OneShot" null)
            (`self.CE_CheckSolved` :!label _label_2)
            (else
              (`PrimitiveComponent.SetMaterial` _smn_amarela 0 (`self.M_White`)))))
        (:`1`
          (if (`self.bWire1Connected`)
            (`PrimitiveComponent.SetMaterial` _smn_vermelha 0 (`self.M_Blue`))
            (`GameplayStatics.PlaySound2D` "/Game/Birra_New/SFX/Bluezone_BC0241_interface_beep_transmission_004.Bluezone_BC0241_interface_beep_transmission_004" 0.5 1.0 0.0 "/Game/Birra_New/Managers/Audio/5_Concurrency/CONC_Machine_OneShot.CONC_Machine_OneShot" null)
            (goto _label_2)
            (else
              (`PrimitiveComponent.SetMaterial` _smn_vermelha 0 (`self.M_White`)))))
        (:`3`
          (if (`self.bWire3Connected`)
            (`PrimitiveComponent.SetMaterial` _smn_azul 0 (`self.M_Yellow`))
            (`GameplayStatics.PlaySound2D` "/Game/Birra_New/SFX/Bluezone_BC0241_interface_beep_transmission_004.Bluezone_BC0241_interface_beep_transmission_004" 0.5 1.0 0.0 "/Game/Birra_New/Managers/Audio/5_Concurrency/CONC_Machine_OneShot.CONC_Machine_OneShot" null)
            (goto _label_2)
            (else
              (`PrimitiveComponent.SetMaterial` _smn_azul 0 (`self.M_White`)))))
        (:`4`
          (goto _label))))))

(event `self.w.OnComponentBeginOverlap`
  (params (OverlappedComponent :type "PrimitiveComponent Object Reference") (OtherActor :type "Actor Object Reference") (OtherComp :type "PrimitiveComponent Object Reference") (OtherBodyIndex :type Integer) (bFromSweep :type Boolean) (SweepResult :type "HitResult Structure (by ref)"))
  (cast `/Game/ChildrenOfAndromeda/Character/BP_Character/BP_Resident_HorrorV1` OtherActor)
  (`self.EnableInput` (`GameplayStatics.GetPlayerController` 0))
  (set `self.bPuzzleActive` true)
  (`KismetSystemLibrary.PrintString` "Hello"))

(event `Key|One`
  (params (Key :type "Key Structure"))
  (:`Pressed`
    (if (`self.bPuzzleActive`)
      (if (`self.bWire1Connected`)
        (set `self.bWire1Connected` false)
        (else
          (set `self.bWire1Connected` true)))
      (`self.CE_UpdateWireState` 1 true))))

(event `Key|Two`
  (params (Key :type "Key Structure"))
  (:`Pressed`
    (if (`self.bPuzzleActive`)
      (if (`self.bWire2Connected`)
        (set `self.bWire2Connected` false)
        (else
          (set `self.bWire2Connected` true)))
      (`self.CE_UpdateWireState` 4 true))))

(event `self.w.OnComponentEndOverlap`
  (params (OverlappedComponent :type "PrimitiveComponent Object Reference") (OtherActor :type "Actor Object Reference") (OtherComp :type "PrimitiveComponent Object Reference") (OtherBodyIndex :type Integer))
  (cast `/Game/ChildrenOfAndromeda/Character/BP_Character/BP_Resident_HorrorV1` OtherActor)
  (`self.DisableInput` (`GameplayStatics.GetPlayerController` 0))
  (set `self.bPuzzleActive` false))

(event `Key|Three`
  (params (Key :type "Key Structure"))
  (:`Pressed`
    (if (`self.bPuzzleActive`)
      (if (`self.bWire3Connected`)
        (set `self.bWire3Connected` false)
        (else
          (set `self.bWire3Connected` true)))
      (`self.CE_UpdateWireState` 3 true))))

(event `self.ReceiveBeginPlay`
  (`PrimitiveComponent.SetMaterial` (`self.SMN_Vermelha`) 0 "/Game/Birra_New/10_Arduino/BPs/Ard_Branco.Ard_Branco")
  (`PrimitiveComponent.SetMaterial` (`self.SMN_Azul`) 0 "/Game/Birra_New/10_Arduino/BPs/Ard_Branco.Ard_Branco")
  (`PrimitiveComponent.SetMaterial` (`self.SMN_Amarela`) 0 "/Game/Birra_New/10_Arduino/BPs/Ard_Branco.Ard_Branco")
  (set `self.bWire1Connected` false)
  (set `self.bWire2Connected` false)
  (set `self.bWire3Connected` false)
  (set `self.bSolved` false)
  (set `self.bPuzzleActive` false))

(fn `UserConstructionScript`)