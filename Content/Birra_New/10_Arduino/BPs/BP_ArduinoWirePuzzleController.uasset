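; Controller actor that links an Arduino wire puzzle over a serial COM port to an in-game three-wire puzzle.
; After BeginPlay it opens the port, sends a greeting and polls lines on a looping timer.
; Filtered lines update board status and puzzle wires 1–3 from hardware wires 1, 4 and 3, while disconnect messages are dropped.
; Helpers send reset, lock and unlock commands; solved/failed parsing sits in unconnected nodes.
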(event `Key|One`
  (params (Key :type "Key Structure")))

(event `Key|Three`
  (params (Key :type "Key Structure")))

(event `Key|Zero`
  (params (Key :type "Key Structure")))

(event `Key|Five`
  (params (Key :type "Key Structure")))

(event `Key|Eight`
  (params (Key :type "Key Structure")))

(event `Key|Two`
  (params (Key :type "Key Structure")))

(event `Key|Four`
  (params (Key :type "Key Structure")))

(event `Key|Nine`
  (params (Key :type "Key Structure")))

(event `Key|Six`
  (params (Key :type "Key Structure")))

(event `DebugParseLine`
  (params (DebugLine :type String))
  (if (`self.bEnableManualDebug`)
    (`self.ParseArduinoLine` DebugLine)))

(event `self.ReceiveEndPlay`
  (params (EndPlayReason :type "EEndPlayReason Enum" :default "Destroyed"))
  (bind _serialport (`self.SerialPort`))
  (`KismetSystemLibrary.K2_ClearTimer` null "PollArduino")
  (`/Engine/EditorBlueprintResources/StandardMacros.IsValid` _serialport
    (:`Is Valid`
      (if (`self.bSerialOpen`)
        (`SerialCom.Close` _serialport)
        (set `self.bSerialOpen` false)
        (set `self.bBoardDetected` false)
        (set `self.bArduinoReady` false)
        (`KismetSystemLibrary.PrintString` "arduino COM fechada en Endplay")
        (else
          (set `self.bBoardDetected` false)
          (set `self.bArduinoReady` false))))))

(event `self.ReceiveBeginPlay`
  (`self.EnableInput` (`GameplayStatics.GetPlayerController` 0))
  (`KismetSystemLibrary.Delay` 1.0)
  (`self.OpenArduinoConnection`))

(event `OnWireChanged`
  (if (`self.bDebugArduino`)
    (`KismetSystemLibrary.PrintString` (`KismetStringLibrary.Concat_StrStr` "Wire changed | Connected:" (`KismetStringLibrary.Conv_IntToString` (`self.ConnectedWireCount`))))
    (`self.ED_WirePuzzleChanged`)))

(event `OnPuzzleSolved`
  (`KismetSystemLibrary.PrintString` "WIRE PUZZLE SOLVED" true true (struct :`G` 0.66 :`B` 1.0 :`A` 1.0) 55.0)
  (`self.ED_WirePuzzleSolved`)
  (`self.TriggerSolvedGameplay`))

(event `DebugPrintSerialPortScan`
  (set `self.CurrentScanPort ` (`self.ScanMinPort`))
  (`KismetSystemLibrary.PrintString` "Serial Scan")
  (`self.DebugPrintSerialPortScan`))

(event `OnPuzzleFailed`
  (`KismetSystemLibrary.PrintString` "WIRE PUZZLE FAILED")
  (`self.ED_WirePuzzleFailed`)
  (`self.TriggerFailedGamePlay`))

(event `DebugPrintCurrentSerialPort`
  (if (> (`self.CurrentScanPort `) (`self.ScanMaxPort`))
    (`KismetSystemLibrary.PrintString` "SERIAL SCAN END")
    (else
      (set `self.CurrentScanPort ` (+ (`self.CurrentScanPort `) 1))
      (`KismetSystemLibrary.Delay` (`self.DebugScanDelay `)))))

(event `TriggerSolvedGameplay`
  (if (`self.bUseSolvedTargetActor`)
    (`/Engine/EditorBlueprintResources/StandardMacros.IsValid` (`self.SolvedTargetActor`)
      (:`Is Valid`
        (`KismetSystemLibrary.PrintString` "Valid"))
      (:`Is Not Valid`
        (`KismetSystemLibrary.PrintString` "InValid")))))

(event `TriggerFailedGamePlay`
  (if (`self.bUseFailedTargetActor`)
    (`/Engine/EditorBlueprintResources/StandardMacros.IsValid` (`self.FailedTargetActor`)
      (:`Is Valid`
        (`KismetSystemLibrary.PrintString` "Valid"))
      (:`Is Not Valid`
        (`KismetSystemLibrary.PrintString` "InValid")))))

(fn `CanProcessArduinoLine`
  (params (`LineToCheck ` :type String))
  (returns (bCanProcess :type Boolean))
  (locals (CleanLine :type String))
  (if (`KismetStringLibrary.Contains` `LineToCheck ` "DISCONNECTED")
    (return false)
    (elif (`self.bSerialOpen`)
      (`/Engine/EditorBlueprintResources/StandardMacros.IsValid` (`self.SerialPort`)
        (:`Is Valid`
          (if (`self.bPuzzleSolved`)
            (if (`KismetStringLibrary.Contains` `LineToCheck ` "RESET")
              (return true)
              (else
                (return false)))
            (elif (`self.bPuzzleActive`)
              (return true)
              (elif (`KismetStringLibrary.Contains` `LineToCheck ` "RESET")
                (return true)
                (else
                  (return false))))))
        (:`Is Not Valid`
          (return false)))
      (else
        (return false)))))

(fn `NewFunction`)

(fn `OpenArduinoConnection`
  (set `self.bSerialOpen` false)
  (if (`self.bSerialOpen`)
    (`KismetSystemLibrary.PrintString` "Aberto")
    (`KismetSystemLibrary.K2_SetTimer` null "StartArduinoHandshake" (`self.ReadInterval`))
    (else
      (bind (_bopened _returnvalue) (`SerialCom.OpenComPort` (`self.PortName`) (`self.BaudRate`)))
      (set `self.SerialPort` _returnvalue)
      (bind _output_get (set `self.bSerialOpen` _bopened))
      (if _output_get
        (`KismetSystemLibrary.PrintString` "Arduino Aberto")
        (`KismetSystemLibrary.K2_SetTimer` null "StartArduinoHandshake" (`self.ReadInterval`))
        (else
          (`KismetSystemLibrary.PrintString` "Arduino Fechado")
          (set `self.bSerialOpen` false)
          (set `self.bBoardDetected` false)
          (set `self.bArduinoReady` false))))))

(fn `ParseArduinoLine`
  (params (LineToParse :type String))
  (bind _threewirepuzzleref_final (`self.ThreeWirePuzzleRef_Final`))
  (bind _threewirepuzzleref_final_2 (`self.ThreeWirePuzzleRef_Final`))
  (bind _threewirepuzzleref_final_3 (`self.ThreeWirePuzzleRef_Final`))
  (if (`self.bDebugArduino`)
    (`KismetSystemLibrary.PrintString` LineToParse))
  (if (`KismetStringLibrary.Contains` LineToParse "BOARD:READY")
    (set `self.bBoardDetected` true)
    (set `self.bArduinoReady` true)
    (`KismetSystemLibrary.PrintString` "Arduino Board Ready")
    (elif (`KismetStringLibrary.Contains` LineToParse "PONG")
      (set `self.bBoardDetected` true)
      (`KismetSystemLibrary.PrintString` "Arduino Pong Received")
      (return)
      (else
        (`|ExecutionSequence`
          (:`then_0`
            (if (`KismetStringLibrary.Contains` LineToParse "WIRE:1:CONNECTED")
              (`self.UpdateConnectedWireCount`)
              (`/Engine/EditorBlueprintResources/StandardMacros.IsValid` _threewirepuzzleref_final_2
                (:`Is Valid`
                  (set `/Game/Birra_New/10_Arduino/BPs/BP_ThreeWireDoorPuzzle.bWire1Connected` true _threewirepuzzleref_final_2)
                  (`/Game/Birra_New/10_Arduino/BPs/BP_ThreeWireDoorPuzzle.CE_UpdateWireState` _threewirepuzzleref_final_2 1 true)))
              (elif (`KismetStringLibrary.Contains` LineToParse "WIRE:1:DISCONNECTED")
                (`self.UpdateConnectedWireCount`)
                (`/Engine/EditorBlueprintResources/StandardMacros.IsValid` _threewirepuzzleref_final_2
                  (:`Is Valid`
                    (set `/Game/Birra_New/10_Arduino/BPs/BP_ThreeWireDoorPuzzle.bWire1Connected` false _threewirepuzzleref_final_2)
                    (`/Game/Birra_New/10_Arduino/BPs/BP_ThreeWireDoorPuzzle.CE_UpdateWireState` _threewirepuzzleref_final_2 1 false))))))
          (:`then_1`
            (if (`KismetStringLibrary.Contains` LineToParse "WIRE:4:CONNECTED")
              (`self.UpdateConnectedWireCount`)
              (`/Engine/EditorBlueprintResources/StandardMacros.IsValid` _threewirepuzzleref_final_3
                (:`Is Valid`
                  (set `/Game/Birra_New/10_Arduino/BPs/BP_ThreeWireDoorPuzzle.bWire2Connected` true _threewirepuzzleref_final_3)
                  (`/Game/Birra_New/10_Arduino/BPs/BP_ThreeWireDoorPuzzle.CE_UpdateWireState` _threewirepuzzleref_final_3 4 true)))
              (elif (`KismetStringLibrary.Contains` LineToParse "WIRE:4:DISCONNECTED")
                (`self.UpdateConnectedWireCount`))))
          (:`then_2`
            (if (`KismetStringLibrary.Contains` LineToParse "WIRE:3:CONNECTED")
              (`self.UpdateConnectedWireCount`)
              (`/Engine/EditorBlueprintResources/StandardMacros.IsValid` _threewirepuzzleref_final
                (:`Is Valid`
                  (set `/Game/Birra_New/10_Arduino/BPs/BP_ThreeWireDoorPuzzle.bWire3Connected` true _threewirepuzzleref_final)
                  (`/Game/Birra_New/10_Arduino/BPs/BP_ThreeWireDoorPuzzle.CE_UpdateWireState` _threewirepuzzleref_final 3 true)))
              (elif (`KismetStringLibrary.Contains` LineToParse "WIRE:3:DISCONNECTED")
                _))))))))

(fn `PollArduino`
  (if (`self.bSerialOpen`)
    (bind (_bsuccess _returnvalue) (`SerialCom.Readln` (`self.SerialPort`)))
    (bind _output_get (set `self.LastLine` _returnvalue))
    (`KismetSystemLibrary.PrintString` (`KismetStringLibrary.Concat_StrStr` "FODASSEEEEEEEE" (`KismetStringLibrary.Concat_StrStr` "Arduino Last Line ->" _output_get)) true true (struct :`R` 1.0 :`G` 0.375824 :`A` 1.0) 5.0)
    (bind _bcanprocess (`self.CanProcessArduinoLine` _output_get))
    (if _bcanprocess
      (`self.ParseArduinoLine` _output_get)
      (elif (`self.bDebugArduino`)
        (`KismetSystemLibrary.PrintString` "Ignored arduino line")
        (else
          (return))))))

(fn `ResetPuzzleState`
  (set `self.Wire1Connected` false)
  (set `self.Wire2Connected` false)
  (set `self.Wire3Connected` false)
  (set `self.Wire4Connected` false)
  (set `self.ConnectedWireCount` 0)
  (set `self.bPuzzleSolved` false)
  (set `self.bPuzzleFailed` false)
  (set `self.bPuzzleActive` true)
  (if (`self.bDebugArduino`)
    (`KismetSystemLibrary.PrintString` "Wire Puzzle Reset")
    (set `self.bArduinoReady` (`self.bArduinoReady`))
    (set `self.bBoardDetected` (`self.bBoardDetected`))
    (`self.ED_WirePuzzleReset`)))

(fn `SendArduinoCommand`
  (params (Command :type String))
  (returns (bSent :type Boolean))
  (bind _serialport (`self.SerialPort`))
  (if (`self.bSerialOpen`)
    (`/Engine/EditorBlueprintResources/StandardMacros.IsValid` _serialport
      (:`Is Valid`
        (if (`KismetStringLibrary.Contains` Command "DISCONNECTED")
          (return false)
          (else
            (`SerialCom.Println` _serialport Command)
            (if (`self.bDebugArduino`)
              (`KismetSystemLibrary.PrintString` (`KismetStringLibrary.Concat_StrStr` "Send to Arduino" Command))
              (return true)))))
      (:`Is Not Valid`
        (`KismetSystemLibrary.PrintString` "Comando Arduino Falha: SerialPort Closed")
        (return false)))
    (else
      (`KismetSystemLibrary.PrintString` "Comando Arduino Falha: Serial Closed")
      (return false))))

(fn `SendHelloToArduino`
  (`KismetSystemLibrary.PrintString` "yoyoyo")
  (`self.SendArduinoCommand` "Estou aqui"))

(fn `SendLockToArduino`
  (bind _bsent (`self.SendArduinoCommand` "LOCK"))
  (if _bsent
    (set `self.bPuzzleActive` false)
    (else
      (return))))

(fn `SendPingToArduino`
  (`self.SendArduinoCommand` "PING"))

(fn `SendResetToArduino`
  (bind _bsent (`self.SendArduinoCommand` "RESET"))
  (if _bsent
    (`self.SendResetToArduino`)
    (else
      (return))))

(fn `SendUnlockToArduino`
  (bind _bsent (`self.SendArduinoCommand` "UNLOCK"))
  (if _bsent
    (bind _output_get (set `self.bPuzzleActive` true))
    (`KismetSystemLibrary.PrintString` (`KismetStringLibrary.Concat_StrStr` "Puzzle Active" (`KismetStringLibrary.Conv_BoolToString` _output_get)) true true (struct :`R` 1.0 :`G` 0.852737 :`A` 1.0) 40.0)
    (else
      (return))))

(fn `StartArduinoHandshake`
  (if (`self.bSerialOpen`)
    (`self.SendHelloToArduino`)
    (`KismetSystemLibrary.K2_SetTimer` null "PollArduino" (`self.ReadInterval`) true)
    (else
      (`KismetSystemLibrary.PrintString` "Cancelado"))))

(fn `UpdateConnectedWireCount`
  (set `self.ConnectedWireCount` 0)
  (if (`self.Wire1Connected`)
    (set `self.ConnectedWireCount` (+ (`self.ConnectedWireCount`) 1))
    (elif (`self.Wire2Connected`)
      (set `self.ConnectedWireCount` (+ (`self.ConnectedWireCount`) 1))
      (elif (`self.Wire3Connected`)
        (set `self.ConnectedWireCount` (+ (`self.ConnectedWireCount`) 1))
        (elif (`self.Wire4Connected`)
          (set `self.ConnectedWireCount` (+ (`self.ConnectedWireCount`) 1)))))))

(fn `UserConstructionScript`)