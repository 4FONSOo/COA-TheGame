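; Test Blueprint that checks for an Arduino board over a serial COM port using a PING/PONG handshake.
; On BeginPlay it opens the configured port, waits briefly, then sends PING and starts a looping timer.
; The timer reads lines until one contains PONG, then flags the board as detected and stops, printing debug status throughout.
; EndPlay closes the port.
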(event `ReadArduino`
  (if (not (`self.bBoardDetected`))
    (bind (_bsuccess _returnvalue) (`SerialCom.Readln` (stale `self.ReceiveBeginPlay` _output_get)))
    (bind _output_get (set `self.LastLine` _returnvalue))
    (if (`KismetStringLibrary.Contains` _output_get "PONG")
      (set `self.bBoardDetected` true)
      (`KismetSystemLibrary.PrintString` "ARDUINO DETECTED")
      (`KismetSystemLibrary.K2_ClearAndInvalidateTimerHandle` (stale `self.ReceiveBeginPlay` _output_get_2))
      (else
        (`KismetSystemLibrary.PrintString` "ERRO NO PONG")))))

(event `self.ReceiveBeginPlay`
  (bind (_bopened _returnvalue) (`SerialCom.OpenComPort` (`self.PortNumber`) (`self.BaudRate`)))
  (bind _output_get (set `self.SerialPortRef` _returnvalue))
  (`KismetSystemLibrary.PrintString` (`KismetSystemLibrary.GetDisplayName` _output_get))
  (`KismetSystemLibrary.Delay` 2.0)
  (if (`SerialCom.IsOpened` _output_get)
    (`KismetSystemLibrary.PrintString` "SERIAL OPEN OK")
    (`SerialCom.Println` _output_get "PING")
    (bind _returnvalue_2 (`KismetSystemLibrary.K2_SetTimerDelegate` (delegate `ReadArduino`) 0.2 true))
    (bind _output_get_2 (set `self.DetectionTimerHandle` _returnvalue_2))
    (else
      (`KismetSystemLibrary.PrintString` "SERIAL OPEN FAILED"))))

(event `self.ReceiveEndPlay`
  (params (EndPlayReason :type "EEndPlayReason Enum" :default "Destroyed"))
  (`/Engine/EditorBlueprintResources/StandardMacros.IsValid` (stale `self.ReceiveBeginPlay` _output_get)
    (:`Is Valid`
      (`SerialCom.Close` (stale `self.ReceiveBeginPlay` _output_get)))))

(fn `UserConstructionScript`)