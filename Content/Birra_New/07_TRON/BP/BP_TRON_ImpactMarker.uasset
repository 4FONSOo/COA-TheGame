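; Short-lived impact marker actor for the TRON level that shows light, Niagara VFX and sound at a hit point.
; BeginPlay applies ImpactScale and destroys the actor after ImpactLifetime.
; InitializeImpactFeedback orients it to the surface normal, sets the color and triggers feedback; its lifetime input is stored but unused here.
; With valid VFX and sound, the light hides immediately and the actor optionally self-destructs, without a timed fade.
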(event `StartImpactMarker`
  (bind _impactscale (`self.ImpactScale`))
  (`self.SetActorScale3D` (`KismetMathLibrary.MakeVector` _impactscale _impactscale _impactscale))
  (`KismetSystemLibrary.Delay` (`self.ImpactLifetime`))
  (`self.FinishImpactMarker`))

(event `FinishImpactMarker`
  (if true
    (`self.K2_DestroyActor`)
    (else
      (`self.SetActorHiddenInGame` true))))

(event `self.ReceiveBeginPlay`
  (`self.StartImpactMarker`))

(fn `FadeOutImpactFeedback`
  (`SceneComponent.SetVisibility` (`self.PointLight_Impact`) false false)
  (if (`self.bAutoDestroyAfterFade`)
    (`self.K2_DestroyActor`)))

(fn `InitializeImpactFeedback`
  (params (InImpactLocation :type "Vector Structure") (InImpactNormal :type "Vector Structure") (InImpactColor :type "LinearColor Structure") (InImpactLifetime :type "Float (double-precision)"))
  (`self.K2_SetActorLocationAndRotation` InImpactLocation (`KismetMathLibrary.MakeRotFromZ` InImpactNormal))
  (set `self.ImpactColor` InImpactColor)
  (set `self.ImpactLifetime_VFX` InImpactLifetime)
  (`self.PlayImpactFeedback`))

(fn `PlayImpactFeedback`
  (bind _pointlight_impact (`self.PointLight_Impact`))
  (bind _impactvfx (`self.ImpactVFX`))
  (bind _impactsound (`self.ImpactSound`))
  (`SceneComponent.SetVisibility` _pointlight_impact true false)
  (`LightComponent.SetIntensity` _pointlight_impact (`self.ImpactLightIntensity`))
  (`LocalLightComponent.SetAttenuationRadius` _pointlight_impact (`self.ImpactLightRadius`))
  (`LightComponent.SetLightColor` _pointlight_impact (`self.ImpactColor`) true)
  (`/Engine/EditorBlueprintResources/StandardMacros.IsValid` _impactvfx
    (:`Is Valid`
      (`NiagaraFunctionLibrary.SpawnSystemAtLocation` _impactvfx (`self.K2_GetActorLocation`) (`self.K2_GetActorRotation`) (`KismetMathLibrary.Conv_DoubleToVector` (`self.ImpactVFXScale`)) true true "None" false)
      (`/Engine/EditorBlueprintResources/StandardMacros.IsValid` _impactsound
        (:`Is Valid`
          (`GameplayStatics.SpawnSoundAtLocation` _impactsound (`self.K2_GetActorLocation`) (struct) (`self.ImpactSoundVolume`) (`self.ImpactSoundPitch`) 0.0 null null)
          (`self.FadeOutImpactFeedback`))))))

(fn `UserConstructionScript`)