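; Spawner actor for TRON beams, fired on behalf of a resident owner or through debug keys and scene start/end points.
; Fire functions set start, end and direction, optionally line tracing for the endpoint, then spawn a beam initialized from BeamConfig.
; Traced shots place a color-matched impact marker, and resident traced shots add optional muzzle sound and VFX.
; Stopping kills the tracked beam and clears its marker; respawning repeats this, then fires after a short delay.
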(event `self.ReceiveBeginPlay`
  (if (`self.bEnableDebugInput`)
    (`self.EnableInput` (`GameplayStatics.GetPlayerController` 0))))

(event `OnCurrentBeamFinished`
  (`self.ClearImpactMarker`)
  (set `self.CurrentBeamRef` null)
  (set `self.bBeamActive` false))

(event `RespawnTRONBeam`
  (`self.StopCurrentTRONBeam`)
  (`KismetSystemLibrary.Delay` 0.5)
  (`self.SpawnTRONBeam`))

(event `Key|Five`
  (params (Key :type "Key Structure"))
  (:`Pressed`
    (if (`self.bEnableDebugInput`)
      (`self.Debug_FireContinuous`))))

(event `Key|Six`
  (params (Key :type "Key Structure"))
  (:`Pressed`
    (if (`self.bEnableDebugInput`)
      (`self.StopCurrentTRONBeam`))))

(event `Key|Seven`
  (params (Key :type "Key Structure"))
  (:`Pressed`
    (if (`self.bEnableDebugInput`)
      (`self.Debug_FireTraceContinuous`))))

(event `Key|Eight`
  (params (Key :type "Key Structure"))
  (:`Pressed`
    (if (`self.bEnableDebugInput`)
      (`self.Debug_FireTraceImpact`))))

(fn `CalculateBeamEndFromTrace`
  (params (InStartLocation :type "Vector Structure") (InFireDirection :type "Vector Structure"))
  (returns (OutEndLocation :type "Vector Structure") (bHit :type Boolean) (OutHitResult :type "HitResult Structure"))
  (locals (NormalizedDirection :type "Vector Structure" :default (0.0 0.0 0.0)) (TraceEnd :type "Vector Structure"))
  (bind _output_get (set `local.NormalizedDirection` (`KismetMathLibrary.Normal` InFireDirection)))
  (bind _output_get_2 (set `local.TraceEnd` (+ InStartLocation (* _output_get (`self.MaxBeamDistance`)))))
  (bind (_outhit _returnvalue) (`KismetSystemLibrary.LineTraceSingle` InStartLocation _output_get_2 (`self.TraceChannel`)))
  (if _returnvalue
    (bind _output_get_3 (set `self.bLastTraceHit` true))
    (return (`.Location` (`GameplayStatics.BreakHitResult` _outhit)) _output_get_3 _outhit)
    (else
      (bind _output_get_4 (set `self.bLastTraceHit` false))
      (bind _output_get_5 (set `self.LastTraceHit` (struct)))
      (return (`local.TraceEnd`) _output_get_4 _output_get_5))))

(fn `ClearImpactMarker`
  (bind _currentimpactmarkerref (`self.CurrentImpactMarkerRef`))
  (`/Engine/EditorBlueprintResources/StandardMacros.IsValid` _currentimpactmarkerref
    (:`Is Valid`
      (`self.K2_DestroyActor` _currentimpactmarkerref)
      (set `self.CurrentImpactMarkerRef` null))
    (:`Is Not Valid`
      (return))))

(fn `Debug_FireContinuous`
  (set `self.CurrentStartLocation` (`SceneComponent.K2_GetComponentLocation` (`self.Scene_StartPoint`)))
  (set `self.CurrentEndLocation` (`SceneComponent.K2_GetComponentLocation` (`self.Scene_EndPoint`)))
  (set `self.CurrentFireDirection` (`SceneComponent.GetForwardVector` (`self.Arrow_Direction`)))
  (set `self.bCurrentImpactBeam` false)
  (`self.SpawnTRONBeam`))

(fn `Debug_FireImpact`
  (set `self.CurrentStartLocation` (`SceneComponent.K2_GetComponentLocation` (`self.Scene_StartPoint`)))
  (set `self.CurrentEndLocation` (`SceneComponent.K2_GetComponentLocation` (`self.Scene_EndPoint`)))
  (set `self.CurrentFireDirection` (`SceneComponent.GetForwardVector` (`self.Arrow_Direction`)))
  (set `self.bCurrentImpactBeam` false)
  (`self.SpawnTRONBeam`))

(fn `Debug_FireTraceContinuous`
  (locals (Const :type "Float (double-precision)" :default -1.0))
  (bind _returnvalue (`SceneComponent.K2_GetComponentLocation` (`self.Scene_StartPoint`)))
  (bind _returnvalue_2 (`SceneComponent.GetForwardVector` (`self.Arrow_Direction`)))
  (bind (_outendlocation _bhit _outhitresult) (`self.CalculateBeamEndFromTrace` _returnvalue _returnvalue_2))
  (set `self.CurrentStartLocation` _returnvalue)
  (set `self.CurrentEndLocation` _outendlocation)
  (set `self.CurrentFireDirection` _returnvalue_2)
  (set `self.bCurrentImpactBeam` _bhit)
  (`|ExecutionSequence`
    (:`then_0`
      (if _bhit
        (bind (_bblockinghit _binitialoverlap _time _distance _location _impactpoint _normal) (`GameplayStatics.BreakHitResult` _outhitresult))
        (`self.SpawnImpactMarker` _location _normal)
        (elif (`self.bSpawnImpactMarkerWithoutHit`)
          (`self.SpawnImpactMarker` (`self.CurrentEndLocation`) (* (`self.CurrentFireDirection`) (`local.Const`)))
          (`self.SpawnTRONBeam`))))
    (:`then_1`
      (`self.SpawnTRONBeam`))))

(fn `Debug_FireTraceImpact`
  (locals (Const_ :type "Float (double-precision)" :default -1.0))
  (bind _returnvalue (`SceneComponent.K2_GetComponentLocation` (`self.Scene_StartPoint`)))
  (bind _returnvalue_2 (`SceneComponent.GetForwardVector` (`self.Arrow_Direction`)))
  (bind (_outendlocation _bhit _outhitresult) (`self.CalculateBeamEndFromTrace` _returnvalue _returnvalue_2))
  (set `self.CurrentStartLocation` _returnvalue)
  (set `self.CurrentEndLocation` _outendlocation)
  (set `self.CurrentFireDirection` _returnvalue_2)
  (set `self.bCurrentImpactBeam` true)
  (`|ExecutionSequence`
    (:`then_0`
      (if _bhit
        (bind (_bblockinghit _binitialoverlap _time _distance _location _impactpoint _normal) (`GameplayStatics.BreakHitResult` _outhitresult))
        (`self.SpawnImpactMarker` _location _normal)
        (elif (`self.bSpawnImpactMarkerWithoutHit`)
          (`self.SpawnImpactMarker` (`self.CurrentEndLocation`) (* (`self.CurrentFireDirection`) (`local.Const_`)))
          (`self.SpawnTRONBeam`))))
    (:`then_1`
      (`self.SpawnTRONBeam`))))

(fn `FireTRONFromResident`
  (params (InResidentOwner :type "/Game/ChildrenOfAndromeda/Character/BP_Character/BP_Resident_HorrorV1 Object Reference") (InStartLocation :type "Vector Structure") (InFireDirection :type "Vector Structure") (bAsImpactBeam :type Boolean))
  (set `self.ResidentOwnerRef` InResidentOwner)
  (set `self.bUseResidentOwner` true)
  (set `self.bCurrentImpactBeam` bAsImpactBeam)
  (bind _output_get (set `self.CurrentFireDirection` (`KismetMathLibrary.Normal` InFireDirection)))
  (set `self.CurrentStartLocation` InStartLocation)
  (set `self.CurrentEndLocation` (* (+ InStartLocation _output_get) (`self.DefaultBeamDistance`)))
  (`self.SpawnTRONBeam`))

(fn `FireTRONFromResident_WithTrace`
  (params (InResidentOwner :type "/Game/ChildrenOfAndromeda/Character/BP_Character/BP_Resident_HorrorV1 Object Reference") (InStartLocation :type "Vector Structure") (InFireDirection :type "Vector Structure") (bForceImpactMode :type Boolean))
  (locals (Const :type "Float (double-precision)" :default -1.0))
  (set `self.ResidentOwnerRef` InResidentOwner)
  (set `self.bUseResidentOwner` true)
  (bind (_outendlocation _bhit _outhitresult) (`self.CalculateBeamEndFromTrace` InStartLocation InFireDirection))
  (bind _output_get (set `self.CurrentStartLocation` InStartLocation))
  (set `self.CurrentEndLocation` _outendlocation)
  (bind _output_get_2 (set `self.CurrentFireDirection` (`KismetMathLibrary.Normal` InFireDirection)))
  (set `self.bCurrentImpactBeam` _bhit)
  (`self.PlayTRONFireFeedback` _output_get _output_get_2)
  (`|ExecutionSequence`
    (:`then_0`
      (if _bhit
        (bind (_bblockinghit _binitialoverlap _time _distance _location _impactpoint _normal) (`GameplayStatics.BreakHitResult` _outhitresult))
        (`self.SpawnImpactMarker` _location _normal)
        (elif (`self.bSpawnImpactMarkerWithoutHit`)
          (`self.SpawnImpactMarker` (`self.CurrentEndLocation`) (* (`self.CurrentFireDirection`) (`local.Const`)))
          (`self.SpawnTRONBeam` :!label _label))))
    (:`then_1`
      (goto _label))))

(fn `PlayTRONFireFeedback`
  (params (InStartLocation :type "Vector Structure") (InFireDirection :type "Vector Structure"))
  (if (`self.bUseTRONFireSound`)
    (`GameplayStatics.SpawnSoundAtLocation` (`self.TRONFireSound`) InStartLocation (struct) (`self.FireSoundVolume`) (`self.FireSoundPitch`) 0.0 null null)
    (if (`self.bUseTRONFireVFX`)
      (`NiagaraFunctionLibrary.SpawnSystemAtLocation` (`self.TRONFireVFX`) InStartLocation (`KismetMathLibrary.MakeRotFromX` InFireDirection) (`KismetMathLibrary.Conv_DoubleToVector` (`self.FireVFXScale`))))))

(fn `SetBeamStartAndEnd`
  (params (InStartLocation :type "Vector Structure") (InEndLocation :type "Vector Structure") (InFireDirection :type "Vector Structure"))
  (set `self.CurrentStartLocation` InStartLocation)
  (set `self.CurrentEndLocation` InEndLocation)
  (set `self.CurrentFireDirection` InFireDirection))

(fn `SpawnImpactMarker`
  (params (InImpactLocation :type "Vector Structure") (InImpactNormal :type "Vector Structure"))
  (bind _beamconfig_beamcolor (break `/Game/Birra_New/07_TRON/Structs/ST_TRONBeamConfig` (`self.BeamConfig`)))
  (`self.ClearImpactMarker`)
  (bind _returnvalue (`|SpawnActorFromClass` (`self.ImpactMarkerClass`) (`KismetMathLibrary.MakeTransform` InImpactLocation (`KismetMathLibrary.MakeRotFromZ` InImpactNormal)) "Undefined" "MultiplyWithRoot" null null))
  (bind _output_get (set `self.CurrentImpactMarkerRef` _returnvalue))
  (`/Game/Birra_New/07_TRON/BP/BP_TRON_ImpactMarker.InitializeImpactFeedback` _output_get InImpactLocation InImpactNormal _beamconfig_beamcolor 0.35))

(fn `SpawnTRONBeam`
  (bind _returnvalue (`|SpawnActorFromClass` (`self.BeamClass`) (`KismetMathLibrary.MakeTransform` (`self.CurrentStartLocation`)) "Undefined" "MultiplyWithRoot" null null))
  (bind _output_get (set `self.CurrentBeamRef` _returnvalue))
  (set `self.bBeamActive` true)
  (`/Game/Birra_New/07_TRON/BP/BP_TRON_Beam.InitializeBeamFromConfig` _output_get (`self.CurrentStartLocation`) (`self.CurrentEndLocation`) (`self.BeamConfig`) (`self.bDefaultImpactBeam`)))

(fn `SpawnTRONImpactFeedback`)

(fn `StopCurrentTRONBeam`
  (bind _currentbeamref (`self.CurrentBeamRef`))
  (`/Engine/EditorBlueprintResources/StandardMacros.IsValid` _currentbeamref
    (:`Is Valid`
      (`/Game/Birra_New/07_TRON/BP/BP_TRON_Beam.ForceKillBeam` _currentbeamref)
      (set `self.CurrentBeamRef` null)
      (set `self.bBeamActive` false)
      (`self.ClearImpactMarker`)
      (if (`self.bDebugSpawner`)
        (`KismetSystemLibrary.PrintString` "TRON Beam Stopped")))
    (:`Is Not Valid`
      (set `self.bBeamActive` false)
      (return))))

(fn `UserConstructionScript`)