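; TRON-style beam actor that stretches layered core and glow meshes between start and end points, with cross-glow meshes currently hidden.
; Init functions place and scale it, create dynamic materials and set color, noise and glow parameters.
; Timers hold the beam, then a looping TickFade drives tail noise dissolve, or vertical fade for impact beams.
; Finishing or force-killing calls the finished dispatcher, then destroys or hides the actor.
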(fn `ApplyMaterialParameters`
  (bind (_beamconfig_beamcolor _beamconfig_coreintensity _beamconfig_glowintensity _beamconfig_corewidth _beamconfig_innerglowwidth _beamconfig_outerglowwidth _beamconfig_beamlifetime _beamconfig_impactholdtime _beamconfig_fadeduration _beamconfig_noisespeed _beamconfig_noisescale _beamconfig_wavespeed _beamconfig_wavestrength) (break `/Game/Birra_New/07_TRON/Structs/ST_TRONBeamConfig` (`self.BeamConfig`)))
  (bind _mid_innerglow (`self.MID_InnerGlow`))
  (bind _mid_outerglow (`self.MID_OuterGlow`))
  (bind _mid_crossglow01 (`self.MID_CrossGlow01`))
  (bind _mid_crossglow02 (`self.MID_CrossGlow02`))
  (bind (_beamconfig_beamcolor_2 _beamconfig_coreintensity_2 _beamconfig_glowintensity_2 _beamconfig_corewidth_2 _beamconfig_innerglowwidth_2 _beamconfig_outerglowwidth_2 _beamconfig_beamlifetime_2 _beamconfig_impactholdtime_2 _beamconfig_fadeduration_2 _beamconfig_noisespeed_2 _beamconfig_noisescale_2 _beamconfig_wavespeed_2 _beamconfig_wavestrength_2) (break `/Game/Birra_New/07_TRON/Structs/ST_TRONBeamConfig` (`self.BeamConfig`)))
  (bind _dissolveamount (`self.DissolveAmount`))
  (bind _verticalfadeamount (`self.VerticalFadeAmount`))
  (bind _dissolveamount_2 (`self.DissolveAmount`))
  (bind _verticalfadeamount_2 (`self.VerticalFadeAmount`))
  (bind _mid_core (`self.MID_Core`))
  (`/Engine/EditorBlueprintResources/StandardMacros.IsValid` _mid_core
    (:`Is Valid`
      (`MaterialInstanceDynamic.SetVectorParameterValue` _mid_core "BeamColor" _beamconfig_beamcolor_2)
      (`MaterialInstanceDynamic.SetScalarParameterValue` _mid_core "EmissiveIntensity" _beamconfig_coreintensity_2)
      (`MaterialInstanceDynamic.SetScalarParameterValue` _mid_core "LayerOpacity" 1.0)
      (`MaterialInstanceDynamic.SetScalarParameterValue` _mid_core "EdgeSoftness" 0.08)
      (`MaterialInstanceDynamic.SetScalarParameterValue` _mid_core "DissolveAmount" (`self.DissolveAmount`))
      (`MaterialInstanceDynamic.SetScalarParameterValue` _mid_core "VerticalFadeAmount" (`self.VerticalFadeAmount`))
      (`MaterialInstanceDynamic.SetScalarParameterValue` _mid_core "NoiseScale" _beamconfig_noisescale_2)
      (`MaterialInstanceDynamic.SetScalarParameterValue` _mid_core "NoiseSpeed" _beamconfig_noisespeed_2)
      (`MaterialInstanceDynamic.SetScalarParameterValue` _mid_core "WaveSpeed" _beamconfig_wavespeed_2)
      (`MaterialInstanceDynamic.SetScalarParameterValue` _mid_core "WaveStrength" (* _beamconfig_wavestrength_2 0.6))
      (`/Engine/EditorBlueprintResources/StandardMacros.IsValid` _mid_innerglow
        (:`Is Valid`
          (`MaterialInstanceDynamic.SetVectorParameterValue` _mid_innerglow "BeamColor" _beamconfig_beamcolor_2)
          (`MaterialInstanceDynamic.SetScalarParameterValue` _mid_innerglow "EmissiveIntensity" _beamconfig_glowintensity_2)
          (`MaterialInstanceDynamic.SetScalarParameterValue` _mid_innerglow "LayerOpacity" 0.55)
          (`MaterialInstanceDynamic.SetScalarParameterValue` _mid_innerglow "EdgeSoftness" 0.25)
          (`MaterialInstanceDynamic.SetScalarParameterValue` _mid_innerglow "DissolveAmount" _dissolveamount_2)
          (`MaterialInstanceDynamic.SetScalarParameterValue` _mid_innerglow "VerticalFadeAmount" _verticalfadeamount_2)
          (`MaterialInstanceDynamic.SetScalarParameterValue` _mid_innerglow "NoiseScale" (* _beamconfig_noisescale_2 0.8))
          (`MaterialInstanceDynamic.SetScalarParameterValue` _mid_innerglow "NoiseSpeed" _beamconfig_noisespeed_2)
          (`MaterialInstanceDynamic.SetScalarParameterValue` _mid_innerglow "WaveSpeed" _beamconfig_wavespeed_2)
          (`MaterialInstanceDynamic.SetScalarParameterValue` _mid_innerglow "WaveStrength" _beamconfig_wavestrength_2)
          (`/Engine/EditorBlueprintResources/StandardMacros.IsValid` _mid_outerglow
            (:`Is Valid`
              (`MaterialInstanceDynamic.SetVectorParameterValue` _mid_outerglow "BeamColor" _beamconfig_beamcolor)
              (`MaterialInstanceDynamic.SetScalarParameterValue` _mid_outerglow "EmissiveIntensity" (* _beamconfig_glowintensity_2 0.45))
              (`MaterialInstanceDynamic.SetScalarParameterValue` _mid_outerglow "LayerOpacity" 0.25)
              (`MaterialInstanceDynamic.SetScalarParameterValue` _mid_outerglow "EdgeSoftness" 0.55)
              (`MaterialInstanceDynamic.SetScalarParameterValue` _mid_outerglow "DissolveAmount" _dissolveamount_2)
              (`MaterialInstanceDynamic.SetScalarParameterValue` _mid_outerglow "VerticalFadeAmount" _verticalfadeamount_2)
              (`MaterialInstanceDynamic.SetScalarParameterValue` _mid_outerglow "NoiseScale" (* _beamconfig_noisescale_2 0.55))
              (`MaterialInstanceDynamic.SetScalarParameterValue` _mid_outerglow "NoiseSpeed" _beamconfig_noisespeed_2)
              (`MaterialInstanceDynamic.SetScalarParameterValue` _mid_outerglow "WaveSpeed" 0.0)
              (`MaterialInstanceDynamic.SetScalarParameterValue` _mid_outerglow "WaveStrength" 0.0)
              (`/Engine/EditorBlueprintResources/StandardMacros.IsValid` _mid_crossglow01
                (:`Is Valid`
                  (`MaterialInstanceDynamic.SetVectorParameterValue` _mid_crossglow01 "BeamColor" _beamconfig_beamcolor)
                  (`MaterialInstanceDynamic.SetScalarParameterValue` _mid_crossglow01 "EmissiveIntensity" (* _beamconfig_glowintensity 0.65))
                  (`MaterialInstanceDynamic.SetScalarParameterValue` _mid_crossglow01 "LayerOpacity" 0.35)
                  (`MaterialInstanceDynamic.SetScalarParameterValue` _mid_crossglow01 "EdgeSoftness" 0.4)
                  (`MaterialInstanceDynamic.SetScalarParameterValue` _mid_crossglow01 "DissolveAmount" _dissolveamount)
                  (`MaterialInstanceDynamic.SetScalarParameterValue` _mid_crossglow01 "VerticalFadeAmount" _verticalfadeamount)
                  (`MaterialInstanceDynamic.SetScalarParameterValue` _mid_crossglow01 "NoiseScale" (* _beamconfig_noisescale 0.7))
                  (`MaterialInstanceDynamic.SetScalarParameterValue` _mid_crossglow01 "NoiseSpeed" (* _beamconfig_noisespeed 0.9))
                  (`MaterialInstanceDynamic.SetScalarParameterValue` _mid_crossglow01 "WaveSpeed" (* _beamconfig_wavespeed 0.9))
                  (`MaterialInstanceDynamic.SetScalarParameterValue` _mid_crossglow01 "WaveStrength" _beamconfig_wavestrength)
                  (`/Engine/EditorBlueprintResources/StandardMacros.IsValid` _mid_crossglow02
                    (:`Is Valid`
                      (`MaterialInstanceDynamic.SetVectorParameterValue` _mid_crossglow02 "BeamColor" _beamconfig_beamcolor)
                      (`MaterialInstanceDynamic.SetScalarParameterValue` _mid_crossglow02 "EmissiveIntensity" (* _beamconfig_glowintensity 0.55))
                      (`MaterialInstanceDynamic.SetScalarParameterValue` _mid_crossglow02 "LayerOpacity" 0.3)
                      (`MaterialInstanceDynamic.SetScalarParameterValue` _mid_crossglow02 "EdgeSoftness" 0.45)
                      (`MaterialInstanceDynamic.SetScalarParameterValue` _mid_crossglow02 "DissolveAmount" _dissolveamount)
                      (`MaterialInstanceDynamic.SetScalarParameterValue` _mid_crossglow02 "VerticalFadeAmount" _verticalfadeamount)
                      (`MaterialInstanceDynamic.SetScalarParameterValue` _mid_crossglow02 "NoiseScale" (* _beamconfig_noisescale 0.65))
                      (`MaterialInstanceDynamic.SetScalarParameterValue` _mid_crossglow02 "NoiseSpeed" (* _beamconfig_noisespeed 0.85))
                      (`MaterialInstanceDynamic.SetScalarParameterValue` _mid_crossglow02 "WaveSpeed" (* _beamconfig_wavespeed 0.85))
                      (`MaterialInstanceDynamic.SetScalarParameterValue` _mid_crossglow02 "WaveStrength" (* _beamconfig_wavestrength 1.1)))))))))))))

(fn `ApplyMaterialParameters_Clean`
  (bind _mid_core (`self.MID_Core`))
  (bind _mid_innerglow (`self.MID_InnerGlow`))
  (bind (_beamconfig_beamcolor _beamconfig_coreintensity _beamconfig_glowintensity _beamconfig_corewidth _beamconfig_innerglowwidth _beamconfig_outerglowwidth _beamconfig_beamlifetime _beamconfig_impactholdtime _beamconfig_fadeduration _beamconfig_noisespeed _beamconfig_noisescale _beamconfig_wavespeed _beamconfig_wavestrength) (break `/Game/Birra_New/07_TRON/Structs/ST_TRONBeamConfig` (`self.BeamConfig`)))
  (bind (_beamconfig_beamcolor_2 _beamconfig_coreintensity_2 _beamconfig_glowintensity_2 _beamconfig_corewidth_2 _beamconfig_innerglowwidth_2 _beamconfig_outerglowwidth_2 _beamconfig_beamlifetime_2 _beamconfig_impactholdtime_2 _beamconfig_fadeduration_2 _beamconfig_noisespeed_2 _beamconfig_noisescale_2 _beamconfig_wavespeed_2 _beamconfig_wavestrength_2) (break `/Game/Birra_New/07_TRON/Structs/ST_TRONBeamConfig` (`self.BeamConfig`)))
  (`MaterialInstanceDynamic.SetVectorParameterValue` _mid_core "BeamColor" (`self.BeamColor`))
  (`MaterialInstanceDynamic.SetScalarParameterValue` _mid_core "EmissiveIntensity" _beamconfig_coreintensity_2)
  (`MaterialInstanceDynamic.SetScalarParameterValue` _mid_core "LayerOpacity" 1.0)
  (`MaterialInstanceDynamic.SetScalarParameterValue` _mid_core "EdgeSoftness" 8.0)
  (`MaterialInstanceDynamic.SetScalarParameterValue` _mid_core "DissolveAmount" (`self.DissolveAmount`))
  (`MaterialInstanceDynamic.SetScalarParameterValue` _mid_core "VerticalFadeAmount" (`self.VerticalFadeAmount`))
  (`MaterialInstanceDynamic.SetScalarParameterValue` _mid_core "NoiseScale" _beamconfig_noisescale_2)
  (`MaterialInstanceDynamic.SetScalarParameterValue` _mid_core "NoiseSpeed" _beamconfig_noisespeed_2)
  (`MaterialInstanceDynamic.SetScalarParameterValue` _mid_core "WaveSpeed" _beamconfig_wavespeed_2)
  (`MaterialInstanceDynamic.SetScalarParameterValue` _mid_core "WaveStrength" _beamconfig_wavestrength_2)
  (`MaterialInstanceDynamic.SetVectorParameterValue` _mid_innerglow "BeamColor" (`self.BeamColor`))
  (`MaterialInstanceDynamic.SetScalarParameterValue` _mid_innerglow "EmissiveIntensity" (* _beamconfig_glowintensity 0.45))
  (`MaterialInstanceDynamic.SetScalarParameterValue` _mid_innerglow "LayerOpacity" 0.35)
  (`MaterialInstanceDynamic.SetScalarParameterValue` _mid_innerglow "EdgeSoftness" 3.0)
  (`MaterialInstanceDynamic.SetScalarParameterValue` _mid_innerglow "DissolveAmount" (`self.DissolveAmount`))
  (`MaterialInstanceDynamic.SetScalarParameterValue` _mid_innerglow "VerticalFadeAmount" (`self.VerticalFadeAmount`))
  (`MaterialInstanceDynamic.SetScalarParameterValue` _mid_innerglow "NoiseScale" (* _beamconfig_noisescale 0.6))
  (`MaterialInstanceDynamic.SetScalarParameterValue` _mid_innerglow "NoiseSpeed" (* _beamconfig_noisescale 0.5)))

(fn `ApplyRuntimeFadeParameters`
  (bind _mid_core (`self.MID_Core`))
  (bind _mid_innerglow (`self.MID_InnerGlow`))
  (bind _dissolveamount (`self.DissolveAmount`))
  (bind _verticalfadeamount (`self.VerticalFadeAmount`))
  (bind _dissolveamount_2 (`self.DissolveAmount`))
  (bind _verticalfadeamount_2 (`self.VerticalFadeAmount`))
  (bind _mid_outerglow (`self.MID_OuterGlow`))
  (bind _mid_crossglow01 (`self.MID_CrossGlow01`))
  (bind _mid_crossglow02 (`self.MID_CrossGlow02`))
  (`/Engine/EditorBlueprintResources/StandardMacros.IsValid` _mid_core
    (:`Is Valid`
      (`MaterialInstanceDynamic.SetScalarParameterValue` _mid_core "DissolveAmount" (`self.DissolveAmount`))
      (`MaterialInstanceDynamic.SetScalarParameterValue` _mid_core "VerticalFadeAmount" (`self.VerticalFadeAmount`))
      (`/Engine/EditorBlueprintResources/StandardMacros.IsValid` _mid_innerglow
        (:`Is Valid`
          (`MaterialInstanceDynamic.SetScalarParameterValue` _mid_innerglow "DissolveAmount" _dissolveamount_2)
          (`MaterialInstanceDynamic.SetScalarParameterValue` _mid_innerglow "VerticalFadeAmount" _verticalfadeamount_2)
          (`/Engine/EditorBlueprintResources/StandardMacros.IsValid` _mid_outerglow
            (:`Is Valid`
              (`MaterialInstanceDynamic.SetScalarParameterValue` _mid_outerglow "DissolveAmount" _dissolveamount)
              (`MaterialInstanceDynamic.SetScalarParameterValue` _mid_outerglow "VerticalFadeAmount" _verticalfadeamount)
              (`/Engine/EditorBlueprintResources/StandardMacros.IsValid` _mid_crossglow01
                (:`Is Valid`
                  (`MaterialInstanceDynamic.SetScalarParameterValue` _mid_crossglow01 "DissolveAmount" _dissolveamount_2)
                  (`MaterialInstanceDynamic.SetScalarParameterValue` _mid_crossglow01 "VerticalFadeAmount" _verticalfadeamount_2)
                  (`/Engine/EditorBlueprintResources/StandardMacros.IsValid` _mid_crossglow02
                    (:`Is Valid`
                      (`MaterialInstanceDynamic.SetScalarParameterValue` _mid_crossglow02 "DissolveAmount" _dissolveamount)
                      (`MaterialInstanceDynamic.SetScalarParameterValue` _mid_crossglow02 "VerticalFadeAmount" _verticalfadeamount))))))))))))

(fn `BeginImpactFade`
  (set `self.CurrentState` "NewEnumerator3")
  (set `self.FadeElapsed` 0.0)
  (set `self.FadeMode` "NewEnumerator2")
  (set `self.DissolveAmount` 0.0)
  (set `self.VerticalFadeAmount` 0.0)
  (`self.ApplyRuntimeFadeParameters`)
  (bind _returnvalue (`KismetSystemLibrary.K2_SetTimer` null "TickFade" (`self.FadeTickInterval`) true))
  (set `self.FadeTimerHandle` _returnvalue))

(fn `BeginTailDissolve`
  (set `self.CurrentState` "NewEnumerator3")
  (set `self.FadeElapsed` 0.0)
  (set `self.FadeMode` "NewEnumerator1")
  (set `self.DissolveAmount` 0.0)
  (set `self.VerticalFadeAmount` 0.0)
  (`self.ApplyRuntimeFadeParameters`)
  (bind _returnvalue (`KismetSystemLibrary.K2_SetTimer` null "TickFade" (`self.FadeTickInterval`) true))
  (set `self.NewVar` _returnvalue))

(fn `CalculateBeamData`
  (bind _endlocation (`self.EndLocation`))
  (bind _startlocation (`self.StartLocation`))
  (set `self.BeamLength` (`KismetMathLibrary.VSize` (- _endlocation _startlocation)))
  (set `self.BeamRotation` (`KismetMathLibrary.FindLookAtRotation` _startlocation _endlocation)))

(fn `ClearBeamTimers`
  (`KismetSystemLibrary.K2_ClearAndInvalidateTimerHandle` (`self.LifeTimerHandle`))
  (`KismetSystemLibrary.K2_ClearAndInvalidateTimerHandle` (`self.ImpactHoldTimerHandle`))
  (`KismetSystemLibrary.K2_ClearAndInvalidateTimerHandle` (`self.FadeTimerHandle`)))

(fn `CreateDynamicMaterials`
  (bind _crossglowsourcematerial (`self.CrossGlowSourceMaterial`))
  (bind _returnvalue (`PrimitiveComponent.CreateDynamicMaterialInstance` (`self.SM_Core`) 0 (`self.CoreSourceMaterial`) "None"))
  (set `self.MID_Core` _returnvalue)
  (bind _returnvalue_2 (`PrimitiveComponent.CreateDynamicMaterialInstance` (`self.SM_InnerGlow`) 0 (`self.InnerGlowSourceMaterial`) "None"))
  (set `self.MID_InnerGlow` _returnvalue_2)
  (bind _returnvalue_3 (`PrimitiveComponent.CreateDynamicMaterialInstance` (`self.SM_OuterGlow`) 0 (`self.OuterGlowSourceMaterial`) "None"))
  (set `self.MID_OuterGlow` _returnvalue_3)
  (bind _returnvalue_4 (`PrimitiveComponent.CreateDynamicMaterialInstance` (`self.SM_CrossGlow_01`) 0 _crossglowsourcematerial "None"))
  (set `self.MID_CrossGlow01` _returnvalue_4)
  (bind _returnvalue_5 (`PrimitiveComponent.CreateDynamicMaterialInstance` (`self.SM_CrossGlow_02`) 0 _crossglowsourcematerial "None"))
  (set `self.MID_CrossGlow02` _returnvalue_5)
  (`SceneComponent.SetVisibility` (`self.SM_CrossGlow_01`) false false)
  (`SceneComponent.SetVisibility` (`self.SM_CrossGlow_02`) false false))

(fn `FinishBeam`
  (if (`self.bHasFinished`)
    (return)
    (else
      (`self.ClearBeamTimers`)
      (set `self.CurrentState` "NewEnumerator4")
      (set `self.DissolveAmount` 1.0)
      (set `self.VerticalFadeAmount` 1.0)
      (`self.ApplyRuntimeFadeParameters`)
      (`self.ED_TRONBeamFinished`)
      (if (`self.bIsAutoDestroy`)
        (`self.K2_DestroyActor`)
        (else
          (`self.SetActorHiddenInGame` true)
          (`self.SetActorEnableCollision` false))))))

(fn `ForceKillBeam`
  (if (`self.bHasFinished`)
    (return)
    (else
      (`self.ClearBeamTimers`)
      (set `self.FadeMode` "NewEnumerator3")
      (set `self.DissolveAmount` 1.0)
      (set `self.VerticalFadeAmount` 1.0)
      (set `self.CurrentState` "NewEnumerator3")
      (`self.ApplyRuntimeFadeParameters`)
      (`self.ED_TRONBeamFinished`)
      (if (`self.bIsAutoDestroy`)
        (`self.K2_DestroyActor`)
        (else
          (`self.SetBeamComponentsVisible` false))))))

(fn `InitializeBeam`
  (params (InStartLocation :type "Vector Structure") (InEndLocation :type "Vector Structure") (InFadeMode :type "/Game/Birra_New/07_TRON/Enums/E_TRONFadeMode Enum" :default "NewEnumerator0") (InBeamColor :type "LinearColor Structure") (bInImpactBeam :type Boolean))
  (set `self.StartLocation` InStartLocation)
  (set `self.EndLocation` InEndLocation)
  (set `self.FadeMode` InFadeMode)
  (set `self.BeamColor` InBeamColor)
  (set `self.bIsImpactBeam` bInImpactBeam)
  (set `self.CurrentState` "NewEnumerator1")
  (`self.CalculateBeamData`)
  (`self.UpdateBeamTransform`)
  (`self.CreateDynamicMaterials`)
  (`self.ApplyMaterialParameters_Clean`)
  (`self.StartBeamLifetime`))

(fn `InitializeBeamFromConfig`
  (params (InStartLocation :type "Vector Structure") (InEndLocation :type "Vector Structure") (InConfig :type "/Game/Birra_New/07_TRON/Structs/ST_TRONBeamConfig Structure") (bInImpactBeam :type Boolean))
  (bind (_beamcolor _coreintensity _glowintensity _corewidth _innerglowwidth _outerglowwidth _beamlifetime _impactholdtime _fadeduration _noisespeed _noisescale _wavespeed _wavestrength _fademode) (break `/Game/Birra_New/07_TRON/Structs/ST_TRONBeamConfig` InConfig))
  (set `self.bHasFinished` false)
  (set `self.StartLocation` InStartLocation)
  (set `self.EndLocation` InEndLocation)
  (set `self.BeamConfig` InConfig)
  (set `self.bUseStructConfig` true)
  (bind _output_get (set `self.bIsImpactBeam` bInImpactBeam))
  (`KismetSystemLibrary.PrintString` (`KismetStringLibrary.Conv_BoolToString` _output_get))
  (set `self.CurrentState` "NewEnumerator1")
  (set `self.BeamColor` _beamcolor)
  (set `self.FadeMode` _fademode)
  (`self.CalculateBeamData`)
  (`self.UpdateBeamTransform`)
  (`self.CreateDynamicMaterials`)
  (`self.ApplyMaterialParameters_Clean`)
  (`self.StartBeamLifetime`))

(fn `SetBeamComponentsVisible`
  (params (BIsVisible :type Boolean))
  (bind _sm_core (`self.SM_Core`))
  (bind _sm_crossglow_02 (`self.SM_CrossGlow_02`))
  (bind _sm_innerglow (`self.SM_InnerGlow`))
  (bind _sm_outerglow (`self.SM_OuterGlow`))
  (bind _sm_crossglow_01 (`self.SM_CrossGlow_01`))
  (`SceneComponent.SetVisibility` _sm_core BIsVisible false)
  (`SceneComponent.SetVisibility` _sm_innerglow BIsVisible false)
  (`SceneComponent.SetVisibility` _sm_outerglow BIsVisible false)
  (`SceneComponent.SetVisibility` _sm_crossglow_01 BIsVisible false)
  (`SceneComponent.SetVisibility` _sm_crossglow_02 BIsVisible false)
  (`PrimitiveComponent.SetCollisionEnabled` _sm_core "NoCollision")
  (`PrimitiveComponent.SetCollisionEnabled` _sm_innerglow "NoCollision")
  (`PrimitiveComponent.SetCollisionEnabled` _sm_outerglow "NoCollision")
  (`PrimitiveComponent.SetCollisionEnabled` _sm_crossglow_01 "NoCollision")
  (`PrimitiveComponent.SetCollisionEnabled` _sm_crossglow_02 "NoCollision"))

(fn `SetTRONColor`
  (params (NewColor :type "LinearColor Structure"))
  (bind _mid_core (`self.MID_Core`))
  (bind _mid_innerglow (`self.MID_InnerGlow`))
  (bind _mid_outerglow (`self.MID_OuterGlow`))
  (bind _mid_crossglow01 (`self.MID_CrossGlow01`))
  (bind _mid_crossglow02 (`self.MID_CrossGlow02`))
  (set `self.BeamColor` NewColor)
  (`/Engine/EditorBlueprintResources/StandardMacros.IsValid` _mid_core
    (:`Is Valid`
      (`MaterialInstanceDynamic.SetVectorParameterValue` _mid_core "BeamColor" NewColor)
      (`/Engine/EditorBlueprintResources/StandardMacros.IsValid` _mid_innerglow
        (:`Is Valid`
          (`MaterialInstanceDynamic.SetVectorParameterValue` _mid_innerglow "BeamColor" NewColor)
          (`/Engine/EditorBlueprintResources/StandardMacros.IsValid` _mid_outerglow
            (:`Is Valid`
              (`MaterialInstanceDynamic.SetVectorParameterValue` _mid_outerglow "BeamColor" NewColor)
              (`/Engine/EditorBlueprintResources/StandardMacros.IsValid` _mid_crossglow01
                (:`Is Valid`
                  (`MaterialInstanceDynamic.SetVectorParameterValue` _mid_crossglow01 "BeamColor" NewColor)
                  (`/Engine/EditorBlueprintResources/StandardMacros.IsValid` _mid_crossglow02
                    (:`Is Valid`
                      (`MaterialInstanceDynamic.SetVectorParameterValue` _mid_crossglow02 "BeamColor" NewColor))))))))))))

(fn `StartBeamLifetime`
  (bind _bisimpactbeam (`self.bIsImpactBeam`))
  (bind (_beamconfig_beamcolor _beamconfig_coreintensity _beamconfig_glowintensity _beamconfig_corewidth _beamconfig_innerglowwidth _beamconfig_outerglowwidth _beamconfig_beamlifetime _beamconfig_impactholdtime) (break `/Game/Birra_New/07_TRON/Structs/ST_TRONBeamConfig` (`self.BeamConfig`)))
  (`KismetSystemLibrary.PrintString` "Entrei no start")
  (`KismetSystemLibrary.PrintString` (`KismetStringLibrary.Concat_StrStr` "Impact?" (`KismetStringLibrary.Conv_BoolToString` _bisimpactbeam)))
  (if _bisimpactbeam
    (set `self.CurrentState` "NewEnumerator2")
    (bind _returnvalue (`KismetSystemLibrary.K2_SetTimer` null "BeginImpactFade" _beamconfig_impactholdtime))
    (set `self.ImpactHoldTimerHandle` _returnvalue)
    (`KismetSystemLibrary.PrintString` "TAIL TIMER STARTED")
    (else
      (set `self.CurrentState` "NewEnumerator1")
      (bind _returnvalue_2 (`KismetSystemLibrary.K2_SetTimer` null "BeginTailDissolve" _beamconfig_beamlifetime))
      (set `self.LifeTimerHandle` _returnvalue_2)
      (`KismetSystemLibrary.PrintString` "TAIL TIMER STARTED"))))

(fn `TickFade`
  (bind (_beamconfig_beamcolor _beamconfig_coreintensity _beamconfig_glowintensity _beamconfig_corewidth _beamconfig_innerglowwidth _beamconfig_outerglowwidth _beamconfig_beamlifetime _beamconfig_impactholdtime _beamconfig_fadeduration) (break `/Game/Birra_New/07_TRON/Structs/ST_TRONBeamConfig` (`self.BeamConfig`)))
  (bind _returnvalue (`KismetMathLibrary.FClamp` (/ (`self.FadeElapsed`) _beamconfig_fadeduration)))
  (set `self.FadeElapsed` (+ (`self.FadeElapsed`) (`self.FadeTickInterval`)))
  (switch `/Game/Birra_New/07_TRON/Enums/E_TRONFadeMode` (`self.FadeMode`)
    (:`NewEnumerator0`
      (return))
    (:`NewEnumerator1`
      (set `self.DissolveAmount` _returnvalue)
      (set `self.VerticalFadeAmount` 0.0)
      (`self.ApplyRuntimeFadeParameters`))
    (:`NewEnumerator2`
      (set `self.VerticalFadeAmount` _returnvalue)
      (set `self.DissolveAmount` 0.0)
      (`self.ApplyRuntimeFadeParameters`))
    (:`NewEnumerator3`
      (set `self.DissolveAmount` 0.0)
      (set `self.VerticalFadeAmount` 0.0)
      (`self.ApplyRuntimeFadeParameters`)))
  (if (>= _returnvalue 1.0)
    (`self.FinishBeam`)))

(fn `UpdateBeamTransform`
  (locals (Constant_1 :type "Float (double-precision)" :default 0.5))
  (bind _startlocation (`self.StartLocation`))
  (bind (_beamconfig_beamcolor _beamconfig_coreintensity _beamconfig_glowintensity _beamconfig_corewidth _beamconfig_innerglowwidth _beamconfig_outerglowwidth) (break `/Game/Birra_New/07_TRON/Structs/ST_TRONBeamConfig` (`self.BeamConfig`)))
  (bind _returnvalue (/ (`self.BeamLength`) (`self.MeshBaseLength`)))
  (`self.K2_SetActorLocation` (+ (* (- (`self.EndLocation`) _startlocation) (`local.Constant_1`)) _startlocation))
  (`self.K2_SetActorRotation` (`self.BeamRotation`))
  (`SceneComponent.SetRelativeScale3D` (`self.SM_Core`) (`KismetMathLibrary.MakeVector` _beamconfig_corewidth _returnvalue 1.0))
  (`SceneComponent.SetRelativeScale3D` (`self.SM_InnerGlow`) (`KismetMathLibrary.MakeVector` _beamconfig_innerglowwidth _returnvalue 1.0))
  (`SceneComponent.SetRelativeScale3D` (`self.SM_OuterGlow`) (`KismetMathLibrary.MakeVector` _beamconfig_outerglowwidth _returnvalue 1.0))
  (`SceneComponent.SetRelativeScale3D` (`self.SM_CrossGlow_01`) (`KismetMathLibrary.MakeVector` _beamconfig_innerglowwidth _returnvalue 1.0))
  (`SceneComponent.SetRelativeScale3D` (`self.SM_CrossGlow_02`) (`KismetMathLibrary.MakeVector` (* _beamconfig_outerglowwidth 0.5) _returnvalue 1.0)))

(fn `UserConstructionScript`
  (`self.CalculateBeamData`)
  (`self.UpdateBeamTransform`)
  (`self.CreateDynamicMaterials`)
  (`self.ApplyMaterialParameters`)
  (`self.ApplyRuntimeFadeParameters`))