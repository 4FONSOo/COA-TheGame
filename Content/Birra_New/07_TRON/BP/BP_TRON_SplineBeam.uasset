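; TRON-style beam actor that lays spline meshes along a path, with left and right cameras looking ahead along it.
; BeginPlay rebuilds the spline from preset points, then shows the full beam with cameras at the path's end.
; UpdateBeamGrowth reveals and trims segments by progress, which the construction script uses for editor preview.
; The timeline that would animate growth and cameras is disconnected, so nothing animates at runtime.
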(event `StartGrowBeam`
  (`self.ClearSplineMeshes`)
  (`self.BuildSplineBeam`)
  (`self.UpdateBeamGrowth` 1.0))

(event `self.ReceiveBeginPlay`
  (`self.StartGrowBeam`)
  (`self.BuildSplineFromPresetArray`))

(event `BuildSplineFromPresetArray`
  (bind _spline_tronpath (`self.Spline_TRONPath`))
  (`SplineComponent.ClearSplinePoints` _spline_tronpath false)
  (for (_array_element _array_index) (`self.PresetSplinePoints`)
    (`SplineComponent.AddSplinePoint` _spline_tronpath (break `/Game/Birra_New/07_TRON/Structs/ST_TRON_SplinePresetPoint` _array_element) "Local" false)
    (`SplineComponent.SetRotationAtSplinePoint` _spline_tronpath _array_index (`.Rotation_14_DF272F8B4C8CD41ED61DE4802E617461` (break `/Game/Birra_New/07_TRON/Structs/ST_TRON_SplinePresetPoint` _array_element)) "Local" false)
    (`SplineComponent.SetTangentsAtSplinePoint` _spline_tronpath _array_index (`.ArriveTangent_13_0FF84F604B63C3C2AC1CFDA46B66AE79` (break `/Game/Birra_New/07_TRON/Structs/ST_TRON_SplinePresetPoint` _array_element)) (`.LeaveTangent_12_9312CFD24D49C211DC35988E5170EA18` (break `/Game/Birra_New/07_TRON/Structs/ST_TRON_SplinePresetPoint` _array_element)) "Local" false)
    (`SplineComponent.SetSplinePointType` _spline_tronpath _array_index "CurveCustomTangent" false))
  (`SplineComponent.UpdateSpline` _spline_tronpath)
  (`self.BuildSplineBeam`)
  (`self.UpdateBeamGrowth` 1.0)
  (`self.UpdateSideCameras` 1.0))

(event `ApplyPresetPointsToSpline`
  (bind _spline_tronpath (`self.Spline_TRONPath`))
  (`SplineComponent.ClearSplinePoints` _spline_tronpath false)
  (for (_array_element _array_index) (`self.PresetSplinePoints`)
    (`SplineComponent.AddSplinePoint` _spline_tronpath (break `/Game/Birra_New/07_TRON/Structs/ST_TRON_SplinePresetPoint` _array_element) "Local" false)
    (`SplineComponent.SetRotationAtSplinePoint` _spline_tronpath _array_index (`.Rotation_14_DF272F8B4C8CD41ED61DE4802E617461` (break `/Game/Birra_New/07_TRON/Structs/ST_TRON_SplinePresetPoint` _array_element)) "Local" false)
    (`SplineComponent.SetTangentsAtSplinePoint` _spline_tronpath _array_index (`.ArriveTangent_13_0FF84F604B63C3C2AC1CFDA46B66AE79` (break `/Game/Birra_New/07_TRON/Structs/ST_TRON_SplinePresetPoint` _array_element)) (`.LeaveTangent_12_9312CFD24D49C211DC35988E5170EA18` (break `/Game/Birra_New/07_TRON/Structs/ST_TRON_SplinePresetPoint` _array_element)) "Local" false)
    (`SplineComponent.SetSplinePointType` _spline_tronpath _array_index "Curve" false))
  (`SplineComponent.UpdateSpline` _spline_tronpath))

(fn `BuildSplineBeam`
  (`self.ClearSplineMeshes`)
  (bind _output_get (set `self.SplineLength` (`SplineComponent.GetSplineLength` (`self.Spline_TRONPath`))))
  (bind _output_get_2 (set `self.SegmentCount` (`KismetMathLibrary.FCeil` (/ _output_get (`KismetMathLibrary.FMax` (`self.SegmentLength`) 1.0)))))
  (for _ (range _output_get_2)
    (bind _returnvalue (`AddComponent|NODE_AddSplineMeshComponent-0` :`bManualAttachment` true))
    (`StaticMeshComponent.SetStaticMesh` _returnvalue (`self.BeamMesh`))
    (`PrimitiveComponent.SetMaterial` _returnvalue 0 (`self.BeamMaterial`))
    (`SplineMeshComponent.SetForwardAxis` _returnvalue "Y" true)
    (`SceneComponent.SetMobility` _returnvalue "Movable")
    (`SceneComponent.SetVisibility` _returnvalue false false)
    (`KismetArrayLibrary.Array_Add` (`self.SplineMeshComponents`) _returnvalue)))

(fn `ClearSplineMeshes`
  (bind _splinemeshcomponents (`self.SplineMeshComponents`))
  (for _array_element _splinemeshcomponents
    (`/Engine/EditorBlueprintResources/StandardMacros.IsValid` _array_element
      (:`Is Valid`
        (`ActorComponent.K2_DestroyComponent` _array_element)
        (`KismetArrayLibrary.Array_Clear` _splinemeshcomponents)))))

(fn `UpdateBeamGrowth`
  (params (Progress :type "Float (double-precision)"))
  (locals (ClampedProgress :type "Float (double-precision)") (CurrentDistance :type "Float (double-precision)") (SegmentStartDistance :type "Float (double-precision)") (SegmentEndDistance :type "Float (double-precision)") (RealSegmentEndDistance :type "Float (double-precision)") (VisibleEndDistance :type "Float (double-precision)") (CurrentSegmentLength :type "Float (double-precision)") (StartLocation :type "Vector Structure") (EndLocation :type "Vector Structure") (StartDirection :type "Vector Structure") (EndDirection :type "Vector Structure") (StartTangent :type "Vector Structure") (EndTangent :type "Vector Structure") (CurrentSplineMesh :type "SplineMeshComponent Object Reference"))
  (bind _segmentlength (`self.SegmentLength`))
  (bind _currentdistance (`local.CurrentDistance`))
  (bind _realsegmentenddistance (`local.RealSegmentEndDistance`))
  (bind _spline_tronpath (`self.Spline_TRONPath`))
  (bind _segmentstartdistance (`local.SegmentStartDistance`))
  (bind _visibleenddistance (`local.VisibleEndDistance`))
  (bind _tangentstrength (`self.TangentStrength`))
  (bind _currentsplinemesh (`local.CurrentSplineMesh`))
  (bind _returnvalue (`KismetMathLibrary.MakeVector2D` (`self.BeamWidth`) (`self.BeamThickness`)))
  (bind _output_get (set `local.ClampedProgress` (`KismetMathLibrary.FClamp` Progress)))
  (set `self.BeamProgress` _output_get)
  (set `local.CurrentDistance` (* _output_get (`self.SplineLength`)))
  (for _index (range (`self.SegmentCount`))
    (bind _output_get_2 (set `local.CurrentSplineMesh` (`|GetArrayItem` (`self.SplineMeshComponents`) _index)))
    (`/Engine/EditorBlueprintResources/StandardMacros.IsValid` _output_get_2
      (:`Is Valid`
        (bind _output_get_3 (set `local.SegmentStartDistance` (* _index _segmentlength)))
        (bind _output_get_4 (set `local.SegmentEndDistance` (+ _output_get_3 _segmentlength)))
        (set `local.RealSegmentEndDistance` (`KismetMathLibrary.FClamp` _output_get_4 0.0 (`self.SplineLength`)))
        (if (<= (`local.CurrentDistance`) (`local.SegmentStartDistance`))
          (`SceneComponent.SetVisibility` (`local.CurrentSplineMesh`) false false)
          (else
            (if (>= _currentdistance _realsegmentenddistance)
              (set `local.VisibleEndDistance` _realsegmentenddistance)
              (else
                (set `local.VisibleEndDistance` _currentdistance)))
            (bind _output_get_5 (set `local.StartLocation` (`SplineComponent.GetLocationAtDistanceAlongSpline` _spline_tronpath _segmentstartdistance "Local")))
            (bind _output_get_6 (set `local.EndLocation` (`SplineComponent.GetLocationAtDistanceAlongSpline` _spline_tronpath _visibleenddistance "Local")))
            (bind _output_get_7 (set `local.StartDirection` (`SplineComponent.GetDirectionAtDistanceAlongSpline` _spline_tronpath _segmentstartdistance "Local")))
            (bind _output_get_8 (set `local.EndDirection` (`SplineComponent.GetDirectionAtDistanceAlongSpline` _spline_tronpath _visibleenddistance "Local")))
            (bind _output_get_9 (set `local.CurrentSegmentLength` (- (`local.VisibleEndDistance`) (`local.SegmentStartDistance`))))
            (bind _output_get_10 (set `local.StartTangent` (* (* _output_get_7 _output_get_9) _tangentstrength)))
            (bind _output_get_11 (set `local.EndTangent` (* (* _output_get_8 _output_get_9) _tangentstrength)))
            (`SplineMeshComponent.SetStartAndEnd` _currentsplinemesh _output_get_5 _output_get_10 _output_get_6 _output_get_11 true)
            (`SplineMeshComponent.SetStartScale` _currentsplinemesh _returnvalue true)
            (`SplineMeshComponent.SetEndScale` _currentsplinemesh _returnvalue true)
            (`SceneComponent.SetVisibility` _currentsplinemesh true false)))))))

(fn `UpdateSideCameras`
  (params (Progress :type "Float (double-precision)"))
  (locals (CameraDistance :type "Float (double-precision)") (BaseLocation :type "Vector Structure" :default (0.0 0.0 0.0)) (RightVector :type "Vector Structure" :default (0.0 0.0 0.0)) (UpVector :type "Vector Structure" :default (0.0 0.0 0.0)) (LeftCameraLocation :type "Vector Structure") (`Right Camera Location` :type "Vector Structure") (LookDistance :type "Float (double-precision)" :default 0.0) (LookTarget :type "Vector Structure" :default (0.0 0.0 0.0)) (SideOffset :type "Vector Structure") (HeightOffset :type "Vector Structure"))
  (bind _spline_tronpath (`self.Spline_TRONPath`))
  (bind _baselocation (`local.BaseLocation`))
  (bind _output_get (set `self.SplineLength` (`SplineComponent.GetSplineLength` _spline_tronpath)))
  (bind _output_get_2 (set `local.CameraDistance` (* _output_get (`KismetMathLibrary.FClamp` Progress))))
  (set `local.BaseLocation` (`SplineComponent.GetLocationAtDistanceAlongSpline` _spline_tronpath _output_get_2 "World"))
  (set `local.RightVector` (`SplineComponent.GetRightVectorAtDistanceAlongSpline` _spline_tronpath _output_get_2 "World"))
  (set `local.UpVector` (`SplineComponent.GetUpVectorAtDistanceAlongSpline` _spline_tronpath _output_get_2 "World"))
  (bind _output_get_3 (set `local.SideOffset` (* (`local.RightVector`) (`self.CameraSideOffset`))))
  (bind _output_get_4 (set `local.HeightOffset` (* (`local.UpVector`) (`self.CameraHeightOffset`))))
  (bind _output_get_5 (set `local.LeftCameraLocation` (+ (- _baselocation _output_get_3) _output_get_4)))
  (`SceneComponent.K2_SetWorldLocation` (`self.Camera Left`) _output_get_5 false false)
  (bind _output_get_6 (set `local.Right Camera Location` (+ (+ _baselocation _output_get_3) _output_get_4)))
  (`SceneComponent.K2_SetWorldLocation` (`self.Camera Right`) _output_get_6 false false)
  (bind _output_get_7 (set `local.LookDistance` (`KismetMathLibrary.FClamp` (+ (`local.CameraDistance`) (`self.CameraLookAheadDistance`)) 0.0 (`self.SplineLength`))))
  (bind _output_get_8 (set `local.LookTarget` (`SplineComponent.GetLocationAtDistanceAlongSpline` (`self.Spline_TRONPath`) _output_get_7 "World")))
  (`SceneComponent.K2_SetWorldRotation` (`self.Camera Left`) (`KismetMathLibrary.FindLookAtRotation` (`local.LeftCameraLocation`) _output_get_8) false false)
  (`SceneComponent.K2_SetWorldRotation` (`self.Camera Right`) (`KismetMathLibrary.FindLookAtRotation` (`local.Right Camera Location`) _output_get_8) false false))

(fn `UserConstructionScript`
  (bind _previewprogress (`self.PreviewProgress`))
  (if (`self.bEditorPreviewBeam`)
    (`self.BuildSplineBeam`)
    (if (`self.bPreviewFullBeam`)
      (`self.UpdateBeamGrowth` 1.0)
      (`self.UpdateSideCameras` 0.0)
      (else
        (`self.UpdateBeamGrowth` _previewprogress)
        (`self.UpdateSideCameras` _previewprogress)))))