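; BP_TRON_TestRig is a test actor for firing a configurable beam between its CubeStart and CubeEnd components.
; It spawns BeamClass at the start point and initializes it with both endpoints, TestBeamConfig and the impact-beam flag.
; Optional number-key input respawns a normal or impact beam, or force-kills the current one; respawning stops the old beam, then waits briefly.
; A separate flag auto-fires a beam on BeginPlay.
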(event `RespawnBeam`
  (`self.StopCurrentBeam`)
  (`KismetSystemLibrary.Delay` 0.05)
  (`self.SpawnTestBeam`))

(event `self.ReceiveBeginPlay`
  (`|ExecutionSequence`
    (:`then_0`
      (if (`self.bAutoFireOnBeginPlay`)
        (`self.SpawnTestBeam`)))
    (:`then_1`
      (if (`self.bEnableKeyboardTest`)
        (`self.EnableInput` (`GameplayStatics.GetPlayerController` 0))))))

(event `Key|One`
  (params (Key :type "Key Structure"))
  (:`Pressed`
    (set `self.bTestAsImpactBeam` false)
    (`self.RespawnBeam`)))

(event `Key|Two`
  (params (Key :type "Key Structure"))
  (:`Pressed`
    (`self.StopCurrentBeam`)))

(event `Key|Three`
  (params (Key :type "Key Structure"))
  (:`Pressed`
    (set `self.bTestAsImpactBeam` false)
    (`self.RespawnBeam`)))

(event `Key|Four`
  (params (Key :type "Key Structure"))
  (:`Pressed`
    (set `self.bTestAsImpactBeam` true)
    (`self.RespawnBeam`)))

(fn `GetEndPoint`
  (returns (EndPoint :type "Vector Structure"))
  (return (`SceneComponent.K2_GetComponentLocation` (`self.Cube_End`))))

(fn `GetStartPoint`
  (returns (StartPoint :type "Vector Structure"))
  (return (`SceneComponent.K2_GetComponentLocation` (`self.Cube_Start`))))

(fn `SpawnTestBeam`
  (bind _startpoint (`self.GetStartPoint`))
  (bind _endpoint (`self.GetEndPoint`))
  (bind _returnvalue (`|SpawnActorFromClass` (`self.BeamClass`) (`KismetMathLibrary.MakeTransform` _startpoint) "Undefined" "MultiplyWithRoot" null null))
  (bind _output_get (set `self.CurrentBeamRef` _returnvalue))
  (`/Game/Birra_New/07_TRON/BP/BP_TRON_Beam.InitializeBeamFromConfig` _output_get _startpoint _endpoint (`self.TestBeamConfig`) (`self.bTestAsImpactBeam`)))

(fn `StopCurrentBeam`
  (bind _currentbeamref (`self.CurrentBeamRef`))
  (`/Engine/EditorBlueprintResources/StandardMacros.IsValid` _currentbeamref
    (:`Is Valid`
      (`/Game/Birra_New/07_TRON/BP/BP_TRON_Beam.ForceKillBeam` _currentbeamref)
      (set `self.CurrentBeamRef` null))))

(fn `UserConstructionScript`)