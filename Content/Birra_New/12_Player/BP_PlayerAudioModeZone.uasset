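; Box trigger zone that switches the player's movement audio mode (normal, tension, panic, recovery, muted) when a Character enters or leaves.
; Overlaps find the character's AC_PlayerMovementAudio_Metal and apply the enter or exit mode, with optional timing and an entry gasp.
; Entry applies only when TriggerOnce and AlreadyTriggered are both already true, so the once-only check looks inverted.
; FireAudioEvent offers one-shot audio actions but is not called here.
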(event `self.Box.OnComponentBeginOverlap`
  (params (OverlappedComponent :type "PrimitiveComponent Object Reference") (OtherActor :type "Actor Object Reference") (OtherComp :type "PrimitiveComponent Object Reference") (OtherBodyIndex :type Integer) (bFromSweep :type Boolean) (SweepResult :type "HitResult Structure (by ref)"))
  (if (== (`self.bAffectOnBeginOverlap`) false)
    _
    (elif (and (== (`self.bTriggerOnce`) true) (== (`self.bAlreadyTriggered`) true))
      (bind _ascharacter (cast `Character` OtherActor))
      (bind _movementaudio (`self.GetPlayerMovementAudioComponent` _ascharacter))
      (`/Engine/EditorBlueprintResources/StandardMacros.IsValid` _movementaudio
        (:`Is Valid`
          (`KismetSystemLibrary.PrintString` (`KismetStringLibrary.Concat_StrStr` "ZONE ENTER | PlayerSpeedXY=" (`KismetStringLibrary.Conv_VectorToString` (`self.GetVelocity` OtherActor))))
          (`self.ApplyModeOnEnter` _movementaudio)
          (set `self.bAlreadyTriggered` true))
        (:`Is Not Valid`
          (`KismetSystemLibrary.PrintString` "bati aqui"))))))

(event `self.Box.OnComponentEndOverlap`
  (params (OverlappedComponent :type "PrimitiveComponent Object Reference") (OtherActor :type "Actor Object Reference") (OtherComp :type "PrimitiveComponent Object Reference") (OtherBodyIndex :type Integer))
  (if (not (== (`self.bAffectOnEndOverlap`) false))
    (bind _ascharacter (cast `Character` OtherActor))
    (bind _movementaudio (`self.GetPlayerMovementAudioComponent` _ascharacter))
    (`/Engine/EditorBlueprintResources/StandardMacros.IsValid` _movementaudio
      (:`Is Valid`
        (`self.ApplyModeOnExit` _movementaudio)))))

(fn `ApplyModeOnEnter`
  (params (MovementAudioComponent :type "/Game/Birra_New/12_Player/AC_PlayerMovementAudio_Metal Object Reference"))
  (bind _modeduration (`self.ModeDuration`))
  (bind _returnvalue (== (`self.bUseDuration`) true))
  (`/Engine/EditorBlueprintResources/StandardMacros.IsValid` MovementAudioComponent
    (:`Is Valid`
      (`|ExecutionSequence`
        (:`then_0`
          (if (== (`self.bDebug`) true)
            (`KismetSystemLibrary.PrintString` "BP_PlayerAudioModeZone: Apply Mode On Enter")))
        (:`then_1`
          (switch `/Game/Birra_New/12_Player/E_PlayerAudioMode` (`self.ModeOnEnter`)
            (:`NewEnumerator0`
              (`/Game/Birra_New/12_Player/AC_PlayerMovementAudio_Metal.SetAudioMode` MovementAudioComponent "NewEnumerator0"))
            (:`NewEnumerator1`
              (`/Game/Birra_New/12_Player/AC_PlayerMovementAudio_Metal.SetAudioMode` MovementAudioComponent "NewEnumerator1"))
            (:`NewEnumerator2`
              (if _returnvalue
                (`/Game/Birra_New/12_Player/AC_PlayerMovementAudio_Metal.SetPanicModeForDuration` MovementAudioComponent _modeduration)
                (else
                  (`/Game/Birra_New/12_Player/AC_PlayerMovementAudio_Metal.SetAudioMode` MovementAudioComponent "NewEnumerator2"))))
            (:`NewEnumerator3`
              (if _returnvalue
                (`/Game/Birra_New/12_Player/AC_PlayerMovementAudio_Metal.SetRecoveryMode` MovementAudioComponent _modeduration)
                (else
                  (`/Game/Birra_New/12_Player/AC_PlayerMovementAudio_Metal.SetAudioMode` MovementAudioComponent "NewEnumerator3"))))
            (:`NewEnumerator4`
              (`/Game/Birra_New/12_Player/AC_PlayerMovementAudio_Metal.SetAudioMode` MovementAudioComponent "NewEnumerator4")))
          (if (== (`self.bPlayGaspOnEnter`) true)
            (`/Game/Birra_New/12_Player/AC_PlayerMovementAudio_Metal.PlayPanicGasp` MovementAudioComponent)))))
    (:`Is Not Valid`
      (return))))

(fn `ApplyModeOnExit`
  (params (MovementAudioComponent :type "/Game/Birra_New/12_Player/AC_PlayerMovementAudio_Metal Object Reference"))
  (bind _returnvalue (== (`self.bUseDuration`) true))
  (`/Engine/EditorBlueprintResources/StandardMacros.IsValid` MovementAudioComponent
    (:`Is Valid`
      (`|ExecutionSequence`
        (:`then_0`
          (if (== (`self.bDebug`) true)
            (`KismetSystemLibrary.PrintString` "BP_PlayerAudioModeZone: Apply Mode On Exit")))
        (:`then_1`
          (switch `/Game/Birra_New/12_Player/E_PlayerAudioMode` (`self.ModeOnExit`)
            (:`NewEnumerator0`
              (`/Game/Birra_New/12_Player/AC_PlayerMovementAudio_Metal.ResetPlayerAudioToNormal` MovementAudioComponent))
            (:`NewEnumerator1`
              (`/Game/Birra_New/12_Player/AC_PlayerMovementAudio_Metal.SetAudioMode` MovementAudioComponent "NewEnumerator1"))
            (:`NewEnumerator2`
              (if _returnvalue
                (`/Game/Birra_New/12_Player/AC_PlayerMovementAudio_Metal.SetPanicMode` MovementAudioComponent true)
                (else
                  (`/Game/Birra_New/12_Player/AC_PlayerMovementAudio_Metal.SetAudioMode` MovementAudioComponent "NewEnumerator2"))))
            (:`NewEnumerator3`
              (if _returnvalue
                (`/Game/Birra_New/12_Player/AC_PlayerMovementAudio_Metal.SetRecoveryMode` MovementAudioComponent (`self.ModeDuration`))
                (else
                  (`/Game/Birra_New/12_Player/AC_PlayerMovementAudio_Metal.SetAudioMode` MovementAudioComponent "NewEnumerator3"))))
            (:`NewEnumerator4`
              (`/Game/Birra_New/12_Player/AC_PlayerMovementAudio_Metal.SetAudioMode` MovementAudioComponent "NewEnumerator4"))))))
    (:`Is Not Valid`
      (return))))

(fn `FireAudioEvent`
  (params (MovementAudioComponent :type "/Game/Birra_New/12_Player/AC_PlayerMovementAudio_Metal Object Reference"))
  (bind _audioeventduration (`self.AudioEventDuration`))
  (`/Engine/EditorBlueprintResources/StandardMacros.IsValid` MovementAudioComponent
    (:`Is Valid`
      (`|ExecutionSequence`
        (:`then_0`
          (if (== (`self.bDebug`) true)
            (`KismetSystemLibrary.PrintString` "BP_PlayerAudioEventTrigger: Fire Audio Event")))
        (:`then_1`
          (switch `/Game/Birra_New/12_Player/E_PlayerAudioTriggerEvent` (`self.PlayerAudioTrigger`)
            (:`NewEnumerator0`
              (`/Game/Birra_New/12_Player/AC_PlayerMovementAudio_Metal.SetPanicModeForDuration` MovementAudioComponent _audioeventduration))
            (:`NewEnumerator1`
              (`/Game/Birra_New/12_Player/AC_PlayerMovementAudio_Metal.SetRecoveryMode` MovementAudioComponent _audioeventduration))
            (:`NewEnumerator2`
              (`/Game/Birra_New/12_Player/AC_PlayerMovementAudio_Metal.PlayPanicGasp` MovementAudioComponent))
            (:`NewEnumerator3`
              (`/Game/Birra_New/12_Player/AC_PlayerMovementAudio_Metal.MutePlayerMovementAudioForDuration` MovementAudioComponent _audioeventduration))
            (:`NewEnumerator4`
              (`/Game/Birra_New/12_Player/AC_PlayerMovementAudio_Metal.SetPlayerAudioMasterVolume` MovementAudioComponent (`self.AudioEventVolumeValue`)))
            (:`NewEnumerator5`
              (`/Game/Birra_New/12_Player/AC_PlayerMovementAudio_Metal.ResetPlayerAudioToNormal` MovementAudioComponent))
            (:`NewEnumerator6`
              (`/Game/Birra_New/12_Player/AC_PlayerMovementAudio_Metal.SetAudioMode` MovementAudioComponent "NewEnumerator1"))
            (:`NewEnumerator7`
              (`/Game/Birra_New/12_Player/AC_PlayerMovementAudio_Metal.SetPanicMode` MovementAudioComponent true))))))
    (:`Is Not Valid`
      (return))))

(fn `GetPlayerMovementAudioComponent`
  (params (TargetActor :type "Actor Object Reference"))
  (returns (MovementAudio :type "/Game/Birra_New/12_Player/AC_PlayerMovementAudio_Metal Object Reference"))
  (`/Engine/EditorBlueprintResources/StandardMacros.IsValid` TargetActor
    (:`Is Valid`
      (return (`self.GetComponentByClass` TargetActor "/Game/Birra_New/12_Player/AC_PlayerMovementAudio_Metal.AC_PlayerMovementAudio_Metal_C")))
    (:`Is Not Valid`
      (return null))))

(fn `UserConstructionScript`)