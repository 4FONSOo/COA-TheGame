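; Unfinished player Character component for metal-surface movement audio: footsteps, landings, scrapes, breathing and heartbeat, with panic and recovery modes.
; Tick advances cooldown timers, derives movement state from falling, crouch and horizontal speed, then calls exhaustion, breathing, heartbeat and landing updates.
; Footstep gating currently sits inside the panic and recovery expiry branches.
; Most functions, including mode setters and playback, are empty stubs; unconnected PrintString placeholders mark intended sound nodes.
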(event `self.ReceiveBeginPlay`
  (bind _ownercharacter (`self.OwnerCharacter`))
  (`self.InitOwnerReferences`)
  (`self.ResetRuntimeValues`)
  (`/Engine/EditorBlueprintResources/StandardMacros.IsValid` _ownercharacter
    (:`Is Valid`
      (set `self.LastOwnerLocation` (`Actor.K2_GetActorLocation` _ownercharacter))
      (set `self.TimeSinceLastStep` 999.0)
      (set `self.TimeSinceLastLanding` 999.0)
      (set `self.TimeSinceLastScrape` 999.0)
      (set `self.TimeSinceLastStopStep` 999.0)
      (set `self.TimeSinceLastRecoveryBreath` 999.0)
      (set `self.TimeSinceLastPanicGasp` 999.0)
      (set `self.TimeSinceLastPanicTrigger` 999.0)
      (set `self.CurrentFootIndex` 0)
      (set `self.CurrentAudioMode` "NewEnumerator0")
      (set `self.PreviousAudioMode` "NewEnumerator0")
      (set `self.CurrentMovementState` "NewEnumerator0")
      (set `self.PreviousMovementState` "NewEnumerator0"))))

(event `self.ReceiveTick`
  (params (DeltaSeconds :type "Float (single-precision)"))
  (bind _returnvalue (`Actor.K2_GetActorLocation` (`self.OwnerCharacter`)))
  (`/Engine/EditorBlueprintResources/StandardMacros.IsValid` (`self.OwnerCharacter`)
    (:`Is Valid`
      (set `self.TimeSinceLastStep` (+ DeltaSeconds (`self.TimeSinceLastStep`)))
      (set `self.TimeSinceLastLanding` (+ DeltaSeconds (`self.TimeSinceLastLanding`)))
      (set `self.TimeSinceLastScrape` (+ DeltaSeconds (`self.TimeSinceLastScrape`)))
      (set `self.TimeSinceLastStopStep` (+ DeltaSeconds (`self.TimeSinceLastStopStep`)))
      (set `self.TimeSinceLastRecoveryBreath` (+ DeltaSeconds (`self.TimeSinceLastRecoveryBreath`)))
      (set `self.TimeSinceLastPanicGasp` (+ DeltaSeconds (`self.TimeSinceLastPanicGasp`)))
      (set `self.TimeSinceLastPanicTrigger` (+ DeltaSeconds (`self.TimeSinceLastPanicTrigger`)))
      (set `self.PreviousMovementState` (`self.CurrentMovementState`))
      (`self.UpdateMovementState`)
      (`self.UpdateRunExhaustion`)
      (`self.UpdateBreathingState`)
      (`self.UpdateBreathingVolume`)
      (`self.UpdateHeartbeatTarget`)
      (`self.HandleLandingDetection`)
      (if (== (`self.bPanicHasDuration`) true)
        (bind _output_get (set `self.PanicRemainingTime` (- (`self.PanicRemainingTime`) DeltaSeconds)))
        (if (<= _output_get 0.0)
          (set `self.bPanicHasDuration` true)
          (`self.SetRecoveryMode`)
          (if (== (`self.bRecoveryHasDuration`) true)
            (bind _output_get_2 (set `self.RecoveryRemainingTime` (- (`self.RecoveryRemainingTime`) DeltaSeconds)))
            (if (<= _output_get_2 0.0)
              (set `self.bRecoveryHasDuration` false)
              (`self.ResetPlayerAudioToNormal`)
              (if (== (`self.bPlayerMovementAudioEnabled`) false)
                (set `self.LastOwnerLocation` _returnvalue)
                (else
                  ; Verificar O node no false
                  (if (`|EnumEquality` (`self.CurrentAudioMode`) "NewEnumerator4")
                    (bind _output_get_3 (set `self.LastOwnerLocation` _returnvalue))
                    (else
                      (bind _shouldprocess (`self.ShouldProcessFootsteps`))
                      (if _shouldprocess
                        (set `self.LastOwnerLocation` _output_get_3)
                        (else
                          (`self.AccumulateFootstepDistance`)
                          (set `self.LastOwnerLocation` _output_get_3)
                          (`self.GetHorizontalSpeed`)
                          (set `self.PreviousHorizontalSpeed` 0.0))))))))))))))

(event `self.ReceiveEndPlay`
  (params (EndPlayReason :type "EEndPlayReason Enum" :default "Destroyed"))
  (`self.StopBreathingLoop`)
  (`self.StopHeartbeat`)
  (`KismetSystemLibrary.K2_ClearAndInvalidateTimerHandle` (`self.HeartbeatTimerHandle`)))

(event `CE_UnmutePlayerMovementAudio`
  (set `self.bPlayerMovementAudioEnabled` true)
  (`self.ResetPlayerAudioToNormal`))

(event `CE_EndPanicDuration`
  (set `self.bPanicHasDuration` false)
  ; defaultRecoveryMode
  (`self.SetRecoveryMode`))

(event `CE_EndRecoveryDuration`
  (set `self.bRecoveryHasDuration` false)
  (`self.ResetPlayerAudioToNormal`))

(event `CE_PlayHeartbeatBeat`
  (`self.PlayHeartbeatBeat`))

(fn `AccumulateFootstepDistance`)

(fn `ApplyAudioModeModifiers`)

(fn `CalculateFootstepPitch`)

(fn `CalculateFootstepVolume`)

(fn `CalculateLandingVolume`)

(fn `DebugAudioMode`)

(fn `DebugFootstep`)

(fn `ForceFootstep`)

(fn `GetCurrentStrideDistance`)

(fn `GetFootstepTraceHit`)

(fn `GetHorizontalSpeed`
  (returns (HorizontalSpeed :type "Float (double-precision)"))
  (return (`KismetMathLibrary.VSize` (`KismetMathLibrary.MakeVector` (.x (`Actor.GetVelocity` (`self.OwnerCharacter`))) (.y (`Actor.GetVelocity` (`self.OwnerCharacter`)))))))

(fn `GetRandomSoundFromArrayNoRepeat`)

(fn `GetRunExhaustionAlpha`)

(fn `HandleLandingDetection`)

(fn `InitOwnerReferences`
  (bind _output_get (set `self.OwnerActor` (`self.GetOwner`)))
  (bind _ascharacter (cast `Character` _output_get)
    (:`then`
      (bind _output_get_2 (set `self.OwnerCharacter` _ascharacter))
      (set `self.OwnerMovement` (`Character.CharacterMovement` _output_get_2))
      (set `self.OwnerCapsule` (`Character.CapsuleComponent` _output_get_2)))
    (:`CastFailed`
      (`KismetSystemLibrary.PrintString` "AC_PlayerMovementAudio_Metal: Owner is not Character"))))

(fn `MutePlayerMovementAudioForDuration`)

(fn `PlayFootstepSound`)

(fn `PlayHeartbeatBeat`)

(fn `PlayPanicGasp`)

(fn `PlayRecoveryBreath`)

(fn `ResetFootstepAccumulator`)

(fn `ResetPlayerAudioToNormal`)

(fn `ResetRuntimeValues`
  (set `self.AccumulatedDistance` 0.0)
  (set `self.CurrentFootIndex` 0)
  (set `self.bWasMoving` false)
  (set `self.bWasRunning` false)
  (set `self.bIsRunningLongEnough` false)
  (set `self.bWasFalling` false)
  (set `self.PeakFallSpeed` 0.0)
  (set `self.CurrentRunTime` 0.0)
  (set `self.ContinuousRunTime` 0.0)
  (set `self.RunExhaustionAlpha` 0.0)
  (set `self.CurrentBreathingVolume` 0.0)
  (set `self.TargetBreathingVolume` 0.0)
  (set `self.bHeartbeatActive` false)
  (set `self.CurrentHeartbeatInterval` 0.0)
  (set `self.TargetHeartbeatInterval` 0.0)
  (set `self.bPanicHasDuration` false)
  (set `self.PanicRemainingTime` 0.0)
  (set `self.bRecoveryHasDuration` false)
  (set `self.RecoveryRemainingTime` 0.0)
  (set `self.LastWalkSoundIndex` -1)
  (set `self.LastRunSoundIndex` -1)
  (set `self.LastCrouchSoundIndex` -1)
  (set `self.LastLandingSoundIndex` -1)
  (set `self.LastScrapeSoundIndex` -1)
  (set `self.LastStopSoundIndex` -1)
  (set `self.LastRecoveryBreathIndex` -1)
  (set `self.LastPanicGaspIndex` -1)
  (set `self.LastHeartbeatIndex` -1))

(fn `SelectFootstepSound`)

(fn `SetAudioMode`)

(fn `SetPanicMode`)

(fn `SetPanicModeForDuration`)

(fn `SetPlayerAudioMasterVolume`)

(fn `SetPlayerMovementAudioEnabled`)

(fn `SetRecoveryMode`)

(fn `SetTensionMode`)

(fn `ShouldProcessFootsteps`
  (returns (ShouldProcess :type Boolean))
  (if (`|EnumEquality` (`self.CurrentMovementState`) "NewEnumerator0")
    (set `self.AccumulatedDistance` 0.0)
    (if (and (== (`self.bWasMoving`) true) (>= (`self.PreviousHorizontalSpeed`) (`self.StopStepMinPreviousSpeed`)) (>= (`self.TimeSinceLastStopStep`) (`self.StopStepCooldown`)) (== (`self.bUseStopStep`) true))
      (`self.TriggerStopStep`)
      (else
        (set `self.bWasMoving` true)
        (return false)))
    (elif (`|EnumEquality` (`self.CurrentMovementState`) "NewEnumerator4")
      (set `self.AccumulatedDistance` 0.0)
      (set `self.bWasMoving` false)
      (return false)
      (else
        (bind _horizontalspeed (`self.GetHorizontalSpeed`))
        (if (< _horizontalspeed (`self.MinSpeedToStep`))
          (return false)
          (elif (< (`self.TimeSinceLastStep`) (`self.AbsoluteMinStepInterval`))
            (return false)
            (elif (and (== (`self.bUseStartMovingDelay`) false) (== (`self.bWasMoving`) false))
              (bind _output_get (set `self.TimeSinceStartedMoving` (+ (`self.TimeSinceStartedMoving`) (`GameplayStatics.GetWorldDeltaSeconds`))))
              (if (< _output_get (`self.StartMovingDelay`))
                (return false))
              (else
                (set `self.bWasMoving` false)
                (if (< (`self.TimeSinceLastStep`) (`self.MinTimeBetweenSteps`))
                  (return false)
                  (else
                    (return true)))))))))))

(fn `StartBreathingLoop`)

(fn `StartHeartbeat`)

(fn `StopBreathingLoop`)

(fn `StopHeartbeat`)

(fn `ToggleFoot`)

(fn `TriggerFootstep`)

(fn `TriggerFootstepLanding`)

(fn `TriggerScrapeChance`)

(fn `TriggerStopStep`)

(fn `UpdateBreathingState`)

(fn `UpdateBreathingVolume`)

(fn `UpdateHeartbeatTarget`)

(fn `UpdateMovementState`
  (bind _ownermovement (`self.OwnerMovement`))
  (`/Engine/EditorBlueprintResources/StandardMacros.IsValid` _ownermovement
    (:`Is Valid`
      (if (`NavMovementInterface.IsFalling` _ownermovement)
        (set `self.CurrentMovementState` "NewEnumerator4")
        (return)
        (else
          (bind _horizontalspeed (`self.GetHorizontalSpeed`))
          (if (< _horizontalspeed (`self.MinSpeedToStep`))
            (set `self.CurrentMovementState` "NewEnumerator0")
            (return)
            (elif (`Character.bIsCrouched` (`self.OwnerCharacter`))
              (set `self.CurrentMovementState` "NewEnumerator3")
              (return)
              (elif (>= _horizontalspeed (`self.RunSpeedThreshold`))
                (set `self.CurrentMovementState` "NewEnumerator2")
                (return)
                (else
                  (set `self.CurrentMovementState` "NewEnumerator1"))))))))
    (:`Is Not Valid`
      (set `self.CurrentMovementState` "NewEnumerator0")
      (return))))

(fn `UpdateRunExhaustion`)