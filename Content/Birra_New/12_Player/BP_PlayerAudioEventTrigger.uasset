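; Trigger volume that changes the player's movement audio state when BP_Resident_HorrorV1 enters its box.
; On begin overlap it calls the AC_PlayerMovementAudio_Metal action chosen by EventToFire, such as panic, recovery, tension, gasp, mute, volume or reset.
; TriggerOnce limits it to a single firing.
; With CleanOverlap set, leaving the box stops breathing and heartbeat, resets audio to normal and clears footstep tracking.
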(event `self.Box.OnComponentBeginOverlap`
  (params (OverlappedComponent :type "PrimitiveComponent Object Reference") (OtherActor :type "Actor Object Reference") (OtherComp :type "PrimitiveComponent Object Reference") (OtherBodyIndex :type Integer) (bFromSweep :type Boolean) (SweepResult :type "HitResult Structure (by ref)"))
  (bind _duration (`self.Duration`))
  (bind _asbp_resident_horror_v1 (cast `/Game/ChildrenOfAndromeda/Character/BP_Character/BP_Resident_HorrorV1` OtherActor))
  (if (not (and (== (`self.bTriggerOnce`) true) (== (`self.bAlreadyTriggered`) true)))
    (bind _returnvalue (`self.GetComponentByClass` _asbp_resident_horror_v1 "/Game/Birra_New/12_Player/AC_PlayerMovementAudio_Metal.AC_PlayerMovementAudio_Metal_C"))
    (`/Engine/EditorBlueprintResources/StandardMacros.IsValid` _returnvalue
      (:`Is Valid`
        (switch `/Game/Birra_New/12_Player/E_PlayerAudioTriggerEvent` (`self.EventToFire`)
          (:`NewEnumerator0`
            (`/Game/Birra_New/12_Player/AC_PlayerMovementAudio_Metal.SetPanicModeForDuration` _returnvalue _duration))
          (:`NewEnumerator1`
            (`/Game/Birra_New/12_Player/AC_PlayerMovementAudio_Metal.SetRecoveryMode` _returnvalue _duration))
          (:`NewEnumerator2`
            (`/Game/Birra_New/12_Player/AC_PlayerMovementAudio_Metal.PlayPanicGasp` _returnvalue))
          (:`NewEnumerator3`
            (`/Game/Birra_New/12_Player/AC_PlayerMovementAudio_Metal.MutePlayerMovementAudioForDuration` _returnvalue _duration))
          (:`NewEnumerator4`
            (`/Game/Birra_New/12_Player/AC_PlayerMovementAudio_Metal.SetPlayerAudioMasterVolume` _returnvalue (`self.VolumeValue`)))
          (:`NewEnumerator5`
            (`/Game/Birra_New/12_Player/AC_PlayerMovementAudio_Metal.ResetPlayerAudioToNormal` _returnvalue))
          (:`NewEnumerator6`
            (`/Game/Birra_New/12_Player/AC_PlayerMovementAudio_Metal.SetTensionMode` _returnvalue true))
          (:`NewEnumerator7`
            (`/Game/Birra_New/12_Player/AC_PlayerMovementAudio_Metal.SetPanicMode` _returnvalue true)))
        (set `self.bAlreadyTriggered` true)))))

(event `self.Box.OnComponentEndOverlap`
  (params (OverlappedComponent :type "PrimitiveComponent Object Reference") (OtherActor :type "Actor Object Reference") (OtherComp :type "PrimitiveComponent Object Reference") (OtherBodyIndex :type Integer))
  (bind _asbp_resident_horror_v1 (cast `/Game/ChildrenOfAndromeda/Character/BP_Character/BP_Resident_HorrorV1` OtherActor))
  (if (`self.bCleanOverlap`)
    (bind _returnvalue (`self.GetComponentByClass` _asbp_resident_horror_v1 "/Game/Birra_New/12_Player/AC_PlayerMovementAudio_Metal.AC_PlayerMovementAudio_Metal_C"))
    (`/Engine/EditorBlueprintResources/StandardMacros.IsValid` _returnvalue
      (:`Is Valid`
        (`/Game/Birra_New/12_Player/AC_PlayerMovementAudio_Metal.StopBreathingLoop` _returnvalue)
        (`/Game/Birra_New/12_Player/AC_PlayerMovementAudio_Metal.StopHeartbeat` _returnvalue)
        (`/Game/Birra_New/12_Player/AC_PlayerMovementAudio_Metal.ResetPlayerAudioToNormal` _returnvalue)
        (set `/Game/Birra_New/12_Player/AC_PlayerMovementAudio_Metal.AccumulatedDistance` 0.0 _returnvalue)
        (set `/Game/Birra_New/12_Player/AC_PlayerMovementAudio_Metal.TimeSinceLastStep` 0.0 _returnvalue)
        (set `/Game/Birra_New/12_Player/AC_PlayerMovementAudio_Metal.bWasMoving` false _returnvalue)))))

(fn `UserConstructionScript`)