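; Base light unit Blueprint that drives a lamp mesh's emissive material and its light component through states like Off, Normal, Emergency, Alarm, Flicker and Broken.
; BeginPlay creates a dynamic material, caches the light component and sets Off emissive.
; On/off commands and pump multipliers feed ApplyLightOutput, with broken units optionally ignoring commands.
; TurnOn sets Normal but applies Off intensity and emissive values, unlike ReapplyCurrentState, which uses per-state values.
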(event `/Game/Birra_New/Managers/Lights/4_Interfaces/BPI_LightControllable.Light_TurnOn`
  (`self.TurnOn`))

(event `/Game/Birra_New/Managers/Lights/4_Interfaces/BPI_LightControllable.Light_TurnOff`
  (`self.TurnOff`))

(event `self.ReceiveBeginPlay`
  (`self.CreateLampDynamicMaterial`)
  (`self.CacheActiveLightComponent`)
  (`self.ApplyStartupMaterialState`))

(fn `ApplyLightOutput`
  (params (InColor :type "LinearColor Structure") (InIntensity :type "Float (double-precision)") (InEmissiveStrength :type "Float (double-precision)") (bEnableLight :type Boolean))
  (bind _activelightcomponent (`self.ActiveLightComponent`))
  (`/Engine/EditorBlueprintResources/StandardMacros.IsValid` _activelightcomponent
    (:`Is Valid`
      (`SceneComponent.SetVisibility` _activelightcomponent bEnableLight false)
      (`LightComponent.SetIntensity` _activelightcomponent (* InIntensity (`self.IntensityMultiplier`)))
      (`LightComponent.SetLightColor` _activelightcomponent InColor true)
      (`self.SetLampEmissive` InColor (* InEmissiveStrength (`self.EmissiveMultiplier`))))
    (:`Is Not Valid`
      (`self.SetLampEmissive` InColor InEmissiveStrength))))

(fn `ApplyStartupMaterialState`
  (bind _normalcolor (`self.NormalColor`))
  (bind _emissivenormalstrength (`self.EmissiveNormalStrength`))
  (set `self.CurrentState` "NewEnumerator0")
  (set `self.PreviousState` "NewEnumerator0")
  (switch `/Game/Birra_New/Managers/Lights/5_Enums/E_LightState` "NewEnumerator0"
    (:`NewEnumerator0`
      (set `self.bIsBroken` false)
      (`self.SetLampEmissive` _normalcolor (`self.EmissiveOffStrength`)))
    (:`NewEnumerator1`
      (set `self.bIsBroken` false)
      (`self.SetLampEmissive` _normalcolor _emissivenormalstrength))
    (:`NewEnumerator2`
      (set `self.bIsBroken` false)
      (`self.SetLampEmissive` (`self.EmergencyColor`) (`self.EmissiveEmergencyStrength`)))
    (:`NewEnumerator3`
      (set `self.bIsBroken` false)
      (`self.SetLampEmissive` (`self.AlarmColor`) (`self.EmissiveAlarmStrength`)))
    (:`NewEnumerator4`
      (set `self.bIsBroken` false)
      (`self.SetLampEmissive` _normalcolor _emissivenormalstrength))
    (:`NewEnumerator5`
      (set `self.bIsBroken` true)
      (`self.SetLampEmissive` (`self.BrokenColor`) (`self.EmissiveBrokenStrength`)))))

(fn `CacheActiveLightComponent`
  (bind _returnvalue (`self.GetComponentByClass` "/Script/Engine.LightComponent"))
  (`/Engine/EditorBlueprintResources/StandardMacros.IsValid` _returnvalue
    (:`Is Valid`
      (bind _aslight_component (cast `LightComponent` _returnvalue))
      (set `self.ActiveLightComponent` _aslight_component))))

(fn `ClearPumpState`
  (set `self.IntensityMultiplier` 1.0)
  (set `self.EmissiveMultiplier` 1.0)
  (set `self.bIsPumped` false)
  (`self.ReapplyCurrentState`))

(fn `CreateLampDynamicMaterial`
  (bind _staticmesh_lamp (`self.StaticMesh_Lamp`))
  (bind _returnvalue (`PrimitiveComponent.CreateDynamicMaterialInstance` _staticmesh_lamp 0 "/Game/Birra_New/Managers/Lights/6_Materiais/M_Lamp_Emissive.M_Lamp_Emissive" "None"))
  (bind _output_get (set `self.DynamicMaterialRef` _returnvalue))
  (`PrimitiveComponent.SetMaterial` _staticmesh_lamp 0 _output_get))

(fn `ReapplyCurrentState`
  (bind _normalcolor (`self.NormalColor`))
  (switch `/Game/Birra_New/Managers/Lights/5_Enums/E_LightState` (`self.CurrentState`)
    (:`NewEnumerator0`
      (`self.ApplyLightOutput` _normalcolor (`self.OffIntensity`) (`self.EmissiveOffStrength`) :!label _label))
    (:`NewEnumerator1`
      (`self.ApplyLightOutput` _normalcolor (`self.NormalIntensity`) (`self.EmissiveNormalStrength`) true :!label _label_2))
    (:`NewEnumerator2`
      (`self.ApplyLightOutput` (`self.EmergencyColor`) (`self.EmergencyIntensity`) (`self.EmissiveEmergencyStrength`) true :!label _label_3))
    (:`NewEnumerator3`
      (`self.ApplyLightOutput` (`self.AlarmColor`) (`self.AlarmIntensity`) (`self.EmissiveAlarmStrength`) true :!label _label_4))
    (:`NewEnumerator4`
      (switch `/Game/Birra_New/Managers/Lights/5_Enums/E_LightState` (`self.PreviousState`)
        (:`NewEnumerator0`
          (goto _label))
        (:`NewEnumerator1`
          (goto _label_2))
        (:`NewEnumerator2`
          (goto _label_3))
        (:`NewEnumerator3`
          (goto _label_4))
        (:`NewEnumerator4`
          (`self.ApplyLightOutput` (`self.NormalColor`) (`self.NormalIntensity`) (`self.EmissiveNormalStrength`) true))
        (:`NewEnumerator5`
          (`self.ApplyLightOutput` (`self.BrokenColor`) (`self.BrokenIntensity`) (`self.EmissiveBrokenStrength`)))))
    (:`NewEnumerator5`
      (`self.ApplyLightOutput` (`self.BrokenColor`) (`self.BrokenIntensity`) (`self.EmissiveBrokenStrength`)))))

(fn `SetLampEmissive`
  (params (InColor :type "LinearColor Structure") (InStrength :type "Float (double-precision)"))
  (bind _dynamicmaterialref (`self.DynamicMaterialRef`))
  (`/Engine/EditorBlueprintResources/StandardMacros.IsValid` _dynamicmaterialref
    (:`Is Valid`
      (`MaterialInstanceDynamic.SetVectorParameterValue` _dynamicmaterialref "EmissiveColor" InColor)
      (`MaterialInstanceDynamic.SetScalarParameterValue` _dynamicmaterialref "EmissiveStrength" InStrength))))

(fn `SetPumpState`
  (params (NewIntensityMultiplier :type "Float (double-precision)" :default 2.0) (NewEmissiveMultiplier :type "Float (double-precision)" :default 1.5))
  (if (not (and (`self.bIsBroken`) (`self.bIgnoreCommandsWhenBroken`)))
    (set `self.IntensityMultiplier` NewIntensityMultiplier)
    (set `self.EmissiveMultiplier` NewEmissiveMultiplier)
    (set `self.bIsPumped` false)
    (`self.ReapplyCurrentState`)))

(fn `TurnOff`
  (if (not (and (`self.bIsBroken`) (`self.bIgnoreCommandsWhenBroken`)))
    (set `self.PreviousState` (`self.CurrentState`))
    (set `self.CurrentState` "NewEnumerator0")
    (`self.ApplyLightOutput` (`self.NormalColor`) (`self.OffIntensity`) (`self.EmissiveOffStrength`))))

(fn `TurnOn`
  (if (not (and (`self.bIsBroken`) (`self.bIgnoreCommandsWhenBroken`)))
    (set `self.PreviousState` (`self.CurrentState`))
    (set `self.CurrentState` "NewEnumerator1")
    (`self.ApplyLightOutput` (`self.NormalColor`) (`self.OffIntensity`) (`self.EmissiveOffStrength`) true)))

(fn `UserConstructionScript`)