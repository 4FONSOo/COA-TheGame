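; Level controller that runs global light actions on all BP_LightUnit_Base actors via start/end trigger boxes, with random obscure sounds.
; Actions apply at once or through a shuffled, randomly timed queue.
; Optional number-key test sequences add timed auto-revert, but the buffer clears before matching.
; Only TurnOnAll is wired among the all-light functions; off, pump, de-pump, flicker and deflicker are empty, though per-light pump works.
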(event `self.ReceiveBeginPlay`
  (if (`self.bEnableManualTestInput`)
    (`self.EnableInput` (`GameplayStatics.GetPlayerController` 0))
    (`self.RefreshAllLights`)
    (else
      (`self.RefreshAllLights`))))

(event `Key|One`
  (params (Key :type "Key Structure"))
  (:`Pressed`
    (`self.RegisterManualKey` "\"1\"")))

(event `Key|Four`
  (params (Key :type "Key Structure"))
  (:`Pressed`
    (`self.RegisterManualKey` "\"4\"")))

(event `Key|Seven`
  (params (Key :type "Key Structure"))
  (:`Pressed`
    (`self.RegisterManualKey` "\"7\"")))

(event `Key|Two`
  (params (Key :type "Key Structure"))
  (:`Pressed`
    (`self.RegisterManualKey` "\"2\"")))

(event `Key|Five`
  (params (Key :type "Key Structure"))
  (:`Pressed`
    (`self.RegisterManualKey` "\"5\"")))

(event `Key|Three`
  (params (Key :type "Key Structure"))
  (:`Pressed`
    (`self.RegisterManualKey` "\"3\"")))

(event `Key|Six`
  (params (Key :type "Key Structure"))
  (:`Pressed`
    (`self.RegisterManualKey` "\"6\"")))

(event `self.Box_StartTrigger.OnComponentBeginOverlap`
  (params (OverlappedComponent :type "PrimitiveComponent Object Reference") (OtherActor :type "Actor Object Reference") (OtherComp :type "PrimitiveComponent Object Reference") (OtherBodyIndex :type Integer) (bFromSweep :type Boolean) (SweepResult :type "HitResult Structure (by ref)"))
  (if (`self.bOnlyPlayerTriggers`)
    (cast `Character` OtherActor)
    (`self.StartGlobalLightEvent`)
    (else
      (`/Engine/EditorBlueprintResources/StandardMacros.IsValid` OtherActor
        (:`Is Valid`
          (`self.StartGlobalLightEvent`))))))

(event `self.Box_EndTrigger.OnComponentBeginOverlap`
  (params (OverlappedComponent :type "PrimitiveComponent Object Reference") (OtherActor :type "Actor Object Reference") (OtherComp :type "PrimitiveComponent Object Reference") (OtherBodyIndex :type Integer) (bFromSweep :type Boolean) (SweepResult :type "HitResult Structure (by ref)"))
  (if (`self.bOnlyPlayerTriggers`)
    (cast `Character` OtherActor)
    (`self.StopGlobalLightEvent`)
    (else
      (`/Engine/EditorBlueprintResources/StandardMacros.IsValid` OtherActor
        (:`Is Valid`
          (`self.StopGlobalLightEvent`))))))

(fn `ApplyActionToLight`
  (params (TargetLight :type "/Game/Birra_New/Managers/Lights/0_BPs/BP_LightUnit_Base Object Reference") (Action :type "/Game/Birra_New/Managers/Lights/5_Enums/E_GlobalLightAction Enum" :default "NewEnumerator0"))
  (`/Engine/EditorBlueprintResources/StandardMacros.IsValid` TargetLight
    (:`Is Valid`
      (switch `/Game/Birra_New/Managers/Lights/5_Enums/E_GlobalLightAction` Action
        (:`NewEnumerator0`
          (`self.TurnOnAll`))
        (:`NewEnumerator1`
          (`self.TurnOffAll`))
        (:`NewEnumerator2`
          (`/Game/Birra_New/Managers/Lights/0_BPs/BP_LightUnit_Base.SetPumpState` TargetLight (`self.PumpIntensityMultiplier`) (`self.PumpEmissiveMultiplier`)))
        (:`NewEnumerator3`
          (`self.DePumpAll`))
        (:`NewEnumerator4`
          (`self.FlickerAll`))
        (:`NewEnumerator5`
          (`self.DeflickerAll`))))))

(fn `AutoRevertManualAction`
  (switch `/Game/Birra_New/Managers/Lights/5_Enums/E_GlobalLightAction` (`self.CurrentGlobalAction`)
    (:`NewEnumerator0`
      (`self.TurnOnAll`))
    (:`NewEnumerator1`
      (`self.TurnOffAll`))
    (:`NewEnumerator2`
      (`self.PumpAll`))
    (:`NewEnumerator3`
      (`self.DePumpAll`))
    (:`NewEnumerator4`
      (`self.FlickerAll`))
    (:`NewEnumerator5`
      (`self.DeflickerAll`))
    (:`NewEnumerator6`
      (`self.DePumpAll`)
      (`self.DeflickerAll`))))

(fn `BuildSequentialLightQueue`
  (bind _sequentiallightsqueue (`self.SequentialLightsQueue`))
  (`KismetArrayLibrary.Array_Clear` _sequentiallightsqueue)
  (if (`self.bRefreshBeforeCommand`)
    (`self.RefreshAllLights`)
    (for _array_element (`self.AllLights`)
      (`/Engine/EditorBlueprintResources/StandardMacros.IsValid` _array_element
        (:`Is Valid`
          (`KismetArrayLibrary.Array_Add` _sequentiallightsqueue _array_element))))
    (`KismetArrayLibrary.Array_Shuffle` _sequentiallightsqueue)))

(fn `CancelSequentialGlobalAction`
  (`KismetSystemLibrary.K2_ClearAndInvalidateTimerHandle` (`self.SequentialTimerHandle`))
  (`KismetArrayLibrary.Array_Clear` (`self.SequentialLightsQueue`))
  (set `self.bSequentialInProgress` false))

(fn `CheckManualSequence`
  (switch `string` (`self.ManualKeyBuffer`)
    (:`111`
      (`self.ExecuteManualGlobalLightAction` "NewEnumerator0"))
    (:`222`
      (`self.ExecuteManualGlobalLightAction` "NewEnumerator1"))
    (:`333`
      (`self.ExecuteManualGlobalLightAction` "NewEnumerator2"))
    (:`444`
      (`self.ExecuteManualGlobalLightAction` "NewEnumerator3"))
    (:`555`
      (`self.ExecuteManualGlobalLightAction` "NewEnumerator4"))
    (:`666`
      (`self.ExecuteManualGlobalLightAction` "NewEnumerator5"))
    (:`777`
      (`self.ExecuteRandomGlobalLightAction` "NewEnumerator0")
      (`self.ScheduleManualAutoRevert`)
      (`self.ClearManualKeyBuffer`))))

(fn `ClearManualKeyBuffer`
  (set `self.ManualKeyBuffer` "\"\""))

(fn `DeflickerAll`)

(fn `DePumpAll`)

(fn `ExecuteGlobalLightAction`
  (params (Action :type "/Game/Birra_New/Managers/Lights/5_Enums/E_GlobalLightAction Enum" :default "NewEnumerator0"))
  (if (`self.bPlaySoundOnGlobalAction`)
    (`self.CancelSequentialGlobalAction`)
    (`self.PlayObscureSound`))
  (bind _output_get (set `self.CurrentGlobalAction` Action))
  (if (`self.bUseSequentialGlobalActions`)
    (`self.ExecuteGlobalLightActionSequential` _output_get)
    (else
      (switch `/Game/Birra_New/Managers/Lights/5_Enums/E_GlobalLightAction` _output_get
        (:`NewEnumerator0`
          (`self.TurnOnAll`))
        (:`NewEnumerator1`
          (`self.TurnOffAll`))
        (:`NewEnumerator2`
          (`self.PumpAll`))
        (:`NewEnumerator3`
          (`self.DePumpAll`))
        (:`NewEnumerator4`
          (`self.FlickerAll`))
        (:`NewEnumerator5`
          (`self.DeflickerAll`))))))

(fn `ExecuteGlobalLightActionSequential`
  (params (Action :type "/Game/Birra_New/Managers/Lights/5_Enums/E_GlobalLightAction Enum" :default "NewEnumerator0"))
  (if (`|EnumEquality` Action "NewEnumerator6")
    (`self.ExecuteRandomGlobalLightAction` Action)
    (else
      (`KismetSystemLibrary.K2_ClearAndInvalidateTimerHandle` (`self.SequentialTimerHandle`))
      (set `self.CurrentSequentialAction` Action)
      (set `self.bSequentialInProgress` true)
      (`self.BuildSequentialLightQueue`)
      (`self.ProcessNextSequentialLight`))))

(fn `ExecuteManualGlobalLightAction`
  (params (Action :type "/Game/Birra_New/Managers/Lights/5_Enums/E_GlobalLightAction Enum" :default "NewEnumerator0"))
  (`self.ExecuteGlobalLightAction` Action)
  (`self.ScheduleManualAutoRevert`))

(fn `ExecuteRandomGlobalLightAction`
  (params (Action :type "/Game/Birra_New/Managers/Lights/5_Enums/E_GlobalLightAction Enum" :default "NewEnumerator0"))
  (`self.PlayObscureSound`)
  (set `self.CurrentGlobalAction` Action)
  (switch `int` (`KismetMathLibrary.RandomIntegerInRange` 0 5)
    (:`0`
      (`self.TurnOnAll`))
    (:`1`
      (`self.TurnOffAll`))
    (:`2`
      (`self.PumpAll`))
    (:`3`
      (`self.DePumpAll`))
    (:`4`
      (`self.FlickerAll`))
    (:`5`
      (`self.DeflickerAll`))))

(fn `FlickerAll`)

(fn `GetRandomManualDuration`
  (returns (Duration :type "Float (double-precision)"))
  (return (`KismetMathLibrary.RandomFloatInRange` (`self.ManualEffectDurationMin`) (`self.ManualEffectDurationMax`))))

(fn `GetRandomObscureSound`
  (returns (SelectedSound :type "SoundBase Object Reference"))
  (bind _obscuresoundarray (`self.ObscureSoundArray`))
  (bind _returnvalue (`KismetArrayLibrary.Array_Length` _obscuresoundarray))
  (if (> _returnvalue 0)
    (return (`|GetArrayItem` _obscuresoundarray (`KismetMathLibrary.RandomIntegerInRange` 0 (- _returnvalue 1))))
    (else
      (return null))))

(fn `PlayObscureSound`
  (bind _returnvalue (`KismetMathLibrary.RandomFloatInRange` (`self.PitchMin`) (`self.PitchMax`)))
  (bind _returnvalue_2 (`KismetMathLibrary.RandomFloatInRange` (`self.VolumeMin`) (`self.VolumeMax`)))
  (bind _selectedsound (`self.GetRandomObscureSound`))
  (`/Engine/EditorBlueprintResources/StandardMacros.IsValid` _selectedsound
    (:`Is Valid`
      (if (`self.bUse2DSound`)
        (`GameplayStatics.SpawnSound2D` _selectedsound _returnvalue_2 _returnvalue 0.0 null)
        (else
          (`GameplayStatics.SpawnSoundAtLocation` _selectedsound (`SceneComponent.K2_GetComponentLocation` (`self.AudioOrigin`)) (struct) _returnvalue_2 _returnvalue 0.0 null null))))))

(fn `ProcessNextSequentialLight`
  (locals (NewLocalVar :type "/Game/Birra_New/Managers/Lights/0_BPs/BP_LightUnit_Base Object Reference"))
  (bind _sequentiallightsqueue (`self.SequentialLightsQueue`))
  (bind _returnvalue (`KismetArrayLibrary.Array_Length` _sequentiallightsqueue))
  (bind _returnvalue_2 (`KismetMathLibrary.RandomIntegerInRange` 0 (- _returnvalue 1)))
  (if (> _returnvalue 0)
    (bind _output_get (set `local.NewLocalVar` (`|GetArrayItem` _sequentiallightsqueue _returnvalue_2)))
    (`self.ApplyActionToLight` _output_get (`self.CurrentSequentialAction`))
    (`KismetArrayLibrary.Array_Remove` _sequentiallightsqueue _returnvalue_2)
    (bind _returnvalue_3 (`KismetSystemLibrary.K2_SetTimer` null "ProcessNextSequentialLight" (`KismetMathLibrary.RandomFloatInRange` (`self.SequentialDelayMin`) (`self.SequentialDelayMax`))))
    (set `self.SequentialTimerHandle` _returnvalue_3)
    (else
      (set `self.bSequentialInProgress` false)
      (`KismetSystemLibrary.K2_ClearAndInvalidateTimerHandle` (`self.SequentialTimerHandle`)))))

(fn `PumpAll`)

(fn `RefreshAllLights`
  (bind _alllights (`self.AllLights`))
  (`KismetArrayLibrary.Array_Clear` _alllights)
  (bind _outactors (`GameplayStatics.GetAllActorsOfClass` "/Game/Birra_New/Managers/Lights/0_BPs/BP_LightUnit_Base.BP_LightUnit_Base_C"))
  (for _array_element _outactors
    (bind _asbp_light_unit_base (cast `/Game/Birra_New/Managers/Lights/0_BPs/BP_LightUnit_Base` _array_element))
    (if (`self.bUseIgnoredLights`)
      (if (not (`KismetArrayLibrary.Array_Contains` (`self.IgnoredLights`) _asbp_light_unit_base))
        (`KismetArrayLibrary.Array_Add` _alllights _asbp_light_unit_base))
      (else
        (`KismetArrayLibrary.Array_Add` _alllights _asbp_light_unit_base))))
  (`KismetSystemLibrary.PrintString` (`KismetTextLibrary.Conv_TextToString` (`|FormatText` "Global Lights Found: {Length}" (`KismetArrayLibrary.Array_Length` _alllights))) true true (struct :`R` 1.0 :`A` 1.0) 10.0))

(fn `RegisterManualKey`
  (params (KeyChar :type String))
  (bind _output_get (set `self.ManualKeyBuffer` (`KismetStringLibrary.Concat_StrStr` KeyChar (`self.ManualKeyBuffer`))))
  (if (> (`KismetStringLibrary.Len` _output_get) 3)
    (set `self.ManualKeyBuffer` (`KismetStringLibrary.Right` _output_get 3))
    (`KismetSystemLibrary.K2_ClearAndInvalidateTimerHandle` (`self.ManualSequenceTimerHandle`))
    (`KismetSystemLibrary.K2_SetTimer` null "ClearManualKeyBuffer" (`self.ManualSequenceResetDelay`))
    (set `self.ManualKeyBuffer` "")
    (`self.CheckManualSequence`)))

(fn `ScheduleManualAutoRevert`
  (if (`self.bAutoRevertManualAction`)
    (`KismetSystemLibrary.K2_ClearAndInvalidateTimerHandle` (`self.ManualRevertTimerHandle`))
    (bind _duration (`self.GetRandomManualDuration`))
    (bind _returnvalue (`KismetSystemLibrary.K2_SetTimer` null "AutoRevertManualAction" _duration))
    (set `self.ManualRevertTimerHandle` _returnvalue)))

(fn `StartGlobalLightEvent`
  (if (not (`self.bGlobalEventActive`))
    (set `self.bGlobalEventActive` true)
    (`self.ExecuteGlobalLightAction` (`self.StartGlobalAction`))))

(fn `StopGlobalLightEvent`
  (if (not (`self.bGlobalEventActive`))
    (set `self.bGlobalEventActive` false)
    (`self.ExecuteGlobalLightAction` (`self.StopGlobalAction`))))

(fn `TurnOffAll`)

(fn `TurnOnAll`
  (if (`self.bRefreshBeforeCommand`)
    (`self.RefreshAllLights`))
  (for _array_element (`self.AllLights`)
    (`/Engine/EditorBlueprintResources/StandardMacros.IsValid` _array_element
      (:`Is Valid`
        (`/Game/Birra_New/Managers/Lights/0_BPs/BP_LightUnit_Base.TurnOn` _array_element)))))

(fn `UserConstructionScript`)