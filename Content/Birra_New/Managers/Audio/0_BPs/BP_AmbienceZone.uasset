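; BP_AmbienceZone is a trigger volume that fades an ambience sound in when an actor enters its box and out when one leaves.
; An option restricts triggering to the BP_Resident_HorrorV1 player, and another starts the sound on BeginPlay.
; SetupAmbience applies the configured sound, pitch and volume to the audio component.
; An IsActive flag prevents repeated fades, without counting how many actors remain inside.
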(event `self.ReceiveBeginPlay`
  (`self.SetupAmbience`)
  (if (`self.bStartActive`)
    (`self.FadeInAmbience`)))

(event `self.ZoneBox.OnComponentBeginOverlap`
  (params (OverlappedComponent :type "PrimitiveComponent Object Reference") (OtherActor :type "Actor Object Reference") (OtherComp :type "PrimitiveComponent Object Reference") (OtherBodyIndex :type Integer) (bFromSweep :type Boolean) (SweepResult :type "HitResult Structure (by ref)"))
  (if (`self.bOnlyPlayerTriggers`)
    (cast `/Game/ChildrenOfAndromeda/Character/BP_Character/BP_Resident_HorrorV1` OtherActor)
    (`self.FadeInAmbience`)
    (else
      (`self.FadeInAmbience`))))

(event `self.ZoneBox.OnComponentEndOverlap`
  (params (OverlappedComponent :type "PrimitiveComponent Object Reference") (OtherActor :type "Actor Object Reference") (OtherComp :type "PrimitiveComponent Object Reference") (OtherBodyIndex :type Integer))
  (if (`self.bOnlyPlayerTriggers`)
    (cast `/Game/ChildrenOfAndromeda/Character/BP_Character/BP_Resident_HorrorV1` OtherActor)
    (`self.FadeOutAmbience`)
    (else
      (`self.FadeOutAmbience`))))

(fn `FadeInAmbience`
  (if (not (`self.bIsActive`))
    (`/Engine/EditorBlueprintResources/StandardMacros.IsValid` (`self.AmbienceSound`)
      (:`Is Valid`
        (`self.SetupAmbience`)
        (`AudioComponent.FadeIn` (`self.Audio_Ambience`) (`self.FadeInTime`) (`self.VolumeTarget`) 0.0 "Linear")
        (set `self.bIsActive` true)))))

(fn `FadeOutAmbience`
  (if (`self.bIsActive`)
    (`AudioComponent.FadeOut` (`self.Audio_Ambience`) (`self.FadeOutTime`) 0.0 "Linear")
    (set `self.bIsActive` false)))

(fn `SetupAmbience`
  (bind _ambiencesound (`self.AmbienceSound`))
  (bind _audio_ambience (`self.Audio_Ambience`))
  (`/Engine/EditorBlueprintResources/StandardMacros.IsValid` _ambiencesound
    (:`Is Valid`
      (`AudioComponent.SetSound` _audio_ambience _ambiencesound)
      (`AudioComponent.SetPitchMultiplier` _audio_ambience (`self.PitchMultiplier`))
      (`AudioComponent.SetVolumeMultiplier` _audio_ambience (`self.VolumeTarget`))
      (return))
    (:`Is Not Valid`
      (return))))

(fn `UserConstructionScript`)