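; BP_MachineSound is an actor that plays machine audio through an Off, Starting, Running, Stopping and Broken state machine.
; Start, stop, broken and running functions fade the AudioLoop component in or out, with the first three also spawning one-shot sounds at the actor's location.
; BeginPlay configures the loop and stores StartupState, but its switch reads a literal Off, so the loop always begins stopped.
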(event `self.ReceiveBeginPlay`
  (bind _audio_loop (`self.Audio_Loop`))
  (bind _volumemultiplier (`self.VolumeMultiplier`))
  (bind _brokensound (`self.BrokenSound`))
  (`self.SetupMachineSound`)
  (set `self.CurrentMachineState` (`self.StartupState`))
  (switch `/Game/Birra_New/Managers/Audio/4_Enums/E_MachineAudioState` "NewEnumerator0"
    (:`NewEnumerator0`
      (set `self.bIsLoopPlaying` false)
      (`AudioComponent.Stop` _audio_loop))
    (:`NewEnumerator1`
      (set `self.CurrentMachineState` "NewEnumerator0"))
    (:`NewEnumerator2`
      (`/Engine/EditorBlueprintResources/StandardMacros.IsValid` (`self.LoopSound`)
        (:`Is Valid`
          (`AudioComponent.FadeIn` _audio_loop (`self.FadeInTime`) _volumemultiplier 0.0 "Linear")
          (set `self.bIsLoopPlaying` false)
          (set `self.CurrentMachineState` "NewEnumerator2"))))
    (:`NewEnumerator3`
      (set `self.CurrentMachineState` "NewEnumerator0"))
    (:`NewEnumerator4`
      (set `self.CurrentMachineState` "NewEnumerator4")
      (`/Engine/EditorBlueprintResources/StandardMacros.IsValid` _brokensound
        (:`Is Valid`
          (`GameplayStatics.SpawnSoundAtLocation` _brokensound (`self.K2_GetActorLocation`) (struct) _volumemultiplier (`self.PitchMultiplier`) 0.0 null null))))))

(fn `SetMachineBroken`
  (bind _brokensound (`self.BrokenSound`))
  (if (not (`|EnumEquality` (`self.CurrentMachineState`) "NewEnumerator4"))
    (set `self.CurrentMachineState` "NewEnumerator4")
    (if (`self.bIsLoopPlaying`)
      (`AudioComponent.FadeOut` (`self.Audio_Loop`) (`self.FadeOutTime`) 0.0 "Linear")
      (set `self.bIsLoopPlaying` false)
      (`/Engine/EditorBlueprintResources/StandardMacros.IsValid` _brokensound
        (:`Is Valid`
          (`GameplayStatics.SpawnSoundAtLocation` _brokensound (`self.K2_GetActorLocation`) (struct) (`self.VolumeMultiplier`) (`self.PitchMultiplier`) 0.0 (`self.AttenuationSettings`) (`self.OneShotConcurrencySettings`)))))))

(fn `SetMachineRunning`
  (if (not (`|EnumEquality` (`self.CurrentMachineState`) "NewEnumerator2"))
    (set `self.CurrentMachineState` "NewEnumerator2")
    (`self.SetupMachineSound`)
    (`/Engine/EditorBlueprintResources/StandardMacros.IsValid` (`self.LoopSound`)
      (:`Is Valid`
        (`AudioComponent.FadeIn` (`self.Audio_Loop`) (`self.FadeInTime`) (`self.VolumeMultiplier`) 0.0 "Linear")
        (set `self.bIsLoopPlaying` true))
      (:`Is Not Valid`
        (set `self.bIsLoopPlaying` false)))))

(fn `SetupMachineSound`
  (bind _loopsound (`self.LoopSound`))
  (bind _audio_loop (`self.Audio_Loop`))
  (`/Engine/EditorBlueprintResources/StandardMacros.IsValid` _loopsound
    (:`Is Valid`
      (`AudioComponent.SetSound` _audio_loop _loopsound)
      (`AudioComponent.SetVolumeMultiplier` _audio_loop (`self.VolumeMultiplier`))
      (`AudioComponent.SetPitchMultiplier` _audio_loop (`self.PitchMultiplier`))
      (return))
    (:`Is Not Valid`
      (return))))

(fn `StartMachineSound`
  (bind _startsound (`self.StartSound`))
  (switch `/Game/Birra_New/Managers/Audio/4_Enums/E_MachineAudioState` (`self.CurrentMachineState`)
    (:`NewEnumerator0`
      (set `self.CurrentMachineState` "NewEnumerator1")
      (`/Engine/EditorBlueprintResources/StandardMacros.IsValid` _startsound
        (:`Is Valid`
          (`GameplayStatics.SpawnSoundAtLocation` _startsound (`self.K2_GetActorLocation`) (struct) (`self.VolumeMultiplier`) (`self.PitchMultiplier`) 0.0 (`self.AttenuationSettings`) (`self.OneShotConcurrencySettings`))
          (`self.SetupMachineSound`)
          (`/Engine/EditorBlueprintResources/StandardMacros.IsValid` (`self.LoopSound`)
            (:`Is Valid`
              (`AudioComponent.FadeIn` (`self.Audio_Loop`) (`self.FadeInTime`) (`self.VolumeMultiplier`) 0.0 "Linear")
              (set `self.bIsLoopPlaying` true)
              (set `self.CurrentMachineState` "NewEnumerator2"))
            (:`Is Not Valid`
              (set `self.CurrentMachineState` "NewEnumerator2")
              (set `self.bIsLoopPlaying` false))))))))

(fn `StopMachineSound`
  (bind _stopsound (`self.StopSound`))
  (bind _stopsound_2 (`self.StopSound`))
  (bind _stopsound_3 (`self.StopSound`))
  (switch `/Game/Birra_New/Managers/Audio/4_Enums/E_MachineAudioState` (`self.CurrentMachineState`)
    (:`NewEnumerator1`
      (set `self.CurrentMachineState` "NewEnumerator3")
      (if (`self.bIsLoopPlaying`)
        (`AudioComponent.FadeOut` (`self.Audio_Loop`) (`self.FadeOutTime`) 0.0 "Linear")
        (set `self.bIsLoopPlaying` false)
        (`/Engine/EditorBlueprintResources/StandardMacros.IsValid` _stopsound
          (:`Is Valid`
            (`GameplayStatics.SpawnSoundAtLocation` _stopsound (`self.K2_GetActorLocation`) (struct) (`self.VolumeMultiplier`) (`self.PitchMultiplier`) 0.0 (`self.AttenuationSettings`) (`self.OneShotConcurrencySettings`))
            (set `self.CurrentMachineState` "NewEnumerator0")))))
    (:`NewEnumerator2`
      (set `self.CurrentMachineState` "NewEnumerator3")
      (if (`self.bIsLoopPlaying`)
        (`AudioComponent.FadeOut` (`self.Audio_Loop`) (`self.FadeOutTime`) 0.0 "Linear")
        (set `self.bIsLoopPlaying` false)
        (`/Engine/EditorBlueprintResources/StandardMacros.IsValid` _stopsound_2
          (:`Is Valid`
            (`GameplayStatics.SpawnSoundAtLocation` _stopsound_2 (`self.K2_GetActorLocation`) (struct) (`self.VolumeMultiplier`) (`self.PitchMultiplier`) 0.0 (`self.AttenuationSettings`) (`self.OneShotConcurrencySettings`))
            (set `self.CurrentMachineState` "NewEnumerator0")))))
    (:`NewEnumerator4`
      (set `self.CurrentMachineState` "NewEnumerator3")
      (if (`self.bIsLoopPlaying`)
        (`AudioComponent.FadeOut` (`self.Audio_Loop`) (`self.FadeOutTime`) 0.0 "Linear")
        (set `self.bIsLoopPlaying` false)
        (`/Engine/EditorBlueprintResources/StandardMacros.IsValid` _stopsound_3
          (:`Is Valid`
            (`GameplayStatics.SpawnSoundAtLocation` _stopsound_3 (`self.K2_GetActorLocation`) (struct) (`self.VolumeMultiplier`) (`self.PitchMultiplier`) 0.0 (`self.AttenuationSettings`) (`self.OneShotConcurrencySettings`))
            (set `self.CurrentMachineState` "NewEnumerator0")))))))

(fn `UserConstructionScript`)