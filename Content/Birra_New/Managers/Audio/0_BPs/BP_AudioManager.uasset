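; BP_AudioManager is a central audio manager that controls a global alarm and plays 2D sounds.
; It keeps a BP_AlarmSoundController reference, either registered externally or optionally auto-found as the first instance at BeginPlay and before start or stop calls.
; Alarm functions forward to that controller, though SetGlobalAlarmLevel calls itself unconditionally before setting the level, so it recurses endlessly.
; PlayGlobal2DSound scales requested volume and pitch by global multipliers.
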(event `self.ReceiveBeginPlay`
  (`self.SetupAudioManager`))

(fn `PlayGlobal2DSound`
  (params (SoundToPlay :type "SoundBase Object Reference") (VolumeOverride :type "Float (double-precision)" :default 1.0) (PitchOverride :type "Float (double-precision)" :default 1.0))
  (`/Engine/EditorBlueprintResources/StandardMacros.IsValid` SoundToPlay
    (:`Is Valid`
      (`GameplayStatics.SpawnSound2D` SoundToPlay (* VolumeOverride (`self.GlobalVolumeMultiplier`)) (* PitchOverride (`self.GlobalPitchMultiplier`)) 0.0 null))))

(fn `RegisterAlarmController`
  (params (NewAlarmController :type "/Game/Birra_New/Managers/Audio/0_BPs/BP_AlarmSoundController Object Reference"))
  (`/Engine/EditorBlueprintResources/StandardMacros.IsValid` NewAlarmController
    (:`Is Valid`
      (set `self.AlarmControllerRef` NewAlarmController))))

(fn `SetGlobalAlarmLevel`
  (params (NewAlarmLevel :type Integer))
  (bind _alarmcontrollerref (`self.AlarmControllerRef`))
  (`self.SetGlobalAlarmLevel` NewAlarmLevel)
  (`/Engine/EditorBlueprintResources/StandardMacros.IsValid` _alarmcontrollerref
    (:`Is Valid`
      (set `/Game/Birra_New/Managers/Audio/0_BPs/BP_AlarmSoundController.AlarmLevel` NewAlarmLevel _alarmcontrollerref))))

(fn `SetupAudioManager`
  (`/Engine/EditorBlueprintResources/StandardMacros.IsValid` (`self.AlarmControllerRef`)
    (:`Is Valid`
      (return))
    (:`Is Not Valid`
      (if (`self.bAutoFindAlarmController`)
        (bind _outactors (`GameplayStatics.GetAllActorsOfClass` "/Game/Birra_New/Managers/Audio/0_BPs/BP_AlarmSoundController.BP_AlarmSoundController_C"))
        (if (> (`KismetArrayLibrary.Array_Length` _outactors) 0)
          (set `self.AlarmControllerRef` (`|GetArrayItem` _outactors))
          (return)
          (else
            (return)))
        (else
          (return))))))

(fn `StartGlobalAlarm`
  (bind _alarmcontrollerref (`self.AlarmControllerRef`))
  (`self.SetupAudioManager`)
  (`/Engine/EditorBlueprintResources/StandardMacros.IsValid` _alarmcontrollerref
    (:`Is Valid`
      (`/Game/Birra_New/Managers/Audio/0_BPs/BP_AlarmSoundController.StartAlarm` _alarmcontrollerref))))

(fn `StopGlobalAlarm`
  (bind _alarmcontrollerref (`self.AlarmControllerRef`))
  (`self.SetupAudioManager`)
  (`/Engine/EditorBlueprintResources/StandardMacros.IsValid` _alarmcontrollerref
    (:`Is Valid`
      (`/Game/Birra_New/Managers/Audio/0_BPs/BP_AlarmSoundController.StopAlarm` _alarmcontrollerref))))

(fn `UserConstructionScript`)