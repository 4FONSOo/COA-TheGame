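; A trigger-box actor that plays a random sound from an array, as 2D or at SoundOrigin, when overlapped.
; Overlaps proceed only when OnlyPlayerTriggers is set and the actor is BP_FirstPersonCharacter; with the flag off, nothing plays.
; An optional delay precedes playback, which randomizes volume and pitch and applies concurrency settings.
; TriggerOnce blocks replays by setting HasTriggered after playback, and ResetTrigger clears it.
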(event `self.TriggerBox.OnComponentBeginOverlap`
  (params (OverlappedComponent :type "PrimitiveComponent Object Reference") (OtherActor :type "Actor Object Reference") (OtherComp :type "PrimitiveComponent Object Reference") (OtherBodyIndex :type Integer) (bFromSweep :type Boolean) (SweepResult :type "HitResult Structure (by ref)"))
  (if (`self.bOnlyPlayerTriggers`)
    (cast `/Game/FirstPerson/Blueprints/BP_FirstPersonCharacter` OtherActor)
    (`self.Check TriggerOnce`)))

(event `Check TriggerOnce`
  (if (`self.bTriggerOnce`)
    (if (not (`self.bHasTriggered`))
      (`self.Delay Check`))
    (else
      (`self.Delay Check`))))

(event `Delay Check`
  (bind _btriggeronce (`self.bTriggerOnce`))
  (if (> (`self.DelayBeforePlay`) 0.0)
    (`KismetSystemLibrary.Delay` (`self.DelayBeforePlay`))
    (`self.PlayOneShotSound`)
    (if _btriggeronce
      (set `self.bHasTriggered` true))
    (else
      (`self.PlayOneShotSound`)
      (if _btriggeronce
        (set `self.bHasTriggered` true)))))

(fn `GetSelectedSound`
  (returns (SelectedSound :type "SoundBase Object Reference"))
  (bind _soundarray (`self.SoundArray`))
  (bind _returnvalue (`KismetArrayLibrary.Array_Length` _soundarray))
  (if (<= _returnvalue 0)
    (return null)
    (else
      (return (`|GetArrayItem` _soundarray (`KismetMathLibrary.RandomIntegerInRange` 0 (- _returnvalue 1)))))))

(fn `PlayOneShotSound`
  (bind _concurrencysettings (`self.ConcurrencySettings`))
  (bind _returnvalue (`KismetMathLibrary.RandomFloatInRange` (`self.PitchMin`) (`self.PitchMax`)))
  (bind _returnvalue_2 (`KismetMathLibrary.RandomFloatInRange` (`self.VolumeMin`) (`self.VolumeMax`)))
  (bind _selectedsound (`self.GetSelectedSound`))
  (`/Engine/EditorBlueprintResources/StandardMacros.IsValid` _selectedsound
    (:`Is Valid`
      (if (`self.bUse2D`)
        (`GameplayStatics.SpawnSound2D` _selectedsound _returnvalue_2 _returnvalue 0.0 _concurrencysettings)
        (else
          (`GameplayStatics.SpawnSoundAtLocation` _selectedsound (`SceneComponent.K2_GetComponentLocation` (`self.SoundOrigin`)) (struct) _returnvalue_2 _returnvalue 0.0 (`self.AttenuationSettings`) _concurrencysettings))))))

(fn `ResetTrigger`
  (set `self.bHasTriggered` false))

(fn `UserConstructionScript`)