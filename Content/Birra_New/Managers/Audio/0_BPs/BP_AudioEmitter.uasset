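; Placeable audio emitter actor that wraps an AudioMain component to play a configurable sound, optionally starting on BeginPlay.
; SetupEmitter applies the sound, volume, pitch and optional attenuation, and runs at BeginPlay and before each play.
; Play and Stop fade, guarded by an IsPlaying flag, while ForceStop cuts immediately.
; StopEmitter reuses FadeInTime as its fade-out duration and targets VolumeMultiplier rather than zero.
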(event `self.ReceiveBeginPlay`
  (`self.SetupEmitter`)
  (if (`self.bAutoPlay`)
    (`self.PlayEmitter`)))

(fn `ForceStopEmitter`
  (`AudioComponent.Stop` (`self.Audio_Main`))
  (set `self.bIsPlaying` false))

(fn `PlayEmitter`
  (if (not (`self.bIsPlaying`))
    (`/Engine/EditorBlueprintResources/StandardMacros.IsValid` (`self.SoundToPlay`)
      (:`Is Valid`
        (`self.SetupEmitter`)
        (`AudioComponent.FadeIn` (`self.Audio_Main`) (`self.FadeInTime`) (`self.VolumeMultiplier`) 0.0 "Linear")
        (set `self.bIsPlaying` true)))))

(fn `SetupEmitter`
  (bind _attenuationsettings (`self.AttenuationSettings`))
  (`/Engine/EditorBlueprintResources/StandardMacros.IsValid` (`self.SoundToPlay`)
    (:`Is Valid`
      (`AudioComponent.SetSound` (`self.Audio_Main`) null)
      (set `self.VolumeMultiplier` (`self.VolumeMultiplier`))
      (set `self.PitchMultiplier` (`self.PitchMultiplier`))
      (`/Engine/EditorBlueprintResources/StandardMacros.IsValid` _attenuationsettings
        (:`Is Valid`
          (set `AudioComponent.AttenuationSettings` _attenuationsettings (`self.Audio_Main`)))
        (:`Is Not Valid`
          (return))))
    (:`Is Not Valid`
      (return))))

(fn `StopEmitter`
  (if (`self.bIsPlaying`)
    (`AudioComponent.FadeOut` (`self.Audio_Main`) (`self.FadeInTime`) (`self.VolumeMultiplier`) "Linear")
    (set `self.bIsPlaying` false)))

(fn `UserConstructionScript`)