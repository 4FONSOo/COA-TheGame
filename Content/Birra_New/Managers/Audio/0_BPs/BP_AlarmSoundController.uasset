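; Alarm audio controller actor that runs a looping alarm with one-shot start and stop sounds at its location.
; BeginPlay configures the loop and calls StartAlarm when AlarmLevel is positive.
; StartAlarm only plays if AlarmActive is already set, otherwise setting that flag, while StopAlarm fades out.
; SetAlarmLevel always zeroes the level, and PlayRandomIntercom is uncalled here, with an inverted array-length check.
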(event `self.ReceiveBeginPlay`
  (`self.SetupAlarm`)
  (if (> (`self.AlarmLevel`) 0)
    (`self.StartAlarm`)
    (else
      (set `self.bAlarmActive` false))))

(fn `PlayRandomIntercom`
  (bind _intercomarray (`self.IntercomArray`))
  (bind _audio_intercom (`self.Audio_Intercom`))
  (bind _returnvalue (`KismetArrayLibrary.Array_Length` _intercomarray))
  (bind _output (`|GetArrayItem` _intercomarray (`KismetMathLibrary.RandomIntegerInRange` 0 (- _returnvalue 1))))
  (if (<= _returnvalue 0)
    (`/Engine/EditorBlueprintResources/StandardMacros.IsValid` _output
      (:`Is Valid`
        (`AudioComponent.SetSound` _audio_intercom _output)
        (`AudioComponent.SetVolumeMultiplier` _audio_intercom (`self.VolumeMultiplier`))
        (`AudioComponent.SetPitchMultiplier` _audio_intercom (`self.PitchMultiplier`))
        (`AudioComponent.Play` _audio_intercom 0.0)))))

(fn `SetAlarmLevel`
  (bind _output_get (set `self.AlarmLevel` 0))
  (if (<= (== _output_get 0) 0)
    (`self.StopAlarm`)
    (else
      (`self.StartAlarm`))))

(fn `SetupAlarm`
  (bind _alarmloopsound (`self.AlarmLoopSound`))
  (bind _audio_alarmloop (`self.Audio_AlarmLoop`))
  (`/Engine/EditorBlueprintResources/StandardMacros.IsValid` _alarmloopsound
    (:`Is Valid`
      (`AudioComponent.SetSound` _audio_alarmloop _alarmloopsound)
      (`AudioComponent.SetVolumeMultiplier` _audio_alarmloop (`self.VolumeMultiplier`))
      (`AudioComponent.SetPitchMultiplier` _audio_alarmloop (`self.PitchMultiplier`))
      (return))
    (:`Is Not Valid`
      (return))))

(fn `StartAlarm`
  (bind _alarmstartsound (`self.AlarmStartSound`))
  (bind _audio_alarmloop (`self.Audio_AlarmLoop`))
  (bind _volumemultiplier (`self.VolumeMultiplier`))
  (bind _fadeintime (`self.FadeInTime`))
  (if (`self.bAlarmActive`)
    (`/Engine/EditorBlueprintResources/StandardMacros.IsValid` _alarmstartsound
      (:`Is Valid`
        (`GameplayStatics.SpawnSoundAtLocation` _alarmstartsound (`self.K2_GetActorLocation`) (struct) (`self.VolumeMultiplier`) (`self.PitchMultiplier`) 0.0 (`self.AttenuationSettings`) (`self.AlarmOneShotConcurrencySettings`))
        (`self.SetupAlarm`)
        (`/Engine/EditorBlueprintResources/StandardMacros.IsValid` (`self.AlarmLoopSound`)
          (:`Is Valid`
            (`AudioComponent.FadeIn` _audio_alarmloop _fadeintime _volumemultiplier 0.0 "Linear")
            (if (`self.bPlayIntercomOnAlarmStart`)
              (`AudioComponent.FadeIn` _audio_alarmloop _fadeintime _volumemultiplier 0.0 "Linear"))))))
    (else
      (set `self.bAlarmActive` true))))

(fn `StopAlarm`
  (bind _alarmstopsound (`self.AlarmStopSound`))
  (if (`self.bAlarmActive`)
    (set `self.bAlarmActive` false)
    (`AudioComponent.FadeOut` (`self.Audio_AlarmLoop`) (`self.FadeOutTime`) 0.0 "Linear")
    (`/Engine/EditorBlueprintResources/StandardMacros.IsValid` _alarmstopsound
      (:`Is Valid`
        (`GameplayStatics.SpawnSoundAtLocation` _alarmstopsound (`self.K2_GetActorLocation`) (struct) (`self.VolumeMultiplier`) (`self.PitchMultiplier`) 0.0 (`self.AttenuationSettings`) (`self.AlarmOneShotConcurrencySettings`))))))

(fn `UserConstructionScript`)