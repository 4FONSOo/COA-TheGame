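; Player footsteps component that plays randomized footstep sounds for its owning Character.
; Tick accumulates horizontal travel against a crouch, walk or run step distance, though this logic is gated on an invalid movement component.
; PlayFootstep picks a sound, preferring the metal set over default, and line-traces down from an offset foot position.
; Only the right-foot trace-miss path spawns the sound with random volume and pitch and toggles the foot.
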(event `self.ReceiveBeginPlay`
  ; Alterar este
  (bind _ascharacter (cast `Character` (`self.GetOwner`)))
  (bind _output_get (set `self.OwnerCharacter` _ascharacter))
  (set `self.OwnerMovement` (`Character.CharacterMovement` _output_get))
  (set `self.LastActorLocation` (`self.K2_GetActorLocation` _output_get)))

(event `self.ReceiveTick`
  (params (DeltaSeconds :type "Float (single-precision)"))
  (bind _ownercharacter (`self.OwnerCharacter`))
  (bind _returnvalue (`self.K2_GetActorLocation` _ownercharacter))
  (if (`self.bFootstepsEnabled`)
    (`/Engine/EditorBlueprintResources/StandardMacros.IsValid` _ownercharacter
      (:`Is Valid`
        (`/Engine/EditorBlueprintResources/StandardMacros.IsValid` (`self.OwnerMovement`)
          (:`Is Not Valid`
            (bind _returnvalue_2 (`self.CanPlayFootstep`))
            (if _returnvalue_2
              (set `self.CurrentLocation` _returnvalue)
              (bind _output_get (set `self.DeltaDistance` (`KismetMathLibrary.VSizeXY` (- (`self.CurrentLocation`) (`self.LastActorLocation`)))))
              (bind _output_get_2 (set `self.DistanceAccumulator` (+ (`self.DistanceAccumulator`) _output_get)))
              (bind _returnvalue_3 (`self.GetCurrentStepDistance`))
              (bind _output_get_3 (set `self.CurrentStepDistance` _returnvalue_3))
              (if (>= _output_get_3 _output_get_2)
                (`self.PlayFootstep`)
                (set `self.DistanceAccumulator` 0.0))
              (else
                (set `self.LastActorLocation` _returnvalue)
                (set `self.DistanceAccumulator` 0.0)))))))))

(fn `CanPlayFootstep`
  (returns (ReturnValue :type Boolean))
  (bind _ownercharacter (`self.OwnerCharacter`))
  (bind _ownermovement (`self.OwnerMovement`))
  (if (`self.bFootstepsEnabled`)
    (`/Engine/EditorBlueprintResources/StandardMacros.IsValid` _ownercharacter
      (:`Is Valid`
        (if (`NavMovementInterface.IsFalling` _ownermovement)
          _
          (elif (`NavMovementComponent.IsMovingOnGround` _ownermovement)
            (return (> (`KismetMathLibrary.VSizeXY` (`self.GetVelocity` _ownercharacter)) (`self.MinSpeedForFootsteps`)))
            (else
              _))))
      (:`Is Not Valid`
        _)))
  (return false))

(fn `GetCurrentStepDistance`
  (returns (ReturnValue :type "Float (double-precision)"))
  (bind _ownercharacter (`self.OwnerCharacter`))
  (bind _walkstepdistance (`self.WalkStepDistance`))
  (`/Engine/EditorBlueprintResources/StandardMacros.IsValid` _ownercharacter
    (:`Is Valid`
      (if (`Character.bIsCrouched` _ownercharacter)
        (return (`self.CrouchStepDistance`))
        (elif (>= (`KismetMathLibrary.VSizeXY` (`self.GetVelocity` _ownercharacter)) (`self.RunSpeedThreshold`))
          (return (`self.RunStepDistance`))
          (else
            (return _walkstepdistance)))))
    (:`Is Not Valid`
      (return _walkstepdistance))))

(fn `GetRandomFootstepSound`
  (returns (SelectedSound :type "SoundBase Object Reference"))
  (bind _footstep_metal (`self.Footstep_Metal`))
  (bind _footstep_default (`self.Footstep_Default`))
  (bind _returnvalue (`KismetArrayLibrary.Array_Length` _footstep_default))
  (bind _returnvalue_2 (`KismetArrayLibrary.Array_Length` _footstep_metal))
  (if (> _returnvalue_2 0)
    (return (`|GetArrayItem` _footstep_metal (`KismetMathLibrary.RandomIntegerInRange` 0 (- _returnvalue_2 1))))
    (elif (> _returnvalue 0)
      (return (`|GetArrayItem` _footstep_default (`KismetMathLibrary.RandomIntegerInRange` 0 (- 0 _returnvalue))))
      (else
        (return null)))))

(fn `PlayFootstep`
  (locals (BaseLocation :type "Vector Structure" :default (0.0 0.0 0.0)) (ForwardOffset :type "Vector Structure") (RightOffset :type "Vector Structure") (SideOffset :type "Vector Structure") (StepLocation :type "Vector Structure") (RandomVolume :type "Float (double-precision)" :default 0.0) (`Const -1` :type "Float (double-precision)" :default -1.0) (RandomPitch :type "Float (double-precision)" :default 0.0) (TraceStart :type "Vector Structure" :default (0.0 0.0 0.0)) (TraceEnd :type "Vector Structure") (SoundLocation :type "Vector Structure"))
  (bind _ownercharacter (`self.OwnerCharacter`))
  (bind _footforwardoffset (`self.FootForwardOffset`))
  (`/Engine/EditorBlueprintResources/StandardMacros.IsValid` _ownercharacter
    (:`Is Valid`
      (bind _selectedsound (`self.GetRandomFootstepSound`))
      (`/Engine/EditorBlueprintResources/StandardMacros.IsValid` _selectedsound
        (:`Is Valid`
          (set `local.BaseLocation` (`self.K2_GetActorLocation` _ownercharacter))
          (set `local.ForwardOffset` (* (`self.GetActorForwardVector` _ownercharacter) _footforwardoffset))
          (bind _output_get (set `local.RightOffset` (* (`self.GetActorRightVector` _ownercharacter) _footforwardoffset)))
          (if (`self.bLeftFootNext`)
            (set `local.SideOffset` (* _output_get (`local.Const -1`)))
            (else
              (bind _output_get_2 (set `local.SideOffset` _output_get))
              (bind _output_get_3 (set `local.StepLocation` (+ (`local.BaseLocation`) (`local.ForwardOffset`) _output_get_2)))
              (bind _output_get_4 (set `local.TraceStart` _output_get_3))
              (bind _output_get_5 (set `local.TraceEnd` (- _output_get_4 (`KismetMathLibrary.MakeVector` 0.0 0.0 (`self.FootTraceDistance`)))))
              (bind (_outhit _returnvalue) (`KismetSystemLibrary.LineTraceSingle` _output_get_4 _output_get_5 "TraceTypeQuery1"))
              (if _returnvalue
                (set `local.SoundLocation` (`.ImpactPoint` (`GameplayStatics.BreakHitResult` _outhit)))
                (else
                  (bind _output_get_6 (set `local.SoundLocation` _output_get_3))
                  (bind _output_get_7 (set `local.RandomVolume` (`KismetMathLibrary.RandomFloatInRange` (`self.VolumeMin`) (`self.VolumeMax`))))
                  (bind _output_get_8 (set `local.RandomPitch` (`KismetMathLibrary.RandomFloatInRange` (`self.PitchMin`) (`self.PitchMax`))))
                  (`GameplayStatics.SpawnSoundAtLocation` _selectedsound _output_get_6 (struct) _output_get_7 _output_get_8 0.0 (`self.AttenuationSettings`) (`self.ConcurrencySettings`))
                  (set `self.bLeftFootNext` (not (`self.bLeftFootNext`))))))))
        (:`Is Not Valid`
          (return))))
    (:`Is Not Valid`
      (return))))

(fn `UserConstructionScript`)