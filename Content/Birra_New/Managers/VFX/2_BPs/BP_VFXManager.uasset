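; BP_VFXManager is a Blueprint manager that spawns, tracks and stops Niagara effects defined in a VFX library.
; Location and attached spawns use a library lookup, currently fed "None" instead of the requested ID, then register components in ActiveVFX with tag, owner and looping data.
; Effects stop by component or by tag, and a reverse-index sweep prunes invalid or inactive entries after tag stops.
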(fn `ClearInvalidVFXRefs`
  (returns (RemovedCount :type Integer))
  (locals (LocalRemovedCount :type Integer) (LocalLastIndex :type Integer))
  (bind _activevfx (`self.ActiveVFX`))
  (set `local.LocalRemovedCount` 0)
  (bind _output_get (set `local.LocalLastIndex` (- (`KismetArrayLibrary.Array_Length` _activevfx) 1)))
  (if (>= _output_get 0)
    (for _index (range (+ _output_get 1))
      (bind _returnvalue (- _output_get _index))
      (bind (_output_vfx_id _output_vfxtag _output_niagaracomponentref) (break `/Game/Birra_New/Managers/VFX/3_Structs/ST_ActiveVFXData` (`|GetArrayItem` _activevfx _returnvalue)))
      (`/Engine/EditorBlueprintResources/StandardMacros.IsValid` _output_niagaracomponentref
        (:`Is Valid`
          (if (not (`ActorComponent.IsActive` _output_niagaracomponentref))
            (`KismetArrayLibrary.Array_Remove` _activevfx _returnvalue)
            (set `local.LocalRemovedCount` (+ (`local.LocalRemovedCount`) 1))))
        (:`Is Not Valid`
          (`KismetArrayLibrary.Array_Remove` _activevfx _returnvalue)
          (bind _output_get_2 (set `local.LocalRemovedCount` (+ (`local.LocalRemovedCount`) 1)))
          (return _output_get_2))))
    (else
      (return 0))))

(fn `FindVFXDataByID`
  (params (InVFX_ID :type Name))
  (returns (bFound :type Boolean) (OutVFXData :type "/Game/Birra_New/Managers/VFX/3_Structs/ST_VFXData Structure"))
  (for _array_element (`self.VFXLibrary`)
    (if (== (`.VFX_ID_4_A68A69974CEE54B673E6B98A5544C5F0` (break `/Game/Birra_New/Managers/VFX/3_Structs/ST_VFXData` _array_element)) InVFX_ID)
      (return true _array_element)))
  (return false))

(fn `RegisterActiveVFX`
  (params (InVFX_ID :type Name) (InVFXTag :type Name) (InNiagaraComponent :type "NiagaraComponent Object Reference") (InOwnerActor :type "Actor Object Reference") (bInLooping :type Boolean))
  (`/Engine/EditorBlueprintResources/StandardMacros.IsValid` InNiagaraComponent
    (:`Is Valid`
      (`KismetArrayLibrary.Array_Add` (`self.ActiveVFX`) (make `/Game/Birra_New/Managers/VFX/3_Structs/ST_ActiveVFXData` InVFX_ID InVFXTag InNiagaraComponent InOwnerActor bInLooping)))
    (:`Is Not Valid`
      (return))))

(fn `SpawnVFXAtLocation`
  (params (InVFX_ID :type Name) (InLocation :type "Vector Structure") (InRotation :type "Rotator Structure") (InScale :type "Vector Structure" :default (1.0 1.0 1.0)) (InTagOverride :type Name) (InOwnerActor :type "Actor Object Reference"))
  (returns (bSpawned :type Boolean) (OutNiagaraComponent :type "NiagaraComponent Object Reference"))
  (bind (_bfound _outvfxdata) (`self.FindVFXDataByID` "None"))
  (if _bfound
    (bind (_vfx_id _niagarasystem _blooping _bautodestroy _defaultlifetime _defaultscale _defaulttag) (break `/Game/Birra_New/Managers/VFX/3_Structs/ST_VFXData` _outvfxdata))
    (`/Engine/EditorBlueprintResources/StandardMacros.IsValid` _niagarasystem
      (:`Is Valid`
        (bind _returnvalue (`NiagaraFunctionLibrary.SpawnSystemAtLocation` _niagarasystem InLocation InRotation InScale _bautodestroy true "None" false))
        (if (== InTagOverride "None")
          (`self.RegisterActiveVFX` InVFX_ID _defaulttag _returnvalue InOwnerActor _blooping)
          (return false _returnvalue)
          (else
            (`self.RegisterActiveVFX` InVFX_ID InTagOverride _returnvalue InOwnerActor _blooping)
            (return false _returnvalue))))
      (:`Is Not Valid`
        (return false null)))
    (else
      (return false null))))

(fn `SpawnVFXAttached`
  (params (InVFX_ID :type Name) (InAttachToComponent :type "SceneComponent Object Reference") (InSocketName :type Name) (InRelativeLocation :type "Vector Structure") (InRelativeRotation :type "Rotator Structure") (InScale :type "Vector Structure" :default (1.0 1.0 1.0)) (InTagOverride :type Name) (InOwnerActor :type "Actor Object Reference"))
  (returns (bSpawned :type Boolean) (OutNiagaraComponent :type "NiagaraComponent Object Reference"))
  (`/Engine/EditorBlueprintResources/StandardMacros.IsValid` InAttachToComponent
    (:`Is Valid`
      (bind (_bfound _outvfxdata) (`self.FindVFXDataByID` "None"))
      (if _bfound
        (bind (_vfx_id _niagarasystem _blooping _bautodestroy _defaultlifetime _defaultscale _defaulttag) (break `/Game/Birra_New/Managers/VFX/3_Structs/ST_VFXData` _outvfxdata))
        (`/Engine/EditorBlueprintResources/StandardMacros.IsValid` _niagarasystem
          (:`Is Valid`
            (bind _returnvalue (`NiagaraFunctionLibrary.SpawnSystemAttached` _niagarasystem InAttachToComponent InSocketName InRelativeLocation InRelativeRotation "KeepRelativeOffset" _bautodestroy false))
            ; Alternativa para Node. O activate pode sair
            (`SceneComponent.SetRelativeScale3D` _returnvalue InScale)
            (`ActorComponent.Activate` _returnvalue false)
            (if (== InTagOverride "None")
              (`self.RegisterActiveVFX` InVFX_ID _defaulttag _returnvalue null _blooping)
              (return true null)
              (else
                (`self.RegisterActiveVFX` InTagOverride _defaulttag _returnvalue InOwnerActor _blooping)
                (return true null))))
          (:`Is Not Valid`
            (return false null)))
        (else
          (return false null))))
    (:`Is Not Valid`
      (return false null))))

(fn `StopAllVFXByTag`
  (params (InVFXTag :type Name))
  (returns (StoppedCount :type Integer))
  (locals (LocalStoppedCount :type Integer))
  (for _array_element (`self.ActiveVFX`)
    (if (== (`.VFXTag_11_A49743F94DA6B98270F39DADCDF4855E` (break `/Game/Birra_New/Managers/VFX/3_Structs/ST_ActiveVFXData` _array_element)) InVFXTag)
      (`/Engine/EditorBlueprintResources/StandardMacros.IsValid` (`.NiagaraComponentRef_12_D08840C74D8C06EA56498F99B7CF2BC1` (break `/Game/Birra_New/Managers/VFX/3_Structs/ST_ActiveVFXData` _array_element))
        (:`Is Valid`
          (`ActorComponent.Deactivate` (`.NiagaraComponentRef_12_D08840C74D8C06EA56498F99B7CF2BC1` (break `/Game/Birra_New/Managers/VFX/3_Structs/ST_ActiveVFXData` _array_element)))
          (set `local.LocalStoppedCount` (+ (`local.LocalStoppedCount`) 1))))))
  (`self.ClearInvalidVFXRefs`)
  (return (`local.LocalStoppedCount`)))

(fn `StopVFX`
  (params (InNiagaraComponent :type "NiagaraComponent Object Reference"))
  (returns (bStopped :type Boolean))
  (bind _activevfx (`self.ActiveVFX`))
  (`/Engine/EditorBlueprintResources/StandardMacros.IsValid` InNiagaraComponent
    (:`Is Valid`
      (`ActorComponent.Deactivate` InNiagaraComponent)
      (for (_array_element _array_index) _activevfx
        (if (== InNiagaraComponent (`.NiagaraComponentRef_12_D08840C74D8C06EA56498F99B7CF2BC1` (break `/Game/Birra_New/Managers/VFX/3_Structs/ST_ActiveVFXData` _array_element)))
          (`KismetArrayLibrary.Array_Remove` _activevfx _array_index)
          (break)))
      (return true))
    (:`Is Not Valid`
      (return false))))

(fn `UserConstructionScript`)