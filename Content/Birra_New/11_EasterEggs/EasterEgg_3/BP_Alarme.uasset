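; BP_Alarme is a rotating alarm light actor for an easter egg, switched on through the LigarAlarme event.
; LigarAlarme sets AlarmeAtivo and makes LuzAlarme visible, after which Tick yaws PivotRotacao at Velocidade scaled by delta time.
; When Randomizer is set, BeginPlay randomly reverses the spin direction by negating Velocidade.
; The Blueprint has no logic to switch the alarm back off.
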(event `self.ReceiveBeginPlay`
  (if (`self.Randomizer`)
    (if (`KismetMathLibrary.RandomBool`)
      (set `self.Velocidade` (* (`self.Velocidade`) -1.0)))))

(event `self.ReceiveTick`
  (params (DeltaSeconds :type "Float (single-precision)"))
  (if (`self.AlarmeAtivo`)
    (`SceneComponent.K2_AddLocalRotation` (`self.Pivot_Rotacao`) (`KismetMathLibrary.MakeRotator` 0.0 0.0 (* DeltaSeconds (`self.Velocidade`))) false false)))

(event `LigarAlarme`
  (set `self.AlarmeAtivo` true)
  (`SceneComponent.SetVisibility` (`self.Luz_Alarme`) true false))

(fn `UserConstructionScript`)