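; BP_EE_VideoMonitor is an easter egg monitor that plays a video on its screen mesh when externally triggered.
; PlayVideoFromTrigger checks playing, cooldown and play-once flags, then swaps slot 0 to the video material and opens the source.
; Media player callbacks start playback from opening and, at the end, restore the idle material and begin a timed cooldown.
; Those callbacks are bound only when UseAudio is true; otherwise BeginPlay just mutes the sound.
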(event `OnVideoOpened`
  (params (OpenedUrl :type String))
  (bind _mediaplayer (`self.MediaPlayer`))
  (`MediaPlayer.Seek` _mediaplayer (`KismetMathLibrary.MakeTimespan` 0))
  (`MediaPlayer.Play` _mediaplayer))

(event `self.ReceiveBeginPlay`
  (bind _mediaplayer (`self.MediaPlayer`))
  (bind _mediaplayer_2 (`self.MediaPlayer`))
  (bind _mediasound (`self.MediaSound`))
  (`PrimitiveComponent.SetMaterial` (`self.SM_Screen`) (`self.ScreenMaterialIndex`) (`self.IdleMaterial`))
  (`MediaPlayer.SetLooping` _mediaplayer false)
  (`MediaSoundComponent.SetMediaPlayer` (`self.MediaSound`) _mediaplayer)
  (if (`self.bUseAudio`)
    (`MediaSoundComponent.SetMediaPlayer` _mediasound _mediaplayer)
    (`SynthComponent.SetVolumeMultiplier` _mediasound (`self.AudioVolume`))
    (add `MediaPlayer.OnMediaOpened` _mediaplayer_2 (delegate `OnVideoOpened`))
    (add `MediaPlayer.OnEndReached` _mediaplayer_2 (delegate `OnVideoFinished`))
    (else
      (`SynthComponent.SetVolumeMultiplier` _mediasound 0.0))))

(event `OnVideoFinished`
  (`self.StopVideo`))

(event `PlayVideoFromTrigger`
  (if (`self.bIsPlayingVideo`)
    _
    (elif (`self.bOnCooldown`)
      _
      (elif (not (and (`self.bPlayOnlyOnce`) (`self.bHasPlayed`)))
        (set `self.bIsPlayingVideo` true)
        (set `self.bHasPlayed` true)
        (`PrimitiveComponent.SetMaterial` (`self.SM_Screen`) 0 (`self.VideoMaterial`))
        (`MediaPlayer.OpenSource` (`self.MediaPlayer`) (`self.MediaSource`))))))

(event `StopVideo`
  (`MediaPlayer.Pause` (`self.MediaPlayer`))
  (`PrimitiveComponent.SetMaterial` (`self.SM_Screen`) (`self.ScreenMaterialIndex`) (`self.IdleMaterial`))
  (set `self.bIsPlayingVideo` false)
  (set `self.bOnCooldown` true)
  (bind _returnvalue (`KismetSystemLibrary.K2_SetTimerDelegate` (delegate `ResetVideoCooldown`) (`self.CooldownAfterPlay`)))
  (set `self.CooldownTimerHandle` _returnvalue))

(event `ResetVideoCooldown`
  (set `self.bOnCooldown` false))

(fn `UserConstructionScript`)