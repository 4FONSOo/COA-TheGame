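; One-shot Easter egg intercom that lets the player play a recording with E while inside its trigger.
; Overlap toggles input and a widget prompt, which stays hidden once played.
; A delay-chained sequence drives Voice, Static and FX audio through system message, game over line, static burst, power down and distant bang, then sets the panel material.
; A looping timer randomly flickers a red point light until the burst.
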(event `self.ReceiveBeginPlay`
  (bind _prompt (`self.Prompt`))
  (bind _asbp_resident_horror_v1 (cast `/Game/ChildrenOfAndromeda/Character/BP_Character/BP_Resident_HorrorV1` (`GameplayStatics.GetPlayerCharacter` 0)))
  (set `self.PlayerRef` _asbp_resident_horror_v1)
  (`SceneComponent.SetVisibility` _prompt false false)
  (bind _aswbp_ee2_interact_prompt (cast `/Game/Birra_New/11_EasterEggs/EasterEgg_2/WBP_EE2_InteractPrompt` (`WidgetComponent.GetUserWidgetObject` _prompt)))
  (`/Game/Birra_New/11_EasterEggs/EasterEgg_2/WBP_EE2_InteractPrompt.SetPromptText` _aswbp_ee2_interact_prompt "PLAY RECORDING")
  (`/Game/Birra_New/11_EasterEggs/EasterEgg_2/WBP_EE2_InteractPrompt.SetKeyText` _aswbp_ee2_interact_prompt "E")
  (`LightComponent.SetIntensity` (`self.PointLight_Red`) 0.0)
  (`AudioComponent.Stop` (`self.Voice`))
  (`AudioComponent.Stop` (`self.Static`))
  (`AudioComponent.Stop` (`self.FX`))
  (set `self.bPlayerInside` false)
  (set `self.bAlreadyPlayed` false)
  (set `self.bSequenceRunning` false)
  (set `self.bFlickerActive` false))

(event `self.InteractionTrigger.OnComponentBeginOverlap`
  (params (OverlappedComponent :type "PrimitiveComponent Object Reference") (OtherActor :type "Actor Object Reference") (OtherComp :type "PrimitiveComponent Object Reference") (OtherBodyIndex :type Integer) (bFromSweep :type Boolean) (SweepResult :type "HitResult Structure (by ref)"))
  (bind _prompt (`self.Prompt`))
  (if (== OtherActor (`self.PlayerRef`))
    (bind _output_get (set `self.PlayerControllerRef` (`GameplayStatics.GetPlayerController` 0)))
    (set `self.bPlayerInside` true)
    (if (`self.bAlreadyPlayed`)
      (`SceneComponent.SetVisibility` _prompt false false)
      (`self.EnableInput` _output_get)
      (`KismetSystemLibrary.PrintString` "EE2 ALREADY PLAYED - PROMPT HIDDEN")
      (else
        (`SceneComponent.SetHiddenInGame` _prompt false false)
        (`SceneComponent.SetVisibility` _prompt true false)
        (bind _aswbp_ee2_interact_prompt (cast `/Game/Birra_New/11_EasterEggs/EasterEgg_2/WBP_EE2_InteractPrompt` (`WidgetComponent.GetUserWidgetObject` _prompt)))
        (`/Game/Birra_New/11_EasterEggs/EasterEgg_2/WBP_EE2_InteractPrompt.SetPromptText` _aswbp_ee2_interact_prompt "PLAY RECORDING")
        (`/Game/Birra_New/11_EasterEggs/EasterEgg_2/WBP_EE2_InteractPrompt.SetKeyText` _aswbp_ee2_interact_prompt "E")
        (`self.EnableInput` _output_get)
        (`KismetSystemLibrary.PrintString` "EE2 Prompt Show")))))

(event `self.InteractionTrigger.OnComponentEndOverlap`
  (params (OverlappedComponent :type "PrimitiveComponent Object Reference") (OtherActor :type "Actor Object Reference") (OtherComp :type "PrimitiveComponent Object Reference") (OtherBodyIndex :type Integer))
  (if (== OtherActor (`self.PlayerRef`))
    (set `self.bPlayerInside` false)
    (`SceneComponent.SetVisibility` (`self.Prompt`) false false)
    (`self.DisableInput` (stale `self.InteractionTrigger.OnComponentBeginOverlap` _output_get))))

(event `Key|E`
  (params (Key :type "Key Structure"))
  (:`Pressed`
    (if (`self.bPlayerInside`)
      (if (`self.bAlreadyPlayed`)
        _
        (elif (not (`self.bSequenceRunning`))
          (`self.CE_StartIntercomSequence`)
          (`SceneComponent.SetVisibility` (`self.Prompt`) false false))))))

(event `CE_StartIntercomSequence`
  (bind _fx (`self.FX`))
  (bind _static (`self.Static`))
  (bind _fx_2 (`self.FX`))
  (bind _voice (`self.Voice`))
  (bind _fx_3 (`self.FX`))
  (bind _fx_4 (`self.FX`))
  (set `self.bSequenceRunning` true)
  (set `self.bAlreadyPlayed` true)
  (`SceneComponent.SetVisibility` (`self.Prompt`) false false)
  (`AudioComponent.SetSound` _fx (`self.SFX_ButtonClick`))
  (`AudioComponent.Play` _fx 0.0)
  (`self.CE_StartRedFlicker`)
  (`KismetSystemLibrary.Delay` (`self.Delay_AfterClick`))
  (`AudioComponent.SetSound` _static (`self.SFX_StaticLoop`))
  (`AudioComponent.Play` _static 0.0)
  (`AudioComponent.SetSound` _fx_2 (`self.SFX_Beep`))
  (`AudioComponent.Play` _fx_2 0.0)
  (`KismetSystemLibrary.Delay` (`self.Delay_BeforeSystemMessage`))
  (`AudioComponent.SetSound` _voice (`self.VO_SystemMessage`))
  (`AudioComponent.Play` _voice 0.0)
  (`KismetSystemLibrary.Delay` (`self.SystemMessageDuration`))
  (`KismetSystemLibrary.Delay` (`self.Delay_BeforeGameOver`))
  (`AudioComponent.SetSound` _voice (`self.VO_GameOver`))
  (`AudioComponent.Play` _voice 0.0)
  (`KismetSystemLibrary.Delay` (`self.GameOverDuration`))
  (`KismetSystemLibrary.Delay` (`self.Delay_BeforeStaticBurst`))
  (`AudioComponent.Stop` (`self.Static`))
  (`AudioComponent.SetSound` _fx_3 (`self.SFX_StaticBurst`))
  (`AudioComponent.Play` _fx_3 0.0)
  (`self.CE_StopRedFlicker`)
  (`LightComponent.SetIntensity` (`self.PointLight_Red`) 0.0)
  (`AudioComponent.SetSound` _fx_4 (`self.SFX_PowerDown`))
  (`AudioComponent.Play` _fx_4 0.0)
  (`KismetSystemLibrary.Delay` (`self.Delay_BeforeDistantBang`))
  (`AudioComponent.SetSound` _fx_4 (`self.SFX_DistantBang`))
  (`AudioComponent.Play` _fx_4 0.0)
  (`PrimitiveComponent.SetMaterial` (`self.IntercomPanel`) 0 null)
  (set `self.bSequenceRunning` false))

(event `CE_StartRedFlicker`
  (set `self.bFlickerActive` true)
  (bind _returnvalue (`KismetSystemLibrary.K2_SetTimerDelegate` (delegate `CE_FlickerTick`) (`self.FlickerInterval`) true))
  (set `self.FlickerTimerHandle` _returnvalue))

(event `CE_FlickerTick`
  (bind _pointlight_red (`self.PointLight_Red`))
  (if (`self.bFlickerActive`)
    (if (< (`KismetMathLibrary.RandomFloatInRange` 0.0) (`self.FlickerChanceOff`))
      (`LightComponent.SetIntensity` _pointlight_red 0.0)
      (else
        (`LightComponent.SetIntensity` _pointlight_red (`KismetMathLibrary.RandomFloatInRange` (`self.FlickerMinIntensity`) (`self.FlickerMaxIntensity`)))))
    (else
      (`LightComponent.SetIntensity` _pointlight_red 0.0))))

(event `CE_StopRedFlicker`
  (set `self.bFlickerActive` false)
  (`KismetSystemLibrary.K2_ClearAndInvalidateTimerHandle` (`self.FlickerTimerHandle`))
  (`LightComponent.SetIntensity` (`self.PointLight_Red`) 0.0))

(fn `UserConstructionScript`)