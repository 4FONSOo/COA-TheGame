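; Replicated health component that gives its owning actor health, damage, healing, death and an optional player HUD.
; Authority-gated Interaction functions change health, with server-to-multicast events and RepNotifies driving event dispatchers for other Blueprints.
; At zero health the client removes its HUD and requests respawn from the server.
; Unless custom respawn is set, player pawns respawn at a random PlayerStart and get repossessed, optionally after a delayed multicast ragdoll.
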(event `self.ReceiveBeginPlay`
  ;[0 0 0] Will be fired once the component is activated
  (`KismetSystemLibrary.Delay` 0.2)
  (if (`self.Locally Controlled`)
    (`self.Server: Initiate Component`)
    (`self.Initiate Component`
      (:`Out`
        (`self.On Component Initialized`)
        (`self.Create User Widget`)))))

(event `self.ReceiveEndPlay`
  (params (EndPlayReason :type "EEndPlayReason Enum" :default "Destroyed"))
  ;[0 0 0] When component ends play
  (`self.On Component End Play`))

(event `Default`)

(event `Server: Initiate Component`
  ;[0 0 0] Replicated Dispatchers
  ;;[1 0 0.8607] Initates the component on server
  (`self.Initiate Component`))

(event `Server: Damage Received Dispatcher`
  ;[0 0 0] Replicated Dispatchers
  ;;[1 0 0.8627] Damage Received Dispatcher
  (`self.Multi: Damage Received Dispatcher`))

(event `Server: On Health Added Dispatcher`
  ;[0 0 0] Replicated Dispatchers
  ;;[1 0 0.8627] Health Added Dispatcher
  (`self.Multi: On Health Added Dispatcher`))

(event `Server: On Health Restored Dispatcher`
  ;[0 0 0] Replicated Dispatchers
  ;;[1 0 0.8627] Health Restored Dispatcher
  (`self.Multi: On Health Restored Dispatcher`))

(event `Server: On Owner Killed Dispatcher`
  ;[0 0 0] Replicated Dispatchers
  ;;[1 0 0.8627] On Owner Killed Dispatcher
  (`self.Multi: On Owner Killed Dispatcher`))

(event `Multi: Damage Received Dispatcher`
  ;[0 0 0] Replicated Dispatchers
  ;;[1 0 0.8627] Damage Received Dispatcher
  (`self.On Damage Received`))

(event `Multi: On Health Added Dispatcher`
  ;[0 0 0] Replicated Dispatchers
  ;;[1 0 0.8627] Health Added Dispatcher
  (`self.On Health Added`))

(event `Multi: On Health Restored Dispatcher`
  ;[0 0 0] Replicated Dispatchers
  ;;[1 0 0.8627] Health Restored Dispatcher
  (`self.On Health Restored`))

(event `Multi: On Owner Killed Dispatcher`
  ;[0 0 0] Replicated Dispatchers
  ;;[1 0 0.8627] On Owner Killed Dispatcher
  (`self.On Owner Killed`))

(event `Client: Kill Owner`
  (bind _hud_widget_reference (`self.HUD Widget Reference`))
  ;[0 0 0] Kill & Respawn Logic
  ;;[1 0 0.8627] First Remove HUD widget as client then start kill logic
  (`/Engine/EditorBlueprintResources/StandardMacros.IsValid` _hud_widget_reference
    (:`Is Valid`
      (`Widget.RemoveFromParent` _hud_widget_reference))
    (:`Is Not Valid`
      _))
  (`self.Server: Respawn`))

(event `Server: Respawn`
  ;[0 0 0] Kill & Respawn Logic
  ;;[1 0 0.8627] Check if no custom spawn logic should be used
  (if (not (`.CustomRespawn_8_A282399F433FE071C6A8CBB4A317851F` (break `/Game/RHS/Blueprints/Struct/Component_Related/ST_RHSS` (`self.Component Settings`))))
    ;;[1 0 0.8627] Check if owner controller can be obtained
    (if (`.Success` (`self.Get Owner Controller`))
      ;;[1 0 0.8627] Check if ragdoll should be used
      (if (not (`.Ragdoll_12_FCCE27A14EA511DF349C949EFFF80A61` (break `/Game/RHS/Blueprints/Struct/Component_Related/ST_RHSS` (`self.Component Settings`))))
        ;;[1 0 0.8627] Get random Player start as new spawn
        (bind _outactors (`GameplayStatics.GetAllActorsOfClass` "/Script/Engine.PlayerStart" :!label _label))
        ;;[1 0 0.8627] Spawn new at given transform
        (bind _returnvalue (`|SpawnActorFromClass` (`GameplayStatics.GetObjectClass` (`self.GetOwner`)) (`Actor.GetTransform` (`KismetArrayLibrary.Array_Random` _outactors)) "AdjustIfPossibleButAlwaysSpawn" "OverrideRootScale" null null))
        ;;[1 0 0.8627] Make controller of this owner possess new
        (bind _aspawn (cast `Pawn` _returnvalue))
        (`Controller.Possess` (`self.Get Owner Controller`) _aspawn)
        ;;[1 0 0.8627] Destroy owner
        (`Actor.K2_DestroyActor` (`self.GetOwner`))
        (else
          ;;[1 0 0.8627] Play ragdoll death animation
          (`|ExecutionSequence`
            (:`then_0`
              (`KismetSystemLibrary.Delay` 7.0)
              (goto _label))
            (:`then_1`
              (`self.Multi: Ragdoll Death`))))))))

(event `Multi: Ragdoll Death`
  ;[0 0 0] Kill & Respawn Logic
  ;;[1 0 0.8627] Simulate a ragdoll on character (Replicate to all)
  (if (`.Ragdoll_12_FCCE27A14EA511DF349C949EFFF80A61` (break `/Game/RHS/Blueprints/Struct/Component_Related/ST_RHSS` (`self.Component Settings`)))
    (bind _ascharacter (cast `Character` (`self.GetOwner`)))
    (`PrimitiveComponent.SetSimulatePhysics` (`Character.Mesh` _ascharacter) true)
    (`CharacterMovementComponent.DisableMovement` (`Character.CharacterMovement` _ascharacter))))

(fn `Bundle Component Data`
  (returns (Output_Get :type "/Game/RHS/Blueprints/Struct/Component_Related/ST_RHSD Structure"))
  (locals (RHSD :type "/Game/RHS/Blueprints/Struct/Component_Related/ST_RHSD Structure"))
  ;[0 0 0] Bundles the most important component data into a data bundle that you can use later. For example, if you want to save player health values between sessions. Is supposed to be called from the outside.
  (bind _output_get (set `local.RHSD` (make `/Game/RHS/Blueprints/Struct/Component_Related/ST_RHSD` (`self.Component Settings`) (`self.Maximal Health`) (`self.Current Health`))))
  (return _output_get))

(fn `Get Owner Controller`
  (returns (Controller :type "Controller Object Reference") (Success :type Boolean))
  ;[0 0 0] Returns the controller of the current owner (if owner is pawn)
  (if (`.IsPlayer?_5_965A17F34B0A3900D62C5BA3E36E2BB9` (break `/Game/RHS/Blueprints/Struct/Component_Related/ST_RHSS` (`self.Component Settings`)))
    (bind _aspawn (cast `Pawn` (`self.GetOwner`))
      (:`then`
        (return (`Pawn.GetController` _aspawn) true))
      (:`CastFailed`
        (return null false)))
    (else
      (return null false))))

(fn `Interaction: Add Health`
  (params (Health :type "Float (double-precision)"))
  ;[0 0 0] Increase the owners health. Is intended to be called from outside. Dont use inside of component.
  (`/Engine/EditorBlueprintResources/ActorComponentMacros.Switch Has Authority`
    (:`Authority`
      (`self.Increase Owner Health` Health
        (:`Out`
          (`self.Server: On Health Added Dispatcher`)
          (return))))))

(fn `Interaction: Apply Damage`
  (params (Damage :type "Float (double-precision)"))
  ;[0 0 0] Decrease the owners health. Is intended to be called from outside. Dont use inside of component.
  (`/Engine/EditorBlueprintResources/ActorComponentMacros.Switch Has Authority`
    (:`Authority`
      (`self.Decrease Owner Health` Damage
        (:`Out`
          (`self.Server: Damage Received Dispatcher`)
          (return))))))

(fn `Interaction: Instant Kill`
  ;[0 0 0] Instantly kills the owner of this component. Is intended to be called from outside. Dont use inside of component.
  (`/Engine/EditorBlueprintResources/ActorComponentMacros.Switch Has Authority`
    (:`Authority`
      (`self.Decrease Owner Health` (`self.Current Health`)
        (:`Out`
          (return))))))

(fn `Interaction: Restore Health`
  ;[0 0 0] Restore the owners health. Will fill the owners health to 100% immediatly. Is intended to be called from outside. Dont use inside of component.
  (`/Engine/EditorBlueprintResources/ActorComponentMacros.Switch Has Authority`
    (:`Authority`
      (`self.Increase Owner Health` (`self.Maximal Health`)
        (:`Out`
          (`self.Server: On Health Restored Dispatcher`)
          (return))))))

(fn `Locally Controlled`
  (returns (ReturnValue :type Boolean))
  (bind _instigator (`Actor.Instigator` (`self.GetOwner`)))
  ;[0 0 0] Essentially gets the instigator of the pawn that owns this component and returns if the pawn is controlled by a local machine. If the instigator is not valid for any reason, it will return false.
  (`/Engine/EditorBlueprintResources/StandardMacros.IsValid` _instigator
    (:`Is Valid`
      (return (`Pawn.IsLocallyControlled` _instigator)))
    (:`Is Not Valid`
      (return false))))

(fn `OnRep_Current Health`
  (`self.On Health Data Changed`))

(fn `OnRep_Dead`)

(fn `OnRep_HUD Widget Reference`)

(fn `OnRep_Maximal Health`
  (`self.On Health Data Changed`))

(fn `Return Death State`
  (returns (Dead :type Boolean))
  ;[0 0 0] Returns the "Dead" state of this component. Should be used from the outside to retain information, since dead var is private.
  (return (`self.Dead`)))

(fn `Return Health Data`
  (returns (`Maximal Health` :type "Float (double-precision)") (`Current Health` :type "Float (double-precision)"))
  ;[0 0 0] Returns the health values. Function is intended to be used by third party blueprints, trying to access the component from the outside.
  (return (`self.Maximal Health`) (`self.Current Health`)))

(fn `Return Percentage`
  (returns (Percentage :type "Float (double-precision)"))
  ;[0 0 0] Returns the current health percentage
  (return (`KismetMathLibrary.FClamp` (/ (`self.Current Health`) (`self.Maximal Health`)))))