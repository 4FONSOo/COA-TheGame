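; BP_EmergencyLight is an emergency light actor that blinks a light and switches BP_Alarme alarms on and off.
; BeginPlay adds the Alarme01 child actor to the Alarmes array, which LigarEmergencyLights and DesligarAlarmes loop over.
; Separately, StartEmergencyLight sets a looping timer that toggles EmergencyLight visibility.
; StopEmergencyLight hides the light and clears the active flag but never clears that timer.
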(event `self.ReceiveBeginPlay`
  (bind _asbp_alarme (cast `/Game/Birra_New/11_EasterEggs/EasterEgg_3/BP_Alarme` (`ChildActorComponent.ChildActor` (`self.Alarme_01`))))
  (`KismetArrayLibrary.Array_Add` (`self.Alarmes`) _asbp_alarme))

(event `LigarEmergencyLights`
  (for _array_element (`self.Alarmes`)
    (`/Engine/EditorBlueprintResources/StandardMacros.IsValid` _array_element
      (:`Is Valid`
        (`/Game/Birra_New/11_EasterEggs/EasterEgg_3/BP_Alarme.LigarAlarme` _array_element)))))

(event `DesligarAlarmes`
  (for _array_element (`self.Alarmes`)
    (`/Engine/EditorBlueprintResources/StandardMacros.IsValid` _array_element
      (:`Is Valid`
        (`/Game/Birra_New/11_EasterEggs/EasterEgg_3/BP_Alarme.DesligarAlarme` _array_element)))))

(event `StartEmergencyLight`
  (if (not (`self.bEmergencyActive`))
    (set `self.bEmergencyActive` true)
    (`KismetSystemLibrary.K2_SetTimerDelegate` (delegate `BlinkEmergencyLight`) (`self.BlinkInterval`) true)))

(event `BlinkEmergencyLight`
  (if (`self.bEmergencyActive`)
    (bind _output_get (set `self.bLightVisible` (not (`self.bLightVisible`))))
    (`SceneComponent.SetVisibility` (`self.EmergencyLight`) _output_get false)))

(event `StopEmergencyLight`
  (set `self.bEmergencyActive` false)
  (set `self.bLightVisible` false)
  (`SceneComponent.SetVisibility` (`self.EmergencyLight`) false false))

(fn `UserConstructionScript`)