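; Exterior door actor that slides its mesh between closed and open positions, with audio on each OpenDoor or CloseDoor.
; An IsOpen flag guards both events, which play the TL_OpenExteriorDoor timeline forward or in reverse to lerp the mesh's relative location.
; BeginPlay caches the closed location, adds OpenOffset to OpenLocation's own value rather than the closed location, and also plays the timeline without changing IsOpen.
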(event `self.ReceiveBeginPlay`
  (bind _output_get (set `self.ClosedLocation` (`SceneComponent.RelativeLocation` (`self.DoorMesh`))))
  (bind _output_get_2 (set `self.OpenLocation` (+ (`self.OpenLocation`) (`self.OpenOffset`))))
  (bind (_direction _alpha) (`Timeline|TL_OpenExteriorDoor` :!label _label)
    (:`Update`
      (`SceneComponent.K2_SetRelativeLocation` (`self.DoorMesh`) (`KismetMathLibrary.VLerp` _output_get _output_get_2 _alpha) false false))))

(event `OpenDoor`
  (if (not (`self.bIsOpen`))
    (set `self.bIsOpen` true)
    (`AudioComponent.Play` (`self.ExteriorDoorAudio`) 0.0)
    (goto _label :!via `PlayFromStart`)))

(event `CloseDoor`
  (if (`self.bIsOpen`)
    (set `self.bIsOpen` false)
    (`AudioComponent.Play` (`self.ExteriorDoorAudio`) 0.0)
    (goto _label :!via `ReverseFromEnd`)))

(fn `UserConstructionScript`)