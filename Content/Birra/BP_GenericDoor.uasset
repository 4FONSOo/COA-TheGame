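; BP_GenericDoor is a sliding door actor that other logic opens and closes through the OpenDoor and CloseDoor events.
; BeginPlay takes the placed mesh position as open, derives the closed position from ClosedOffset, and plays the close timeline.
; The timeline lerps the mesh's relative location, running forward to close and reversed to open.
; IsClosed guards against repeated calls, and both directions play the same audio component.
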(event `self.ReceiveBeginPlay`
  (set `self.OpenLocation` (`SceneComponent.RelativeLocation` (`self.DoorMesh`)))
  (bind _output_get (set `self.ClosedLocation` (+ (`self.OpenLocation`) (`self.ClosedOffset`))))
  (bind (_direction _alpha) (`Timeline|TL_CloseDoor` :!label _label)
    (:`Update`
      (`SceneComponent.K2_SetRelativeLocation` (`self.DoorMesh`) (`KismetMathLibrary.VLerp` (`self.OpenLocation`) _output_get _alpha) false false))))

(event `CloseDoor`
  (if (not (`self.bIsClosed`))
    (set `self.bIsClosed` true)
    (`AudioComponent.Play` (`self.DoorCloseAudio`) 0.0)
    (goto _label :!via `PlayFromStart`)))

(event `OpenDoor`
  (if (`self.bIsClosed`)
    (set `self.bIsClosed` false)
    (`AudioComponent.Play` (`self.DoorCloseAudio`) 0.0)
    (goto _label :!via `ReverseFromEnd`)))

(fn `UserConstructionScript`)