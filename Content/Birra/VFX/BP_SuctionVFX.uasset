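; BP_SuctionVFX is an actor that plays a Niagara suction effect aimed at a target location.
; StartVFX rotates the actor to look at the target with yaw flipped 180 degrees, and activates the Niagara component only if it is not already active.
; StopVFX deactivates it, and the effect starts switched off on BeginPlay, with a VFXActive flag tracking its state.
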(event `self.ReceiveBeginPlay`
  (set `self.bVFXActive` false)
  (`ActorComponent.Deactivate` (`self.SuctionNiagara`)))

(event `StartVFX`
  (params (TargetLocation :type "Vector Structure"))
  (`self.K2_SetActorRotation` (`KismetMathLibrary.MakeRotator` (.roll (`KismetMathLibrary.FindLookAtRotation` (`self.K2_GetActorLocation`) TargetLocation)) (.pitch (`KismetMathLibrary.FindLookAtRotation` (`self.K2_GetActorLocation`) TargetLocation)) (+ (.yaw (`KismetMathLibrary.FindLookAtRotation` (`self.K2_GetActorLocation`) TargetLocation)) 180.0)))
  (if (not (`self.bVFXActive`))
    (set `self.bVFXActive` true)
    (`ActorComponent.Activate` (`self.SuctionNiagara`) true)))

(event `StopVFX`
  (set `self.bVFXActive` false)
  (`ActorComponent.Deactivate` (`self.SuctionNiagara`)))

(fn `UserConstructionScript`)