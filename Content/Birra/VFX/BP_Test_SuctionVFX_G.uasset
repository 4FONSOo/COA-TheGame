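; Test actor for previewing a suction Niagara effect on a key press.
; On BeginPlay it deactivates the TestNiagara component and prints a ready message.
; Pressing G restarts the effect with a reset and sets VFXPlaying.
; When AutoStop is set, it deactivates the effect after TestDuration, printing debug messages along the way.
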(event `self.ReceiveBeginPlay`
  (set `self.bVFXPlaying` false)
  (`ActorComponent.Deactivate` (`self.TestNiagara`))
  (`KismetSystemLibrary.PrintString` "BP VFX TEST READY - PRESS G"))

(event `Key|G`
  (params (Key :type "Key Structure"))
  (bind _testniagara (`self.TestNiagara`))
  (:`Pressed`
    (`KismetSystemLibrary.PrintString` "Pressed")
    (`ActorComponent.Deactivate` _testniagara)
    (`ActorComponent.Activate` _testniagara true)
    (set `self.bVFXPlaying` true)
    (if (`self.bAutoStop`)
      (`KismetSystemLibrary.Delay` (`self.TestDuration`))
      (`ActorComponent.Deactivate` _testniagara)
      (`KismetSystemLibrary.PrintString` "VFX STOPPED"))))

(fn `UserConstructionScript`)