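; Short-lived Tron-style beam actor that draws a straight beam between two world points and expires after BeamLifetime.
; On BeginPlay, BuildBeam moves the actor to BeamStartWorld and lays a two-point linear spline to BeamEndWorld in local space.
; Core and glow spline meshes stretch cylinders along that line with separate materials and scales.
; InitBeam is an empty stub, and the glow uses GlowStartScale at both ends.
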(event `self.ReceiveBeginPlay`
  (`self.BuildBeam`)
  (`self.SetLifeSpan` (`self.BeamLifetime`)))

(fn `BuildBeam`
  (bind _returnvalue (`KismetMathLibrary.MakeVector` 0.0))
  (bind _beamspline (`self.BeamSpline`))
  (bind _coresplinemesh (`self.CoreSplineMesh`))
  (bind _corestartscale (`self.CoreStartScale`))
  (bind _coreendscale (`self.CoreEndScale`))
  (bind _glowsplinemesh (`self.GlowSplineMesh`))
  (bind _glowstartscale (`self.GlowStartScale`))
  (bind _glowstartscale_2 (`self.GlowStartScale`))
  (bind _returnvalue_2 (`KismetMathLibrary.InverseTransformLocation` (`self.GetTransform`) (`self.BeamEndWorld`)))
  (bind _returnvalue_3 (- _returnvalue_2 _returnvalue))
  (`self.K2_SetActorLocation` (`self.BeamStartWorld`))
  (`SplineComponent.ClearSplinePoints` _beamspline true)
  (`SplineComponent.AddSplinePoint` _beamspline _returnvalue "Local" true)
  (`SplineComponent.AddSplinePoint` _beamspline _returnvalue_2 "Local" true)
  (`SplineComponent.SetSplinePointType` _beamspline 0 "Linear" false)
  (`SplineComponent.SetSplinePointType` _beamspline 1 "Linear" false)
  (`SplineComponent.UpdateSpline` _beamspline)
  (`StaticMeshComponent.SetStaticMesh` _coresplinemesh "/Game/LevelPrototyping/Meshes/SM_Cylinder.SM_Cylinder")
  (`PrimitiveComponent.SetMaterial` _coresplinemesh 0 "/Game/Birra/TronOLD/M_TronBeam_Core3D.M_TronBeam_Core3D")
  (`SplineMeshComponent.SetForwardAxis` _coresplinemesh "Z" true)
  (`SplineMeshComponent.SetStartAndEnd` _coresplinemesh _returnvalue _returnvalue_3 _returnvalue_2 _returnvalue_3 true)
  (`SplineMeshComponent.SetStartScale` _coresplinemesh (`KismetMathLibrary.MakeVector2D` _corestartscale _corestartscale) true)
  (`SplineMeshComponent.SetEndScale` _coresplinemesh (`KismetMathLibrary.MakeVector2D` _coreendscale _coreendscale) true)
  (`StaticMeshComponent.SetStaticMesh` _glowsplinemesh "/Game/LevelPrototyping/Meshes/SM_Cylinder.SM_Cylinder")
  (`PrimitiveComponent.SetMaterial` _glowsplinemesh 0 "/Game/Birra/TronOLD/M_TronBeam_Glow3D.M_TronBeam_Glow3D")
  (`SplineMeshComponent.SetForwardAxis` _glowsplinemesh "Z" true)
  (`SplineMeshComponent.SetStartAndEnd` _glowsplinemesh _returnvalue _returnvalue_3 _returnvalue_2 _returnvalue_3 true)
  (`SplineMeshComponent.SetStartScale` _glowsplinemesh (`KismetMathLibrary.MakeVector2D` _glowstartscale _glowstartscale) true)
  (`SplineMeshComponent.SetEndScale` _glowsplinemesh (`KismetMathLibrary.MakeVector2D` _glowstartscale_2 _glowstartscale_2) true))

(fn `InitBeam`
  (params (StartLocation :type "Vector Structure") (EndLocation :type "Vector Structure")))

(fn `UserConstructionScript`)