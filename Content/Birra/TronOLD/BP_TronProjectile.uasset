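; BP_TronProjectile is a projectile actor with a Niagara visual and a five-second lifespan.
; On a sphere collision hit, it spawns the Tron impact effect aligned to the surface normal and plays an optional pitch-randomized, attenuated sound.
; It then stops movement, disables collision and deactivates its Niagara component.
; The trailing Delay leads nowhere and DestroyActor is unconnected, so only the lifespan removes the actor.
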(event `self.ReceiveBeginPlay`
  (`self.SetLifeSpan` 5.0))

(event `self.Sphere Collision.OnComponentHit`
  (params (HitComponent :type "PrimitiveComponent Object Reference") (OtherActor :type "Actor Object Reference") (OtherComp :type "PrimitiveComponent Object Reference") (NormalImpulse :type "Vector Structure") (Hit :type "HitResult Structure (by ref)"))
  (bind (_bblockinghit _binitialoverlap _time _distance _location _impactpoint _normal) (`GameplayStatics.BreakHitResult` Hit))
  (bind _impactsound (`self.ImpactSound`))
  (`NiagaraFunctionLibrary.SpawnSystemAtLocation` "/Game/Birra/TronOLD/NS_TronImpact.NS_TronImpact" _location (`KismetMathLibrary.MakeRotFromX` _normal))
  (`/Engine/EditorBlueprintResources/StandardMacros.IsValid` _impactsound
    (:`Is Valid`
      (`GameplayStatics.PlaySoundAtLocation` _impactsound _impactpoint (struct) (`self.ImpactVolume`) (`KismetMathLibrary.RandomFloatInRange` (`self.ImpactPitchMin`) (`self.ImpactPitchMax`)) 0.0 "/Game/Birra/TronOLD/ATT_TronImpact.ATT_TronImpact" null null null))
    (:`Is Not Valid`
      _))
  (`MovementComponent.StopMovementImmediately` (`self.ProjectileMovement`))
  (`PrimitiveComponent.SetCollisionEnabled` (`self.Sphere Collision`) "NoCollision")
  (`ActorComponent.Deactivate` (`self.Niagara System`))
  (`KismetSystemLibrary.Delay` 2.0))

(fn `UserConstructionScript`)