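; BP_GenericAlarm is an alarm actor with a light and an audio component that switches itself on shortly after play begins.
; BeginPlay hides the light and silences the audio, then calls StartAlarm after a fixed delay.
; StartAlarm, guarded by an active flag, plays the audio and sets a looping timer that toggles the light's visibility at BlinkInterval.
; The file contains no logic to stop the alarm.
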(event `self.ReceiveBeginPlay`
  (`SceneComponent.SetVisibility` (`self.AlarmLight`) false false)
  (`AudioComponent.Stop` (`self.AlarmAudio`))
  (set `self.bAlarmActive` false)
  (set `self.bLightVisible` false)
  (`KismetSystemLibrary.Delay` 5.0)
  (`self.StartAlarm`))

(event `StartAlarm`
  (if (not (`self.bAlarmActive`))
    (set `self.bAlarmActive` true)
    (`AudioComponent.Play` (`self.AlarmAudio`) 0.0)
    (`KismetSystemLibrary.K2_SetTimerDelegate` (delegate `BlinkAlarmLight`) (`self.BlinkInterval`) true)))

(event `BlinkAlarmLight`
  (bind _output_get (set `self.bLightVisible` (not (`self.bLightVisible`))))
  (`SceneComponent.SetVisibility` (`self.AlarmLight`) _output_get false))

(fn `UserConstructionScript`)