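; Player-operated CCTV terminal for a horror game: inside its box, E switches the view to security cameras with a CRT overlay and camera-list HUD.
; Keys cycle or pick online cameras and pan, tilt or zoom them, pausing the selected camera's surveillance.
; A random timer arms a jump scare that spawns an alien before the viewed camera, plays static, knocks that camera offline permanently and auto-exits the terminal.
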(event `self.ReceiveBeginPlay`
  (bind _output_get (set `self.PCRef` (`GameplayStatics.GetPlayerController` 0)))
  (bind _asbp_resident_horror_v1 (cast `/Game/ChildrenOfAndromeda/Character/BP_Character/BP_Resident_HorrorV1` (`GameplayStatics.GetPlayerCharacter` 0)))
  (set `self.PlayerRef` _asbp_resident_horror_v1)
  (`self.EnableInput` _output_get)
  (`SceneComponent.SetVisibility` (`self.WC_PressE_CCTV`) false false)
  (`SceneComponent.SetVisibility` (`self.TextRender`) false false))

(event `self.BoxColisao.OnComponentBeginOverlap`
  (params (OverlappedComponent :type "PrimitiveComponent Object Reference") (OtherActor :type "Actor Object Reference") (OtherComp :type "PrimitiveComponent Object Reference") (OtherBodyIndex :type Integer) (bFromSweep :type Boolean) (SweepResult :type "HitResult Structure (by ref)"))
  (if (== OtherActor (`self.PlayerRef`))
    (set `self.bPlayerInside` true)
    (if (not (`self.bUsingTerminal`))
      (`SceneComponent.SetVisibility` (`self.WC_PressE_CCTV`) true false)
      (`SceneComponent.SetVisibility` (`self.TextRender`) true false))))

(event `self.BoxColisao.OnComponentEndOverlap`
  (params (OverlappedComponent :type "PrimitiveComponent Object Reference") (OtherActor :type "Actor Object Reference") (OtherComp :type "PrimitiveComponent Object Reference") (OtherBodyIndex :type Integer))
  (bind _busingterminal (`self.bUsingTerminal`))
  (if (== OtherActor (`self.PlayerRef`))
    (if _busingterminal
      (set `self.bPlayerInside` _busingterminal)
      (set `self.bHoldPanLeft` false)
      (set `self.bHoldPanRight` false)
      (set `self.bHoldTiltUp` false)
      (set `self.bHoldTiltDown` false)
      (`SceneComponent.SetVisibility` (`self.WC_PressE_CCTV`) false false)
      (`self.ExitTerminal`))))

(event `ExitTerminal`
  (bind _pcref (`self.PCRef`))
  (bind _currentcctvref (`self.CurrentCCTVRef`))
  (bind _wc_presse_cctv (`self.WC_PressE_CCTV`))
  (bind _crtoverlayref (`self.CRTOverlayRef`))
  (`self.CancelCCTVJumpScare`)
  (`self.CloseTerminalHUD`)
  (`self.ResetActiveCCTV`)
  (`/Engine/EditorBlueprintResources/StandardMacros.IsValid` _currentcctvref
    (:`Is Valid`
      (`/Game/Birra/CCTV/BP_CCTV.ResetCCTVToOrigin` _currentcctvref)
      (`self.StartAllSurveillance`))
    (:`Is Not Valid`
      _))
  (set `self.bUsingTerminal` false)
  (if (`self.bPlayerInside`)
    (`SceneComponent.SetVisibility` _wc_presse_cctv true false)
    (`Controller.ResetIgnoreMoveInput` _pcref)
    (`Controller.ResetIgnoreLookInput` _pcref)
    (`PlayerController.SetViewTargetWithBlend` _pcref (`self.PlayerRef`) 0.15 "VTBlend_Linear" 0.0 false)
    (`/Engine/EditorBlueprintResources/StandardMacros.IsValid` _crtoverlayref
      (:`Is Valid`
        (`Widget.RemoveFromParent` _crtoverlayref)
        (set `self.CRTOverlayRef` null)))
    (else
      (`SceneComponent.SetVisibility` _wc_presse_cctv true false))))

(event `EnterTerminal`
  (bind _pcref (`self.PCRef`))
  (if (> (`KismetArrayLibrary.Array_Length` (`self.Cameras`)) 0)
    (set `self.bUsingTerminal` true)
    (bind _returnvalue (`|CreateWidget` "/Game/Birra/CCTV/WBP_CCTV_CRT_Overlay.WBP_CCTV_CRT_Overlay_C" (`self.PCRef`)))
    (bind _output_get (set `self.CRTOverlayRef` _returnvalue))
    (`UserWidget.AddToViewport` _output_get 50)
    (`SceneComponent.SetVisibility` (`self.WC_PressE_CCTV`) false false)
    (`self.OpenTerminalHUD`)
    (`self.SelectFirstOnlineCamera`)
    (`Controller.SetIgnoreLookInput` _pcref true)
    (`Controller.SetIgnoreMoveInput` _pcref true)
    ; alien
    (`self.ArmCCTVJumpScare`)))

(event `NextCamera`
  (bind _returnvalue (`KismetArrayLibrary.Array_Length` (`self.Cameras`)))
  (if (`self.bUsingTerminal`)
    (for _index (range 1 (+ _returnvalue 1))
      (bind _returnvalue_2 (mod (+ (`self.CurrentIndex`) _index) _returnvalue))
      (bind (_bexists _bonline) (`self.GetCameraStatusByIndex` _returnvalue_2))
      (if (and _bexists _bonline)
        (`self.SelectCameraByIndex` _returnvalue_2)
        (break)))
    (`self.RefreshTerminalHUD`)))

(event `Key|MouseScrollUp`
  (params (Key :type "Key Structure"))
  (:`Pressed`
    (if (`self.bUsingTerminal`)
      (`/Engine/EditorBlueprintResources/StandardMacros.IsValid` (`self.CurrentCCTVRef`)
        (:`Is Valid`
          (`/Game/Birra/CCTV/BP_CCTV.CamZoomIn` (`self.Cameras`)))))))

(event `ResetActiveCCTV`
  (bind _currentcctvref (`self.CurrentCCTVRef`))
  (`/Engine/EditorBlueprintResources/StandardMacros.IsValid` _currentcctvref
    (:`Is Valid`
      (`/Game/Birra/CCTV/BP_CCTV.ResetCCTVToOrigin` _currentcctvref))))

(event `Key|E`
  (params (Key :type "Key Structure"))
  (:`Pressed`
    (if (`self.bPlayerInside`)
      (if (`self.bUsingTerminal`)
        (`self.ExitTerminal`)
        (else
          (`self.EnterTerminal`))))))

(event `Key|MouseScrollDown`
  (params (Key :type "Key Structure"))
  (:`Pressed`
    (if (`self.bUsingTerminal`)
      (`/Engine/EditorBlueprintResources/StandardMacros.IsValid` (`self.CurrentCCTVRef`)
        (:`Is Valid`
          (`/Game/Birra/CCTV/BP_CCTV.CamZoomOut` (`self.Cameras`)))))))

(event `PreviousCamera`
  (bind _returnvalue (`KismetArrayLibrary.Array_Length` (`self.Cameras`)))
  (if (`self.bUsingTerminal`)
    (for _index (range 1 (+ _returnvalue 1))
      (bind _returnvalue_2 (mod (+ (- (`self.CurrentIndex`) _index) _returnvalue) _returnvalue))
      (bind (_bexists _bonline) (`self.GetCameraStatusByIndex` _returnvalue_2))
      (if (and _bexists _bonline)
        (`self.SelectCameraByIndex` _returnvalue_2)
        (break)))
    (`self.RefreshTerminalHUD`)))

(event `Key|W`
  (params (Key :type "Key Structure"))
  (:`Pressed`
    (set `self.bHoldTiltUp` true))
  (:`Released`
    (set `self.bHoldTiltUp` false)))

(event `Key|A`
  (params (Key :type "Key Structure"))
  (:`Pressed`
    (set `self.bHoldPanLeft` true))
  (:`Released`
    (set `self.bHoldPanLeft` false)))

(event `Key|Left`
  (params (Key :type "Key Structure")))

(event `Key|D`
  (params (Key :type "Key Structure"))
  (:`Pressed`
    (set `self.bHoldPanRight` true))
  (:`Released`
    (set `self.bHoldPanRight` false)))

(event `Key|Right`
  (params (Key :type "Key Structure")))

(event `Key|Up`
  (params (Key :type "Key Structure")))

(event `Key|S`
  (params (Key :type "Key Structure"))
  (:`Pressed`
    (set `self.bHoldTiltDown` true))
  (:`Released`
    (set `self.bHoldTiltDown` false)))

(event `self.ReceiveTick`
  (params (DeltaSeconds :type "Float (single-precision)"))
  (bind _currentcctvref (`self.CurrentCCTVRef`))
  (bind _currentcctvref_2 (`self.CurrentCCTVRef`))
  (if (`self.bUsingTerminal`)
    (bind _returnvalue (`self.GetCurrentCCTV`))
    (`/Engine/EditorBlueprintResources/StandardMacros.IsValid` _returnvalue
      (:`Is Valid`
        (`|ExecutionSequence`
          (:`then_0`
            (if (`self.bHoldPanLeft`)
              (`/Game/Birra/CCTV/BP_CCTV.CamPanLeft` _currentcctvref_2)))
          (:`then_1`
            (if (`self.bHoldPanRight`)
              (`/Game/Birra/CCTV/BP_CCTV.CamPanRight` _currentcctvref_2)))
          (:`then_2`
            (if (`self.bHoldTiltUp`)
              (`/Game/Birra/CCTV/BP_CCTV.CamTiltUp` _currentcctvref)))
          (:`then_3`
            (if (`self.bHoldTiltDown`)
              (`/Game/Birra/CCTV/BP_CCTV.CamTiltDown` _currentcctvref))))))))

(event `Key|Down`
  (params (Key :type "Key Structure")))

(event `Key|C`
  (params (Key :type "Key Structure"))
  (:`Pressed`
    (`self.PreviousCamera`)))

(event `Key|Z`
  (params (Key :type "Key Structure"))
  (:`Pressed`
    (`self.NextCamera`)))

(event `StartAllSurveillance`
  (for _array_element (`self.Cameras`)
    (`/Engine/EditorBlueprintResources/StandardMacros.IsValid` _array_element
      (:`Is Valid`
        (`/Game/Birra/CCTV/BP_CCTV.StartSurveillance` _array_element)))))

(event `SelectCameraByIndex`
  (params (NewIndex :type Integer))
  (bind _currentcctvref (`self.CurrentCCTVRef`))
  (bind _output (`|GetArrayItem` (`self.Cameras`) NewIndex))
  (if (`self.bUsingTerminal`)
    (bind (_bexists _bonline) (`self.GetCameraStatusByIndex` NewIndex))
    (if (and _bexists _bonline)
      (`/Engine/EditorBlueprintResources/StandardMacros.IsValid` _output
        (:`Is Valid`
          (bind _output_get (set `self.SelectedCameraRef` _output))
          (`self.ResetActiveCCTV`)
          (set `self.CurrentIndex` NewIndex)
          (set `self.CurrentCCTVRef` _output_get)
          (`/Game/Birra/CCTV/BP_CCTV.StopSurveillance` _currentcctvref)
          (`PlayerController.SetViewTargetWithBlend` (`self.PCRef`) _currentcctvref 0.2 "VTBlend_Linear" 0.0 false)
          (`self.RefreshTerminalHUD`))
        (:`Is Not Valid`
          (`self.RefreshTerminalHUD`)))
      (else
        (`self.RefreshTerminalHUD`)))))

(event `RefreshTerminalHUD`
  (bind _terminalhudref (`self.TerminalHUDRef`))
  (`/Engine/EditorBlueprintResources/StandardMacros.IsValid` _terminalhudref
    (:`Is Valid`
      (`/Game/Birra/CCTV/WBP_CCTV_TerminalHUD.RefreshCameraButtons` _terminalhudref))))

(event `OpenTerminalHUD`
  (`/Engine/EditorBlueprintResources/StandardMacros.IsValid` (`self.TerminalHUDRef`)
    (:`Is Not Valid`
      (bind _returnvalue (`|CreateWidget` "/Game/Birra/CCTV/WBP_CCTV_TerminalHUD.WBP_CCTV_TerminalHUD_C" (`self.PCRef`) self))
      (bind _output_get (set `self.TerminalHUDRef` _returnvalue))
      (`UserWidget.AddToViewport` _output_get 100)
      (`/Game/Birra/CCTV/WBP_CCTV_TerminalHUD.BuildCameraList` _output_get)
      (`/Game/Birra/CCTV/WBP_CCTV_TerminalHUD.RefreshCameraButtons` _output_get))))

(event `CloseTerminalHUD`
  (bind _terminalhudref (`self.TerminalHUDRef`))
  (`/Engine/EditorBlueprintResources/StandardMacros.IsValid` _terminalhudref
    (:`Is Valid`
      (`Widget.RemoveFromParent` _terminalhudref)
      (set `self.TerminalHUDRef` null))))

(event `PlayCCTVJumpScareAudio`
  (bind _jumpscaresfx (`self.JumpScareSFX`))
  (bind _jumpscarestaticsfx (`self.JumpScareStaticSFX`))
  (bind _jumpscareofflinesfx (`self.JumpScareOfflineSFX`))
  (`/Engine/EditorBlueprintResources/StandardMacros.IsValid` _jumpscaresfx
    (:`Is Valid`
      (`GameplayStatics.PlaySound2D` _jumpscaresfx (`self.JumpScareSFXVolume`) (`self.JumpScareSFXPitch`) 0.0 null null)
      (`/Engine/EditorBlueprintResources/StandardMacros.IsValid` _jumpscarestaticsfx
        (:`Is Valid`
          (`GameplayStatics.PlaySound2D` _jumpscarestaticsfx 0.8 1.0 0.0 null null)
          (`/Engine/EditorBlueprintResources/StandardMacros.IsValid` _jumpscareofflinesfx
            (:`Is Valid`
              (`GameplayStatics.PlaySound2D` _jumpscareofflinesfx 0.7 1.0 0.0 null null))))))))

(event `Key|One`
  (params (Key :type "Key Structure"))
  (:`Pressed`
    (if (`self.bUsingTerminal`)
      (`self.SelectCameraByIndex` 0))))

(event `Key|Two`
  (params (Key :type "Key Structure"))
  (:`Pressed`
    (if (`self.bUsingTerminal`)
      (`self.SelectCameraByIndex` 1))))

(event `Key|Three`
  (params (Key :type "Key Structure"))
  (:`Pressed`
    (if (`self.bUsingTerminal`)
      (`self.SelectCameraByIndex` 2))))

(event `ArmCCTVJumpScare`
  (if (`self.bJumpScareEnabled`)
    (if (`self.bUsingTerminal`)
      (if (not (`self.bJumpScareInProgress`))
        (bind _return (`self.HasAnyActiveCCTVCamera`))
        (if _return
          (`KismetSystemLibrary.K2_ClearAndInvalidateTimerHandle` (`self.TH_JumpScare`))
          (bind _returnvalue (`KismetSystemLibrary.K2_SetTimerDelegate` (delegate `OnCCTVJumpScareTimerFinished`) (`KismetMathLibrary.RandomFloatInRange` (`self.JumpScareMinDelay`) (`self.JumpScareMaxDelay`))))
          (set `self.TH_JumpScare` _returnvalue)
          (set `self.bJumpScareArmed` true)
          (`KismetSystemLibrary.PrintString` "JUMPSCARE ARMED" true true (struct :`R` 1.0 :`G` 0.105633 :`A` 1.0)))))))

(event `Key|Four`
  (params (Key :type "Key Structure"))
  (:`Pressed`
    (if (`self.bUsingTerminal`)
      (`self.SelectCameraByIndex` 3))))

(event `Key|H`
  (params (Key :type "Key Structure"))
  (bind _terminalhudref (`self.TerminalHUDRef`))
  (:`Pressed`
    (if (`self.bUsingTerminal`)
      (`/Engine/EditorBlueprintResources/StandardMacros.IsValid` _terminalhudref
        (:`Is Valid`
          (`/Game/Birra/CCTV/WBP_CCTV_TerminalHUD.ToggleControlsPanel` _terminalhudref))))))

(event `OnCCTVJumpScareTimerFinished`
  (bind _currentindex (`self.CurrentIndex`))
  (`KismetSystemLibrary.PrintString` "JUMPSCARE TIMER FINISHED" true true (struct :`R` 1.0 :`G` 0.105633 :`A` 1.0))
  (set `self.bJumpScareArmed` false)
  (if (`self.bUsingTerminal`)
    (if (not (`self.bJumpScareInProgress`))
      (bind _return (`self.HasAnyActiveCCTVCamera`))
      (if _return
        (bind _return_2 (`self.IsCCTVCameraOnline` _currentindex))
        (if _return_2
          (`self.TriggerCCTVJumpScare` _currentindex)
          (else
            (`self.ArmCCTVJumpScare`)))))))

(event `CancelCCTVJumpScare`
  (`KismetSystemLibrary.K2_ClearAndInvalidateTimerHandle` (`self.TH_JumpScare`))
  (`KismetSystemLibrary.K2_ClearAndInvalidateTimerHandle` (`self.TH_JumpScareExit`))
  (set `self.bJumpScareArmed` false)
  (set `self.bJumpScareInProgress` false)
  (`/Engine/EditorBlueprintResources/StandardMacros.IsValid` (`self.ActiveJumpScareAlien`)
    (:`Is Valid`
      (`self.K2_DestroyActor`)
      (set `self.ActiveJumpScareAlien` null))))

(event `TriggerCCTVJumpScare`
  (params (CameraIndex :type Integer))
  (bind _crtoverlayref (`self.CRTOverlayRef`))
  (set `self.bJumpScareInProgress` true)
  (`KismetSystemLibrary.K2_ClearAndInvalidateTimerHandle` (`self.TH_JumpScare`))
  (`self.SpawnJumpScareAlienAtCamera` CameraIndex)
  (`self.PlayCCTVJumpScareAudio`)
  (`/Engine/EditorBlueprintResources/StandardMacros.IsValid` _crtoverlayref
    (:`Is Valid`
      (`/Game/Birra/CCTV/WBP_CCTV_CRT_Overlay.PlayJumpScareStatic` _crtoverlayref (`self.JumpScareExitDelay`)))
    (:`Is Not Valid`
      _))
  (`self.SetCCTVCameraOfflinePermanent` CameraIndex)
  (`self.RefreshCCTVAfterJumpScare`)
  (bind _returnvalue (`KismetSystemLibrary.K2_SetTimerDelegate` (delegate `AutoExitCCTVAfterJumpScare`) (`self.JumpScareExitDelay`)))
  (set `self.TH_JumpScareExit` _returnvalue))

(event `AutoExitCCTVAfterJumpScare`
  (bind _crtoverlayref (`self.CRTOverlayRef`))
  (bind _activejumpscarealien (`self.ActiveJumpScareAlien`))
  (`/Engine/EditorBlueprintResources/StandardMacros.IsValid` _crtoverlayref
    (:`Is Valid`
      (`/Game/Birra/CCTV/WBP_CCTV_CRT_Overlay.StopJumpScareStatic` _crtoverlayref)
      (`/Engine/EditorBlueprintResources/StandardMacros.IsValid` _activejumpscarealien
        (:`Is Valid`
          (`self.K2_DestroyActor` _activejumpscarealien))
        (:`Is Not Valid`
          _))
      (set `self.ActiveJumpScareAlien` null)
      (set `self.bJumpScareInProgress` false)
      (set `self.bJumpScareArmed` false)
      (`self.ExitTerminal`))))

(fn `GetCameraStatusByIndex`
  (params (CameraIndex :type Integer))
  (returns (bExists :type Boolean) (bOnline :type Boolean) (DisplayLabel :type Text) (CameraRef :type "/Game/Birra/CCTV/BP_CCTV Object Reference"))
  (bind _cameras (`self.Cameras`))
  (bind _output (`|GetArrayItem` _cameras CameraIndex))
  (if (`KismetArrayLibrary.Array_IsValidIndex` _cameras CameraIndex)
    (`/Engine/EditorBlueprintResources/StandardMacros.IsValid` _output
      (:`Is Valid`
        (bind _returnvalue (`/Game/Birra/CCTV/BP_CCTV.GetIsOnline` _output))
        (bind _getcctvdisplaylabel (`/Game/Birra/CCTV/BP_CCTV.GetCCTVDisplayLabel` _output))
        (return true _returnvalue _getcctvdisplaylabel _output))
      (:`Is Not Valid`
        _)))
  (return false false "OFFLINE" null))

(fn `GetCurrentCCTV`
  (returns (ReturnValue :type "/Game/Birra/CCTV/BP_CCTV Object Reference"))
  (return (`|GetArrayItem` (`self.Cameras`) (`self.CurrentIndex`))))

(fn `HasAnyActiveCCTVCamera`
  (returns (Return :type Boolean))
  (for (_ _array_index) (`self.Cameras`)
    (bind (_bexists _bonline) (`self.GetCameraStatusByIndex` _array_index))
    (if (and _bexists _bonline)
      (return true)))
  (return false))

(fn `IsCCTVCameraOnline`
  (params (CameraIndex :type Integer))
  (returns (Return :type Boolean))
  (if (< CameraIndex 0)
    (return false)
    (elif (>= CameraIndex (`KismetArrayLibrary.Array_Length` (`self.Cameras`)))
      (return false)
      (else
        (bind (_bexists _bonline) (`self.GetCameraStatusByIndex` CameraIndex))
        (return (and _bexists _bonline))))))

(fn `RefreshCCTVAfterJumpScare`
  (bind _terminalhudref (`self.TerminalHUDRef`))
  (`/Engine/EditorBlueprintResources/StandardMacros.IsValid` _terminalhudref
    (:`Is Valid`
      (`/Game/Birra/CCTV/WBP_CCTV_TerminalHUD.RefreshCameraButtons` _terminalhudref))))

(fn `SelectFirstOnlineCamera`
  (for _index (range (`KismetArrayLibrary.Array_Length` (`self.Cameras`)))
    (bind (_bexists _bonline) (`self.GetCameraStatusByIndex` _index))
    (if (and _bexists _bonline)
      (`self.SelectCameraByIndex` _index)
      (return)))
  (`self.RefreshTerminalHUD`)
  (return))

(fn `SetCameraStatusByIndex`
  (params (CameraIndex :type Integer) (bOnline :type Boolean))
  (bind _cameras (`self.Cameras`))
  (bind _output (`|GetArrayItem` _cameras CameraIndex))
  (if (< CameraIndex 0)
    (return)
    (elif (>= CameraIndex (`KismetArrayLibrary.Array_Length` _cameras))
      (return)
      (else
        (`/Engine/EditorBlueprintResources/StandardMacros.IsValid` _output
          (:`Is Valid`
            (set `/Game/Birra/CCTV/BP_CCTV.bIsOnline` bOnline _output)
            (`/Game/Birra/CCTV/BP_CCTV.StopSurveillance` _output)
            (set `self.CurrentCCTVRef` null)
            (`self.RefreshCCTVAfterJumpScare`)
            (return)))))))

(fn `SetCCTVCameraOfflinePermanent`
  (params (CameraIndex :type Integer))
  (bind _cameras (`self.Cameras`))
  (bind _output (`|GetArrayItem` _cameras CameraIndex))
  (if (< CameraIndex 0)
    (return)
    (elif (>= CameraIndex (`KismetArrayLibrary.Array_Length` _cameras))
      (return)
      (else
        (`KismetArrayLibrary.Array_AddUnique` (`self.JumpScaredCameraIndices`) CameraIndex)
        (`/Engine/EditorBlueprintResources/StandardMacros.IsValid` _output
          (:`Is Valid`
            (`self.SetCameraStatusByIndex` CameraIndex)
            (`/Game/Birra/CCTV/BP_CCTV.StopSurveillance` _output)
            (`KismetSystemLibrary.PrintString` (`KismetStringLibrary.Concat_StrStr` "CAMERA SET OFFLINE = " (`KismetStringLibrary.Conv_IntToString` CameraIndex))))
          (:`Is Not Valid`
            (return)))))))

(fn `SpawnJumpScareAlienAtCamera`
  (params (CameraIndex :type Integer))
  (returns (Actor :type "Actor Object Reference"))
  (bind _output (`|GetArrayItem` (`self.Cameras`) CameraIndex))
  (`/Engine/EditorBlueprintResources/StandardMacros.IsValid` _output
    (:`Is Valid`
      (bind _output_get (set `self.LocalCameraRef` _output))
      (bind _camera (`/Game/Birra/CCTV/BP_CCTV.Camera` _output_get))
      (bind _returnvalue (`|SpawnActorFromClass` "/Game/Birra/CCTV/BP_CCTV_JumpScareAlien.BP_CCTV_JumpScareAlien_C" (`KismetMathLibrary.MakeTransform` (+ (+ (* (`SceneComponent.GetForwardVector` _camera) (`self.JumpScareAlienDistanceFromCamera`)) (`SceneComponent.K2_GetComponentLocation` _camera)) (`self.JumpScareAlienOffset`)) (`SceneComponent.K2_GetComponentRotation` _camera)) "Undefined" "MultiplyWithRoot" null null))
      (bind _output_get_2 (set `self.ActiveJumpScareAlien` _returnvalue))
      (bind _asbp_cctv_jump_scare_alien (cast `/Game/Birra/CCTV/BP_CCTV_JumpScareAlien` _output_get_2))
      (`/Game/Birra/CCTV/BP_CCTV_JumpScareAlien.ActivateJumpScareAlien` _asbp_cctv_jump_scare_alien))
    (:`Is Not Valid`
      (return null))))

(fn `UserConstructionScript`)