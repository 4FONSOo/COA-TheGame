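; BP_CCTV_JumpScareAlien is a jump-scare alien actor that stays hidden and without collision until triggered.
; ActivateJumpScareAlien reveals it, plays a sound, shows a point light and activates a Niagara effect.
; A timeline lerps the alien mesh from a configurable Z offset to its original relative position, while collision remains off.
; A separate event destroys the actor.
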(event `self.ReceiveBeginPlay`
  (`self.SetActorHiddenInGame` true)
  (`self.SetActorEnableCollision` false))

(event `ActivateJumpScareAlien`
  (bind _audiocomponent (`self.AudioComponent`))
  (bind _alienmesh (`self.AlienMesh`))
  (`self.SetActorHiddenInGame` false)
  (`self.SetActorEnableCollision` false)
  (bind _output_get (set `self.RiseEndLocation` (`SceneComponent.RelativeLocation` _alienmesh)))
  (bind _output_get_2 (set `self.RiseStartLocation` (+ _output_get (`KismetMathLibrary.MakeVector` 0.0 0.0 (`self.RiseStartOffsetZ`)))))
  (`SceneComponent.K2_SetRelativeLocation` _alienmesh _output_get_2 false false)
  (`AudioComponent.SetSound` _audiocomponent (`self.AlienSFX`))
  (`AudioComponent.SetVolumeMultiplier` _audiocomponent (`self.AlienSFXVolume`))
  (`AudioComponent.Play` _audiocomponent 0.0)
  (`SceneComponent.SetVisibility` (`self.PointLight`) true false)
  (`ActorComponent.Activate` (`self.NiagaraComponent `) false)
  (bind (_direction _alpha) (`Timeline|TL_AlienRise` :`NewTime` (`self.RiseDuration`) :!via `PlayFromStart`)
    (:`Update`
      (`SceneComponent.K2_SetRelativeLocation` (`self.AlienMesh`) (`KismetMathLibrary.VLerp` (`self.RiseStartLocation`) (`self.RiseEndLocation`) _alpha) false false))))

(event `DestroyJumpScareAlien`
  (`self.K2_DestroyActor`))

(fn `UserConstructionScript`)