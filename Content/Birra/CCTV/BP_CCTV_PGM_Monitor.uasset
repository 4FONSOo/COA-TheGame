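; CCTV program (PGM) monitor that shows feeds from a list of cameras in slots on a widget.
; Shortly after BeginPlay, SetupPGM gets the WBP_CCTV_PGM from its widget component and fills the visible slots in array order.
; Online cameras pass their PGM render target and label to their slot, while offline, invalid or missing cameras show as offline.
; Slots are assigned during setup, with no polling for status changes.
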(event `self.ReceiveBeginPlay`
  (`KismetSystemLibrary.Delay` 0.2)
  (`self.SetupPGM`))

(event `SetupPGM`
  (bind _pgmwidgetref (`self.PGMWidgetRef`))
  (bind _pgmwidgetref_2 (`self.PGMWidgetRef`))
  (bind _currentloopcamera (`self.CurrentLoopCamera`))
  (bind _returnvalue (`KismetArrayLibrary.Array_Length` (`self.Cameras`)))
  (bind _cameralabel (`/Game/Birra/CCTV/BP_CCTV.CameraLabel` _currentloopcamera))
  (bind _pgmrendertarget (`/Game/Birra/CCTV/BP_CCTV.PGMRenderTarget` _currentloopcamera))
  (bind _aswbp_cctv_pgm (cast `/Game/Birra/CCTV/CCTV_RenderTargets/WBP_CCTV_PGM` (`WidgetComponent.GetUserWidgetObject` (`self.Widget_PGM`))))
  (bind _output_get (set `self.PGMWidgetRef` _aswbp_cctv_pgm))
  (if (== _returnvalue 0)
    (`/Game/Birra/CCTV/CCTV_RenderTargets/WBP_CCTV_PGM.SetGlobalOffline` _output_get false)
    (else
      (`/Game/Birra/CCTV/CCTV_RenderTargets/WBP_CCTV_PGM.SetGlobalOffline` _output_get false)
      (for _index (range (`self.VisibleSlots`))
        (if (< _index _returnvalue)
          (bind _output_get_2 (set `self.CurrentLoopCamera` (`|GetArrayItem` (`self.Cameras`) _index)))
          (`/Engine/EditorBlueprintResources/StandardMacros.IsValid` _output_get_2
            (:`Is Valid`
              (if (`/Game/Birra/CCTV/BP_CCTV.bIsOnline` _currentloopcamera)
                (`/Engine/EditorBlueprintResources/StandardMacros.IsValid` _pgmrendertarget
                  (:`Is Valid`
                    (`/Game/Birra/CCTV/CCTV_RenderTargets/WBP_CCTV_PGM.SetSlotFeed` _pgmwidgetref_2 _index _pgmrendertarget _cameralabel)))
                (else
                  (`/Game/Birra/CCTV/CCTV_RenderTargets/WBP_CCTV_PGM.SetSlotOffline` _pgmwidgetref_2 _index _cameralabel)
                  (`/Game/Birra/CCTV/CCTV_RenderTargets/WBP_CCTV_PGM.SetSlotOffline` _pgmwidgetref_2 _index _cameralabel))))
            (:`Is Not Valid`
              (`/Game/Birra/CCTV/CCTV_RenderTargets/WBP_CCTV_PGM.SetSlotOffline` _pgmwidgetref _index "OFFLINE")))
          (else
            (`/Game/Birra/CCTV/CCTV_RenderTargets/WBP_CCTV_PGM.SetSlotOffline` _pgmwidgetref _index "OFFLINE")))))))

(fn `UserConstructionScript`)