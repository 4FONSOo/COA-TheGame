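; CCTV camera actor that sweeps on its own or takes player-driven pan, tilt, zoom and infrared toggle.
; Yaw and pitch pivots turn within clamped limits, zoom steps a clamped FOV, and infrared switches the camera's post-process blend weight.
; While surveillance is active and no player controls it, Tick bounces yaw between its limits at a randomized speed and starting direction.
; A scene capture outputs to the PGM render target; getters expose label and online state.
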(event `self.ReceiveBeginPlay`
  (bind _camera (`self.Camera`))
  (bind _defaultfov (`self.DefaultFOV`))
  (bind _pgmrendertarget (`self.PGMRenderTarget`))
  (`/Engine/EditorBlueprintResources/StandardMacros.IsValid` _pgmrendertarget
    (:`Is Valid`
      (set `SceneCaptureComponent2D.TextureTarget` _pgmrendertarget (`self.SceneCapture_PGM`))
      (set `self.OriginYawRotation` (`SceneComponent.RelativeRotation` (`self.YawPivot`)))
      (set `self.OriginPitchRotation` (`SceneComponent.RelativeRotation` (`self.PitchPivot`)))
      (set `self.OriginFOV` _defaultfov)
      (bind _output_get (set `self.CurrentFOV` _defaultfov))
      (set `self.SurveillanceDirection` (`KismetMathLibrary.SelectFloat` 1.0 -1.0 (`KismetMathLibrary.RandomBool`)))
      (set `self.SurveillanceSpeed` (`KismetMathLibrary.RandomFloatInRange` 6.0 12.0))
      (`CameraComponent.SetFieldOfView` _camera _output_get)
      (`CameraComponent.SetPostProcessBlendWeight` _camera 0.0))))

(event `ResetCCTVToOrigin`
  (bind _defaultfov (`self.DefaultFOV`))
  (`SceneComponent.K2_SetRelativeRotation` (`self.YawPivot`) (`self.OriginYawRotation`) false false)
  (`SceneComponent.K2_SetRelativeRotation` (`self.PitchPivot`) (`self.OriginPitchRotation`) false false)
  (set `self.CurrentFOV` _defaultfov)
  (`CameraComponent.SetFieldOfView` (`self.Camera`) _defaultfov))

(event `CamZoomIn`
  (bind _output_get (set `self.CurrentFOV` (`KismetMathLibrary.FClamp` (- (`self.CurrentFOV`) (`self.ZoomStep`)) (`self.MinFov`) (`self.MaxFov`))))
  (`CameraComponent.SetFieldOfView` (`self.Camera`) _output_get))

(event `StartSurveillance`
  (set `self.bPlayerControllingThisCam` false)
  (set `self.bSurveillanceActive` true))

(event `CamZoomOut`
  (bind _output_get (set `self.CurrentFOV` (`KismetMathLibrary.FClamp` (+ (`self.CurrentFOV`) (`self.ZoomStep`)) (`self.MinFov`) (`self.MaxFov`))))
  (`CameraComponent.SetFieldOfView` (`self.Camera`) _output_get))

(event `StopSurveillance`
  (set `self.bPlayerControllingThisCam` true)
  (set `self.bSurveillanceActive` false)
  (`CameraComponent.SetFieldOfView` (`self.Camera`) (`self.CurrentFOV`)))

(event `CamTiltUp`
  (bind _pitchpivot (`self.PitchPivot`))
  (`SceneComponent.K2_SetRelativeRotation` _pitchpivot (`KismetMathLibrary.MakeRotator` 0.0 (`KismetMathLibrary.FClamp` (+ (.pitch (`SceneComponent.RelativeRotation` _pitchpivot)) (`self.TiltStep`)) (`self.MinPitch`) (`self.MaxPitch`))) false false))

(event `CamTiltDown`
  (bind _pitchpivot (`self.PitchPivot`))
  (`SceneComponent.K2_SetRelativeRotation` _pitchpivot (`KismetMathLibrary.MakeRotator` 0.0 (`KismetMathLibrary.FClamp` (- (.pitch (`SceneComponent.RelativeRotation` _pitchpivot)) (`self.TiltStep`)) (`self.MinPitch`) (`self.MaxPitch`))) false false))

(event `CamPanLeft`
  (bind _yawpivot (`self.YawPivot`))
  (`SceneComponent.K2_SetRelativeRotation` _yawpivot (`KismetMathLibrary.MakeRotator` 0.0 0.0 (`KismetMathLibrary.FClamp` (- (.yaw (`SceneComponent.RelativeRotation` _yawpivot)) (`self.PanStep`)) (`self.MinYaw`) (`self.MaxYaw`))) false false))

(event `CamPanRight`
  (bind _yawpivot (`self.YawPivot`))
  (`SceneComponent.K2_SetRelativeRotation` _yawpivot (`KismetMathLibrary.MakeRotator` 0.0 0.0 (`KismetMathLibrary.FClamp` (+ (.yaw (`SceneComponent.RelativeRotation` _yawpivot)) (`self.PanStep`)) (`self.MinYaw`) (`self.MaxYaw`))) false false))

(event `ToggleInfraRed`
  (bind _camera (`self.Camera`))
  (if (`self.bInfraRedOn`)
    (set `self.bInfraRedOn` false)
    (`CameraComponent.SetPostProcessBlendWeight` _camera 0.0)
    (else
      (set `self.bInfraRedOn` true)
      (`CameraComponent.SetPostProcessBlendWeight` _camera 1.0))))

(event `self.ReceiveTick`
  (params (DeltaSeconds :type "Float (single-precision)"))
  (bind _maxyaw (`self.MaxYaw`))
  (bind _minyaw (`self.MinYaw`))
  (bind _returnvalue (+ (.yaw (`SceneComponent.RelativeRotation` (`self.YawPivot`))) (* (* (`self.SurveillanceDirection`) (`self.SurveillanceSpeed`)) DeltaSeconds)))
  (if (`self.bSurveillanceActive`)
    (if (not (`self.bPlayerControllingThisCam`))
      (set `self.SurveillanceTargetYaw` (`KismetMathLibrary.FClamp` _returnvalue _minyaw _maxyaw))
      (`|ExecutionSequence`
        (:`then_0`
          (if (<= _returnvalue _minyaw)
            (set `self.SurveillanceDirection` 1.0)))
        (:`then_1`
          (if (>= _returnvalue _maxyaw)
            (set `self.SurveillanceDirection` -1.0)))
        (:`then_2`
          (`SceneComponent.K2_SetRelativeRotation` (`self.YawPivot`) (`KismetMathLibrary.MakeRotator` 0.0 0.0 (`self.SurveillanceTargetYaw`)) false false))))))

(fn `ApplyCurrentFOV`
  (`CameraComponent.SetFieldOfView` (`self.Camera`) (`self.CurrentFOV`)))

(fn `GetCCTVDisplayLabel`
  (returns (GetCCTVDisplayLabel :type Text))
  (return (`self.CameraLabel`)))

(fn `GetIsOnline`
  (returns (ReturnValue :type Boolean))
  (return (`self.bIsOnline`)))

(fn `UserConstructionScript`)